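; BP_Locker is an interactable locker that players hide in.
; ServerInteract calls a likely multicast event that, behind a cooldown, clears IsHiding on tracked players and swings the door on a timeline with open and close sounds.
; When the swing finishes, it plays a radial camera shake and marks those players hiding.
; While IsEffective is set, trigger overlaps track players, and leaving the trigger clears their hiding state.
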(event OnComponentBeginOverlap(Trigger)
  (params (OverlappedComponent :type Primitive%20Component%20Object%20Reference) (OtherActor :type Actor%20Object%20Reference) (OtherComp :type Primitive%20Component%20Object%20Reference) (OtherBodyIndex :type Integer) (bFromSweep :type Boolean) (SweepResult :type Hit%20Result%20Structure%20%28by%20ref%29))
  (if (Variables|Default|GetIsEffective)
    (bind _asbp_player (Utilities|Casting|CastToBP_Player OtherActor))
    (Utilities|Array|Add (Variables|Default|GetPlayers) _asbp_player)))

(event OnComponentEndOverlap(Trigger)
  (params (OverlappedComponent :type Primitive%20Component%20Object%20Reference) (OtherActor :type Actor%20Object%20Reference) (OtherComp :type Primitive%20Component%20Object%20Reference) (OtherBodyIndex :type Integer))
  (if (Variables|Default|GetIsEffective)
    (bind _asbp_player (Utilities|Casting|CastToBP_Player OtherActor))
    (Variables|/Game/Blueprints/Player/BP_Player.BP_Player_C|SetIsHiding _asbp_player false)
    (Utilities|Array|RemoveItem (Variables|Default|GetPlayers) _asbp_player)))

(event Custom|Multi_Locker
  (if (not (Variables|Default|GetCooldown))
    (Variables|Default|SetCooldown true)
    (for _array_element (Variables|Default|GetPlayers)
      (Variables|/Game/Blueprints/Player/BP_Player.BP_Player_C|SetIsHiding _array_element false))
    (Audio|Components|Audio|Play (Variables|Default|GetOpenDoor) 0.0)
    (bind _doorangle (Timeline|MainAnimation PlayFromStart)
      (:Update
        (Transformation|SetRelativeRotation (Variables|Default|GetAxis) (Math|Rotator|MakeRotator 0.0 0.0 (* _doorangle -1.0)) false false))
      (:Finished
        (Default|CameraShake (Utilities|GameInstance) "/Game/Shakes/CS_Locker.CS_Locker_C" (Transformation|GetActorLocation) 3e+02 5e+02 1.0 false)
        (Audio|Components|Audio|Play (Variables|Default|GetCloseDoor) 0.0)
        (for _array_element_2 (Variables|Default|GetPlayers)
          (Variables|/Game/Blueprints/Player/BP_Player.BP_Player_C|SetIsHiding _array_element_2 true))
        (Variables|Default|SetCooldown false)))))

(event EventServerInteract
  (params (WhoInteracted :type Actor%20Object%20Reference))
  (CallFunction|MultiLocker))

(fn ConstructionScript)