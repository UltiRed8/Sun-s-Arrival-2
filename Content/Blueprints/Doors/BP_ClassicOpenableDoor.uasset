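; Classic hinged door that opens, closes, locks and can be smashed by AI, extending a parent door class.
; Server open/close events play timelines driving yaw, flipped by IsInverted, with sounds, a camera shake on closing, and toggling of an optional linked double door.
; Lock state switches the box's Pawn collision between Block and Overlap.
; AI destruction turns the box into a physics body launched by an impulse, with shake and sound.
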(event Custom|UpdateNav
  (Collision|SetCollisionResponsetoChannel (Variables|Default|GetBox) "ECC_Pawn" (select (Variables|Default|GetIsLocked) "ECR_Block" "ECR_Overlap")))

(event Custom|Multi_AIDestroy
  (params (Direction :type Vector))
  (bind _box (Variables|Default|GetBox))
  (if (not (Variables|Default|GetIsDestroyed))
    (Variables|Default|SetIsDestroyed true)
    (Components|Box|SetBoxExtent _box "28.000000,28.000000,28.000000" true)
    (Collision|SetCollisionResponsetoAllChannels _box "ECR_Ignore")
    (Collision|SetCollisionResponsetoChannel _box "ECC_WorldStatic" "ECR_Block")
    (Physics|SetSimulatePhysics _box true)
    (Physics|AddImpulseatLocation _box (* Direction 5e+05) (+ (Transformation|GetWorldLocation (Variables|Default|GetImpactPoint)) (* Direction -1.0)) "None")
    (Default|CameraShake (Utilities|GameInstance) "/Game/Shakes/CS_DoorDestroyed.CS_DoorDestroyed_C" (Transformation|GetActorLocation) 8e+02 1.6e+03 1.0 false)
    (Audio|Components|Audio|Play (Variables|Default|GetDestroyDoor) 0.0)))

(event Custom|Multi_OpenSound
  (Audio|Components|Audio|Play (Variables|Default|GetOpenDoor) 0.0))

(event Custom|Multi_CloseSound
  (Audio|Components|Audio|Play (Variables|Default|GetCloseDoor) 0.0))

(event Custom|Server_ToggleDouble
  (bind _doubledoor (Variables|Default|GetDoubleDoor))
  (Utilities|IsValid _doubledoor
    (:Is%20Valid
      (Default|ServerToggleDoor _doubledoor))))

(event EventServerUnlock
  (|CallParentFunction)
  (CallFunction|UpdateNav))

(event EventBeginPlay
  (|CallParentFunction)
  (CallFunction|UpdateNav))

(event EventServerOpenDoor
  (if (not (Variables|Default|GetIsDestroyed))
    (CallFunction|ServerToggleDouble)
    (CallFunction|MultiOpenSound)
    (bind _rotation (Timeline|OpenDoorAnim PlayFromStart)
      (:Update
        (CallFunction|UpdateDoorData "0, 0, 0" (Math|Rotator|MakeRotator 0.0 0.0 (* _rotation (Math|Float|SelectFloat -1.0 1.0 (Variables|Default|GetIsInverted))))))
      (:Finished
        (|CallParentFunction)))))

(event EventServerCloseDoor
  (if (not (Variables|Default|GetIsDestroyed))
    (CallFunction|ServerToggleDouble)
    (bind _rotation (Timeline|CloseDoorAnim PlayFromStart)
      (:Update
        (CallFunction|UpdateDoorData "0, 0, 0" (Math|Rotator|MakeRotator 0.0 0.0 (* _rotation (Math|Float|SelectFloat -1.0 1.0 (Variables|Default|GetIsInverted))))))
      (:Finished
        (CallFunction|MultiCloseSound)
        (Default|CameraShake (Utilities|GameInstance) "/Game/Shakes/CS_ClassicDoor.CS_ClassicDoor_C" (Transformation|GetActorLocation) 6e+02 1.2e+03 1.0 false)
        (|CallParentFunction)))))

(fn ConstructionScript
  (|CallParentFunction)
  (if (Variables|Default|GetIsInverted)
    (Transformation|AddRelativeRotation (Variables|Default|GetArrow) (Math|Rotator|MakeRotator 0.0 0.0 1.8e+02) false false)))