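; Base door actor that holds open, locked and toggle state and lets a player open or close it through server-named events.
; Interaction checks for BP_Player and CanBeToggledByPlayer, then toggles if unlocked, using CanToggle as a re-entry guard.
; Open and close only set state and re-arm the guard, while UpdateDoorData separately positions the Axis component.
; Doors flagged open at BeginPlay reset and run through the toggle path.
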(event Custom|Server_OpenDoor
  ;[0.03844 0.15 0 0.5] Open and Close Door
  (Variables|Default|SetIsOpen true)
  (Variables|Default|SetCanToggle true))

(event Custom|Server_CloseDoor
  ;[0.03844 0.15 0 0.5] Open and Close Door
  (Variables|Default|SetIsOpen false)
  (Variables|Default|SetCanToggle true))

(event Custom|Server_ToggleDoor
  ;[0.03844 0.15 0 0.5] Open and Close Door
  (if (not (Variables|Default|GetIsLocked))
    (if (Variables|Default|GetCanToggle)
      (Variables|Default|SetCanToggle false)
      (if (Variables|Default|GetIsOpen)
        (CallFunction|ServerCloseDoor)
        (else
          (CallFunction|ServerOpenDoor))))))

(event Custom|UpdateDoorData
  (params (Location :type Vector) (Rotation :type Rotator))
  (Transformation|SetRelativeTransform (Variables|Default|GetAxis) (Math|Transform|MakeTransform Location Rotation "1.000000,1.000000,1.000000") false false))

(event Custom|Server_Unlock
  ;[0.03844 0.15 0 0.5] Open and Close Door
  (Variables|Default|SetIsLocked false))

(event EventServerInteract
  (params (WhoInteracted :type Actor%20Object%20Reference))
  (Utilities|Casting|CastToBP_Player WhoInteracted)
  (if (Variables|Default|GetCanBeToggledByPlayer)
    (CallFunction|ServerToggleDoor)))

(event EventBeginPlay
  (if (Variables|Default|GetIsOpen)
    (Variables|Default|SetIsOpen false)
    (CallFunction|ServerToggleDoor)))

(fn ConstructionScript)