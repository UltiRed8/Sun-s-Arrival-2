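; BP_PanelDoor is a child door Blueprint for a sliding panel door with a keycard reader indicator.
; Server open and close events trigger the same multicast sound, play separate timelines that feed a Y location into UpdateDoorData, then call the parent event on completion.
; The open multicast sets the Cylinder to the keycard success material.
; The construction script also applies that material when the door is open or player-toggleable.
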(event Custom|Multi_Sound
  (Audio|Components|Audio|Play (Variables|Default|GetOpenDoor) 0.0))

(event Custom|Multi_Open
  (Rendering|Material|SetMaterial (Variables|Default|GetCylinder) 0 "/Game/Materials/Instances/MI_KeycardReaderSuccess.MI_KeycardReaderSuccess"))

(event EventServerOpenDoor
  (CallFunction|MultiSound)
  (bind _position (Timeline|OpenDoorAnim PlayFromStart)
    (:Update
      (CallFunction|UpdateDoorData (Math|Vector|MakeVector 0.0 _position 0.0) "0, 0, 0"))
    (:Finished
      (|CallParentFunction))))

(event EventServerCloseDoor
  (CallFunction|MultiSound)
  (bind _position (Timeline|CloseDoorAnim PlayFromStart)
    (:Update
      (CallFunction|UpdateDoorData (Math|Vector|MakeVector 0.0 _position 0.0) "0, 0, 0"))
    (:Finished
      (|CallParentFunction))))

(fn ConstructionScript
  (if (or (Variables|Default|GetIsOpen) (Variables|Default|GetCanBeToggledByPlayer))
    (CallFunction|MultiOpen))
  (|CallParentFunction))