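; Base networked arcade cabinet that one player at a time can operate, swapping them for a customized stand-in mesh with a name label.
; Interacting switches view and input to the cabinet; releasing Escape or dying hands them back.
; Keys animate joystick and buttons locally, then relay method names through the player to the server's CallMethodByName for remote replication.
; Inputs also feed Konami-code detection for an achievement, and an optional flickering light mimics screen glow.
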(event Custom|Server_CheckDeadPlayer
  (params (DeadPlayer :type BP%20Player%20Object%20Reference))
  (if (== DeadPlayer (Variables|Default|GetActorWhoInteracted))
    (CallFunction|ClientForceRelease)))

(event Custom|Client_ForceRelease
  (CallFunction|StopControl))

(event Custom|Multi_StopControl
  (Rendering|SetActorHiddenInGame (Variables|Default|GetActorWhoInteracted) false)
  (Variables|Default|SetActorWhoInteracted 0)
  (Development|SetHiddeninGame (Variables|Default|GetPlayerMesh) true true)
  (Variables|Default|SetTexture2D "/Game/Textures/T_CursorInteract.T_CursorInteract"))

(event Custom|StopControl
  (bind _returnvalue (Game|GetPlayerController 0))
  (bind _actorwhointeracted (Variables|Default|GetActorWhoInteracted))
  (Game|Player|SetViewTargetwithBlend _returnvalue _actorwhointeracted 0.2 "VTBlend_Linear" 0.0 false)
  (Input|DisableInput self _returnvalue)
  (Input|EnableInput _returnvalue _returnvalue)
  (Input|EnableInput _actorwhointeracted _returnvalue)
  (Default|OntoServerInteractwith (Variables|Default|GetActorWhoInteracted) self))

(event Custom|EnteredInput
  (params (Input :type String))
  (bind _output_get (Variables|Default|SetCurrentInputs (Utilities|String|Append (Variables|Default|GetCurrentInputs) Input)))
  (if (Utilities|String|StartsWith (Variables|Default|GetKonamiCode) _output_get)
    (if (Utilities|Enum|Equal(Enum) (Variables|Default|GetCurrentInputs) (Variables|Default|GetKonamiCode))
      (CallFunction|KonamiCodeTriggered))
    (else
      (Variables|Default|SetCurrentInputs ""))))

(event Custom|Multi_PPressed
  ;[0.15 0.15 0.15 0.5] P
  (if (not (Pawn|IsLocallyControlled (Variables|Default|GetActorWhoInteracted)))
    (Transformation|AddRelativeLocation (Variables|Default|GetButtonA) "0.000000,0.000000,-5.000000" false false)))

(event Custom|Multi_PReleased
  ;[0.15 0.15 0.15 0.5] P
  (if (Pawn|IsLocallyControlled (Variables|Default|GetActorWhoInteracted))
    (CallFunction|StopControl)
    (else
      (Transformation|AddRelativeLocation (Variables|Default|GetButtonA) "0.000000,0.000000,5.000000" false false))))

(event Custom|ReleasedInput
  (params (Input :type String)))

(event Custom|Multi_EPressed
  ;[0.15 0.15 0.15 0.5] Enter
  (if (not (Pawn|IsLocallyControlled (Variables|Default|GetActorWhoInteracted)))
    (Transformation|AddRelativeLocation (Variables|Default|GetButtonF) "0.000000,0.000000,-5.000000" false false)))

(event Custom|Multi_EReleased
  ;[0.15 0.15 0.15 0.5] Enter
  (if (not (Pawn|IsLocallyControlled (Variables|Default|GetActorWhoInteracted)))
    (Transformation|AddRelativeLocation (Variables|Default|GetButtonF) "0.000000,0.000000,5.000000" false false)))

(event Custom|Multi_UpPressed
  ;[0.15 0.15 0.15 0.5] Up
  (if (not (Pawn|IsLocallyControlled (Variables|Default|GetActorWhoInteracted)))
    (Transformation|AddRelativeRotation (Variables|Default|GetJoystickAxis) "20.000000,0.000000,0.000000" false false)))

(event Custom|Multi_UpReleased
  ;[0.15 0.15 0.15 0.5] Up
  (if (not (Pawn|IsLocallyControlled (Variables|Default|GetActorWhoInteracted)))
    (Transformation|AddRelativeRotation (Variables|Default|GetJoystickAxis) "-20.000000,0.000000,0.000000" false false)))

(event Custom|Multi_DownPressed
  ;[0.15 0.15 0.15 0.5] Down
  (if (not (Pawn|IsLocallyControlled (Variables|Default|GetActorWhoInteracted)))
    (Transformation|AddRelativeRotation (Variables|Default|GetJoystickAxis) "-20.000000,0.000000,0.000000" false false)))

(event Custom|KonamiCodeTriggered
  (bind _returnvalue (Actor|GetActorOfClass "/Game/Blueprints/BP_AchievementManager.BP_AchievementManager_C"))
  (Default|Unlock _returnvalue "cheater"))

(event Custom|Multi_DownReleased
  ;[0.15 0.15 0.15 0.5] Down
  (if (not (Pawn|IsLocallyControlled (Variables|Default|GetActorWhoInteracted)))
    (Transformation|AddRelativeRotation (Variables|Default|GetJoystickAxis) "20.000000,0.000000,0.000000" false false)))

(event Custom|Multi_LeftPressed
  ;[0.15 0.15 0.15 0.5] Left
  (if (not (Pawn|IsLocallyControlled (Variables|Default|GetActorWhoInteracted)))
    (Transformation|AddRelativeRotation (Variables|Default|GetJoystickAxis) "0.000000,0.000000,20.000000" false false)))

(event Custom|Multi_LeftReleased
  ;[0.15 0.15 0.15 0.5] Left
  (if (not (Pawn|IsLocallyControlled (Variables|Default|GetActorWhoInteracted)))
    (Transformation|AddRelativeRotation (Variables|Default|GetJoystickAxis) "0.000000,0.000000,-20.000000" false false)))

(event Custom|Multi_RightPressed
  ;[0.15 0.15 0.15 0.5] Right
  (if (not (Pawn|IsLocallyControlled (Variables|Default|GetActorWhoInteracted)))
    (Transformation|AddRelativeRotation (Variables|Default|GetJoystickAxis) "0.000000,0.000000,-20.000000" false false)))

(event Custom|Multi_RightReleased
  ;[0.15 0.15 0.15 0.5] Right
  (if (not (Pawn|IsLocallyControlled (Variables|Default|GetActorWhoInteracted)))
    (Transformation|AddRelativeRotation (Variables|Default|GetJoystickAxis) "0.000000,0.000000,20.000000" false false)))

(event Custom|Multi_APressed
  ;[0.15 0.15 0.15 0.5] A
  (if (not (Pawn|IsLocallyControlled (Variables|Default|GetActorWhoInteracted)))
    (Transformation|AddRelativeLocation (Variables|Default|GetButtonD) "0.000000,0.000000,-5.000000" false false)))

(event Custom|Multi_AReleased
  ;[0.15 0.15 0.15 0.5] A
  (if (not (Pawn|IsLocallyControlled (Variables|Default|GetActorWhoInteracted)))
    (Transformation|AddRelativeLocation (Variables|Default|GetButtonD) "0.000000,0.000000,5.000000" false false)))

(event Custom|Multi_BPressed
  ;[0.15 0.15 0.15 0.5] B
  (if (not (Pawn|IsLocallyControlled (Variables|Default|GetActorWhoInteracted)))
    (Transformation|AddRelativeLocation (Variables|Default|GetButtonC) "0.000000,0.000000,-5.000000" false false)))

(event Custom|Multi_BReleased
  ;[0.15 0.15 0.15 0.5] B
  (if (not (Pawn|IsLocallyControlled (Variables|Default|GetActorWhoInteracted)))
    (Transformation|AddRelativeLocation (Variables|Default|GetButtonC) "0.000000,0.000000,5.000000" false false)))

(event Custom|Multi_XPressed
  ;[0.15 0.15 0.15 0.5] X
  (if (not (Pawn|IsLocallyControlled (Variables|Default|GetActorWhoInteracted)))
    (Transformation|AddRelativeLocation (Variables|Default|GetButtonE) "0.000000,0.000000,-5.000000" false false)))

(event Custom|Multi_XReleased
  ;[0.15 0.15 0.15 0.5] X
  (if (not (Pawn|IsLocallyControlled (Variables|Default|GetActorWhoInteracted)))
    (Transformation|AddRelativeLocation (Variables|Default|GetButtonE) "0.000000,0.000000,5.000000" false false)))

(event Custom|Multi_YPressed
  ;[0.15 0.15 0.15 0.5] Y
  (if (not (Pawn|IsLocallyControlled (Variables|Default|GetActorWhoInteracted)))
    (Transformation|AddRelativeLocation (Variables|Default|GetButtonB) "0.000000,0.000000,-5.000000" false false)))

(event Custom|Multi_YReleased
  ;[0.15 0.15 0.15 0.5] Y
  (if (not (Pawn|IsLocallyControlled (Variables|Default|GetActorWhoInteracted)))
    (Transformation|AddRelativeLocation (Variables|Default|GetButtonB) "0.000000,0.000000,5.000000" false false)))

(event Custom|Multi_Interact
  (params (Target :type BP%20Player%20Object%20Reference))
  (bind _playermesh (Variables|Default|GetPlayerMesh))
  ;[0.15 0.15 0.15 0.5] StartControl
  (bind _output_get (Variables|Default|SetActorWhoInteracted Target))
  (Rendering|SetActorHiddenInGame _output_get true)
  (Rendering|Components|TextRender|SetText (Variables|Default|GetPlayerName) (Utilities|Text|ToText(String) (Variables|/Game/Blueprints/Player/BP_Player.BP_Player_C|GetUsername (Variables|Default|GetActorWhoInteracted))))
  (bind _returnvalue (Rendering|Material|CreateDynamicMaterialInstance _playermesh 1 "/Game/Models/Player/MAT_Player2.MAT_Player2" "None" :!class /Script/Engine.PrimitiveComponent))
  (Rendering|Material|SetScalarParameterValue _returnvalue "HueShift" (Variables|/Game/Blueprints/Player/BP_Player.BP_Player_C|GetHueShift (Variables|Default|GetActorWhoInteracted)) :!class /Script/Engine.MaterialInstanceDynamic)
  (Rendering|Material|SetScalarParameterValue _returnvalue "Brightness" (Variables|/Game/Blueprints/Player/BP_Player.BP_Player_C|GetBrightness (Variables|Default|GetActorWhoInteracted)) :!class /Script/Engine.MaterialInstanceDynamic)
  (Rendering|Material|SetScalarParameterValue _returnvalue "Saturation" (Variables|/Game/Blueprints/Player/BP_Player.BP_Player_C|GetSaturation (Variables|Default|GetActorWhoInteracted)) :!class /Script/Engine.MaterialInstanceDynamic)
  (Development|SetHiddeninGame _playermesh false true)
  (Variables|Default|SetTexture2D "/Game/Textures/T_CursorNormal.T_CursorNormal"))

(event EventTick
  (params (DeltaSeconds :type Float%20%28single-precision%29))
  (bind _returnvalue (Game|GetPlayerController 0))
  (bind _playername (Variables|Default|GetPlayerName))
  (bind _returnvalue_2 (Pawn|GetControlledPawn _returnvalue))
  ;[0.15 0.15 0.15 0.5] Event tick
  (if (!= _returnvalue_2 self)
    (Transformation|SetWorldRotation _playername (Math|Rotator|FindLookatRotation (Transformation|GetWorldLocation _playername) (+ (Transformation|GetActorLocation _returnvalue_2) "0.000000,0.000000,70.000000")) false false)))

(event EventBeginPlay
  (bind _rectlight (Variables|Default|GetRectLight))
  ;[0.15 0.15 0.15 0.5] Beginplay
  (if (Variables|Default|GetHasLightEffect)
    (if (Variables|Default|GetIsTurnedOn)
      (Rendering|Components|Light|SetIntensity _rectlight (Math|Random|RandomFloatinRange 1.2e+03 3.6e+03) :!label _label)
      (Utilities|FlowControl|Delay 0.5)
      (Rendering|Components|Light|SetLightColor _rectlight (+ (Variables|Default|GetScreenLight) (Math|Random|RandomFloatinRange -0.1 0.1)) true)
      (goto _label))))

(event EventServerInteract
  (params (WhoInteracted :type Actor%20Object%20Reference))
  ;[0.15 0.15 0.15 0.5] StartControl
  (if (Variables|Default|GetIsTurnedOn)
    (Variables|Default|GetActorWhoInteracted
      (:then)
      (:else
        (bind _asbp_player (Utilities|Casting|CastToBP_Player WhoInteracted))
        (bind _output_get (Variables|Default|SetActorWhoInteracted _asbp_player))
        (CallFunction|MultiInteract _output_get)
        (Default|FromServerInteractwith _output_get self)))))

(event EventOntoServerInteract
  (params (MethodName :type String))
  (if (Utilities|Array|IsEmpty MethodName)
    (CallFunction|MultiStopControl)
    (else
      (Utilities|CallMethodbyName MethodName))))

(event EventClientInteract
  (bind _returnvalue (Game|GetPlayerController 0))
  ;[0.15 0.15 0.15 0.5] StartControl
  (Game|Player|SetViewTargetwithBlend _returnvalue self 0.2 "VTBlend_Linear" 0.0 false)
  (Input|DisableInput (Pawn|GetControlledPawn _returnvalue) _returnvalue)
  (Input|EnableInput self _returnvalue)
  (Input|DisableInput _returnvalue _returnvalue)
  (bind _returnvalue_2 (Actor|GetActorOfClass "/Game/Blueprints/BP_AchievementManager.BP_AchievementManager_C"))
  (Default|Unlock _returnvalue_2 "arcade"))

(event Input|KeyboardEvents|Escape
  (params (Key :type Key%20Structure :default "None"))
  (bind _self self)
  (bind _buttona (Variables|Default|GetButtonA))
  (bind _actorwhointeracted (Variables|Default|GetActorWhoInteracted))
  ;[0.15 0.15 0.15 0.5] P
  (:Pressed
    (Transformation|AddRelativeLocation _buttona "0.000000,0.000000,-5.000000" false false)
    (CallFunction|EnteredInput "P")
    (Default|OntoServerInteractwith _actorwhointeracted _self "Multi_PPressed"))
  (:Released
    (Transformation|AddRelativeLocation _buttona "0.000000,0.000000,5.000000" false false)
    (CallFunction|ReleasedInput "P")
    (Default|OntoServerInteractwith _actorwhointeracted _self "Multi_PReleased")))

(event Input|KeyboardEvents|Enter
  (params (Key :type Key%20Structure :default "None"))
  (bind _self self)
  (bind _buttonf (Variables|Default|GetButtonF))
  (bind _actorwhointeracted (Variables|Default|GetActorWhoInteracted))
  ;[0.15 0.15 0.15 0.5] Enter
  (:Pressed
    (Transformation|AddRelativeLocation _buttonf "0.000000,0.000000,-5.000000" false false)
    (CallFunction|EnteredInput "E")
    (Default|OntoServerInteractwith _actorwhointeracted _self "Multi_EPressed"))
  (:Released
    (Transformation|AddRelativeLocation _buttonf "0.000000,0.000000,5.000000" false false)
    (CallFunction|ReleasedInput "E")
    (Default|OntoServerInteractwith _actorwhointeracted _self "Multi_EReleased")))

(event Input|KeyboardEvents|Up
  (params (Key :type Key%20Structure :default "None"))
  (bind _self self)
  (bind _actorwhointeracted (Variables|Default|GetActorWhoInteracted))
  (bind _joystickaxis (Variables|Default|GetJoystickAxis))
  ;[0.15 0.15 0.15 0.5] Up
  (:Pressed
    (Transformation|AddRelativeRotation _joystickaxis "20.000000,0.000000,0.000000" false false)
    (CallFunction|EnteredInput "U")
    (Default|OntoServerInteractwith _actorwhointeracted _self "Multi_UpPressed"))
  (:Released
    (Transformation|AddRelativeRotation _joystickaxis "-20.000000,0.000000,0.000000" false false)
    (CallFunction|ReleasedInput "U")
    (Default|OntoServerInteractwith _actorwhointeracted _self "Multi_UpReleased")))

(event Input|KeyboardEvents|Down
  (params (Key :type Key%20Structure :default "None"))
  (bind _self self)
  (bind _actorwhointeracted (Variables|Default|GetActorWhoInteracted))
  (bind _joystickaxis (Variables|Default|GetJoystickAxis))
  ;[0.15 0.15 0.15 0.5] Down
  (:Pressed
    (Transformation|AddRelativeRotation _joystickaxis "-20.000000,0.000000,0.000000" false false)
    (CallFunction|EnteredInput "D")
    (Default|OntoServerInteractwith _actorwhointeracted _self "Multi_DownPressed"))
  (:Released
    (Transformation|AddRelativeRotation _joystickaxis "20.000000,0.000000,0.000000" false false)
    (CallFunction|ReleasedInput "D")
    (Default|OntoServerInteractwith _actorwhointeracted _self "Multi_DownReleased")))

(event Input|KeyboardEvents|Left
  (params (Key :type Key%20Structure :default "None"))
  (bind _self self)
  (bind _actorwhointeracted (Variables|Default|GetActorWhoInteracted))
  (bind _joystickaxis (Variables|Default|GetJoystickAxis))
  ;[0.15 0.15 0.15 0.5] Left
  (:Pressed
    (Transformation|AddRelativeRotation _joystickaxis "0.000000,0.000000,20.000000" false false)
    (CallFunction|EnteredInput "L")
    (Default|OntoServerInteractwith _actorwhointeracted _self "Multi_LeftPressed"))
  (:Released
    (Transformation|AddRelativeRotation _joystickaxis "0.000000,0.000000,-20.000000" false false)
    (CallFunction|ReleasedInput "L")
    (Default|OntoServerInteractwith _actorwhointeracted _self "Multi_LeftReleased")))

(event Input|KeyboardEvents|Right
  (params (Key :type Key%20Structure :default "None"))
  (bind _self self)
  (bind _actorwhointeracted (Variables|Default|GetActorWhoInteracted))
  (bind _joystickaxis (Variables|Default|GetJoystickAxis))
  ;[0.15 0.15 0.15 0.5] Right
  (:Pressed
    (Transformation|AddRelativeRotation _joystickaxis "0.000000,0.000000,-20.000000" false false)
    (CallFunction|EnteredInput "R")
    (Default|OntoServerInteractwith _actorwhointeracted _self "Multi_RightPressed"))
  (:Released
    (Transformation|AddRelativeRotation _joystickaxis "0.000000,0.000000,20.000000" false false)
    (CallFunction|ReleasedInput "R")
    (Default|OntoServerInteractwith _actorwhointeracted _self "Multi_RightReleased")))

(event Input|KeyboardEvents|A
  (params (Key :type Key%20Structure :default "None"))
  (bind _self self)
  (bind _actorwhointeracted (Variables|Default|GetActorWhoInteracted))
  (bind _buttond (Variables|Default|GetButtonD))
  ;[0.15 0.15 0.15 0.5] A
  (:Pressed
    (Transformation|AddRelativeLocation _buttond "0.000000,0.000000,-5.000000" false false)
    (CallFunction|EnteredInput "A")
    (Default|OntoServerInteractwith _actorwhointeracted _self "Multi_APressed"))
  (:Released
    (Transformation|AddRelativeLocation _buttond "0.000000,0.000000,5.000000" false false)
    (CallFunction|ReleasedInput "A")
    (Default|OntoServerInteractwith _actorwhointeracted _self "Multi_AReleased")))

(event Input|KeyboardEvents|B
  (params (Key :type Key%20Structure :default "None"))
  (bind _self self)
  (bind _actorwhointeracted (Variables|Default|GetActorWhoInteracted))
  (bind _buttonc (Variables|Default|GetButtonC))
  ;[0.15 0.15 0.15 0.5] B
  (:Pressed
    (Transformation|AddRelativeLocation _buttonc "0.000000,0.000000,-5.000000" false false)
    (CallFunction|EnteredInput "B")
    (Default|OntoServerInteractwith _actorwhointeracted _self "Multi_BPressed"))
  (:Released
    (Transformation|AddRelativeLocation _buttonc "0.000000,0.000000,5.000000" false false)
    (CallFunction|ReleasedInput "B")
    (Default|OntoServerInteractwith _actorwhointeracted _self "Multi_BReleased")))

(event Input|KeyboardEvents|X
  (params (Key :type Key%20Structure :default "None"))
  (bind _self self)
  (bind _buttone (Variables|Default|GetButtonE))
  (bind _actorwhointeracted (Variables|Default|GetActorWhoInteracted))
  ;[0.15 0.15 0.15 0.5] X
  (:Pressed
    (Transformation|AddRelativeLocation _buttone "0.000000,0.000000,-5.000000" false false)
    (CallFunction|EnteredInput "X")
    (Default|OntoServerInteractwith _actorwhointeracted _self "Multi_XPressed"))
  (:Released
    (Transformation|AddRelativeLocation _buttone "0.000000,0.000000,5.000000" false false)
    (CallFunction|ReleasedInput "X")
    (Default|OntoServerInteractwith _actorwhointeracted _self "Multi_XReleased")))

(event Input|KeyboardEvents|Y
  (params (Key :type Key%20Structure :default "None"))
  (bind _self self)
  (bind _actorwhointeracted (Variables|Default|GetActorWhoInteracted))
  (bind _buttonb (Variables|Default|GetButtonB))
  ;[0.15 0.15 0.15 0.5] Y
  (:Pressed
    (Transformation|AddRelativeLocation _buttonb "0.000000,0.000000,-5.000000" false false)
    (CallFunction|EnteredInput "Y")
    (Default|OntoServerInteractwith _actorwhointeracted _self "Multi_YPressed"))
  (:Released
    (Transformation|AddRelativeLocation _buttonb "0.000000,0.000000,5.000000" false false)
    (CallFunction|ReleasedInput "Y")
    (Default|OntoServerInteractwith _actorwhointeracted _self "Multi_YReleased")))

(fn ConstructionScript
  (Rendering|Components|Light|SetLightColor (Variables|Default|GetRectLight) (Variables|Default|GetScreenLight) true))