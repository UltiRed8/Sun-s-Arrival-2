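; BP_DVManager is the Darkventure manager that tracks interactable objects and picks the one nearest the player character.
; On BeginPlay it caches the BP_DVCharacter, and its Register event adds interactables to an array.
; GetClosestInteractable linearly scans that array and returns the nearest entry whose own InteractionDistance covers the character, or None if none is in range.
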(event Custom|Register
  (params (Interactable :type BP%20DV%20Interactable%20Object%20Reference%20%28by%20ref%29))
  (Utilities|Array|Add (Variables|Default|GetInteractives) Interactable))

(event EventBeginPlay
  (bind _returnvalue (Actor|GetActorOfClass "/Game/Blueprints/Darkventure/BP_DVCharacter.BP_DVCharacter_C"))
  (Variables|Default|SetCharacter _returnvalue))

(fn ConstructionScript)

(fn GetClosestInteractable
  (LocalVariables|SetInteractable 0)
  (LocalVariables|SetDistance 999999.0)
  (for _array_element (Variables|Default|GetInteractives)
    (if (<= (Transformation|GetDistanceTo _array_element (Variables|Default|GetCharacter)) (Variables|/Game/Blueprints/Darkventure/BP_DVInteractable.BP_DVInteractable_C|GetInteractionDistance _array_element))
      (Utilities|IsValid (LocalVariables|GetInteractable)
        (:Is%20Valid
          (if (< (Transformation|GetDistanceTo _array_element (Variables|Default|GetCharacter)) (LocalVariables|GetDistance))
            (LocalVariables|SetInteractable _array_element :!label _label)
            (LocalVariables|SetDistance (Transformation|GetDistanceTo _array_element (Variables|Default|GetCharacter)))))
        (:Is%20Not%20Valid
          (goto _label)))))
  (return (LocalVariables|GetInteractable)))