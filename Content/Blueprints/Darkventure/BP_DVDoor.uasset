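; BP_DVDoor is a two-gate door in Darkventure that teleports the player between its ends on interaction.
; BeginPlay caches the BP_DVCharacter and BP_DVMusicManager actors found in the level.
; Interact compares the character's distance to GateA and GateB, then teleports it to the farther gate with zero rotation.
; It then has the music manager play that destination gate's music, followed by a short trailing delay.
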(event EventInteract
  (bind _gatea (Variables|Default|GetGateA))
  (bind _gateb (Variables|Default|GetGateB))
  (bind _character (Variables|Default|GetCharacter))
  (bind _character_2 (Variables|Default|GetCharacter))
  (bind _musicmanager (Variables|Default|GetMusicManager))
  (bind _returnvalue (Transformation|GetActorLocation _character))
  (bind _returnvalue_2 (Transformation|GetWorldLocation _gateb))
  (bind _returnvalue_3 (Transformation|GetWorldLocation _gatea))
  (if (< (Math|Vector|Distance(Vector) _returnvalue _returnvalue_3) (Math|Vector|Distance(Vector) _returnvalue _returnvalue_2))
    (Transformation|Teleport _character_2 _returnvalue_2 "0, 0, 0")
    (Default|SetMusic _musicmanager (Variables|Default|GetMusicGateB))
    (else
      (Transformation|Teleport _character_2 _returnvalue_3 "0, 0, 0")
      (Default|SetMusic _musicmanager (Variables|Default|GetMusicGateA))))
  (Utilities|FlowControl|Delay 0.2))

(event EventBeginPlay
  (bind _returnvalue (Actor|GetActorOfClass "/Game/Blueprints/Darkventure/BP_DVCharacter.BP_DVCharacter_C"))
  (Variables|Default|SetCharacter _returnvalue)
  (bind _returnvalue_2 (Actor|GetActorOfClass "/Game/Blueprints/Darkventure/BP_DVMusicManager.BP_DVMusicManager_C"))
  (Variables|Default|SetMusicManager _returnvalue_2))

(fn ConstructionScript)