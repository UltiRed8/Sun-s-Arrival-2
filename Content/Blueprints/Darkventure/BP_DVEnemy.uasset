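; BP_DVEnemy is a Darkventure enemy that belongs to the room it stands in, with an empty Activate event.
; On BeginPlay it traces a short line downward, and if it hits a BP_DVRoom it registers with that room and stores the reference.
; When a BP_DVCharacter overlaps its Box, it tells the stored room to activate its enemies rather than activating only itself.
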(event OnComponentBeginOverlap(Box)
  (params (OverlappedComponent :type Primitive%20Component%20Object%20Reference) (OtherActor :type Actor%20Object%20Reference) (OtherComp :type Primitive%20Component%20Object%20Reference) (OtherBodyIndex :type Integer) (bFromSweep :type Boolean) (SweepResult :type Hit%20Result%20Structure%20%28by%20ref%29))
  (Utilities|Casting|CastToBP_DVCharacter OtherActor)
  (bind _room (Variables|Default|GetRoom)
    (:then
      (Default|ActivateEnemies _room))
    (:else)))

(event Custom|Activate)

(event EventBeginPlay
  (bind _returnvalue (Transformation|GetActorLocation))
  (bind (_outhit _returnvalue_2) (Collision|LineTraceByChannel _returnvalue (+ _returnvalue "0.000000,0.000000,-50.000000") "TraceTypeQuery1" false 0 "None"))
  (if _returnvalue_2
    (bind _asbp_dvroom (Utilities|Casting|CastToBP_DVRoom (.HitActor (Collision|BreakHitResult _outhit))))
    (Default|RegisterEnemy _asbp_dvroom self)
    (Variables|Default|SetRoom _asbp_dvroom)))

(fn ConstructionScript)