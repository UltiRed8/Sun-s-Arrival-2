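; BP_DVMusicManager tracks the current Darkventure music state: exterior, interior, unknown presence or one of two battle variants.
; SetMusic runs Update only on a change; BeginPlay runs it one tick late.
; Update selects the matching sound, broadcasts OnMusicChanged and passes a per-state rhythm value to registered actors.
; Actors join the rhythm list through RegisterActor, and playback itself is not handled here.
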(event Custom|Update
  (bind _music (Variables|Default|GetMusic))
  (bind _returnvalue (Utilities|Select :Index _music :NewEnumerator0 "/Game/Audio/Musics/Darkventure/SW_DVExterior.SW_DVExterior" :NewEnumerator1 "/Game/Audio/Musics/Darkventure/SW_DVInterior.SW_DVInterior" :NewEnumerator2 "/Game/Audio/Musics/Darkventure/SW_DVUnknownPresence.SW_DVUnknownPresence" :NewEnumerator3 "/Game/Audio/Musics/Darkventure/SW_DVBattle.SW_DVBattle" :NewEnumerator4 "/Game/Audio/Musics/Darkventure/SW_DVBattleAlternative.SW_DVBattleAlternative"))
  (Variables|Default|SetCurrentMusic _returnvalue)
  (Default|CallOnMusicChanged _returnvalue)
  (for _array_element (Variables|Default|GetRhythmActors)
    (Default|SetRhythm _array_element (Utilities|Select :Index _music :NewEnumerator0 1.375 :NewEnumerator1 1.375 :NewEnumerator2 0.6875 :NewEnumerator3 2.75 :NewEnumerator4 2.75))))

(event Custom|SetMusic
  (params (Music :type E_DVMusic%20Enum :default "NewEnumerator0"))
  (if (Utilities|Enum|NotEqual(Enum) Music (Variables|Default|GetMusic))
    (Variables|Default|SetMusic Music)
    (CallFunction|Update)))

(event Custom|RegisterActor
  (params (NewItem :type BP%20DV%20Rhythmed%20Actor%20Object%20Reference%20%28by%20ref%29))
  (Utilities|Array|AddUnique (Variables|Default|GetRhythmActors) NewItem))

(event EventBeginPlay
  (Utilities|FlowControl|DelayUntilNextTick)
  (CallFunction|Update))

(fn ConstructionScript)