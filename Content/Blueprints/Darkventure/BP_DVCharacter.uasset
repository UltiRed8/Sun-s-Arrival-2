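; BP_DVCharacter is the Darkventure character, handling planar movement and interaction through Enhanced Input.
; Move input offsets the actor in world X/Y without sweep, scaled by delta time.
; A debug-drawn box trace on Visibility, reaching slightly beyond each step, blocks movement on a hit.
; Interact asks the BP_DVManager found at BeginPlay for the closest interactable and calls its Interact.
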(event Input|EnhancedActionEvents|EnhancedInputActionIA_Move
  (params (ActionValue :type Vector%202D%20Structure) (ElapsedSeconds :type Float%20%28double-precision%29) (TriggeredSeconds :type Float%20%28double-precision%29) (InputAction :type Input%20Action%20Object%20Reference :default "/Game/Inputs/Actions/IA_Move.IA_Move"))
  (bind _returnvalue (Transformation|GetActorLocation))
  (bind _returnvalue_2 (Math|Vector|MakeVector (.x ActionValue) (.y ActionValue) 0.0))
  (bind _returnvalue_3 (Collision|BoxTraceByChannel (+ _returnvalue "0.000000,0.000000,1.000000") (+ _returnvalue (* _returnvalue_2 5.0 (Utilities|Time|GetWorldDeltaSeconds) 1e+02) "0.000000,0.000000,1.000000") "32.000000,32.000000,0.000000" "0, 0, 0" "TraceTypeQuery1" false 0 "ForOneFrame"))
  (if (not _returnvalue_3)
    (Transformation|AddActorWorldOffset (* _returnvalue_2 4.0 (Utilities|Time|GetWorldDeltaSeconds) 1e+02))))

(event Input|EnhancedActionEvents|EnhancedInputActionIA_Interact
  (params (ActionValue :type Boolean) (ElapsedSeconds :type Float%20%28double-precision%29) (TriggeredSeconds :type Float%20%28double-precision%29) (InputAction :type Input%20Action%20Object%20Reference :default "/Game/Inputs/Actions/IA_Interact.IA_Interact"))
  (:Started
    (bind _manager (Variables|Default|GetManager)
      (:then
        (bind _interactable1 (Default|GetClosestInteractable _manager))
        (Utilities|IsValid _interactable1
          (:Is%20Valid
            (Default|Interact _interactable1))))
      (:else))))

(event EventBeginPlay
  (bind _returnvalue (Actor|GetActorOfClass "/Game/Blueprints/Darkventure/BP_DVManager.BP_DVManager_C"))
  (Variables|Default|SetManager _returnvalue))

(fn ConstructionScript)