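; Elevator door with a child-actor press button that calls its connected elevator.
; On BeginPlay it binds to the button's trigger, which tells the elevator to go to this door if the reference is valid.
; Open and close events play or reverse one timeline that slides two door panels in mirrored directions along local Y, with a FlipFlop toggle event alternating them.
; Opening also prints a debug "Hello".
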(event Custom|ToggleDoor
  (Utilities|FlowControl|FlipFlop
    (:A
      (CallFunction|OpenDoor))
    (:B
      (CallFunction|CloseDoor))))

(event Custom|OnTriggered_Event
  (bind _connectedelevator (Variables|Default|GetConnectedElevator)
    (:then
      (Default|Goto _connectedelevator self))
    (:else)))

(event Custom|OpenDoor
  (Development|PrintString "Hello")
  (bind _dooropening (Timeline|Timeline Play)
    (:Update
      (Transformation|SetRelativeLocation (Variables|Default|GetDoorA) (Math|Vector|MakeVector -6.3e+02 _dooropening 2e+02) false false)
      (Transformation|SetRelativeLocation (Variables|Default|GetDoorB) (Math|Vector|MakeVector -6.3e+02 (* _dooropening -1.0) 2e+02) false false))))

(event Custom|CloseDoor
  (bind _dooropening (Timeline|Timeline Reverse)
    (:Update
      (Transformation|SetRelativeLocation (Variables|Default|GetDoorA) (Math|Vector|MakeVector -6.3e+02 _dooropening 2e+02) false false)
      (Transformation|SetRelativeLocation (Variables|Default|GetDoorB) (Math|Vector|MakeVector -6.3e+02 (* _dooropening -1.0) 2e+02) false false))))

(event EventBeginPlay
  (bind _asbp_press_button (Utilities|Casting|CastToBP_PressButton (Variables|/Script/Engine.ChildActorComponent|GetChildActor (Variables|Default|GetChildActor))))
  (EventDispatchers|AssignOnTriggered _asbp_press_button (delegate Custom|OnTriggered_Event)))

(fn ConstructionScript)