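; Elevator actor that carries players between a list of floor actors, each linked back to it on BeginPlay.
; On authority, the first GoTo call spawns a labeled press button per floor, whose trigger calls GoTo for that floor.
; GoTo toggles floor doors and closes its sliding doors by reversing a timeline.
; Once closed, authority starts a timeline lerping the actor's height to the target, then opens the doors on arrival.
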(event Custom|GoTo
  (params (Floor :type BP%20Elevator%20Door%20Object%20Reference))
  (Networking|SwitchHasAuthority
    (:Authority
      (CallFunction|GenerateButtons))
    (:Remote
      _))
  (if (!= Floor (Variables|Default|GetFloor))
    (Variables|Default|GetIsMoving
      (:then)
      (:else
        (Variables|Default|SetIsMoving true)
        (Variables|Default|SetTargetZ (.z (Transformation|GetActorLocation Floor)))
        (Variables|Default|SetStartingZ (.z (Transformation|GetActorLocation)))
        (bind _floor (Variables|Default|GetFloor)
          (:then
            (Default|ToggleDoor _floor))
          (:else
            _))
        (Variables|Default|SetFloor Floor)
        (CallFunction|CloseDoor)))))

(event Custom|CloseDoor
  (bind (_direction _dooropening) (Timeline|Timeline Reverse)
    (:Update
      (Transformation|SetRelativeLocation (Variables|Default|GetDoorA) (Math|Vector|MakeVector -6e+02 _dooropening 2e+02) false false)
      (Transformation|SetRelativeLocation (Variables|Default|GetDoorB) (Math|Vector|MakeVector -6e+02 (* _dooropening -1.0) 2e+02) false false))
    (:Finished
      (switch Utilities|FlowControl|Switch|SwitchonETimelineDirection _direction
        (:Backward
          (Networking|SwitchHasAuthority
            (:Authority
              (CallFunction|Move (Variables|Default|GetTargetZ)))))))))

(event Custom|OpenDoor
  (bind (_direction _dooropening) (Timeline|Timeline Play)
    (:Update
      (Transformation|SetRelativeLocation (Variables|Default|GetDoorA) (Math|Vector|MakeVector -6e+02 _dooropening 2e+02) false false)
      (Transformation|SetRelativeLocation (Variables|Default|GetDoorB) (Math|Vector|MakeVector -6e+02 (* _dooropening -1.0) 2e+02) false false))
    (:Finished
      (switch Utilities|FlowControl|Switch|SwitchonETimelineDirection _direction
        (:Backward
          (Networking|SwitchHasAuthority
            (:Authority
              (CallFunction|Move (Variables|Default|GetTargetZ)))))))))

(event Custom|Move
  (params (TargetZ :type Float%20%28double-precision%29))
  (bind _returnvalue (Transformation|GetActorLocation))
  (Variables|Default|SetTargetZ TargetZ)
  (bind _progress (Timeline|Elevator PlayFromStart)
    (:Update
      (Transformation|SetActorLocation (Math|Vector|MakeVector (.x _returnvalue) (.y _returnvalue) (Math|Float|Lerp (Variables|Default|GetStartingZ) (Variables|Default|GetTargetZ) _progress)) false false))
    (:Finished
      (Networking|SwitchHasAuthority
        (:Authority
          (Default|ToggleDoor (Variables|Default|GetFloor))
          (CallFunction|OpenDoor)
          (Variables|Default|SetIsMoving false))))))

(event Custom|GenerateButtons
  (Utilities|FlowControl|DoOnce false
    (:Completed
      (for (_array_element _array_index) (Variables|Default|GetFloors)
        (bind _returnvalue (AddComponent|AddChildActorComponent false (Math|Transform|MakeTransform (+ (Variables|/Script/Engine.SceneComponent|GetRelativeLocation (Variables|Default|GetScene)) (* "0.000000,50.000000,0.000000" _array_index)) "0, 0, 0" "1.000000,1.000000,1.000000")))
        (bind _asbp_elevator_press_button (Utilities|Casting|CastToBP_ElevatorPressButton (Variables|/Script/Engine.ChildActorComponent|GetChildActor _returnvalue)))
        (Default|SetText _asbp_elevator_press_button (Variables|/Game/Blueprints/BP_ElevatorDoor.BP_ElevatorDoor_C|GetDoorLabel _array_element))
        (Variables|/Game/Blueprints/GPE/BP_ElevatorPressButton.BP_ElevatorPressButton_C|SetFloor _asbp_elevator_press_button _array_element)
        (EventDispatchers|AssignOnTriggered _asbp_elevator_press_button (delegate Custom|OnTriggered_Event))))))

(event Custom|OnTriggered_Event
  (params (Floor :type BP%20Elevator%20Door%20Object%20Reference))
  (CallFunction|Goto Floor))

(event EventBeginPlay
  (for _array_element (Variables|Default|GetFloors)
    (Variables|/Game/Blueprints/BP_ElevatorDoor.BP_ElevatorDoor_C|SetConnectedElevator _array_element self)))

(fn ConstructionScript)