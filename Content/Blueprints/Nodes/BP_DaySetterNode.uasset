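; BP_DaySetterNode is a triggerable node that switches the level's lighting to day.
; On Trigger it hides the night directional light, shows the day one, sets a fixed exponential height fog density, then calls the parent Trigger.
; It switches on the game instance's extra gamemode first, but every mode leads to the same result.
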(event EventTrigger
  (switch Utilities|FlowControl|Switch|SwitchonE_ExtrasGamemodes (Variables|/Game/BP_GameInstance.BP_GameInstance_C|GetExtraGamemode (Utilities|GameInstance))
    (:NewEnumerator0
      _)
    (:NewEnumerator1
      _)
    (:NewEnumerator2
      _)
    (:NewEnumerator3
      _))
  (Rendering|SetVisibility (Variables|/Script/Engine.Light|GetLightComponent (Variables|Default|GetNightDirectionalLight)) false false)
  (Rendering|SetVisibility (Variables|/Script/Engine.Light|GetLightComponent (Variables|Default|GetDayDirectionalLight)) true false)
  (Class|ExponentialHeightFogComponent|SetFogDensity (Variables|/Script/Engine.ExponentialHeightFog|GetComponent (Variables|Default|GetExponentialHeightFog)) 0.0109)
  (|CallParentFunction))

(fn ConstructionScript
  (|CallParentFunction))