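; Tutorial trigger volume that shows a text hint widget while the locally controlled player overlaps its box.
; One tick after BeginPlay, ReplaceText swaps up to four input placeholders in the text for key names from the active Enhanced Input key profile, matched by mapping name.
; Box overlap creates UW_Tutorial with that text and end overlap removes it, with a DoOnce on entry for single-trigger instances.
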(event OnComponentBeginOverlap(Box)
  (params (OverlappedComponent :type Primitive%20Component%20Object%20Reference) (OtherActor :type Actor%20Object%20Reference) (OtherComp :type Primitive%20Component%20Object%20Reference) (OtherBodyIndex :type Integer) (bFromSweep :type Boolean) (SweepResult :type Hit%20Result%20Structure%20%28by%20ref%29))
  (bind _asbp_player (Utilities|Casting|CastToBP_Player OtherActor))
  (if (Pawn|IsLocallyControlled _asbp_player)
    (if (Variables|Default|GetIsSingleTrigger)
      (Utilities|FlowControl|DoOnce false
        (:Completed
          _)))
    (Variables|Default|GetUI
      (:then)
      (:else
        (bind _returnvalue (UserInterface|CreateWidget "/Game/Widgets/UW_Tutorial.UW_Tutorial_C" (Game|GetPlayerController 0) (Variables|Default|GetText)))
        (bind _output_get (Variables|Default|SetUI _returnvalue))
        (UserInterface|Viewport|AddtoViewport _output_get 0)))))

(event OnComponentEndOverlap(Box)
  (params (OverlappedComponent :type Primitive%20Component%20Object%20Reference) (OtherActor :type Actor%20Object%20Reference) (OtherComp :type Primitive%20Component%20Object%20Reference) (OtherBodyIndex :type Integer))
  (bind _asbp_player (Utilities|Casting|CastToBP_Player OtherActor))
  (if (Pawn|IsLocallyControlled _asbp_player)
    (bind _ui (Variables|Default|GetUI)
      (:then
        (Default|Remove _ui)
        (Variables|Default|SetUI 0))
      (:else))))

(event EventBeginPlay
  (Utilities|FlowControl|DelayUntilNextTick)
  (bind _output_get (Variables|Default|SetStringText (Utilities|String|ToString(Text) (Variables|Default|GetText))))
  (bind _output (CallFunction|ReplaceText _output_get "{Input1}" (Variables|Default|GetMapping1)))
  (bind _output_get_2 (Variables|Default|SetStringText _output))
  (bind _output_2 (CallFunction|ReplaceText _output_get_2 "{Input2}" (Variables|Default|GetMapping2)))
  (bind _output_get_3 (Variables|Default|SetStringText _output_2))
  (bind _output_3 (CallFunction|ReplaceText _output_get_3 "{Input3}" (Variables|Default|GetMapping3)))
  (bind _output_get_4 (Variables|Default|SetStringText _output_3))
  (bind _output_4 (CallFunction|ReplaceText _output_get_4 "{Input4}" (Variables|Default|GetMapping4)))
  (Variables|Default|SetText (Utilities|Text|ToText(String) _output_4)))

(fn ConstructionScript)

(fn ReplaceText
  (params (Input :type String) (Replace :type String) (WithKeyID :type Name))
  (if (== WithKeyID "None")
    (return Input)
    (else
      (bind _values (Utilities|Map|Values (Variables|/Script/EnhancedInput.EnhancedPlayerMappableKeyProfile|GetPlayerMappedKeys (Class|EnhancedInputUserSettings|GetActiveKeyProfile (Class|EnhancedInputSubsystemInterface|GetUserSettings (PlayerController|LocalPlayerSubsystems|GetEnhancedInputLocalPlayerSubsystem (Game|GetPlayerController 0)))))))
      (bind _array_element (Utilities|Array|ForEachLoopwithBreak _values :!label _label)
        (:LoopBody
          (bind _valuepin (Utilities|Set|ForEachLoop(Set) (Utilities|Struct|BreakKeyMappingRow _array_element) :!label _label_2)
            (:then
              (if (== (.MappingName (Utilities|Struct|BreakPlayerKeyMapping _valuepin)) WithKeyID)
                (Utilities|FlowControl|Sequence
                  (:then_0
                    (goto _label_2 BreakPin))
                  (:then_1
                    (goto _label Break))
                  (:then_2
                    (return (Utilities|String|Replace Input Replace (Utilities|String|ToString(Text) (Class|KismetInputLibrary|KeyGetDisplayName (.CurrentKey (Utilities|Struct|BreakPlayerKeyMapping _valuepin)) false))))))))))))))