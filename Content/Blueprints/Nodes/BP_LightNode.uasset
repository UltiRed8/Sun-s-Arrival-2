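; BP_LightNode is a triggerable node that switches a target light and a target wall light to a configured new state.
; Trigger calls a server event and then the parent's Trigger.
; The server event relays to a multi event, apparently a multicast for replication, which calls SetState on whichever targets are valid.
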(event Custom|Server_Trigger
  (CallFunction|MultiTrigger))

(event Custom|Multi_Trigger
  (bind _targetlight (Variables|Default|GetTargetLight)
    (:then
      (Default|SetState _targetlight (Variables|Default|GetNewState)))
    (:else
      _))
  (bind _targetwalllight (Variables|Default|GetTargetWallLight)
    (:then
      (Default|SetState _targetwalllight (Variables|Default|GetNewState)))
    (:else)))

(event EventTrigger
  (CallFunction|ServerTrigger)
  (|CallParentFunction))

(fn ConstructionScript
  (|CallParentFunction))