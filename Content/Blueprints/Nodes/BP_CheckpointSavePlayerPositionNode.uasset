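; Trigger node that saves the player's current position as the checkpoint position.
; When triggered, it proceeds only if the room manager is fully loaded and the node is enabled, then stores the pawn's location with zero rotation and unit scale.
; After a short delay it saves through the game instance and calls the parent trigger, with a DoOnce that resets later to throttle repeat saves.
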(event EventTrigger
  (bind _returnvalue (Actor|GetActorOfClass "/Game/Blueprints/GPE/Rooms/BP_RoomManager.BP_RoomManager_C"))
  (if (Variables|/Game/Blueprints/GPE/Rooms/BP_RoomManager.BP_RoomManager_C|GetIsFullyLoaded _returnvalue)
    (if (Variables|Default|GetIsEnabled)
      (Utilities|FlowControl|DoOnce false :!label _label
        (:Completed
          (Variables|/Game/Saves/SG_Checkpoint.SG_Checkpoint_C|SetPlayerPosition (Utilities|GetCheckpoint) (Math|Transform|MakeTransform (Transformation|GetActorLocation (Game|Player|GetPlayerPawn 0)) "0, 0, 0" "1.000000,1.000000,1.000000"))
          (Utilities|FlowControl|Delay 0.2)
          (Default|SaveSave (Utilities|GameInstance))
          (|CallParentFunction)
          (Utilities|FlowControl|Delay 1e+01)
          (goto _label Reset))))))

(fn ConstructionScript
  (|CallParentFunction))