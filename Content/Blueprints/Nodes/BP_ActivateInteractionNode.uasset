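; BP_ActivateInteractionNode is a trigger node that makes a list of interaction actors interactable.
; Trigger calls a server event that multicasts the activation and saves a checkpoint bool keyed by the node's location string.
; The activation sets each actor's CanInteract and switches any custom cursor component to the interact texture.
; BeginPlay reads that checkpoint and reapplies the activation if it was saved as true.
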(event Custom|Multi_UpdateActivation
  (if (Utilities|Array|IsNotEmpty (Variables|Default|GetInteractionsActorToActivate))
    (for _array_element (Variables|Default|GetInteractionsActorToActivate)
      (Variables|/Game/Blueprints/GPE/BP_InteractableActor.BP_InteractableActor_C|SetCanInteract _array_element true)
      (Utilities|IsValid (Variables|/Game/Blueprints/GPE/BP_InteractableActor.BP_InteractableActor_C|GetBP_CustomCursorComponent _array_element)
        (:Is%20Valid
          (Variables|/Game/Blueprints/Components/BP_CustomCursorComponent.BP_CustomCursorComponent_C|SetCursorTexture (Variables|/Game/Blueprints/GPE/BP_InteractableActor.BP_InteractableActor_C|GetBP_CustomCursorComponent _array_element) "/Game/Textures/T_CursorInteract.T_CursorInteract"))))))

(event Custom|Server_UpdateActivation
  (CallFunction|MultiUpdateActivation)
  (Utilities|CheckpointSaveBool (Utilities|String|ToString(Vector) (Transformation|GetActorLocation)) true))

(event EventBeginPlay
  (|CallParentFunction)
  (bind (_success _bool) (Utilities|CheckpointGetBool (Utilities|String|ToString(Vector) (Transformation|GetActorLocation))))
  (if _success
    (if _bool
      (if (Utilities|Array|IsNotEmpty (Variables|Default|GetInteractionsActorToActivate))
        (for _array_element (Variables|Default|GetInteractionsActorToActivate)
          (Variables|/Game/Blueprints/GPE/BP_InteractableActor.BP_InteractableActor_C|SetCanInteract _array_element true)
          (Utilities|IsValid (Variables|/Game/Blueprints/GPE/BP_InteractableActor.BP_InteractableActor_C|GetBP_CustomCursorComponent _array_element)
            (:Is%20Valid
              (Variables|/Game/Blueprints/Components/BP_CustomCursorComponent.BP_CustomCursorComponent_C|SetCursorTexture (Variables|/Game/Blueprints/GPE/BP_InteractableActor.BP_InteractableActor_C|GetBP_CustomCursorComponent _array_element) "/Game/Textures/T_CursorInteract.T_CursorInteract"))))))))

(event EventTrigger
  (CallFunction|ServerUpdateActivation)
  (|CallParentFunction))

(fn ConstructionScript
  (|CallParentFunction))