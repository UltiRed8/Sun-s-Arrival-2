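; BP_DoorNode is a triggerable node that unlocks a target door and optionally toggles it.
; On Trigger it calls ServerUnlock on a valid TargetDoor, then ServerToggleDoor if ShouldToggleDoor is set.
; It then casts the door to BP_PanelDoor and calls MultiOpen before running the parent Trigger.
; A missing door goes straight to the parent Trigger, while a failed cast ends without calling it.
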(event EventTrigger
  (bind _targetdoor (Variables|Default|GetTargetDoor)
    (:then
      (Default|ServerUnlock _targetdoor)
      (if (Variables|Default|GetShouldToggleDoor)
        (Default|ServerToggleDoor _targetdoor))
      (bind _asbp_panel_door (Utilities|Casting|CastToBP_PanelDoor (Variables|Default|GetTargetDoor)))
      (Default|MultiOpen _asbp_panel_door))
    (:else
      _))
  (|CallParentFunction))

(fn ConstructionScript
  (|CallParentFunction))