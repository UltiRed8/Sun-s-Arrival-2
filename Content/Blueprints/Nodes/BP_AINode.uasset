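; AI node that puts its assigned Enemy into its default state when triggered, then runs the parent node's trigger.
; Triggering runs a MultiTrigger event and saves a checkpoint bool keyed by the node's world location.
; On BeginPlay it reads that saved bool and replays the trigger if it was set, so activation carries over through checkpoints.
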(event Custom|Multi_Trigger
  (bind _enemy (Variables|Default|GetEnemy))
  (Utilities|IsValid _enemy
    (:Is%20Valid
      (Default|DefaultState _enemy)
      (|CallParentFunction))))

(event EventBeginPlay
  (|CallParentFunction)
  (bind (_success _bool) (Utilities|CheckpointGetBool (Utilities|String|ToString(Vector) (Transformation|GetActorLocation))))
  (if _success
    (if _bool
      (CallFunction|MultiTrigger))))

(event EventTrigger
  (CallFunction|MultiTrigger)
  (Utilities|CheckpointSaveBool (Utilities|String|ToString(Vector) (Transformation|GetActorLocation)) true))

(fn ConstructionScript
  (|CallParentFunction))