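; BP_CounterNode is a trigger node that passes a Trigger on to its parent logic only when its countdown reaches exactly zero.
; Each Trigger decrements Counter and saves the value as a checkpoint integer.
; BeginPlay restores any saved count, using the actor's location string as the save ID, so each node's identity depends on its position.
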(event EventBeginPlay
  (|CallParentFunction)
  (bind (_success _int) (Utilities|CheckpointGetInt (Utilities|String|ToString(Vector) (Transformation|GetActorLocation))))
  (if _success
    (Variables|Default|SetCounter _int)))

(event EventTrigger
  (bind _result (Math|Integer|DecrementInt (Variables|Default|GetCounter))
    (:%20%20
      (Utilities|CheckpointSaveInt (Utilities|String|ToString(Vector) (Transformation|GetActorLocation)) _result)
      (if (== _result 0)
        (|CallParentFunction)))))

(fn ConstructionScript
  (|CallParentFunction))