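; Base node actor for chaining triggers between actors placed in a level.
; Trigger calls Trigger on every entry in its Nodes array, passing the signal downstream with no delay or condition.
; EditorTick draws red debug arrows from the node to each linked entry to visualise the connections.
; The construction script adds a child actor component.
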(event Custom|Trigger
  (for _array_element (Variables|Default|GetNodes)
    (CallFunction|Trigger _array_element)))

(event EventEditorTick
  (for _array_element (Variables|Default|GetNodes)
    (Rendering|Debug|DrawDebugArrow (Transformation|GetActorLocation) (Transformation|GetActorLocation _array_element) 5e+03 "(R=1.000000,G=0.000000,B=0.000000,A=1.000000)" 0.0 5.0)))

(fn ConstructionScript
  (AddComponent|AddChildActorComponent false))