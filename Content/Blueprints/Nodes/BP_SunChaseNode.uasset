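; Level node that starts the Sun chase phase, saving a checkpoint flag by location to replay setup on load.
; Setup awards no-map/no-flashlight achievements, teleports the player, streams in F2_SunPhase, locks doors, clears enemies, kills lights, raises alarms and calls the elevator.
; Sun initializes after a delay on fresh triggers, immediately on restore, and can move once a timer sees the player leave the node.
; Trigger boxes fire gated camera-shake rumbles with distant explosions.
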(event Custom|Setup
  (params (WithInit :type Boolean))
  (bind _asbp_game_instance (Utilities|GameInstance))
  (bind _checkpoint (Variables|/Game/BP_GameInstance.BP_GameInstance_C|GetCheckpoint _asbp_game_instance))
  (if (Variables|/Game/Saves/SG_Checkpoint.SG_Checkpoint_C|GetHasUsedMapDevice _checkpoint)
    _
    (else
      (Default|UnlockAchievement _asbp_game_instance "ACH_NoMapDevice")))
  (if (Variables|/Game/Saves/SG_Checkpoint.SG_Checkpoint_C|GetHasUsedFlashlight _checkpoint)
    _
    (else
      (Default|UnlockAchievement _asbp_game_instance "ACH_NoFlashlight")))
  (|CallParentFunction)
  (Utilities|FlowControl|Sequence
    (:then_0
      (bind _returnvalue (Actor|GetActorOfClass "/Game/Blueprints/Player/BP_Player.BP_Player_C"))
      (bind _output_get (Variables|Default|SetPlayerRef _returnvalue))
      (if (Variables|/Game/Blueprints/Player/BP_Player.BP_Player_C|GetFlashlightStatus _output_get)
        _
        (else
          (Default|ToggleFlashlight _output_get)))
      (Transformation|SetActorLocation _returnvalue (Transformation|GetActorLocation) false false)
      (Pawn|SetControlRotation (Game|GetPlayerController 0) (Transformation|GetActorRotation))
      (switch Utilities|FlowControl|Switch|SwitchonE_ExtrasGamemodes (Variables|/Game/BP_GameInstance.BP_GameInstance_C|GetExtraGamemode (Utilities|GameInstance))
        (:NewEnumerator0
          _)
        (:NewEnumerator2
          _)
        (:NewEnumerator3
          _))
      (bind _outactors (Actor|GetAllActorsOfClass "/Game/Blueprints/Decoratives/BP_Alarm.BP_Alarm_C"))
      (for _array_element _outactors
        (Default|SetActive _array_element))
      (Class|GameplayStatics|LoadStreamLevelbySoftObjectPtr "/Game/Levels/SubLevelsFactory2/F2_SunPhase.F2_SunPhase" true true)
      (for _array_element_2 (Variables|Default|GetDoorsToLock)
        (Default|SetForceLocked _array_element_2))
      (bind _outactors_2 (Actor|GetAllActorsOfClass "/Game/Blueprints/Enemies/BP_EndoBase.BP_EndoBase_C"))
      (for _array_element_3 _outactors_2
        (Class|KismetSystemLibrary|IsObjectOfSoftClass _array_element_3 "/Game/Blueprints/Enemies/BP_EndoChase.BP_EndoChase_C"
          (:True
            _)
          (:False
            (Class|KismetSystemLibrary|IsObjectOfSoftClass _array_element_3 "/Game/Blueprints/Enemies/BP_EndoLight.BP_EndoLight_C"
              (:True
                _)
              (:False
                (Class|KismetSystemLibrary|IsObjectOfSoftClass _array_element_3 "/Game/Blueprints/Enemies/BP_EndoSight.BP_EndoSight_C"
                  (:True
                    _))))))
        (Actor|DestroyActor _array_element_3))
      (bind _outactors_3 (Actor|GetAllActorsOfClass "/Game/Blueprints/Enemies/BP_StandEndo.BP_StandEndo_C"))
      (for _array_element_4 _outactors_3
        (if (Variables|/Game/Blueprints/Enemies/BP_StandEndo.BP_StandEndo_C|GetIsAttacking _array_element_4)
          (Actor|DestroyActor _array_element_4)))
      (Default|StartFireAmbiance (Variables|Default|GetElevator))
      (bind _outactors_4 (Actor|GetAllActorsOfClass "/Game/Blueprints/GPE/Lights/BP_SuspendedLight.BP_SuspendedLight_C"))
      (for _array_element_5 _outactors_4
        (Default|Off _array_element_5))
      (for _array_element_6 (Variables|Default|GetActorsToDestroy)
        (Actor|DestroyActor _array_element_6))
      (bind _outactors_5 (Actor|GetAllActorsOfClass "/Game/Blueprints/GPE/Lights/BP_WallLight.BP_WallLight_C"))
      (for _array_element_7 _outactors_5
        (Default|Off _array_element_7))
      (Audio|Components|Audio|Play (Variables|Default|GetAudio) 0.0)
      (for _array_element_8 (Variables|Default|GetRumbleTriggers)
        (EventDispatchers|AssignOnPlayerTriggeredBox _array_element_8 (delegate Custom|Rumble)))
      (Variables|/Game/Blueprints/GPE/BP_BigMachine.BP_BigMachine_C|SetConditionsMet (Variables|Default|GetBigMachine) true)
      (Default|CallElevator (Variables|Default|GetElevatorFloor))
      (bind _returnvalue_2 (Utilities|Time|SetTimerbyEvent (delegate Custom|CheckForPlayerMovement) 0.1 true))
      (Variables|Default|SetPlayerMovementCheckTimer _returnvalue_2)
      (for _array_element_9 (Variables|Default|GetAllSAS)
        (Variables|/Game/Blueprints/GPE/BP_SecurityDoor.BP_SecurityDoor_C|SetCanClose _array_element_9 false)))
    (:then_1
      (if WithInit
        (Utilities|FlowControl|Delay 8.7)
        (Default|Init (Variables|Default|GetSun))))))

(event Custom|Rumble
  (bind _rumbleaudio (Variables|Default|GetRumbleAudio))
  (bind _distantexplosion (Variables|Default|GetDistantExplosion))
  (Utilities|FlowControl|Gate false :!label _label
    (:Exit
      (Utilities|FlowControl|Sequence
        (:then_0
          (goto _label Close))
        (:then_1
          (Default|CameraShake (Utilities|GameInstance) "/Game/Shakes/CS_Rumble.CS_Rumble_C" "0, 0, 0" 99999999.0 0.0 0.0 false)
          (Audio|Components|Audio|Play _rumbleaudio (Math|Random|RandomFloatinRange 0.0 5.0))
          (Utilities|FlowControl|Sequence
            (:then_0
              (bind _volume (Timeline|RumbleVolume PlayFromStart)
                (:Update
                  (Audio|Components|Audio|SetVolumeMultiplier _rumbleaudio _volume :!class /Script/Engine.AudioComponent))
                (:Finished
                  (Utilities|FlowControl|Delay 0.2)
                  (goto _label Open))))
            (:then_1
              (Utilities|FlowControl|Delay (Math|Random|RandomFloatinRange 1.0 2.5))
              (Audio|Components|Audio|SetPitchMultiplier _distantexplosion (Math|Random|RandomFloatinRange 0.5 1.5) :!label _label_2)
              (Audio|Components|Audio|Play _distantexplosion 0.0))
            (:then_2
              (Utilities|FlowControl|Delay (Math|Random|RandomFloatinRange 4.0 5.0))
              (goto _label_2))))))))

(event Custom|OnLoadingCompleted_Event
  (bind _returnvalue (Actor|GetActorOfClass "/Game/Blueprints/GPE/Rooms/BP_RoomManager.BP_RoomManager_C"))
  (EventDispatchers|UnbindEventfromOnLoadingCompleted _returnvalue (delegate Custom|OnLoadingCompleted_Event))
  (bind (_success _bool) (Utilities|CheckpointGetBool (Utilities|String|ToString(Vector) (Transformation|GetActorLocation))))
  (if _success
    (if _bool
      (CallFunction|Setup false)
      (Default|Init (Variables|Default|GetSun)))))

(event Custom|CheckForPlayerMovement
  (if (>= (Transformation|GetDistanceTo (Variables|Default|GetPlayerRef) self) 2e+02)
    (Utilities|Time|ClearandInvalidateTimerbyHandle (Variables|Default|GetPlayerMovementCheckTimer))
    (Default|SetCanMove (Variables|Default|GetSun))))

(event EventTrigger
  (Utilities|CheckpointSaveBool (Utilities|String|ToString(Vector) (Transformation|GetActorLocation)) true)
  (CallFunction|Setup true))

(event EventBeginPlay
  (bind _returnvalue (Actor|GetActorOfClass "/Game/Blueprints/GPE/Rooms/BP_RoomManager.BP_RoomManager_C"))
  (EventDispatchers|AssignOnLoadingCompleted _returnvalue (delegate Custom|OnLoadingCompleted_Event)))

(fn ConstructionScript
  (|CallParentFunction))