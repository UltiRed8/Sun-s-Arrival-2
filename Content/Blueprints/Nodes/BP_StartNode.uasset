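; BP_StartNode is a node actor that plays the game's one-time intro once BP_RoomManager finishes loading.
; It runs when active or in packaged builds, using a location-keyed checkpoint to skip straight to enabling input if already played.
; The intro fires StartNode, plays LS_Start between transition widgets with players hidden and timed by delays, then restores input, fires EndNode and awards extra-gamemode achievements.
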(event Custom|OnLoadingCompleted_Event
  (bind _returnvalue (Transformation|GetActorLocation))
  (bind _returnvalue_2 (Game|GetPlayerController 0))
  (bind _returnvalue_3 (Game|GetPlayerController 0))
  (bind _asbp_game_instance (Utilities|GameInstance))
  (bind _returnvalue_4 (Utilities|String|ToString(Vector) _returnvalue))
  (if (or (Variables|Default|GetIsActive) (Class|KismetSystemLibrary|IsPackagedforDistribution))
    (bind (_success _bool) (Utilities|CheckpointGetBool _returnvalue_4))
    (if _success
      (if _bool
        (Input|EnableInput (Pawn|GetControlledPawn _returnvalue_3) _returnvalue_3 :!label _label)
        (else
          (Utilities|CheckpointSaveBool _returnvalue_4 true :!label _label_2)
          (Default|Trigger (Variables|Default|GetStartNode))
          (bind _returnvalue_5 (UserInterface|CreateWidget "/Game/Widgets/UW_Transition.UW_Transition_C" 0 1.5))
          (UserInterface|Viewport|AddtoViewport _returnvalue_5 10)
          (Utilities|FlowControl|Delay 0.5)
          (bind _returnvalue_6 (Sequencer|Player|CreateLevelSequencePlayer "/Game/Sequences/LS_Start.LS_Start"))
          (Sequencer|Player|Play _returnvalue_6 :!class /Script/MovieScene.MovieSceneSequencePlayer)
          (bind _outactors (Actor|GetAllActorsOfClass "/Game/Blueprints/Player/BP_Player.BP_Player_C"))
          (for _array_element _outactors
            (Rendering|SetActorHiddenInGame _array_element true))
          (Utilities|FlowControl|Delay 15.0)
          (bind _returnvalue_7 (UserInterface|CreateWidget "/Game/Widgets/UW_Transition.UW_Transition_C" 0 1.0))
          (UserInterface|Viewport|AddtoViewport _returnvalue_7 10)
          (bind _outactors_2 (Actor|GetAllActorsOfClass "/Game/Blueprints/Player/BP_Player.BP_Player_C"))
          (for _array_element_2 _outactors_2
            (Rendering|SetActorHiddenInGame _array_element_2 false))
          (Input|EnableInput (Pawn|GetControlledPawn _returnvalue_2) _returnvalue_2)
          (Default|Trigger (Variables|Default|GetEndNode))
          (switch Utilities|FlowControl|Switch|SwitchonE_ExtrasGamemodes (Variables|/Game/BP_GameInstance.BP_GameInstance_C|GetExtraGamemode _asbp_game_instance)
            (:NewEnumerator1
              (Class|EOSGameInstance|GiveAchievement _asbp_game_instance "ACH_EXPLORATION"))
            (:NewEnumerator2
              (Class|EOSGameInstance|GiveAchievement _asbp_game_instance "ACH_HARDSTART"))
            (:NewEnumerator3
              (Class|EOSGameInstance|GiveAchievement _asbp_game_instance "ACH_CHAOSSTART")))))
      (else
        (goto _label_2)))
    (else
      (goto _label))))

(event EventBeginPlay
  (bind _returnvalue (Actor|GetActorOfClass "/Game/Blueprints/GPE/Rooms/BP_RoomManager.BP_RoomManager_C"))
  (EventDispatchers|AssignOnLoadingCompleted _returnvalue (delegate Custom|OnLoadingCompleted_Event)))

(event EventDestroyed
  (bind _returnvalue (Actor|GetActorOfClass "/Game/Blueprints/GPE/Rooms/BP_RoomManager.BP_RoomManager_C"))
  (EventDispatchers|UnbindEventfromOnLoadingCompleted _returnvalue (delegate Custom|OnLoadingCompleted_Event)))

(fn ConstructionScript
  (AddComponent|AddChildActorComponent false))