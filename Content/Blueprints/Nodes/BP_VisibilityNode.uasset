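; BP_VisibilityNode is a triggerable node that shows or hides a set of actors.
; Trigger calls a server event, which relays to a multicast event, then runs the parent Trigger.
; The multicast loops over the Actors array and sets each actor's hidden-in-game state from the inverse of ToVisible.
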(event Custom|Multi_UpdateVisibility
  (for _array_element (Variables|Default|GetActors)
    (Rendering|SetActorHiddenInGame _array_element (not (Variables|Default|GetToVisible)))))

(event Custom|Server_UpdateVisibility
  (CallFunction|MultiUpdateVisibility))

(event EventTrigger
  (CallFunction|ServerUpdateVisibility)
  (|CallParentFunction))

(fn ConstructionScript
  (|CallParentFunction))