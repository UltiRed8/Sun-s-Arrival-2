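; BP_ObjectiveNode is a triggerable node that sets a new objective on the player's map device.
; It only arms shortly after BP_RoomManager reports loading completed, then unbinds from that event.
; When armed and triggered, it skips Exploration mode; other modes route through a server event to a multi event that updates the local player's BP_MapDevice.
; The parent Trigger always runs afterwards.
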(event Custom|Multi_SetObjective
  (bind _asbp_player (Utilities|Casting|CastToBP_Player (Pawn|GetControlledPawn (Game|GetPlayerController 0))))
  (bind _asbp_map_device (Utilities|Casting|CastToBP_MapDevice (Variables|/Script/Engine.ChildActorComponent|GetChildActor (Variables|/Game/Blueprints/Player/BP_Player.BP_Player_C|GetMapDeviceActor _asbp_player))))
  (Default|SetNewObjective _asbp_map_device (Variables|Default|GetObjective)))

(event Custom|OnLoadingCompleted_Event
  (Utilities|FlowControl|Delay 0.2)
  (Variables|Default|SetIsValid true)
  (bind _returnvalue (Actor|GetActorOfClass "/Game/Blueprints/GPE/Rooms/BP_RoomManager.BP_RoomManager_C"))
  (EventDispatchers|UnbindEventfromOnLoadingCompleted _returnvalue (delegate Custom|OnLoadingCompleted_Event)))

(event Custom|Server_SetObjective
  (CallFunction|MultiSetObjective))

(event EventBeginPlay
  (bind _returnvalue (Actor|GetActorOfClass "/Game/Blueprints/GPE/Rooms/BP_RoomManager.BP_RoomManager_C"))
  (Utilities|IsValid _returnvalue
    (:Is%20Valid
      (EventDispatchers|AssignOnLoadingCompleted _returnvalue (delegate Custom|OnLoadingCompleted_Event)))))

(event EventTrigger
  (if (Variables|Default|GetIsValid)
    (switch Utilities|FlowControl|Switch|SwitchonE_ExtrasGamemodes (Variables|/Game/BP_GameInstance.BP_GameInstance_C|GetExtraGamemode (Utilities|GameInstance))
      (:NewEnumerator0
        (CallFunction|ServerSetObjective :!label _label))
      (:NewEnumerator1
        _)
      (:NewEnumerator2
        (goto _label))
      (:NewEnumerator3
        (goto _label))))
  (|CallParentFunction))

(fn ConstructionScript
  (|CallParentFunction))