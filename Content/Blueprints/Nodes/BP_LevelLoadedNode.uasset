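; BP_LevelLoadedNode is a node actor that fires its inherited Trigger when level loading completes.
; On BeginPlay it finds BP_RoomManager and binds to its OnLoadingCompleted event, then unbinds and triggers when that event fires.
; If no room manager exists, it triggers after a one-second delay instead.
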(event Custom|OnLoadingCompleted_Event
  (bind _returnvalue (Actor|GetActorOfClass "/Game/Blueprints/GPE/Rooms/BP_RoomManager.BP_RoomManager_C"))
  (EventDispatchers|UnbindEventfromOnLoadingCompleted _returnvalue (delegate Custom|OnLoadingCompleted_Event))
  (CallFunction|Trigger))

(event EventBeginPlay
  (bind _returnvalue (Actor|GetActorOfClass "/Game/Blueprints/GPE/Rooms/BP_RoomManager.BP_RoomManager_C"))
  (Utilities|IsValid _returnvalue
    (:Is%20Valid
      (EventDispatchers|AssignOnLoadingCompleted _returnvalue (delegate Custom|OnLoadingCompleted_Event)))
    (:Is%20Not%20Valid
      (Utilities|FlowControl|Delay 1.0)
      (CallFunction|Trigger))))

(fn ConstructionScript
  (|CallParentFunction))