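; Victory node that ends the game when triggered with BP_BigMachine's conditions met; Exploration mode only runs the parent trigger.
; A win marks the checkpoint completed and saves it along with the current mode's completion flag.
; Multi_Win plays LS_Victory with the player's customization copied onto a skeletal mesh actor, destroys endos and hides players.
; It then shows the victory game-over widget, while a parallel branch grants the mode's achievement.
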(event Custom|Multi_Win
  (bind _returnvalue (Game|GetPlayerController 0))
  (bind _asbp_game_instance (Utilities|GameInstance))
  (bind _skeletalmeshactor (Variables|Default|GetSkeletalMeshActor))
  (Utilities|FlowControl|Sequence
    (:then_0
      (bind _returnvalue_2 (UserInterface|CreateWidget "/Game/Widgets/UW_Transition.UW_Transition_C"))
      (UserInterface|Viewport|AddtoViewport _returnvalue_2 10)
      (Utilities|FlowControl|Delay 0.5)
      (bind _returnvalue_3 (Sequencer|Player|CreateLevelSequencePlayer "/Game/Sequences/LS_Victory.LS_Victory"))
      (Sequencer|Player|Play _returnvalue_3 :!class /Script/MovieScene.MovieSceneSequencePlayer)
      (bind _asbp_player (Utilities|Casting|CastToBP_Player (Pawn|GetControlledPawn (Game|GetPlayerController 0))))
      (bind _returnvalue_4 (AddComponent|AddBPPlayerCustomizationComponent _skeletalmeshactor))
      (Default|Init _returnvalue_4 (Utilities|Array|MakeArray (Variables|/Script/Engine.SkeletalMeshActor|GetSkeletalMeshComponent _skeletalmeshactor)))
      (Default|CopyData (Variables|/Game/Blueprints/Player/BP_Player.BP_Player_C|GetBP_PlayerCustomizationComponent _asbp_player) _returnvalue_4)
      (bind _outactors (Actor|GetAllActorsOfClass "/Game/Blueprints/Enemies/BP_EndoBase.BP_EndoBase_C"))
      (for _array_element _outactors
        (Actor|DestroyActor _array_element))
      (bind _outactors_2 (Actor|GetAllActorsOfClass "/Game/Blueprints/Player/BP_Player.BP_Player_C"))
      (for _array_element_2 _outactors_2
        (Rendering|SetActorHiddenInGame _array_element_2 true))
      (Utilities|FlowControl|Delay 4.9)
      (Sequencer|Player|Pause _returnvalue_3)
      (bind _returnvalue_5 (UserInterface|CreateWidget "/Game/Widgets/UW_GameOver.UW_GameOver_C" _returnvalue true (Ability|HasAuthority _returnvalue)))
      (UserInterface|Viewport|AddtoViewport _returnvalue_5 0))
    (:then_1
      (switch Utilities|FlowControl|Switch|SwitchonE_ExtrasGamemodes (Variables|/Game/BP_GameInstance.BP_GameInstance_C|GetExtraGamemode _asbp_game_instance)
        (:NewEnumerator0
          (Class|EOSGameInstance|GiveAchievement _asbp_game_instance "ACH_ESCAPE"))
        (:NewEnumerator2
          (Class|EOSGameInstance|GiveAchievement _asbp_game_instance "ACH_HARDEND"))
        (:NewEnumerator3
          (Class|EOSGameInstance|GiveAchievement _asbp_game_instance "ACH_CHAOSEND"))))))

(event EventTrigger
  (bind _asbp_game_instance (Utilities|GameInstance))
  (bind _asbp_game_instance_2 (Utilities|GameInstance))
  (switch Utilities|FlowControl|Switch|SwitchonE_ExtrasGamemodes (Variables|/Game/BP_GameInstance.BP_GameInstance_C|GetExtraGamemode (Utilities|GameInstance))
    (:NewEnumerator0
      (bind _returnvalue (Actor|GetActorOfClass "/Game/Blueprints/GPE/BP_BigMachine.BP_BigMachine_C" :!label _label))
      (Utilities|IsValid _returnvalue
        (:Is%20Valid
          (if (Variables|/Game/Blueprints/GPE/BP_BigMachine.BP_BigMachine_C|GetConditionsMet _returnvalue)
            (CallFunction|MultiWin)
            (|CallParentFunction)
            (Variables|/Game/Saves/SG_Checkpoint.SG_Checkpoint_C|SetCompleted (Variables|/Game/BP_GameInstance.BP_GameInstance_C|GetCheckpoint _asbp_game_instance) true)
            (Default|SaveSave _asbp_game_instance)
            (bind _gamecompletion (Default|GetExtras _asbp_game_instance_2))
            (switch Utilities|FlowControl|Switch|SwitchonE_ExtrasGamemodes (Variables|/Game/BP_GameInstance.BP_GameInstance_C|GetExtraGamemode _asbp_game_instance_2)
              (:NewEnumerator0
                (Variables|/Game/Saves/SG_GameCompletion.SG_GameCompletion_C|SetNormalMode _gamecompletion true))
              (:NewEnumerator2
                (Variables|/Game/Saves/SG_GameCompletion.SG_GameCompletion_C|SetHardcoreMode _gamecompletion true))
              (:NewEnumerator3
                (Variables|/Game/Saves/SG_GameCompletion.SG_GameCompletion_C|SetChaosMode _gamecompletion true)))
            (Default|SaveExtras _asbp_game_instance_2)))))
    (:NewEnumerator1
      (|CallParentFunction))
    (:NewEnumerator2
      (goto _label))
    (:NewEnumerator3
      (goto _label))))

(fn ConstructionScript
  (|CallParentFunction))