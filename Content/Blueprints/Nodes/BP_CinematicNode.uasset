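; Node that, when triggered with a living player present, plays a level sequence behind transition widgets, suspending player input and HUD.
; It clears Endo enemies meanwhile, storing transforms and sinking Chase, Light and Sight types underground while hiding Block and attacking Stand ones.
; The authority can skip skippable cinematics by double-pressing Interact, using paired timed gates.
; A multicast end event stops the sequence, restores enemies on authority and returns player control.
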(event Custom|PlayCinematic
  (bind _returnvalue (Game|GetPlayerController 0))
  (bind _asbp_player (Utilities|Casting|CastToBP_Player (Pawn|GetControlledPawn _returnvalue)))
  (Input|DisableInput _asbp_player _returnvalue)
  (bind _returnvalue_2 (UserInterface|CreateWidget "/Game/Widgets/UW_Transition.UW_Transition_C"))
  (UserInterface|Viewport|AddtoViewport _returnvalue_2 10)
  (Utilities|FlowControl|Delay 0.5)
  (Widget|SetVisibility (Variables|/Game/Blueprints/Player/BP_Player.BP_Player_C|GetInGame _asbp_player) "Collapsed")
  (if (Variables|Default|GetCanBeSkipped)
    (Utilities|Authority
      (:Authority
        (bind _returnvalue_3 (UserInterface|CreateWidget "/Game/Widgets/UW_Cinematic.UW_Cinematic_C" (Game|GetPlayerController 0)))
        (UserInterface|Viewport|AddtoViewport _returnvalue_3 0)
        (Variables|Default|SetSkipWidget _returnvalue_3)
        (Input|EnableInput self (Game|GetPlayerController 0)))
      (:Remote
        _)))
  (bind _returnvalue_4 (Sequencer|Player|CreateLevelSequencePlayer (Variables|Default|GetSequence)))
  (Sequencer|Player|Play _returnvalue_4 :!class /Script/MovieScene.MovieSceneSequencePlayer)
  (Variables|Default|SetSequencePlayer _returnvalue_4))

(event Custom|Multi_EndCinematic
  (bind _returnvalue (Game|GetPlayerController 0))
  (Utilities|FlowControl|DoOnce false
    (:Completed
      (Utilities|FlowControl|Sequence
        (:then_0
          (Utilities|FlowControl|Delay 0.5)
          (Sequencer|Player|Stop (Variables|Default|GetSequencePlayer) :!class /Script/MovieScene.MovieSceneSequencePlayer)
          (Utilities|Authority
            (:Authority
              (bind _outactors (Actor|GetAllActorsOfClass "/Game/Blueprints/Player/BP_Player.BP_Player_C"))
              (for _array_element _outactors
                (Variables|/Game/Blueprints/Player/BP_Player.BP_Player_C|SetIsInCinematic _array_element false)
                (bind (_keypin _valuepin) (Utilities|Map|ForEachLoop(Map) (Variables|Default|GetEndosLocations))
                  (:then
                    (Transformation|SetActorLocationAndRotation _valuepin (.Location (Math|Transform|BreakTransform _keypin)) (.Rotation (Math|Transform|BreakTransform _keypin))))
                  (:CompletedPin
                    (bind _outactors_2 (Actor|GetAllActorsOfClass "/Game/Blueprints/Enemies/BP_EndoBlock.BP_EndoBlock_C"))
                    (for _array_element_2 _outactors_2
                      (Rendering|SetActorHiddenInGame _array_element_2 false))
                    (bind _outactors_3 (Actor|GetAllActorsOfClass "/Game/Blueprints/Enemies/BP_StandEndo.BP_StandEndo_C"))
                    (for _array_element_3 _outactors_3
                      (if (Variables|/Game/Blueprints/Enemies/BP_StandEndo.BP_StandEndo_C|GetIsAttacking _array_element_3)
                        (Rendering|SetActorHiddenInGame _array_element_3 false)))))))))
        (:then_1
          (bind _returnvalue_2 (UserInterface|CreateWidget "/Game/Widgets/UW_Transition.UW_Transition_C"))
          (UserInterface|Viewport|AddtoViewport _returnvalue_2 10)
          (Utilities|FlowControl|Delay 0.5)
          (bind _asbp_player (Utilities|Casting|CastToBP_Player (Pawn|GetControlledPawn (Game|GetPlayerController 0))))
          (Widget|SetVisibility (Variables|/Game/Blueprints/Player/BP_Player.BP_Player_C|GetInGame _asbp_player) "Visible")
          (Input|EnableInput (Pawn|GetControlledPawn _returnvalue) _returnvalue))))))

(event Custom|EndCinematic
  (Networking|SwitchHasAuthority
    (:Authority
      (CallFunction|MultiEndCinematic))))

(event Input|EnhancedActionEvents|EnhancedInputActionIA_Interact
  (params (ActionValue :type Boolean) (ElapsedSeconds :type Float%20%28double-precision%29) (TriggeredSeconds :type Float%20%28double-precision%29) (InputAction :type Input%20Action%20Object%20Reference :default "/Game/Inputs/Actions/IA_Interact.IA_Interact"))
  (bind _skipwidget (Variables|Default|GetSkipWidget))
  (:Started
    (Utilities|Authority
      (:Authority
        (Utilities|FlowControl|Sequence
          (:then_0
            (Utilities|FlowControl|Gate true :!label _label
              (:Exit
                (Utilities|FlowControl|DoOnce false
                  (:Completed
                    (Utilities|FlowControl|Sequence
                      (:then_0
                        (CallFunction|MultiEndCinematic))
                      (:then_1
                        (Input|DisableInput self (Game|GetPlayerController 0))
                        (Utilities|IsValid _skipwidget
                          (:Is%20Valid
                            (Default|Close _skipwidget))))))))))
          (:then_1
            (Utilities|FlowControl|Gate false :!label _label_2
              (:Exit
                (Utilities|FlowControl|Sequence
                  (:then_0
                    (goto _label_2 Close))
                  (:then_1
                    (goto _label Open))
                  (:then_2
                    (Utilities|FlowControl|Delay 0.5)
                    (Utilities|FlowControl|Sequence
                      (:then_0
                        (goto _label Close))
                      (:then_1
                        (goto _label_2 Open)))))))))))))

(event EventTrigger
  (|CallParentFunction)
  (bind _outactors (Actor|GetAllActorsOfClass "/Game/Blueprints/Player/BP_Player.BP_Player_C"))
  (bind _array_element (Utilities|Array|ForEachLoopwithBreak _outactors :!label _label)
    (:LoopBody
      (if (not (Variables|/Game/Blueprints/Player/BP_Player.BP_Player_C|GetIsDead _array_element))
        (Utilities|FlowControl|Sequence
          (:then_0
            (goto _label Break))
          (:then_1
            (CallFunction|PlayCinematic)
            (bind _outactors_2 (Actor|GetAllActorsOfClass "/Game/Blueprints/Enemies/BP_EndoBase.BP_EndoBase_C"))
            (for _array_element_2 _outactors_2
              (Class|KismetSystemLibrary|IsObjectOfSoftClass _array_element_2 "/Game/Blueprints/Enemies/BP_EndoChase.BP_EndoChase_C"
                (:True
                  (Utilities|Map|Add (Variables|Default|GetEndosLocations) (Transformation|GetActorTransform _array_element_2) _array_element_2 :!label _label_2)
                  (Transformation|SetActorLocation _array_element_2 (+ (Transformation|GetActorLocation _array_element_2) "0.000000,0.000000,-5000.000000") false false))
                (:False
                  (Class|KismetSystemLibrary|IsObjectOfSoftClass _array_element_2 "/Game/Blueprints/Enemies/BP_EndoLight.BP_EndoLight_C"
                    (:True
                      (goto _label_2))
                    (:False
                      (Class|KismetSystemLibrary|IsObjectOfSoftClass _array_element_2 "/Game/Blueprints/Enemies/BP_EndoSight.BP_EndoSight_C"
                        (:True
                          (goto _label_2))
                        (:False
                          (Class|KismetSystemLibrary|IsObjectOfSoftClass _array_element_2 "/Game/Blueprints/Enemies/BP_EndoBlock.BP_EndoBlock_C"
                            (:True
                              (Rendering|SetActorHiddenInGame _array_element_2 true))))))))))
            (bind _outactors_3 (Actor|GetAllActorsOfClass "/Game/Blueprints/Enemies/BP_StandEndo.BP_StandEndo_C"))
            (for _array_element_3 _outactors_3
              (if (Variables|/Game/Blueprints/Enemies/BP_StandEndo.BP_StandEndo_C|GetIsAttacking _array_element_3)
                (Rendering|SetActorHiddenInGame _array_element_3 true)))
            (bind _outactors_4 (Actor|GetAllActorsOfClass "/Game/Blueprints/Player/BP_Player.BP_Player_C"))
            (for _array_element_4 _outactors_4
              (Variables|/Game/Blueprints/Player/BP_Player.BP_Player_C|SetIsInCinematic _array_element_4 true))))))))

(fn ConstructionScript
  (|CallParentFunction))