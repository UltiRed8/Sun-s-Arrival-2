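; Trigger node that disables every player-position save checkpoint in the level.
; On Trigger it clears IsEnabled on all BP_CheckpointSavePlayerPositionNode actors, saves a true checkpoint bool, then calls the parent Trigger.
; The bool is keyed by the node's world location as a string.
; BeginPlay reads it back and re-runs Trigger when set, so the disabled state is restored from checkpoint data.
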(event EventBeginPlay
  (|CallParentFunction)
  (bind (_success _bool) (Utilities|CheckpointGetBool (Utilities|String|ToString(Vector) (Transformation|GetActorLocation))))
  (if _success
    (if _bool
      (CallFunction|Trigger))))

(event EventTrigger
  (bind _outactors (Actor|GetAllActorsOfClass "/Game/Blueprints/Nodes/BP_CheckpointSavePlayerPositionNode.BP_CheckpointSavePlayerPositionNode_C"))
  (for _array_element _outactors
    (Variables|/Game/Blueprints/Nodes/BP_CheckpointSavePlayerPositionNode.BP_CheckpointSavePlayerPositionNode_C|SetIsEnabled _array_element false))
  (Utilities|CheckpointSaveBool (Utilities|String|ToString(Vector) (Transformation|GetActorLocation)) true)
  (|CallParentFunction))

(fn ConstructionScript
  (|CallParentFunction))