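; BP_ToggleActivationInteractionNode is an interaction node that toggles the activation of a list of target actors when triggered.
; Trigger calls a server update event before running the parent trigger logic.
; The server event relays to a multi event, which calls ToggleActivation on each entry in InteractionsActorToActivate.
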(event Custom|Multi_UpdateActivation
  (if (Utilities|Array|IsNotEmpty (Variables|Default|GetInteractionsActorToActivate))
    (for _array_element (Variables|Default|GetInteractionsActorToActivate)
      (Default|ToggleActivation _array_element))))

(event Custom|Server_UpdateActivation
  (CallFunction|MultiUpdateActivation))

(event EventTrigger
  (CallFunction|ServerUpdateActivation)
  (|CallParentFunction))

(fn ConstructionScript
  (|CallParentFunction))