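; Player component that tracks whether its owning BP_Player is seeing each BP_EndoSight in the level and reports changes to those Endos.
; On BeginPlay it caches the owner and maps every Endo found to a watched flag, initially false.
; Each Tick it rechecks sight per Endo and, only when the result changes, updates the map and calls a server event that passes the new status to that Endo's PlayerStatus.
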(event Custom|Server_SetEndoPlayerStatus
  (params (IsWatching :type Boolean) (Target :type BP%20Endo%20Sight%20Object%20Reference))
  (Default|PlayerStatus Target IsWatching))

(event EventBeginPlay
  (bind _outactors (Actor|GetAllActorsOfClass "/Game/Blueprints/Enemies/BP_EndoSight.BP_EndoSight_C"))
  (for _array_element _outactors
    (Utilities|Map|Add (Variables|Default|GetEndos) _array_element false)
    (bind _asbp_player (Utilities|Casting|CastToBP_Player (Components|GetOwner)))
    (Variables|Default|SetOwner _asbp_player)))

(event EventTick
  (params (DeltaSeconds :type Float%20%28single-precision%29))
  (bind _endos (Variables|Default|GetEndos))
  (bind (_keypin _valuepin) (Utilities|Map|ForEachLoop(Map) _endos)
    (:then
      (bind _returnvalue (Default|CheckIsSeeingSightEndo (Variables|Default|GetOwner) _keypin))
      (if (!= _returnvalue _valuepin)
        (CallFunction|ServerSetEndoPlayerStatus _returnvalue _keypin)
        (Utilities|Map|Add _endos _keypin _returnvalue)))))