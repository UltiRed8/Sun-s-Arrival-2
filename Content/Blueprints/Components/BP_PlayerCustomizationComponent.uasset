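; Player customization component that recolors helmet, hair, clothes, kneepads and boots with replicated hue and brightness values.
; Init creates one dynamic material per template map entry and assigns it to that slot on every supplied mesh.
; SetVariables and CopyData write the values, and each RepNotify calls UpdateMaterials.
; UpdateMaterials retries each tick until instances exist, then sets HueShift and Brightness by array index, so template order must match part order.
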(event Custom|SetVariables
  (params (HelmetHUE :type Float%20%28double-precision%29) (HairHUE :type Float%20%28single-precision%29) (ClothesHUE :type Float%20%28double-precision%29) (KneepadsOuterHUE :type Float%20%28double-precision%29) (KneepadsInnerHUE :type Float%20%28double-precision%29) (BootsHUE :type Float%20%28double-precision%29) (HelmetBrightness :type Float%20%28double-precision%29) (HairBrightness :type Float%20%28double-precision%29) (ClothesBrightness :type Float%20%28double-precision%29) (KneepadsOuterBrightness :type Float%20%28double-precision%29) (KneepadsInnerBrightness :type Float%20%28double-precision%29) (BootsBrightness :type Float%20%28double-precision%29))
  (Variables|Default|SetHelmetHUE HelmetHUE)
  (Variables|Default|SetHairHUE HairHUE)
  (Variables|Default|SetClothesHUE ClothesHUE)
  (Variables|Default|SetKneepadsOuterHUE KneepadsOuterHUE)
  (Variables|Default|SetKneepadsInnerHUE KneepadsInnerHUE)
  (Variables|Default|SetBootsHUE BootsHUE)
  (Variables|Default|SetHelmetBrightness HelmetBrightness)
  (Variables|Default|SetHairBrightness HairBrightness)
  (Variables|Default|SetClothesBrightness ClothesBrightness)
  (Variables|Default|SetKneepadsOuterBrightness KneepadsOuterBrightness)
  (Variables|Default|SetKneepadsInnerBrightness KneepadsInnerBrightness)
  (Variables|Default|SetBootsBrightness BootsBrightness))

(event Custom|Init
  (params (PlayerMesh :type Array%20of%20Primitive%20Component%20Object%20References))
  (if (Utilities|Array|IsEmpty (Variables|Default|GetMaterialsInstances))
    (bind (_keypin _valuepin) (Utilities|Map|ForEachLoop(Map) (Variables|Default|GetInstancesTemplates))
      (:then
        (bind _returnvalue (Rendering|Material|CreateDynamicMaterialInstance _keypin "None" "None" :!class /Script/Engine.KismetMaterialLibrary))
        (Utilities|Array|Add (Variables|Default|GetMaterialsInstances) _returnvalue)
        (for _array_element PlayerMesh
          (Rendering|Material|SetMaterial _array_element _valuepin _returnvalue))))))

(event Custom|UpdateMaterials
  (bind _materialsinstances (Variables|Default|GetMaterialsInstances))
  (if (== (Utilities|Array|Length _materialsinstances) 0) :!label _label
    (Utilities|FlowControl|DelayUntilNextTick)
    (goto _label)
    (else
      (for (_array_element _array_index) _materialsinstances
        (Rendering|Material|SetScalarParameterValue _array_element "HueShift" (Utilities|Array|Get(acopy) (Utilities|Array|MakeArray (Variables|Default|GetHelmetHUE) (Variables|Default|GetHairHUE) (Variables|Default|GetClothesHUE) (Variables|Default|GetKneepadsOuterHUE) (Variables|Default|GetKneepadsInnerHUE) (Variables|Default|GetBootsHUE)) _array_index) :!class /Script/Engine.MaterialInstanceDynamic)
        (Rendering|Material|SetScalarParameterValue _array_element "Brightness" (Utilities|Array|Get(acopy) (Utilities|Array|MakeArray (Variables|Default|GetHelmetBrightness) (Variables|Default|GetHairBrightness) (Variables|Default|GetClothesBrightness) (Variables|Default|GetKneepadsOuterBrightness) (Variables|Default|GetKneepadsInnerBrightness) (Variables|Default|GetBootsBrightness)) _array_index) :!class /Script/Engine.MaterialInstanceDynamic)))))

(event Custom|CopyData
  (params (Target :type BP%20Player%20Customization%20Component%20Object%20Reference))
  (Variables|BP_PlayerCustomizationComponent_C|SetHelmetHUE Target (Variables|Default|GetHelmetHUE))
  (Variables|BP_PlayerCustomizationComponent_C|SetHairHUE Target (Variables|Default|GetHairHUE))
  (Variables|BP_PlayerCustomizationComponent_C|SetClothesHUE Target (Variables|Default|GetClothesHUE))
  (Variables|BP_PlayerCustomizationComponent_C|SetKneepadsOuterHUE Target (Variables|Default|GetKneepadsOuterHUE))
  (Variables|BP_PlayerCustomizationComponent_C|SetKneepadsInnerHUE Target (Variables|Default|GetKneepadsInnerHUE))
  (Variables|BP_PlayerCustomizationComponent_C|SetBootsHUE Target (Variables|Default|GetBootsHUE))
  (Variables|BP_PlayerCustomizationComponent_C|SetHelmetBrightness Target (Variables|Default|GetHelmetBrightness))
  (Variables|BP_PlayerCustomizationComponent_C|SetHairBrightness Target (Variables|Default|GetHairBrightness))
  (Variables|BP_PlayerCustomizationComponent_C|SetClothesBrightness Target (Variables|Default|GetClothesBrightness))
  (Variables|BP_PlayerCustomizationComponent_C|SetKneepadsOuterBrightness Target (Variables|Default|GetKneepadsOuterBrightness))
  (Variables|BP_PlayerCustomizationComponent_C|SetKneepadsInnerBrightness Target (Variables|Default|GetKneepadsInnerBrightness))
  (Variables|BP_PlayerCustomizationComponent_C|SetBootsBrightness Target (Variables|Default|GetBootsBrightness))
  (CallFunction|UpdateMaterials))

(fn OnRepHelmetHUE
  (CallFunction|UpdateMaterials))

(fn OnRepHairHUE
  (CallFunction|UpdateMaterials))

(fn OnRepClothesHUE
  (CallFunction|UpdateMaterials))

(fn OnRepKneepadsOuterHUE
  (CallFunction|UpdateMaterials))

(fn OnRepKneepadsInnerHUE
  (CallFunction|UpdateMaterials))

(fn OnRepBootsHUE
  (CallFunction|UpdateMaterials))

(fn OnRepHelmetBrightness
  (CallFunction|UpdateMaterials))

(fn OnRepHairBrightness
  (CallFunction|UpdateMaterials))

(fn OnRepClothesBrightness
  (CallFunction|UpdateMaterials))

(fn OnRepKneepadsOuterBrightness
  (CallFunction|UpdateMaterials))

(fn OnRepKneepadsInnerBrightness
  (CallFunction|UpdateMaterials))

(fn OnRepBootsBrightness
  (CallFunction|UpdateMaterials))