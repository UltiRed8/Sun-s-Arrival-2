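; Component that streams one sublevel at a time, loading SLVL_A on BeginPlay and swapping to others on request.
; LoadSublevel streams in directly when nothing is loaded; otherwise it queues the target in ToLoad, unloads the current sublevel, then loads the queued one.
; Non-blocking soft-reference streaming calls are followed by loaded and unloaded dispatchers.
; Tick prints the current level name, or a transition banner when none is set, as debug output.
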(event Custom|LoadSublevel
  (params (Level :type World%20Soft%20Object%20Reference))
  (Utilities|IsSoftValid (Variables|Default|GetCurrentlyLoaded)
    (:true
      (Variables|Default|SetToLoad Level)
      (CallFunction|UnloadSublevel))
    (:false
      (Class|GameplayStatics|LoadStreamLevelbySoftObjectPtr Level true false)
      (Default|CallOnSublevelLoaded)
      (Variables|Default|SetCurrentlyLoaded Level)
      (Variables|Default|SetToLoad 0))))

(event Custom|UnloadSublevel
  (bind _toload (Variables|Default|GetToLoad))
  (Class|GameplayStatics|UnloadStreamLevelbySoftObjectPtr (Variables|Default|GetCurrentlyLoaded) false)
  (Default|CallOnSublevelUnloaded)
  (Variables|Default|SetCurrentlyLoaded 0)
  (Utilities|IsSoftValid _toload
    (:true
      (CallFunction|LoadSublevel _toload))))

(event EventTick
  (params (DeltaSeconds :type Float%20%28single-precision%29))
  (bind _currentlyloaded (Variables|Default|GetCurrentlyLoaded))
  (Utilities|IsSoftValid _currentlyloaded
    (:true
      (Development|PrintString (Utilities|String|Append "Current level: " (.RightS (Utilities|String|Split (Utilities|BreakSoftObjectPath (Class|KismetSystemLibrary|ToSoftObjPath(SoftObjRef) _currentlyloaded)) "."))) true false "(R=0.000000,G=1.000000,B=0.000000,A=1.000000)" DeltaSeconds))
    (:false
      (Development|PrintString "======================= LEVEL TRANSITION =======================" true false "(R=1.000000,G=0.000000,B=0.000000,A=1.000000)" DeltaSeconds))))

(event EventBeginPlay
  (CallFunction|LoadSublevel "/Game/Levels/SubLevels/SLVL_A.SLVL_A"))