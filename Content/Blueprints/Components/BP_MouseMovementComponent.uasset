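; Component that captures mouse movement as a gesture, such as repeated strokes or circling, while blocking normal look and move input.
; Capture flags BP_Player, enables owner input and ends fully when the left mouse button is released.
; Look deltas above a threshold are checked by dot product against the target or previous direction, and optionally by cross-product turn sign.
; Enough successes broadcast OnMouseMoved; the target can flip per success for back-and-forth motion.
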(event Custom|Success
  (params (Angle :type Float%20%28double-precision%29) (Direction :type Vector%202D%20Structure))
  (bind _result (Math|Integer|IncrementInt (Variables|Default|GetCurrentAmount))
    (:%20%20
      (if (Variables|Settings|MouseDetection|GetInverseTargetDirectionOnSuccess)
        (Variables|Settings|MouseDetection|SetTargetDirection (* (Variables|Settings|MouseDetection|GetTargetDirection) "(X=-1.000000,Y=-1.000000)")))
      (if (>= _result (Variables|Settings|MouseDetection|GetAmountForSuccess))
        (Variables|Default|SetCurrentAmount 0)
        (Default|CallOnMouseMoved Angle Direction)))))

(event Custom|StartCapturing
  (bind _returnvalue (Game|GetPlayerController 0))
  (Default|SetInputsIgnored (Utilities|GameInstance) true true)
  (Variables|Default|SetCapturing true)
  (Input|EnableInput (Components|GetOwner) _returnvalue)
  (Default|CallOnMouseCapture)
  (bind _asbp_player (Utilities|Casting|CastToBP_Player (Pawn|GetControlledPawn _returnvalue)))
  (Variables|/Game/Blueprints/Player/BP_Player.BP_Player_C|SetIsMouseCaptured _asbp_player true))

(event Custom|SoftStopCapturing
  (Variables|Default|SetCapturing false)
  (Default|CallOnMouseUncaptured))

(event Custom|ForceStopCapturing
  (bind _returnvalue (Game|GetPlayerController 0))
  (Default|SetInputsIgnored (Utilities|GameInstance) false false)
  (CallFunction|SoftStopCapturing)
  (Input|DisableInput (Components|GetOwner) _returnvalue)
  (bind _asbp_player (Utilities|Casting|CastToBP_Player (Pawn|GetControlledPawn _returnvalue)))
  (Variables|/Game/Blueprints/Player/BP_Player.BP_Player_C|SetIsMouseCaptured _asbp_player false))

(event Input|EnhancedActionEvents|EnhancedInputActionIA_Look
  (params (ActionValue :type Vector%202D%20Structure) (ElapsedSeconds :type Float%20%28double-precision%29) (TriggeredSeconds :type Float%20%28double-precision%29) (InputAction :type Input%20Action%20Object%20Reference :default "/Game/Inputs/Actions/IA_Look.IA_Look"))
  (bind _returnvalue (Math|Vector2D|Normalize2D ActionValue))
  (bind _targetdirection (Variables|Settings|MouseDetection|GetTargetDirection))
  (bind _similaritiesneeded (Variables|Settings|MouseDetection|GetSimilaritiesNeeded))
  (bind _directionneeded (Variables|Settings|MouseDetection|GetDirectionNeeded))
  (if (Variables|Default|GetCapturing)
    (if (>= (Math|Vector2D|Vector2DLength ActionValue) (Variables|Settings|MouseDetection|GetThreshold))
      (Utilities|FlowControl|Sequence
        (:then_0
          (if (not (Utilities|Operators|EqualEqual :A (Variables|Default|GetLastVector)))
            (if (or (>= (Math|Vector2D|DotProduct(2D) (select (Utilities|Operators|EqualEqual :A _targetdirection) (Variables|Default|GetLastVector) _targetdirection) _returnvalue) _similaritiesneeded) (<= _similaritiesneeded 0.0))
              (if (or (== _directionneeded 0) (select (== _directionneeded 1) (> (Class|KismetMathLibrary|CrossProduct2D (Variables|Default|GetLastVector) _returnvalue) 0.0) (< (Class|KismetMathLibrary|CrossProduct2D (Variables|Default|GetLastVector) _returnvalue) 0.0)))
                (CallFunction|Success (Class|KismetMathLibrary|CrossProduct2D (Variables|Default|GetLastVector) _returnvalue) _returnvalue))
              (elif (< (Math|Float|Absolute(Float) (Math|Vector2D|DotProduct(2D) (select (Utilities|Operators|EqualEqual :A _targetdirection) (Variables|Default|GetLastVector) _targetdirection) _returnvalue)) (Variables|Settings|MouseDetection|GetAbsoluteFailValue))
                (Variables|Default|SetCurrentAmount 0)))))
        (:then_1
          (Variables|Default|SetLastVector _returnvalue))))))

(event Input|MouseEvents|LeftMouseButton
  (params (Key :type Key%20Structure :default "None"))
  (:Released
    (CallFunction|ForceStopCapturing)))