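; BP_Room is a streaming room trigger that loads and unloads room levels as BP_Player enters or leaves its cube.
; Overlaps adjust a NeedLoading reference count on every room in ToLoad, letting rooms share neighbours.
; A CurrentState switch loads immediately but delays unloading two seconds, cancelled if the room is needed again.
; A gate feeds asynchronous soft-pointer level streaming, while red, green and blue cube materials show the state.
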(event OnComponentBeginOverlap(Cube)
  (params (OverlappedComponent :type Primitive%20Component%20Object%20Reference) (OtherActor :type Actor%20Object%20Reference) (OtherComp :type Primitive%20Component%20Object%20Reference) (OtherBodyIndex :type Integer) (bFromSweep :type Boolean) (SweepResult :type Hit%20Result%20Structure%20%28by%20ref%29))
  (Utilities|Casting|CastToBP_Player OtherActor)
  (for _array_element (Variables|Default|GetToLoad)
    (Math|Integer|IncrementInt (Variables|BP_Room_C|GetNeedLoading _array_element)
      (:%20%20
        (CallFunction|Load _array_element)))))

(event OnComponentEndOverlap(Cube)
  (params (OverlappedComponent :type Primitive%20Component%20Object%20Reference) (OtherActor :type Actor%20Object%20Reference) (OtherComp :type Primitive%20Component%20Object%20Reference) (OtherBodyIndex :type Integer))
  (Utilities|Casting|CastToBP_Player OtherActor)
  (for _array_element (Variables|Default|GetToLoad)
    (Math|Integer|DecrementInt (Variables|BP_Room_C|GetNeedLoading _array_element)
      (:%20%20
        (CallFunction|Unload _array_element)))))

(event Custom|Load
  (switch int (Variables|Default|GetCurrentState)
    (:0
      _)
    (:1
      _))
  (if (>= (Variables|Default|GetNeedLoading) 1)
    (Variables|Default|SetCurrentState 2)
    (Rendering|Material|SetMaterial (Variables|Default|GetCube) 0 "/Game/Materials/Instances/MI_Green.MI_Green")
    (CallFunction|TrueLoad)))

(event Custom|Unload
  (switch int (Variables|Default|GetCurrentState)
    (:2
      (if (<= (Variables|Default|GetNeedLoading) 0)
        (Variables|Default|SetCurrentState 1)
        (Rendering|Material|SetMaterial (Variables|Default|GetCube) 0 "/Game/Materials/Instances/MI_Blue.MI_Blue")
        (Utilities|FlowControl|RetriggerableDelay 2.0)
        (switch int (Variables|Default|GetCurrentState)
          (:1
            (Rendering|Material|SetMaterial (Variables|Default|GetCube) 0 "/Game/Materials/Instances/MI_Red.MI_Red")
            (CallFunction|TrueUnload)))))))

(event Custom|TrueUnload
  (bind _hasdebugs (Variables|Default|GetHasDebugs))
  (bind _roomlevel (Variables|Default|GetRoomLevel))
  (Utilities|OnceGate) ; enters at InB
)

(event Custom|TrueLoad
  (bind _hasdebugs (Variables|Default|GetHasDebugs))
  (bind _roomlevel (Variables|Default|GetRoomLevel))
  (Utilities|OnceGate
    (:OutA
      (if _hasdebugs
        (Development|PrintString "LOAD"))
      (Utilities|IsSoftValid _roomlevel
        (:true
          (Class|GameplayStatics|LoadStreamLevelbySoftObjectPtr _roomlevel true false))))
    (:OutB
      (if _hasdebugs
        (Development|PrintString "UNLOAD"))
      (Utilities|IsSoftValid _roomlevel
        (:true
          (Class|GameplayStatics|UnloadStreamLevelbySoftObjectPtr _roomlevel false))))))

(event EventBeginPlay
  (Rendering|Material|SetMaterial (Variables|Default|GetCube) 0 "/Game/Materials/Instances/MI_Red.MI_Red"))

(fn ConstructionScript)