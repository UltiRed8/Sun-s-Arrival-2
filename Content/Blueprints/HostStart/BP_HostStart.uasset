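; Host-only interactable that starts the game with a skippable intro cinematic, after a first interaction shows a confirmation notification.
; A multicast clears tutorial triggers, plays cinematic audio and transition widgets, and blends to a camera while a timeline scaled to CinematicDelay drives the rail.
; Timed completion and authority-only Skip share one ending that multicasts the view back to pawns and moves all players to a fixed location.
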(event Custom|Skip
  (Networking|SwitchHasAuthority
    (:Authority
      (if (Variables|Default|GetInCinematic)
        (Variables|Default|SetInCinematic false)
        (CallFunction|MultiSkipped)
        (Variables|Default|SetInCinematic false)
        (CallFunction|MultiEndCinematic)
        (bind _outactors (Actor|GetAllActorsOfClass "/Game/Blueprints/Player/BP_Player.BP_Player_C"))
        (for _array_element _outactors
          (Transformation|SetActorLocation _array_element "0.000000,0.000000,200.000000" false false))))))

(event Custom|Multi_StartTransition
  (bind _returnvalue (Game|GetPlayerController 0))
  (Variables|Default|SetInCinematic true)
  (bind _returnvalue_2 (Audio|CreateSound2D "/Game/Audio/Sounds/SW_Cinematic.SW_Cinematic" 1.0 1.0 0.0 0))
  (bind _output_get (Variables|Default|SetSound _returnvalue_2))
  (Audio|Components|Audio|Play _output_get 0.0)
  (bind _outactors (Actor|GetAllActorsOfClass "/Game/Blueprints/Nodes/BP_TutorialTrigger.BP_TutorialTrigger_C"))
  (for _array_element _outactors
    (Utilities|IsValid _array_element
      (:Is%20Valid
        (Actor|DestroyActor _array_element))))
  (bind _returnvalue_3 (UserInterface|CreateWidget "/Game/Widgets/UW_Transition.UW_Transition_C" _returnvalue))
  (UserInterface|Viewport|AddtoViewport _returnvalue_3 2)
  (Utilities|FlowControl|Delay 0.5)
  (if (Variables|Default|GetInCinematic)
    (Game|Player|SetViewTargetwithBlend _returnvalue (Variables|Default|GetCamera) 0.0 "VTBlend_Linear" 0.0 false)
    (Components|Timeline|SetPlayRate (Variables|Default|GetMovementTimeline) (/ 1.0 (Variables|Default|GetCinematicDelay)))
    (Utilities|FlowControl|Sequence
      (:then_0
        (Utilities|FlowControl|Delay (- (Variables|Default|GetCinematicDelay) 0.5))
        (if (Variables|Default|GetInCinematic)
          (bind _returnvalue_4 (UserInterface|CreateWidget "/Game/Widgets/UW_Transition.UW_Transition_C" (Game|GetPlayerController 0)))
          (UserInterface|Viewport|AddtoViewport _returnvalue_4 2)))
      (:then_1
        (bind _percent (Timeline|MovementTimeline PlayFromStart)
          (:Update
            (Variables|/Script/CinematicCamera.CameraRig_Rail|SetCurrentPositionOnRail (Variables|Default|GetCameraRail) _percent)))))))

(event Custom|Multi_Skipped
  (bind _sound (Variables|Default|GetSound))
  (Variables|Default|SetInCinematic false)
  (Utilities|IsValid _sound
    (:Is%20Valid
      (Audio|Components|Audio|Stop _sound))
    (:Is%20Not%20Valid
      _))
  (Utilities|FlowControl|Sequence
    (:then_0
      (bind _percent (Timeline|MovementTimeline Stop)
        (:Update
          (Variables|/Script/CinematicCamera.CameraRig_Rail|SetCurrentPositionOnRail (Variables|Default|GetCameraRail) _percent))))))

(event Custom|Multi_EndCinematic
  (bind _returnvalue (Game|GetPlayerController 0))
  (Game|Player|SetViewTargetwithBlend _returnvalue (Pawn|GetControlledPawn _returnvalue) 0.0 "VTBlend_Linear" 0.0 false))

(event EventServerInteract
  (params (WhoInteracted :type Actor%20Object%20Reference))
  (bind _asbp_player (Utilities|Casting|CastToBP_Player WhoInteracted))
  (if (Pawn|IsLocallyControlled _asbp_player)
    (Utilities|IsValid (Pawn|GetController _asbp_player)
      (:Is%20Valid
        (if (Ability|HasAuthority (Pawn|GetController _asbp_player))
          (Utilities|FlowControl|FlipFlop
            (:A
              (Utilities|FlowControl|DoOnce false
                (:Completed
                  (bind _returnvalue (UserInterface|CreateWidget "/Game/Widgets/UW_Notification.UW_Notification_C" (Game|GetPlayerController 0) "Interact again to start!" "(R=1.000000,G=1.000000,B=1.000000,A=1.000000)"))
                  (UserInterface|Viewport|AddtoViewport _returnvalue 0))))
            (:B
              (Utilities|FlowControl|DoOnce false
                (:Completed
                  (CallFunction|MultiStartTransition)
                  (Utilities|FlowControl|Delay (+ (Variables|Default|GetCinematicDelay) 0.5))
                  (if (Variables|Default|GetInCinematic)
                    (Variables|Default|SetInCinematic false)
                    (CallFunction|MultiEndCinematic)
                    (bind _outactors (Actor|GetAllActorsOfClass "/Game/Blueprints/Player/BP_Player.BP_Player_C"))
                    (for _array_element _outactors
                      (Transformation|SetActorLocation _array_element "0.000000,0.000000,200.000000" false false))))))))))))

(fn ConstructionScript)