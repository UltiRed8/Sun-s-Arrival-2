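; Global inventory Blueprint that tracks coins, deaths and a map of item names to counts.
; BeginPlay restores checkpoint data, except in Exploration mode, which instead fills the map with every keycard.
; Give and remove requests go through server events that adjust stack counts, with a multicast event announcing received items.
; Changes trigger a checkpoint save, storing each item as an indexed "name@count" string.
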(event Custom|GiveItem
  (params (Item :type String%20%28by%20ref%29))
  (CallFunction|ServerGiveItem Item)
  (CallFunction|Save))

(event Custom|RemoveItem
  (params (Item :type String%20%28by%20ref%29))
  (CallFunction|ServerRemoveItem Item)
  (CallFunction|Save))

(event Custom|Server_GiveItem
  (params (NewItem :type String%20%28by%20ref%29))
  (bind _items (Variables|Default|GetItems))
  (bind (_value _returnvalue) (Utilities|Map|Find _items NewItem))
  (Utilities|Map|Add _items NewItem (Math|Integer|SelectInt (+ _value 1) 1 _returnvalue))
  (CallFunction|MultiGiveItem NewItem))

(event Custom|Multi_GiveItem
  (params (ItemName :type String))
  (Default|CallOnItemReceived ItemName))

(event Custom|Server_RemoveItem
  (params (Item :type String%20%28by%20ref%29))
  (bind _items (Variables|Default|GetItems))
  (bind (_value _returnvalue) (Utilities|Map|Find _items Item))
  (if _returnvalue
    (bind _result (Math|Integer|DecrementInt _value)
      (:%20%20
        (if (== _result 0)
          (Utilities|Map|Remove _items Item))))))

(event Custom|Save
  (bind _items (Variables|Default|GetItems))
  (Utilities|CheckpointSaveInt "InventoryCoins" (Variables|Default|GetCoinsBalance))
  (Utilities|CheckpointSaveInt "InventoryDeaths" (Variables|Default|GetDeathsAmount))
  (bind _keys (Utilities|Map|Keys _items))
  (bind _values (Utilities|Map|Values _items))
  (for (_array_element _array_index) _keys
    (Utilities|CheckpointSaveString (Utilities|String|Append "InventoryItem_" (Utilities|String|ToString(Integer) _array_index)) (Utilities|String|Append _array_element "@" (Utilities|String|ToString(Integer) (Utilities|Array|Get(acopy) _values _array_index))))))

(event Custom|IncrementCoins
  (Math|Integer|IncrementInt (Variables|Default|GetCoinsBalance)
    (:%20%20
      (CallFunction|Save))))

(event Custom|IncrementDeath
  (Math|Integer|IncrementInt (Variables|Default|GetDeathsAmount)
    (:%20%20
      (CallFunction|Save))))

(event EventBeginPlay
  (switch Utilities|FlowControl|Switch|SwitchonE_ExtrasGamemodes (Variables|/Game/BP_GameInstance.BP_GameInstance_C|GetExtraGamemode (Utilities|GameInstance))
    (:NewEnumerator0
      (bind (_success _int) (Utilities|CheckpointGetInt "InventoryCoins" :!label _label))
      (if _success
        (Variables|Default|SetCoinsBalance _int))
      (bind (_success_2 _int_2) (Utilities|CheckpointGetInt "InventoryDeaths"))
      (if _success_2
        (Variables|Default|SetDeathsAmount _int_2))
      (bind (_success_out _strings_out) (CallFunction|CheckpointGetStrings "InventoryItem"))
      (if _success_out
        (for _array_element _strings_out
          (Utilities|Map|Add (Variables|Default|GetItems) (.LeftS (Utilities|String|Split _array_element "@")) (Math|Conversions|ToInteger(Byte) (.RightS (Utilities|String|Split _array_element "@")))))))
    (:NewEnumerator1
      (Variables|Default|SetItems (Utilities|Map|MakeMap "Keycard level 0" 0 "Keycard level 1" 0 "Keycard level 2" 0 "Keycard level 3" 0 "Keycard level 4" 0 "Master Keycard" 0)))
    (:NewEnumerator2
      (goto _label))
    (:NewEnumerator3
      (goto _label))))

(fn ConstructionScript)

(fn HasItem
  (params (ItemToFind :type String%20%28by%20ref%29))
  (return (.ReturnValue (Utilities|Map|Find (Variables|Default|GetItems) ItemToFind))))