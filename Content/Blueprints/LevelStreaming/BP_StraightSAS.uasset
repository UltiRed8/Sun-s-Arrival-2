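; Straight airlock (SAS) door that opens when triggered while enabled and can close itself after a delay.
; Open and Close replay a timeline per segment, sliding door parts one after another with slam sounds, then a steam burst.
; A looping alarm sounds during movement, while an indicator light shows disabled, ready, moving or open.
; Cooldown blocks retriggering and clears only when closing finishes, so without auto-close Trigger works once.
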(event Custom|StartAlarm
  (Variables|Default|SetAlarm true)
  (Audio|PlaySoundatLocation "/Game/Audio/Sounds/SW_SasAlarm.SW_SasAlarm" (Transformation|GetWorldLocation (Variables|Default|GetLightA)) "0, 0, 0" 1.0 1.0 0.0 "/Game/Audio/Attenuations/SA_SasAttenuation.SA_SasAttenuation" 0 0 0 :!label _label)
  (Utilities|FlowControl|Delay 0.9)
  (if (Variables|Default|GetAlarm)
    (goto _label)))

(event Custom|Trigger
  (if (Variables|Default|GetIsEnabled)
    (if (not (Variables|Default|GetCooldown))
      (Variables|Default|SetCooldown true)
      (CallFunction|Open)
      (if (Variables|Default|GetClosesAutomatically)
        (Utilities|FlowControl|Delay 8.0)
        (CallFunction|Close)))))

(event Custom|SetEnabled
  (params (IsEnabled :type Boolean))
  (bind _output_get (Variables|Default|SetIsEnabled IsEnabled))
  (Rendering|Material|SetMaterial (Variables|Default|GetLightB) 0 (select _output_get "/Game/Models/EndoEnemy/MAT_RedGlow.MAT_RedGlow" "/Game/Materials/Instances/MI_UnlitBlack.MI_UnlitBlack")))

(event Custom|Close
  (bind _ns_sassteam0 (Variables|Default|GetNS_SasSteam0))
  (Rendering|Material|SetMaterial (Variables|Default|GetLightB) 0 "/Game/Materials/Instances/MI_YellowBlinking.MI_YellowBlinking")
  (CallFunction|StartAlarm)
  (Utilities|FlowControl|Delay 1.6)
  (Audio|PlaySoundatLocation "/Game/Audio/Sounds/SW_SasClosing.SW_SasClosing" (Transformation|GetActorLocation) "0, 0, 0" 2.0 2.0 0.0 "/Game/Audio/Attenuations/SA_SasAttenuation.SA_SasAttenuation" 0 0 0)
  (Utilities|FlowControl|Delay 0.4)
  (Variables|Default|SetPartIndex 5)
  (bind _position (Timeline|Timeline ReverseFromEnd)
    (:Update
      (Transformation|SetRelativeLocation (Utilities|Array|Get(acopy) (Utilities|Array|MakeArray (Variables|Default|GetDoorPart7) (Variables|Default|GetDoorPart6) (Variables|Default|GetDoorPart5) (Variables|Default|GetDoorPart4) (Variables|Default|GetDoorPart3) (Variables|Default|GetDoorPart2) (Variables|Default|GetDoorPart1)) (Variables|Default|GetPartIndex)) (Math|Vector|MakeVector _position 0.0 0.0) false false))
    (:Finished
      (Audio|PlaySoundatLocation "/Game/Audio/Sounds/SW_MetalDoorSlam.SW_MetalDoorSlam" (Transformation|GetActorLocation) "0, 0, 0" 0.5 2.0 0.0 "/Game/Audio/Attenuations/SA_SasAttenuation.SA_SasAttenuation" 0 0 0)
      (Utilities|FlowControl|Delay 0.05)
      (bind _result (Math|Integer|DecrementInt (Variables|Default|GetPartIndex))
        (:%20%20
          (if (>= _result 0)
            (Timeline|Timeline ReverseFromEnd)
            (else
              (Components|Activation|Activate _ns_sassteam0 false)
              (Audio|PlaySoundatLocation "/Game/Audio/Sounds/SW_Steam.SW_Steam" (Transformation|GetActorLocation) "0, 0, 0" 5.0 1.0 0.0 "/Game/Audio/Attenuations/SA_SasAttenuation.SA_SasAttenuation" 0 0 0)
              (Utilities|FlowControl|Delay 0.5)
              (Components|Activation|Deactivate _ns_sassteam0)
              (Variables|Default|SetAlarm false)
              (Utilities|FlowControl|Delay 0.5)
              (Rendering|Material|SetMaterial (Variables|Default|GetLightB) 0 "/Game/Models/EndoEnemy/MAT_RedGlow.MAT_RedGlow")
              (Variables|Default|SetCooldown false))))))))

(event Custom|Open
  (bind _ns_sassteam0 (Variables|Default|GetNS_SasSteam0))
  (Rendering|Material|SetMaterial (Variables|Default|GetLightB) 0 "/Game/Materials/Instances/MI_YellowBlinking.MI_YellowBlinking")
  (CallFunction|StartAlarm)
  (Utilities|FlowControl|Delay 1.6)
  (Audio|PlaySoundatLocation "/Game/Audio/Sounds/SW_SasOpening.SW_SasOpening" (Transformation|GetActorLocation) "0, 0, 0" 1.0 2.0 0.0 "/Game/Audio/Attenuations/SA_SasAttenuation.SA_SasAttenuation" 0 0 0)
  (Utilities|FlowControl|Delay 0.4)
  (Variables|Default|SetPartIndex 0)
  (bind _position (Timeline|PartOpening PlayFromStart)
    (:Update
      (Transformation|SetRelativeLocation (Utilities|Array|Get(acopy) (Utilities|Array|MakeArray (Variables|Default|GetDoorPart7) (Variables|Default|GetDoorPart6) (Variables|Default|GetDoorPart5) (Variables|Default|GetDoorPart4) (Variables|Default|GetDoorPart3) (Variables|Default|GetDoorPart2) (Variables|Default|GetDoorPart1)) (Variables|Default|GetPartIndex)) (Math|Vector|MakeVector _position 0.0 0.0) false false))
    (:Finished
      (Audio|PlaySoundatLocation "/Game/Audio/Sounds/SW_MetalDoorSlam.SW_MetalDoorSlam" (Transformation|GetActorLocation) "0, 0, 0" 0.5 2.0 0.0 "/Game/Audio/Attenuations/SA_SasAttenuation.SA_SasAttenuation" 0 0 0)
      (Utilities|FlowControl|Delay 0.05)
      (bind _result (Math|Integer|IncrementInt (Variables|Default|GetPartIndex))
        (:%20%20
          (if (<= _result 5)
            (Timeline|PartOpening PlayFromStart)
            (else
              (Components|Activation|Activate _ns_sassteam0 false)
              (Audio|PlaySoundatLocation "/Game/Audio/Sounds/SW_Steam.SW_Steam" (Transformation|GetActorLocation) "0, 0, 0" 5.0 1.0 0.0 "/Game/Audio/Attenuations/SA_SasAttenuation.SA_SasAttenuation" 0 0 0)
              (Utilities|FlowControl|Delay 0.5)
              (Components|Activation|Deactivate _ns_sassteam0)
              (Variables|Default|SetAlarm false)
              (Utilities|FlowControl|Delay 0.5)
              (Rendering|Material|SetMaterial (Variables|Default|GetLightB) 0 "/Game/Models/EndoEnemy/MAT_GreenGlow.MAT_GreenGlow"))))))))

(fn ConstructionScript
  (CallFunction|SetEnabled (Variables|Default|GetIsEnabled)))