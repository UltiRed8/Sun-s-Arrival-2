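; BP_TurnSAS is a two-door airlock that swaps between sublevels ZoneA and ZoneB, starting open on side A.
; A lever, or a keycard reader when KeycardID is set, toggles sides, while two buttons each call their own side.
; Each switch closes both doors, waits, requests the zone through the player's BP_SublevelLoaderComponent, then opens that timeline-driven door.
; A cooldown blocks re-triggering, and SetEnabled gates input and button materials.
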(event Custom|SetEnabled
  (params (IsEnabled :type Boolean))
  (bind _output_get (Variables|Default|SetIsEnabled IsEnabled))
  (bind _asbp_press_button (Utilities|Casting|CastToBP_PressButton (Variables|/Script/Engine.ChildActorComponent|GetChildActor (Variables|Default|GetButtonB))))
  (bind _asbp_press_button_2 (Utilities|Casting|CastToBP_PressButton (Variables|/Script/Engine.ChildActorComponent|GetChildActor (Variables|Default|GetButtonA))))
  (Rendering|Material|SetMaterial (Variables|/Game/Blueprints/Interactives/BP_PressButton.BP_PressButton_C|GetCylinder _asbp_press_button) 0 (select _output_get "/Game/Materials/Instances/MI_KeycardReaderIdle.MI_KeycardReaderIdle" "/Game/Materials/Instances/MI_UnlitBlack.MI_UnlitBlack")))

(event Custom|UpdateInteractor
  (bind _keycardreader (Variables|Default|GetKeycardReader))
  (if (Utilities|Array|IsEmpty (Variables|Default|GetKeycardID))
    (Components|DestroyComponent _keycardreader)
    (else
      (Components|DestroyComponent (Variables|Default|GetLever))
      (bind _asbp_keycard_reader (Utilities|Casting|CastToBP_KeycardReader (Variables|/Script/Engine.ChildActorComponent|GetChildActor _keycardreader)))
      (Variables|/Game/Blueprints/Interactives/BP_KeycardReader.BP_KeycardReader_C|SetKeycardID _asbp_keycard_reader (Variables|Default|GetKeycardID)))))

(event Custom|ButtonACall
  (if (Variables|Default|GetIsEnabled)
    (if (not (Variables|Default|GetIsAOpened))
      (if (not (Variables|Default|GetCooldown))
        (Variables|Default|SetCooldown true)
        (Variables|Default|SetIsAOpened true)
        (CallFunction|UpdateDoors)))))

(event Custom|SasToggle
  (if (Variables|Default|GetIsEnabled)
    (if (not (Variables|Default|GetCooldown))
      (Variables|Default|SetCooldown true)
      (Variables|Default|SetIsAOpened (not (Variables|Default|GetIsAOpened)))
      (CallFunction|UpdateDoors))))

(event Custom|UpdateDoors
  (Collision|SetCollisionEnabled (Variables|Default|GetDoorACollider) "QueryAndPhysics")
  (CallFunction|CloseDoorA)
  (CallFunction|CloseDoorB)
  (Utilities|FlowControl|Delay 1.0)
  (if (Variables|Default|GetIsAOpened)
    (CallFunction|LoadZoneA)
    (else
      (CallFunction|LoadZoneB))))

(event Custom|OpenDoorB
  (bind _percent (Timeline|TimelineDoorB Play)
    (:Update
      (Transformation|SetRelativeLocation (Variables|Default|GetDoorB) (+ (* (Math|Vector|GetForwardVector (Variables|/Script/Engine.SceneComponent|GetRelativeRotation (Variables|Default|GetSideB))) (* _percent -2e+02)) "0.000000,300.000000,25.000000") false false))))

(event Custom|CloseDoorB
  (bind _percent (Timeline|TimelineDoorB Reverse)
    (:Update
      (Transformation|SetRelativeLocation (Variables|Default|GetDoorB) (+ (* (Math|Vector|GetForwardVector (Variables|/Script/Engine.SceneComponent|GetRelativeRotation (Variables|Default|GetSideB))) (* _percent -2e+02)) "0.000000,300.000000,25.000000") false false))))

(event Custom|OpenDoorA
  (bind _percent (Timeline|TimelineDoorA Play)
    (:Update
      (Transformation|SetRelativeLocation (Variables|Default|GetDoorA) (+ (* (Math|Vector|GetRightVector (Variables|/Script/Engine.SceneComponent|GetRelativeRotation (Variables|Default|GetSideA))) (* _percent -2e+02) -1) "0.000000,-300.000000,25.000000") false false))))

(event Custom|CloseDoorA
  (bind _percent (Timeline|TimelineDoorA Reverse)
    (:Update
      (Transformation|SetRelativeLocation (Variables|Default|GetDoorA) (+ (* (Math|Vector|GetRightVector (Variables|/Script/Engine.SceneComponent|GetRelativeRotation (Variables|Default|GetSideA))) (* _percent -2e+02) -1) "0.000000,-300.000000,25.000000") false false))))

(event Custom|LoadZoneA
  (bind _keycardreader (Variables|Default|GetKeycardReader))
  ;[0.15 0.15 0.15 0.5] TEMP
  (bind _returnvalue (Actor|GetActorOfClass "/Game/Blueprints/Player/BP_Player.BP_Player_C"))
  (Default|LoadSublevel (Actor|GetComponentbyClass _returnvalue "/Game/Blueprints/Components/BP_SublevelLoaderComponent.BP_SublevelLoaderComponent_C") (Variables|Default|GetZoneA))
  (CallFunction|OpenDoorA)
  (Collision|SetCollisionEnabled (Variables|Default|GetDoorACollider) "NoCollision")
  (Utilities|FlowControl|Delay 1.0)
  (Variables|Default|SetCooldown false)
  (Utilities|IsValid _keycardreader
    (:Is%20Valid
      (bind _asbp_keycard_reader (Utilities|Casting|CastToBP_KeycardReader (Variables|/Script/Engine.ChildActorComponent|GetChildActor _keycardreader)))
      (Default|Reset _asbp_keycard_reader))))

(event Custom|LoadZoneB
  (bind _keycardreader (Variables|Default|GetKeycardReader))
  ;[0.15 0.15 0.15 0.5] TEMP
  (bind _returnvalue (Actor|GetActorOfClass "/Game/Blueprints/Player/BP_Player.BP_Player_C"))
  (Default|LoadSublevel (Actor|GetComponentbyClass _returnvalue "/Game/Blueprints/Components/BP_SublevelLoaderComponent.BP_SublevelLoaderComponent_C") (Variables|Default|GetZoneB))
  (CallFunction|OpenDoorB)
  (Collision|SetCollisionEnabled (Variables|Default|GetDoorBCollider) "NoCollision")
  (Utilities|FlowControl|Delay 1.0)
  (Variables|Default|SetCooldown false)
  (Utilities|IsValid _keycardreader
    (:Is%20Valid
      (bind _asbp_keycard_reader (Utilities|Casting|CastToBP_KeycardReader (Variables|/Script/Engine.ChildActorComponent|GetChildActor _keycardreader)))
      (Default|Reset _asbp_keycard_reader))))

(event Custom|ButtonBCall
  (if (Variables|Default|GetIsEnabled)
    (if (Variables|Default|GetIsAOpened)
      (if (not (Variables|Default|GetCooldown))
        (Variables|Default|SetCooldown true)
        (Variables|Default|SetIsAOpened false)
        (CallFunction|UpdateDoors)))))

(event EventBeginPlay
  (bind _asbp_lever_pillar (Utilities|Casting|CastToBP_LeverPillar (Variables|/Script/Engine.ChildActorComponent|GetChildActor (Variables|Default|GetLever))))
  (EventDispatchers|AssignOnTriggered _asbp_lever_pillar (delegate Custom|SasToggle))
  (bind _asbp_keycard_reader (Utilities|Casting|CastToBP_KeycardReader (Variables|/Script/Engine.ChildActorComponent|GetChildActor (Variables|Default|GetKeycardReader))))
  (EventDispatchers|BindEventtoOnTriggered _asbp_keycard_reader (delegate Custom|SasToggle))
  (bind _asbp_press_button (Utilities|Casting|CastToBP_PressButton (Variables|/Script/Engine.ChildActorComponent|GetChildActor (Variables|Default|GetButtonA))))
  (bind _asbp_press_button_2 (Utilities|Casting|CastToBP_PressButton (Variables|/Script/Engine.ChildActorComponent|GetChildActor (Variables|Default|GetButtonB))))
  (EventDispatchers|AssignOnTriggered _asbp_press_button (delegate Custom|ButtonACall))
  (EventDispatchers|AssignOnTriggered _asbp_press_button_2 (delegate Custom|ButtonBCall))
  (CallFunction|SetEnabled (Variables|Default|GetIsEnabled))
  (CallFunction|OpenDoorA)
  (Collision|SetCollisionEnabled (Variables|Default|GetDoorACollider) "NoCollision")
  (Variables|Default|SetIsAOpened true)
  (CallFunction|UpdateInteractor))

(fn ConstructionScript)