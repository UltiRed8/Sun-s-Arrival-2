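; BP_SplineCable is a construction-time spline cable that can pin its ends to StartActor and EndActor.
; The construction script moves the endpoints, runs a segment cleanup, then adds a scaled CableMesh spline mesh per point pair using local positions and tangents.
; Endpoint snapping requires a valid StartActor and a stored NumPoints below 2, which is only refreshed afterwards during generation.
; Cleanup has inverted validity branches, and new segments are never added to SegmentMeshes.
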(event EventBeginPlay)

(event Collision|EventActorBeginOverlap
  (params (OtherActor :type Actor%20Object%20Reference)))

(event EventTick
  (params (DeltaSeconds :type Float%20%28single-precision%29)))

(fn ConstructionScript
  (CallFunction|UpdateStartEndPoints)
  (CallFunction|ClearOldSegment)
  (CallFunction|GenerateSplineMeshSegments))

(fn UpdateStartEndPoints
  (bind _startactor (Variables|Default|GetStartActor))
  (bind _spline (Variables|Default|GetSpline))
  (bind _endactor (Variables|Default|GetEndActor))
  (Utilities|IsValid _startactor
    (:Is%20Valid
      (if (< (Variables|Default|GetNumPoints) 2)
        (Spline|SetLocationatSplinePoint _spline 0 (Transformation|GetActorLocation _startactor) "World" true)
        (Utilities|IsValid _endactor
          (:Is%20Valid
            (bind _output_get (Variables|Default|SetLastIndex (- (Spline|GetNumberOfSplinePoints _spline) 1)))
            (Spline|SetLocationatSplinePoint _spline _output_get (Transformation|GetActorLocation _endactor) "World" true)
            (Spline|UpdateSpline _spline)))))))

(fn ClearOldSegment
  (bind _segmentmeshes (Variables|Default|GetSegmentMeshes))
  (for _array_element _segmentmeshes
    (Utilities|IsValid _array_element
      (:Is%20Valid
        (Utilities|Array|Clear _segmentmeshes))
      (:Is%20Not%20Valid
        (Components|DestroyComponent _array_element)))))

(fn GenerateSplineMeshSegments
  (bind _spline (Variables|Default|GetSpline))
  (bind _output_get (Variables|Default|SetNumPoints (Spline|GetNumberOfSplinePoints _spline)))
  (for _index (range 0 (- _output_get 2))
    (Variables|Default|SetStartPos (Spline|GetLocationatSplinePoint _spline _index "Local"))
    (Variables|Default|SetStartTangent (Spline|GetTangentatSplinePoint _spline _index "Local"))
    (bind _output_get_2 (Variables|Default|SetNextIndex (+ _index 1)))
    (Variables|Default|SetEndPos (Spline|GetLocationatSplinePoint _spline _output_get_2 "Local"))
    (Variables|Default|SetEndTangent (Spline|GetTangentatSplinePoint _spline _output_get_2 "Local"))
    (bind _returnvalue (AddComponent|AddSplineMeshComponent false))
    (Components|StaticMesh|SetStaticMesh _returnvalue (Variables|Default|GetCableMesh))
    (SplineMesh|SetStartScale _returnvalue "(X=5.000000,Y=5.000000)" true :!class /Script/Engine.SplineMeshComponent)
    (SplineMesh|SetEndScale _returnvalue "(X=5.000000,Y=5.000000)" true :!class /Script/Engine.SplineMeshComponent)
    (SplineMesh|SetStartPosition _returnvalue (Variables|Default|GetStartPos) true)
    (SplineMesh|SetEndPosition _returnvalue (Variables|Default|GetEndPos) true)
    (SplineMesh|SetStartTangent _returnvalue (Variables|Default|GetStartTangent) true :!class /Script/Engine.SplineMeshComponent)
    (SplineMesh|SetEndTangent _returnvalue (Variables|Default|GetEndTangent) true :!class /Script/Engine.SplineMeshComponent)))