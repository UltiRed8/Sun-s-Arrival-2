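; Player map device that shows a render-target map, with a UW_MapDevice widget for the current objective and keycard level.
; Outside Exploration mode, it restores both values from checkpoints and forwards inventory pickups to the widget; new objectives are saved.
; Toggle plays a scale, rotation and antenna timeline with audio, switching the screen material and showing static until unlocked.
; Tick interpolates roll sway from input deltas, gated by the tools-movement setting.
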(event Custom|Toggle
  (bind _audio (Variables|Default|GetAudio))
  (Utilities|FlowControl|FlipFlop
    (:A
      (Audio|Components|Audio|SetSound _audio "/Game/Audio/Sounds/SW_MapDeviceOn.SW_MapDeviceOn")
      (Audio|Components|Audio|Play _audio 0.0)
      (Utilities|FlowControl|Sequence
        (:then_0
          (bind (_direction _size _rotationx _antennarotationx) (Timeline|ToggleAnimation Play)
            (:Update
              (Transformation|SetRelativeScale3D (Variables|Default|GetParent) (Math|Vector|MakeVector _size _size _size))
              (Transformation|SetRelativeRotation (Variables|Default|GetParent) (Math|Rotator|MakeRotator _rotationx 0.0 0.0) false false)
              (Transformation|SetRelativeRotation (Variables|Default|GetAntennaAxis) (Math|Rotator|MakeRotator _antennarotationx 0.0 0.0) false false))
            (:Finished
              (switch Utilities|FlowControl|Switch|SwitchonETimelineDirection _direction
                (:Backward
                  (Transformation|SetRelativeScale3D (Variables|Default|GetParent) (Math|Vector|MakeVector 0.0 0.0 0.0)))))))
        (:then_1
          (Utilities|FlowControl|Delay 0.8)
          (CallFunction|Screenon))))
    (:B
      (Audio|Components|Audio|SetSound _audio "/Game/Audio/Sounds/SW_MapDeviceOff.SW_MapDeviceOff")
      (Audio|Components|Audio|Play _audio 0.0)
      (CallFunction|ScreenOff)
      (Timeline|ToggleAnimation Reverse))))

(event Custom|SetNewObjective
  (params (Text :type Text))
  (bind _returnvalue (Utilities|String|ToString(Text) Text))
  (bind _asuw_map_device (Utilities|Casting|CastToUW_MapDevice (UserInterface|GetWidget (Variables|Default|GetWidget))))
  (Default|SetObjective _asuw_map_device _returnvalue)
  (Utilities|CheckpointSaveString "MapDeviceObjective" _returnvalue))

(event Custom|OnItemReceived_Event
  (params (ItemID :type String))
  (bind _asuw_map_device (Utilities|Casting|CastToUW_MapDevice (UserInterface|GetWidget (Variables|Default|GetWidget))))
  (Default|SetKeycardLevel _asuw_map_device ItemID))

(event Custom|UpdateRoll
  (params (DeltaY :type Float%20%28double-precision%29))
  (if (Variables|Default|GetSmoothRotation)
    (Variables|Default|SetDeltaY DeltaY)))

(event Custom|ScreenOn
  (Rendering|SetVisibility (Variables|Default|GetWidget) true false)
  (Rendering|Material|SetMaterial (Variables|Default|GetDevice) 1 "/Game/Textures/MAT_RT_Map.MAT_RT_Map")
  (if (Variables|Default|GetIsUnlock)
    _
    (else
      (Rendering|SetVisibility (Variables|Default|GetScreenStatic) true false)))
  (Variables|Default|SetIsOpened true))

(event Custom|ScreenOff
  (Rendering|SetVisibility (Variables|Default|GetScreenStatic) false false)
  (Rendering|Material|SetMaterial (Variables|Default|GetDevice) 1 "/Game/Materials/Instances/MI_UnlitBlack.MI_UnlitBlack")
  (Variables|Default|SetIsOpened false))

(event Custom|OnToolsMovementUpdated_Event
  (params (Enabled :type Boolean))
  (Variables|Default|SetSmoothRotation Enabled))

(event Custom|Unlock
  (params (WithSound :type Boolean))
  (bind _audio (Variables|Default|GetAudio))
  (if WithSound
    (Audio|Components|Audio|SetSound _audio "/Game/Audio/Sounds/SW_MapDeviceUnlock.SW_MapDeviceUnlock")
    (Audio|Components|Audio|Play _audio 0.0))
  (Variables|Default|SetIsUnlock true))

(event EventDestroyed
  (EventDispatchers|UnbindEventfromOnToolsMovementUpdated (Variables|/Game/BP_GameInstance.BP_GameInstance_C|GetSettings (Utilities|GameInstance)) (delegate Custom|OnToolsMovementUpdated_Event)))

(event EventBeginPlay
  (bind _asbp_game_instance (Utilities|GameInstance))
  (bind _widget (Variables|Default|GetWidget))
  (bind _settings (Variables|/Game/BP_GameInstance.BP_GameInstance_C|GetSettings _asbp_game_instance))
  (Utilities|TickDelay 2)
  (bind _returnvalue (Game|GetCurrentLevelName true))
  (if (Utilities|Enum|Equal(Enum) _returnvalue "LVL_Tutorial")
    (CallFunction|SetNewObjective "Complete the tutorial."))
  (EventDispatchers|AssignOnToolsMovementUpdated _settings (delegate Custom|OnToolsMovementUpdated_Event))
  (Variables|Default|SetSmoothRotation (Default|GetToolsMovement _settings))
  (switch Utilities|FlowControl|Switch|SwitchonE_ExtrasGamemodes (Variables|/Game/BP_GameInstance.BP_GameInstance_C|GetExtraGamemode _asbp_game_instance)
    (:NewEnumerator0
      (bind (_success _string) (Utilities|CheckpointGetString "MapDeviceObjective" :!label _label))
      (if _success
        (bind _asuw_map_device (Utilities|Casting|CastToUW_MapDevice (UserInterface|GetWidget (Variables|Default|GetWidget)))
          (:then
            (Variables|/Script/UMG.TextBlock|SetText (Variables|/Game/Widgets/UW_MapDevice.UW_MapDevice_C|GetObjectiveText _asuw_map_device) (Utilities|Text|ToText(String) _string)))
          (:CastFailed
            _)))
      (bind (_success_2 _string_2) (Utilities|CheckpointGetString "MapDeviceKeycardLevel"))
      (if _success_2
        (bind _asuw_map_device_2 (Utilities|Casting|CastToUW_MapDevice (UserInterface|GetWidget (Variables|Default|GetWidget)))
          (:then
            (Default|SilentSetKeycardLevel _asuw_map_device_2 _string_2))
          (:CastFailed
            _)))
      (Transformation|SetRelativeScale3D (Variables|Default|GetParent) (Math|Vector|MakeVector 0.0 0.0 0.0))
      (bind _returnvalue_2 (Actor|GetActorOfClass "/Game/Blueprints/Inventory/BP_GlobalInventory.BP_GlobalInventory_C"))
      (EventDispatchers|AssignOnItemReceived _returnvalue_2 (delegate Custom|OnItemReceived_Event))
      (bind _asuw_map_device_3 (Utilities|Casting|CastToUW_MapDevice (UserInterface|GetWidget (Variables|Default|GetWidget))))
      (Variables|/Game/Widgets/UW_MapDevice.UW_MapDevice_C|SetMapDeviceReference _asuw_map_device_3 self))
    (:NewEnumerator1
      (Rendering|SetVisibility _widget false false)
      (Development|SetHiddeninGame _widget true false))
    (:NewEnumerator2
      (goto _label))
    (:NewEnumerator3
      (goto _label))))

(event EventTick
  (params (DeltaSeconds :type Float%20%28single-precision%29))
  (bind _parent (Variables|Default|GetParent))
  (bind _output_get (Variables|Default|SetRoll (Math|Float|Clamp(Float) (* (Variables|Default|GetDeltaY) 1e+01) -25.0 25.0)))
  (Variables|Default|SetDeltaY 0.0)
  (Transformation|SetRelativeRotation _parent (Math|Rotator|MakeRotator (Math|Interpolation|FInterpTo (.roll (Variables|/Script/Engine.SceneComponent|GetRelativeRotation _parent)) _output_get DeltaSeconds 1e+01) 0.0 0.0) false false))

(fn ConstructionScript)