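; Text actor that turns to face the first player's view, keeping its configurable label readable in the world.
; The construction script removes "\n" sequences from the Text variable, writes it to the text render component and applies TextSize as world size.
; Each tick sets the actor's yaw to player 0's control yaw plus a half turn, a yaw-only billboard based on view direction rather than camera position.
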(event EventTick
  (params (DeltaSeconds :type Float%20%28single-precision%29))
  (Transformation|SetActorRotation (Math|Rotator|MakeRotator 0.0 0.0 (+ (.yaw (Pawn|GetControlRotation (Game|GetPlayerController 0) :!class /Script/Engine.Controller)) 1.8e+02))))

(fn ConstructionScript
  (Rendering|Components|TextRender|SetText (Variables|Default|GetTextRender) (Utilities|Text|ToText(String) (Utilities|String|Replace (Utilities|String|ToString(Text) (Variables|Default|GetText)) "\\n" " 
")))
  (Rendering|Components|TextRender|SetWorldSize (Variables|Default|GetTextRender) (Variables|Default|GetTextSize)))