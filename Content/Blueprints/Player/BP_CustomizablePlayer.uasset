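; BP_CustomizablePlayer is a player Blueprint with adjustable colors for helmet, hair, clothes, outer and inner kneepads, and boots.
; On BeginPlay it passes its skeletal mesh to BPPlayerCustomizationComponent for initialization.
; SetData receives a hue and brightness per part and writes them to the HueShift and Brightness parameters of MaterialsInstances.
; Values are matched to materials by array index, so the material order must follow that part order.
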(event Custom|SetData
  (params (HelmetHUE :type Float%20%28double-precision%29) (HairHUE :type Float%20%28single-precision%29) (ClothesHUE :type Float%20%28double-precision%29) (KneepadsOuterHUE :type Float%20%28double-precision%29) (KneepadsInnerHUE :type Float%20%28double-precision%29) (BootsHUE :type Float%20%28double-precision%29) (HelmetBrightness :type Float%20%28double-precision%29) (HairBrightness :type Float%20%28double-precision%29) (ClothesBrightness :type Float%20%28double-precision%29) (KneepadsOuterBrightness :type Float%20%28double-precision%29) (KneepadsInnerBrightness :type Float%20%28double-precision%29) (BootsBrightness :type Float%20%28double-precision%29))
  (for (_array_element _array_index) (Variables|Default|GetMaterialsInstances)
    (Rendering|Material|SetScalarParameterValue _array_element "HueShift" (Utilities|Array|Get(acopy) (Utilities|Array|MakeArray HelmetHUE HairHUE ClothesHUE KneepadsOuterHUE KneepadsInnerHUE BootsHUE) _array_index) :!class /Script/Engine.MaterialInstanceDynamic)
    (Rendering|Material|SetScalarParameterValue _array_element "Brightness" (Utilities|Array|Get(acopy) (Utilities|Array|MakeArray HelmetBrightness HairBrightness ClothesBrightness KneepadsOuterBrightness KneepadsInnerBrightness BootsBrightness) _array_index) :!class /Script/Engine.MaterialInstanceDynamic)))

(event EventBeginPlay
  (Default|Init (Variables|Default|GetBP_PlayerCustomizationComponent) (Utilities|Array|MakeArray (Variables|Default|GetSkeletalMesh))))

(fn ConstructionScript)