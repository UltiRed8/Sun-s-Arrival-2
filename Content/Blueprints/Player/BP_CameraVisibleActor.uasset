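; BP_CameraVisibleActor is a player-related display actor with a text render and a plane, likely meant to be seen by the camera.
; The construction script applies the configurable Text to the text render and DefaultMaterial to the plane.
; When AutoRotate is set, Tick sets its yaw to the player controller's control yaw plus 180 degrees, billboard-style, so it faces back toward the view.
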(event EventBeginPlay)

(event Collision|EventActorBeginOverlap
  (params (OtherActor :type Actor%20Object%20Reference)))

(event EventTick
  (params (DeltaSeconds :type Float%20%28single-precision%29))
  (if (Variables|Default|GetAutoRotate)
    (Transformation|SetActorRotation (Math|Rotator|MakeRotator 0.0 0.0 (+ (.yaw (Pawn|GetControlRotation (Game|GetPlayerController 0) :!class /Script/Engine.Controller)) 1.8e+02)))))

(fn ConstructionScript
  (Rendering|Components|TextRender|SetText (Variables|Default|GetTextRender) (Variables|Default|GetText))
  (Rendering|Material|SetMaterial (Variables|Default|GetPlane) 0 (Variables|Default|GetDefaultMaterial)))