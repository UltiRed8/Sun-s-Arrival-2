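; Player boombox actor that plays music, starting with SW_Toothless, and bounces and flashes in time with it.
; SetMusic starts the audio, then a BPM-timed delay loop calls Light to randomize light color, hop the physics body upright, pulse intensity via timeline and trigger dust.
; The OIIA track also spawns an attached looping level sequence; other tracks call MultiSetBinded.
; Remove destroys the boombox and any sequence once its player list empties.
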(event Custom|SetMusic
  (params (NewSound :type Sound%20Base%20Object%20Reference) (Delay :type Float%20%28single-precision%29) (BPM :type Float%20%28double-precision%29))
  (bind _audio (Variables|Default|GetAudio))
  (Audio|Components|Audio|SetSound _audio NewSound)
  (if (== NewSound "/Game/Audio/Musics/Dances/SW_OIIA.SW_OIIA")
    (bind _outactor (Sequencer|Player|CreateLevelSequencePlayer "/Game/Audio/Musics/Dances/LS_OIIA.LS_OIIA" (Utilities|Struct|MakeMovieSceneSequencePlaybackSettings true (Utilities|Struct|MakeMovieSceneSequenceLoopCount -1))))
    (Variables|Default|SetLevelSequence _outactor)
    (Transformation|AttachActorToActor _outactor self "None" "SnapToTarget" "SnapToTarget" "SnapToTarget" true)
    (Sequencer|Player|Play (Variables|/Script/LevelSequence.LevelSequenceActor|GetSequencePlayer _outactor) :!class /Script/MovieScene.MovieSceneSequencePlayer)
    (else
      (CallFunction|MultiSetBinded)))
  (Audio|Components|Audio|Play _audio 0.0)
  (Utilities|FlowControl|Delay Delay)
  (Utilities|FlowControl|Delay (/ 6e+01 BPM) :!label _label)
  (CallFunction|Light)
  (goto _label))

(event Custom|Light
  (bind _pointlight (Variables|Default|GetPointLight))
  (bind _boombox (Variables|Default|GetBoombox))
  (Rendering|Components|Light|SetLightColor _pointlight (Utilities|Struct|MakeLinearColor (Math|Random|RandomFloatinRange 0.0 1.0) (Math|Random|RandomFloatinRange 0.0 1.0) (Math|Random|RandomFloatinRange 0.0 1.0) 1.0) true)
  (Class|PrimitiveComponent|AddVelocityChangeImpulseatLocation _boombox (Math|Vector|MakeVector 0.0 0.0 1e+02) (Transformation|GetWorldLocation _boombox) "None")
  (Transformation|SetWorldRotation _boombox (Math|Rotator|MakeRotator 0.0 0.0 (.yaw (Transformation|GetWorldRotation _boombox))) false false)
  (bind _intensity (Timeline|LightTimeline PlayFromStart)
    (:Update
      (Rendering|Components|Light|SetIntensity _pointlight (* _intensity 5.0)))
    (:Finished
      (Utilities|FlowControl|Delay 0.1)
      (Components|Activation|Activate (Variables|Default|GetDust) true))))

(event Custom|Stop
  (bind _levelsequence (Variables|Default|GetLevelSequence))
  (Utilities|IsValid _levelsequence
    (:Is%20Valid
      (Actor|DestroyActor _levelsequence))))

(event Custom|Remove
  (params (Player :type BP%20Player%20Object%20Reference%20%28by%20ref%29))
  (bind _players (Variables|Default|GetPlayers))
  (Utilities|Array|RemoveItem _players Player)
  (if (<= (Utilities|Array|Length _players) 0)
    (CallFunction|Stop)
    (Actor|DestroyActor)))

(event Custom|Multi_SetBinded
  (Variables|Default|SetWasLinked true)
  (Development|PrintString "Hello"))

(event EventBeginPlay
  (CallFunction|SetMusic "/Game/Audio/Musics/Dances/SW_Toothless.SW_Toothless" 0.5 1.5e+02)
  (Physics|SetSimulatePhysics (Variables|Default|GetBoombox) true))

(fn ConstructionScript)