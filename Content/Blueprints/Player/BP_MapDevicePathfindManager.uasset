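; Manager for the player map device that lights up the text and floor indicators for a requested destination ID.
; GoToID turns off every entry in AllTexts, then turns on the first one with a matching CustomID.
; That entry's Floor selects the basement, first-floor or second-floor indicator array to switch on.
; Indicator arrays are only ever turned on here, and no route is computed despite the pathfind name.
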(event Custom|TurnOn
  (params (Array :type Array%20of%20BP%20Camera%20Visible%20Text%20Object%20References))
  (for _array_element Array
    (Default|Turnon _array_element)))

(event Custom|GoToID
  (params (ID :type String))
  (for _array_element (Variables|Default|GetAllTexts)
    (Default|TurnOff _array_element))
  (bind _array_element_2 (Utilities|Array|ForEachLoopwithBreak (Variables|Default|GetAllTexts) :!label _label)
    (:LoopBody
      (if (Utilities|Enum|Equal(Enum) (Variables|/Game/Blueprints/Player/BP_CameraVisibleText.BP_CameraVisibleText_C|GetCustomID _array_element_2) ID)
        (Utilities|FlowControl|Sequence
          (:then_0
            (goto _label Break))
          (:then_1
            (Default|Turnon _array_element_2)
            (switch int (Variables|/Game/Blueprints/Player/BP_CameraVisibleText.BP_CameraVisibleText_C|GetFloor _array_element_2)
              (:0
                (CallFunction|Turnon (Variables|Default|GetBasementIndicators)))
              (:1
                (CallFunction|Turnon (Variables|Default|Get1FIndicators)))
              (:2
                (CallFunction|Turnon (Variables|Default|Get2FIndicators))))))))))

(fn ConstructionScript)