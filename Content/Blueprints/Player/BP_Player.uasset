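; Multiplayer player character with switchable first/third-person cameras, sprint-driven FOV, flashlight, map, dance and ragdoll.
; Camera traces set the HUD cursor and drive server-routed interactions, including hold-to-revive on dead players.
; Server, multicast and client events handle death with jumpscare and ragdoll, revival, and defeat when all players are dead.
; Tick updates the map floor parameter, username facing and out-of-world recovery, while OnReps apply name and material colors.
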(event Custom|JumpScare
  (params (NewViewTarget :type Actor%20Object%20Reference))
  ;[0.15 0.15 0.15 0.502] Jumpscare
  (Game|Player|SetViewTargetwithBlend (Game|GetPlayerController 0) NewViewTarget 0.0 "VTBlend_Linear" 0.0 false)
  (Audio|PlaySound2D "/Game/Audio/Sounds/SW_JumpScare.SW_JumpScare" 1.0 1.0 0.0 0 0))

(event Custom|Server_ToggleRagdoll
  ;[0.15 0.15 0.15 0.5] Ragdoll
  (bind _output_get (Variables|Default|SetIsRagdoll (not (Variables|Default|GetIsRagdoll))))
  (if _output_get
    (CallFunction|MultiEnableRagdoll)
    (else
      (CallFunction|MultiDisableRagdoll))))

(event Custom|Multi_DisableRagdoll
  (bind _mesh (Variables|Character|GetMesh))
  ;[0.15 0.15 0.15 0.5] Ragdoll
  (Variables|Default|SetIsRagdoll false)
  (Class|SkeletalMeshComponent|SetAllBodiesSimulatePhysics _mesh false)
  (Transformation|SetRelativeLocationAndRotation _mesh "0.000000,0.000000,-90.000000" "0.000000,-90.000000,0.000000" false false)
  (Variables|Default|SetbUseControllerRotationYaw true)
  (if (Pawn|IsLocallyControlled)
    (CallFunction|GoFirstPerson)))

(event Custom|Multi_Dance
  ;[0.15 0.15 0.15 0.5] Dance
  (Variables|Default|SetIsDancing true)
  (if (Pawn|IsLocallyControlled)
    (CallFunction|GoThirdPerson)))

(event Custom|SetupFlashlightMultiplayer
  ;[0.15 0.15 0.15 0.5] Flashlight visibility for multiplayer
  (Development|SetHiddeninGame (Variables|Default|GetFlashlightLight) (not (Pawn|IsLocallyControlled)) false))

(event Custom|PseudoOrientation
  (bind _returnvalue (Game|GetPlayerController 0))
  (bind _usernamedisplay (Variables|Default|GetUsernameDisplay))
  (bind _returnvalue_2 (Pawn|GetControlledPawn _returnvalue))
  ;[0.15 0.15 0.15 0.5] Pseudo Orientation
  (if (!= _returnvalue_2 self)
    (Transformation|SetWorldRotation _usernamedisplay (Math|Rotator|FindLookatRotation (Transformation|GetWorldLocation _usernamedisplay) (+ (Transformation|GetActorLocation _returnvalue_2) "0.000000,0.000000,70.000000")) false false)))

(event Custom|Server_StopDance
  ;[0.15 0.15 0.15 0.5] Dance
  (CallFunction|MultiStopDance))

(event Custom|Multi_StopDance
  ;[0.15 0.15 0.15 0.5] Dance
  (Variables|Default|SetIsDancing false))

(event Custom|InGameUI
  ;[0.15 0.15 0.15 0.5] In Game UI
  (if (Pawn|IsLocallyControlled)
    (bind _returnvalue (UserInterface|CreateWidget "/Game/Widgets/InGame/UW_InGame.UW_InGame_C" (Game|GetPlayerController 0)))
    (bind _output_get (Variables|Default|SetInGame _returnvalue))
    (UserInterface|Viewport|AddtoViewport _output_get 0)))

(event Custom|OntoServer_InteractWith
  (params (Interactable :type BPI%20Interactable%20Interface) (MethodName :type String))
  (Default|OntoServerInteract Interactable MethodName))

(event Custom|Server_InteractWith
  (params (Target :type BPI%20Interactable%20Interface))
  (Default|ServerInteract Target self))

(event Custom|Server_Dance
  ;[0.15 0.15 0.15 0.5] Dance
  (CallFunction|MultiDance))

(event Custom|FromServer_InteractWith
  (params (Interactable :type BPI%20Interactable%20Interface))
  (Default|ClientInteract Interactable))

(event Custom|UpdateFOV
  (bind _firstpersoncam (Variables|Default|GetFirstPersonCam))
  (bind _thirdpersoncam (Variables|Default|GetThirdPersonCam))
  (bind _isthirdperson (Variables|Default|GetIsThirdPerson))
  (bind _returnvalue (select _isthirdperson _thirdpersoncam _firstpersoncam))
  ;[0.15 0.15 0.15 0.5] Sprint
  (Camera|SetFieldOfView _returnvalue (Math|Interpolation|FInterptoConstant (Variables|/Script/Engine.CameraComponent|GetFieldOfView _returnvalue) (Math|Float|Lerp 9e+01 1e+02 (Math|Float|Clamp(Float) (/ (- (Math|Vector|VectorLength (Transformation|GetVelocity)) 4e+02) 4e+02))) (Utilities|Time|GetWorldDeltaSeconds) 2e+01)))

(event Custom|Client_Death
  (params (KilledBy :type Actor%20Object%20Reference))
  ;[0.15 0.15 0.15 0.5] Death
  (Variables|Default|SetIsDead true)
  (CallFunction|JumpScare KilledBy)
  (bind _outactors (Actor|GetAllActorsOfClass "/Game/Blueprints/Interactives/BP_InteractiveBase.BP_InteractiveBase_C"))
  (for _array_element _outactors
    (Default|ForceStopCapturing (Variables|/Game/Blueprints/Interactives/BP_InteractiveBase.BP_InteractiveBase_C|GetBP_MouseMovementComponent _array_element)))
  (Utilities|FlowControl|Delay 1.0)
  (Game|Player|SetViewTargetwithBlend (Game|GetPlayerController 0) self 0.0 "VTBlend_Linear" 0.0 false)
  (CallFunction|GoThirdPerson)
  (Rendering|SetVisibility (Variables|Default|GetFlashlightLight) false false)
  (bind _returnvalue (Actor|GetActorOfClass "/Game/Blueprints/BP_AchievementManager.BP_AchievementManager_C"))
  (Default|Unlock _returnvalue "first_death"))

(event Custom|Multi_Death
  ;[0.15 0.15 0.15 0.5] Death
  (Development|SetHiddeninGame (Variables|Default|GetDeathLight) false false)
  (Variables|Default|SetIsDead true))

(event Custom|CustomEvent
  (bind _returnvalue (Transformation|GetActorLocation))
  (Rendering|Material|SetScalarParameterValue "/Game/Materials/MPC_MapParameters.MPC_MapParameters" "Floor" (Math|Float|SelectFloat -1.0 (Math|Float|SelectFloat 1.0 0.0 (> (.z _returnvalue) 5e+02)) (< (.z _returnvalue) -1e+02)) :!class /Script/Engine.KismetMaterialLibrary))

(event Custom|Multi_Revive
  ;[0.15 0.15 0.15 0.5] Revive
  (Development|SetHiddeninGame (Variables|Default|GetDeathLight) true false)
  (Variables|Default|SetIsDead false)
  (if (Pawn|IsLocallyControlled)
    (bind _returnvalue (UserInterface|CreateWidget "/Game/Widgets/InGame/UW_BorderFlash.UW_BorderFlash_C" 0 "(R=0.000000,G=1.000000,B=0.000000,A=1.000000)"))
    (UserInterface|Viewport|AddtoViewport _returnvalue 0)))

(event Custom|SensitivityUpdate
  (Variables|Default|SetSensitivity (Math|Float|Clamp(Float) (+ (Variables|/Game/BP_GameInstance.BP_GameInstance_C|GetMouseSensitivity (Utilities|GameInstance)) 1.0) 0.1 5.0)))

(event Custom|Server_RevivePlayer
  (params (Target :type Self%20Object%20Reference))
  ;[0.15 0.15 0.15 0.5] Revive
  (CallFunction|ServerRevive Target))

(event Custom|Server_CheckGame
  (Utilities|FlowControl|Sequence
    (:then_0
      (goto _label_2 Open))
    (:then_1
      (bind _outactors (Actor|GetAllActorsOfClass "BP_Player_C"))
      (bind _array_element (Utilities|Array|ForEachLoopwithBreak _outactors :!label _label)
        (:LoopBody
          (if (not (Variables|BP_Player_C|GetIsDead _array_element))
            (Utilities|FlowControl|Sequence
              (:then_0
                (goto _label_2 Close))
              (:then_1
                (goto _label Break)))))
        (:Completed
          (Utilities|FlowControl|Gate false :!label _label_2
            (:Exit
              (CallFunction|MultiDefeat))))))))

(event Custom|Server_Revive
  ;[0.15 0.15 0.15 0.5] Revive
  (if (Variables|Default|GetIsDead)
    (Variables|Default|SetIsDead false)
    (CallFunction|MultiDisableRagdoll)
    (CallFunction|MultiRevive)))

(event Custom|Multi_Defeat
  (bind _returnvalue (UserInterface|CreateWidget "/Game/Widgets/UW_GameOver.UW_GameOver_C" (Game|GetPlayerController 0) false (Ability|HasAuthority)))
  (UserInterface|Viewport|AddtoViewport _returnvalue 0)
  (bind _returnvalue_2 (Actor|GetActorOfClass "/Game/Blueprints/BP_AchievementManager.BP_AchievementManager_C"))
  (Default|Unlock _returnvalue_2 "defeat"))

(event Custom|UnbindSensitivity
  (EventDispatchers|UnbindEventfromOnSensitivityChanged (Utilities|GameInstance) (delegate Custom|SensitivityUpdate)))

(event Custom|BindSensitivity
  (EventDispatchers|AssignOnSensitivityChanged (Utilities|GameInstance) (delegate Custom|SensitivityUpdate))
  (CallFunction|SensitivityUpdate))

(event Custom|Client_SetBeingRevived
  (params (BeingRevived :type Boolean) (ByUsername :type String))
  (bind _ingame (Variables|Default|GetInGame))
  (Utilities|IsValid _ingame
    (:Is%20Valid
      (Default|SetBeingRevived _ingame BeingRevived ByUsername))))

(event Custom|CheckDeathZone
  (bind _mesh (Variables|Character|GetMesh))
  ;[0.15 0.15 0.15 0.5] DeathZone
  (if (<= (.z (Transformation|GetActorLocation)) -2.4e+03)
    (Transformation|Teleport "0.000000,0.000000,200.000000" "0, 0, 0")
    (if (Variables|Default|GetIsRagdoll)
      (Physics|SetSimulatePhysics _mesh false)
      (Transformation|SetWorldLocation _mesh "0.000000,0.000000,200.000000" false false)
      (Physics|SetSimulatePhysics _mesh true))))

(event Custom|Server_SetBeingRevived
  (params (Player :type Self%20Object%20Reference) (BeingRevived :type Boolean) (ByUsername :type String))
  (Utilities|IsValid Player
    (:Is%20Valid
      (CallFunction|ClientSetBeingRevived Player BeingRevived ByUsername))))

(event Custom|CursorTick
  (bind _thirdpersoncam (Variables|Default|GetThirdPersonCam))
  (bind _firstpersoncam (Variables|Default|GetFirstPersonCam))
  (bind _isthirdperson (Variables|Default|GetIsThirdPerson))
  (bind _ingame (Variables|Default|GetInGame))
  (bind _returnvalue (select _isthirdperson _thirdpersoncam _firstpersoncam))
  (bind _returnvalue_2 (Transformation|GetWorldLocation _returnvalue))
  (if (Pawn|IsLocallyControlled)
    (Utilities|IsValid (Variables|Default|GetInGame)
      (:Is%20Valid
        (bind (_outhit _returnvalue_3) (Collision|LineTraceByChannel _returnvalue_2 (+ _returnvalue_2 (* (Math|Vector|GetForwardVector (Transformation|GetWorldRotation _returnvalue)) (select (Variables|Default|GetIsThirdPerson) 6e+02 3.5e+02))) "TraceTypeQuery1" false 0 "None"))
        (if _returnvalue_3
          (bind _asbp_interactive_base (Utilities|Casting|CastToBP_InteractiveBase (.HitActor (Collision|BreakHitResult _outhit)))
            (:then
              (Default|SetCustomCursor _ingame (Variables|/Game/Blueprints/Interactives/BP_InteractiveBase.BP_InteractiveBase_C|GetTexture2D _asbp_interactive_base)))
            (:CastFailed
              (bind _asbp_classic_openable_door (Utilities|Casting|CastToBP_ClassicOpenableDoor (.HitActor (Collision|BreakHitResult _outhit)))
                (:then
                  (if (and (Variables|/Game/Blueprints/Doors/BP_DoorBase.BP_DoorBase_C|GetCanBeToggledByPlayer _asbp_classic_openable_door) (not (Variables|/Game/Blueprints/Doors/BP_DoorBase.BP_DoorBase_C|GetIsLocked _asbp_classic_openable_door)))
                    (Default|SetCustomCursor _ingame "/Game/Textures/T_CursorInteract.T_CursorInteract" :!label _label)
                    (else
                      (bind _asbp_object_base (Utilities|Casting|CastToBP_ObjectBase (.HitActor (Collision|BreakHitResult _outhit)) :!label _label_2)
                        (:then
                          (if (Variables|/Game/Blueprints/Objects/BP_ObjectBase.BP_ObjectBase_C|GetCanPickup _asbp_object_base)
                            (goto _label)
                            (else
                              _)))
                        (:CastFailed
                          _))
                      (bind _asbp_arcade_base (Utilities|Casting|CastToBP_ArcadeBase (.HitActor (Collision|BreakHitResult _outhit)))
                        (:then
                          (if (Variables|/Game/Blueprints/Interactives/Arcades/BP_ArcadeBase.BP_ArcadeBase_C|GetIsTurnedOn _asbp_arcade_base)
                            (Default|SetCustomCursor _ingame (Variables|/Game/Blueprints/Interactives/Arcades/BP_ArcadeBase.BP_ArcadeBase_C|GetTexture2D _asbp_arcade_base))
                            (else
                              (Utilities|Casting|CastToBP_CraneControls (.HitActor (Collision|BreakHitResult _outhit)) :!label _label_3
                                (:then
                                  (goto _label))
                                (:CastFailed
                                  (Utilities|Casting|CastToBP_Locker (.HitActor (Collision|BreakHitResult _outhit))
                                    (:then
                                      (goto _label))
                                    (:CastFailed
                                      (bind _asbp_host_start (Utilities|Casting|CastToBP_HostStart (.HitActor (Collision|BreakHitResult _outhit)))
                                        (:then
                                          (if (not (Variables|/Game/Blueprints/HostStart/BP_HostStart.BP_HostStart_C|GetInCinematic _asbp_host_start))
                                            (goto _label)))
                                        (:CastFailed
                                          (Default|SetCustomCursor (Variables|Default|GetInGame) "/Game/Textures/T_CursorNormal.T_CursorNormal" :!label _label_4))))))))))
                        (:CastFailed
                          (goto _label_3))))))
                (:CastFailed
                  (goto _label_2)))))
          (else
            (goto _label_4)))))))

(event Custom|Server_Death
  (params (KilledBy :type Actor%20Object%20Reference))
  (bind _self self)
  ;[0.15 0.15 0.15 0.5] Death
  (if (not (Variables|Default|GetIsDead))
    (bind _outactors (Actor|GetAllActorsOfClass "/Game/Blueprints/Interactives/Arcades/BP_ArcadeBase.BP_ArcadeBase_C"))
    (for _array_element _outactors
      (Default|ServerCheckDeadPlayer _array_element _self))
    (bind _outactors_2 (Actor|GetAllActorsOfClass "/Game/Blueprints/MiniGames/Crane/BP_CraneControls.BP_CraneControls_C"))
    (for _array_element_2 _outactors_2
      (Default|ServerCheckDeadPlayer _array_element_2 _self))
    (Variables|Default|SetIsDead true)
    (CallFunction|ClientDeath KilledBy)
    (Utilities|FlowControl|Delay 1.0)
    (CallFunction|MultiEnableRagdoll)
    (CallFunction|MultiDeath)
    (Utilities|FlowControl|RetriggerableDelay 3.0)
    (CallFunction|ServerCheckGame)))

(event Custom|GoFirstPerson
  ;[0.15 0.15 0.15 0.5] Perspectives
  (Variables|Default|SetIsThirdPerson false)
  (CallFunction|UpdatePerspective))

(event Custom|GoThirdPerson
  ;[0.15 0.15 0.15 0.5] Perspectives
  (Variables|Default|SetIsThirdPerson true)
  (CallFunction|UpdatePerspective))

(event Custom|TogglePerspective
  ;[0.15 0.15 0.15 0.5] Perspectives
  (Variables|Default|SetIsThirdPerson (not (Variables|Default|GetIsThirdPerson)))
  (CallFunction|UpdatePerspective))

(event Custom|UpdatePerspective
  (bind _isthirdperson (Variables|Default|GetIsThirdPerson))
  (bind _returnvalue (not _isthirdperson))
  ;[0.15 0.15 0.15 0.5] Perspectives
  (Components|Activation|SetActive (Variables|Default|GetThirdPersonCam) _isthirdperson false)
  (Components|Activation|SetActive (Variables|Default|GetFirstPersonCam) _returnvalue false)
  (Class|PrimitiveComponent|SetOwnerNoSee (Variables|Character|GetMesh) _returnvalue)
  (Transformation|AttachComponentToComponent (Variables|Default|GetFlashlightLight) (select _isthirdperson (Variables|Default|GetThirdPersonFlashlightPoint) (Variables|Default|GetFirstPersonFlashlightPoint)) "Head" "SnapToTarget" "SnapToTarget" "KeepRelative" true)
  (Development|SetHiddeninGame (Variables|Default|GetThirdPersonFlashlight) _returnvalue false)
  (Development|SetHiddeninGame (Variables|Default|GetFirstPersonFlashlight) _isthirdperson false)
  (Variables|Default|SetbUseControllerRotationYaw _returnvalue)
  (Variables|/Script/Engine.CharacterMovementComponent|SetbOrientRotationToMovement (Variables|Character|GetCharacterMovement) (Variables|Default|GetIsThirdPerson)))

(event Custom|Multi_EnableRagdoll
  (bind _mesh (Variables|Character|GetMesh))
  ;[0.15 0.15 0.15 0.5] Ragdoll
  (Variables|Default|SetIsRagdoll true)
  (Class|PrimitiveComponent|WakeAllRigidBodies _mesh)
  (Class|SkeletalMeshComponent|SetAllBodiesSimulatePhysics _mesh true)
  (Variables|Default|SetbUseControllerRotationYaw false)
  (if (Pawn|IsLocallyControlled)
    (CallFunction|GoThirdPerson)))

(event Input|EnhancedActionEvents|EnhancedInputActionIA_Move
  (params (ActionValue :type Vector%202D%20Structure) (ElapsedSeconds :type Float%20%28double-precision%29) (TriggeredSeconds :type Float%20%28double-precision%29) (InputAction :type Input%20Action%20Object%20Reference :default "/Game/Inputs/Actions/IA_Move.IA_Move"))
  (bind _returnvalue (Pawn|GetControlRotation :!class /Script/Engine.Pawn))
  (bind _isdancing (Variables|Default|GetIsDancing))
  (bind _yaw (Math|Rotator|BreakRotator _returnvalue))
  (bind _returnvalue_2 (Math|Rotator|MakeRotator 0.0 0.0 _yaw))
  ;[0.15 0.15 0.15 0.5] Inputs
  (:Triggered
    (Utilities|NotRagdollHiding
      (:true
        (if (Variables|Default|GetIsThirdPerson)
          (if _isdancing
            (CallFunction|ServerStopDance))
          (Pawn|Input|AddMovementInput (Math|Vector|GetForwardVector _returnvalue_2) (.x ActionValue) false)
          (Pawn|Input|AddMovementInput (Math|Vector|GetRightVector _returnvalue_2) (.y ActionValue) false)
          (else
            (if _isdancing
              (CallFunction|ServerStopDance))
            (Pawn|Input|AddMovementInput (+ (* (.x ActionValue) (Transformation|GetActorForwardVector)) (* (.y ActionValue) (Transformation|GetActorRightVector))) 1.0 false)))
        (CallFunction|UpdateFOV)
        (Variables|/Script/Engine.CharacterMovementComponent|SetMaxWalkSpeed (Variables|Character|GetCharacterMovement) (+ 4e+02 (Math|Float|SelectFloat (* 4e+02 (Math|Float|SelectFloat 1.0 (/ (+ (Math|Vector|DotProduct (Transformation|GetActorForwardVector) (Math|Vector|RotateVector (Math|Vector|Normalize (Math|Vector|MakeVector (.x ActionValue) (.y ActionValue) 0.0) 0.0) (Transformation|GetWorldRotation (Variables|Collision|GetCapsuleComponent)))) 1.0) 2.0) (Variables|Default|GetIsThirdPerson))) 0.0 (Variables|Default|GetIsSprinting))) :!label _label))))
  (:Started
    (Variables|Default|SetCanSprint true)
    (CallFunction|ServerSetBeingRevived (Variables|/Game/Widgets/InGame/UW_InGame.UW_InGame_C|GetPlayer (Variables|Default|GetInGame)) false)
    (Default|SetTarget (Variables|Default|GetInGame)))
  (:Canceled
    (Variables|Default|SetCanSprint false :!label _label_2)
    (CallFunction|UpdateFOV)
    (goto _label))
  (:Completed
    (goto _label_2)))

(event Input|EnhancedActionEvents|EnhancedInputActionIA_Look
  (params (ActionValue :type Vector%202D%20Structure) (ElapsedSeconds :type Float%20%28double-precision%29) (TriggeredSeconds :type Float%20%28double-precision%29) (InputAction :type Input%20Action%20Object%20Reference :default "/Game/Inputs/Actions/IA_Look.IA_Look"))
  (bind _sensitivity (Variables|Default|GetSensitivity))
  (bind _returnvalue (* (.x ActionValue) _sensitivity))
  ;[0.15 0.15 0.15 0.5] Inputs
  (Pawn|Input|AddControllerPitchInput (* (.y ActionValue) _sensitivity))
  (Pawn|Input|AddControllerYawInput _returnvalue)
  (if (not (Variables|Default|GetIsMouseCaptured))
    (bind _asbp_map_device (Utilities|Casting|CastToBP_MapDevice (Variables|/Script/Engine.ChildActorComponent|GetChildActor (Variables|Default|GetMapDeviceActor))))
    (Default|UpdateRoll _asbp_map_device _returnvalue)))

(event Input|EnhancedActionEvents|EnhancedInputActionIA_Flashlight
  (params (ActionValue :type Boolean) (ElapsedSeconds :type Float%20%28double-precision%29) (TriggeredSeconds :type Float%20%28double-precision%29) (InputAction :type Input%20Action%20Object%20Reference :default "/Game/Inputs/Actions/IA_Flashlight.IA_Flashlight"))
  (bind _flashlightlight (Variables|Default|GetFlashlightLight))
  ;[0.15 0.15 0.15 0.5] Flashlight
  (:Started
    (if (not (Variables|Default|GetIsDead))
      (if (not (Class|Pawn|IsMoveInputIgnored))
        (Rendering|ToggleVisibility _flashlightlight false)
        (if (Variables|/Script/Engine.SceneComponent|GetbVisible _flashlightlight)
          (Audio|PlaySound2D "/Game/Audio/Sounds/SW_FlashlightOn.SW_FlashlightOn" 1.0 1.0 0.55 0 0)
          (else
            (Audio|PlaySound2D "/Game/Audio/Sounds/SW_FlashlightOff.SW_FlashlightOff" 1.0 1.0 0.9 0 0)))))))

(event Input|EnhancedActionEvents|EnhancedInputActionIA_Sprint
  (params (ActionValue :type Boolean) (ElapsedSeconds :type Float%20%28double-precision%29) (TriggeredSeconds :type Float%20%28double-precision%29) (InputAction :type Input%20Action%20Object%20Reference :default "/Game/Inputs/Actions/IA_Sprint.IA_Sprint"))
  (bind _asbp_game_instance (Utilities|GameInstance))
  (bind _togglesprint (Variables|/Game/BP_GameInstance.BP_GameInstance_C|GetToggleSprint _asbp_game_instance))
  ;[0.15 0.15 0.15 0.5] Sprint
  (:Started
    (if _togglesprint
      (Utilities|FlowControl|FlipFlop
        (:A
          (Variables|Default|SetIsSprinting true :!label _label))
        (:B
          (Variables|Default|SetIsSprinting false :!label _label_2)))
      (else
        (goto _label))))
  (:Canceled
    (if (not _togglesprint) :!label _label_3
      (goto _label_2)))
  (:Completed
    (goto _label_3)))

(event Input|EnhancedActionEvents|EnhancedInputActionIA_Interact
  (params (ActionValue :type Boolean) (ElapsedSeconds :type Float%20%28double-precision%29) (TriggeredSeconds :type Float%20%28double-precision%29) (InputAction :type Input%20Action%20Object%20Reference :default "/Game/Inputs/Actions/IA_Interact.IA_Interact"))
  (bind _ingame (Variables|Default|GetInGame))
  (bind _ingame_2 (Variables|Default|GetInGame))
  (bind _isthirdperson (Variables|Default|GetIsThirdPerson))
  (bind _thirdpersoncam (Variables|Default|GetThirdPersonCam))
  (bind _firstpersoncam (Variables|Default|GetFirstPersonCam))
  (bind _isthirdperson_2 (Variables|Default|GetIsThirdPerson))
  (bind _returnvalue (select _isthirdperson 6e+02 3.5e+02))
  (bind _returnvalue_2 (select _isthirdperson_2 _thirdpersoncam _firstpersoncam))
  (bind _returnvalue_3 (Transformation|GetWorldLocation _returnvalue_2))
  (bind _returnvalue_4 (Transformation|GetWorldRotation _returnvalue_2))
  (bind _returnvalue_5 (Math|Vector|GetForwardVector _returnvalue_4))
  (bind _returnvalue_6 (* _returnvalue_5 _returnvalue))
  (bind _returnvalue_7 (+ _returnvalue_3 _returnvalue_6))
  ;[0.15 0.15 0.15 0.502] Interaction
  (:Started
    (if (not (Variables|Default|GetIsRagdoll))
      (if (not (Class|Pawn|IsMoveInputIgnored))
        (bind (_outhit _returnvalue_8) (Collision|LineTraceByChannel _returnvalue_3 _returnvalue_7 "TraceTypeQuery1" false 0 "None"))
        (if _returnvalue_8
          (if (Utilities|DoesObjectImplementInterface (.HitActor (Collision|BreakHitResult _outhit)) "/Game/Interfaces/BPI_Interactable.BPI_Interactable_C")
            (bind _asbpi_interactable (Utilities|Casting|CastToBPI_Interactable (.HitActor (Collision|BreakHitResult _outhit))))
            (CallFunction|ServerInteractwith _asbpi_interactable)
            (else
              (bind (_outhit_2 _returnvalue_9) (Collision|SphereTraceForObjects _returnvalue_3 _returnvalue_7 75.0 (Utilities|Array|MakeArray "ObjectTypeQuery4") false 0 "None"))
              (if _returnvalue_9
                (bind _asbp_player (Utilities|Casting|CastToBP_Player (.HitActor (Collision|BreakHitResult _outhit_2))))
                (if (Variables|BP_Player_C|GetIsDead _asbp_player)
                  (CallFunction|ServerSetBeingRevived _asbp_player true (Variables|NetworkVariables|GetUsername))
                  (Default|SetTarget _ingame _asbp_player)
                  (Utilities|FlowControl|RetriggerableDelay (Variables|/Game/Widgets/InGame/UW_InGame.UW_InGame_C|GetTimeToComplete _ingame))
                  (Utilities|IsValid (Variables|/Game/Widgets/InGame/UW_InGame.UW_InGame_C|GetPlayer _ingame)
                    (:Is%20Valid
                      (CallFunction|ServerRevivePlayer _asbp_player)))))))))))
  (:Canceled
    (CallFunction|ServerSetBeingRevived (Variables|/Game/Widgets/InGame/UW_InGame.UW_InGame_C|GetPlayer _ingame_2) false :!label _label)
    (Default|SetTarget _ingame_2))
  (:Completed
    (goto _label)))

(event Input|EnhancedActionEvents|EnhancedInputActionIA_Dance
  (params (ActionValue :type Boolean) (ElapsedSeconds :type Float%20%28double-precision%29) (TriggeredSeconds :type Float%20%28double-precision%29) (InputAction :type Input%20Action%20Object%20Reference :default "/Game/Inputs/Actions/IA_Dance.IA_Dance"))
  ;[0.15 0.15 0.15 0.5] Dance
  (:Started
    (if (not (Variables|Default|GetIsDead))
      (if (not (Class|Pawn|IsMoveInputIgnored))
        (CallFunction|ServerDance)))))

(event Input|EnhancedActionEvents|EnhancedInputActionIA_Perspective
  (params (ActionValue :type Boolean) (ElapsedSeconds :type Float%20%28double-precision%29) (TriggeredSeconds :type Float%20%28double-precision%29) (InputAction :type Input%20Action%20Object%20Reference :default "/Game/Inputs/Actions/IA_Perspective.IA_Perspective"))
  ;[0.15 0.15 0.15 0.5] Perspectives
  (:Started
    (if (not (Variables|Default|GetIsDead))
      (if (not (Class|Pawn|IsMoveInputIgnored))
        (CallFunction|TogglePerspective)))))

(event Input|EnhancedActionEvents|EnhancedInputActionIA_Ragdoll
  (params (ActionValue :type Boolean) (ElapsedSeconds :type Float%20%28double-precision%29) (TriggeredSeconds :type Float%20%28double-precision%29) (InputAction :type Input%20Action%20Object%20Reference :default "/Game/Inputs/Actions/IA_Ragdoll.IA_Ragdoll"))
  ;[0.15 0.15 0.15 0.5] Ragdoll
  (:Started
    (if (not (Variables|Default|GetIsDead))
      (if (not (Variables|Default|GetIsHiding))
        (CallFunction|ServerToggleRagdoll)))))

(event Input|EnhancedActionEvents|EnhancedInputActionIA_Map
  (params (ActionValue :type Boolean) (ElapsedSeconds :type Float%20%28double-precision%29) (TriggeredSeconds :type Float%20%28double-precision%29) (InputAction :type Input%20Action%20Object%20Reference :default "/Game/Inputs/Actions/IA_Map.IA_Map"))
  (:Started
    (Utilities|IsValid (Variables|Default|GetInGameMap)
      (:Is%20Valid
        (Default|CustomClose (Variables|Default|GetInGameMap))
        (Variables|Default|SetInGameMap 0))
      (:Is%20Not%20Valid
        (bind _returnvalue (UserInterface|CreateWidget "/Game/Widgets/InGame/UW_Map.UW_Map_C"))
        (bind _output_get (Variables|Default|SetInGameMap _returnvalue))
        (UserInterface|Viewport|AddtoViewport _output_get 0)))))

(event EventDestroyed
  ;[0.15 0.15 0.15 0.5] Destruct Event
  (if (Pawn|IsLocallyControlled)
    (CallFunction|UnbindSensitivity)))

(event EventTick
  (params (DeltaSeconds :type Float%20%28single-precision%29))
  ;[0.15 0.15 0.15 0.5] TickEvent
  (CallFunction|CustomEvent)
  (CallFunction|PseudoOrientation)
  (CallFunction|CursorTick)
  (Networking|SwitchHasAuthority
    (:Authority
      (CallFunction|CheckDeathZone)
      (if (Pawn|IsLocallyControlled)
        (CallFunction|UpdateFOV)))))

(event EventBeginPlay
  ;[0.15 0.15 0.15 0.5] Beginplay
  (CallFunction|SetupFlashlightMultiplayer)
  (CallFunction|InGameUI)
  (if (Pawn|IsLocallyControlled)
    (CallFunction|BindSensitivity)))

(event Input|KeyboardEvents|SpaceBar
  (params (Key :type Key%20Structure :default "None"))
  (:Pressed
    (bind _asbp_map_device (Utilities|Casting|CastToBP_MapDevice (Variables|/Script/Engine.ChildActorComponent|GetChildActor (Variables|Default|GetMapDeviceActor))))
    (Default|Toggle _asbp_map_device)))

(fn ConstructionScript
  (Transformation|AttachComponentToComponent (Variables|Default|GetThirdPersonFlashlight) (Variables|Character|GetMesh) "RightHandSocket" "SnapToTarget" "KeepRelative" "KeepRelative" true))

(fn OnRepHueShift
  (Utilities|IsValid (Variables|Default|GetDynamicMaterial)
    (:Is%20Valid
      _)
    (:Is%20Not%20Valid
      (bind _returnvalue (Rendering|Material|CreateDynamicMaterialInstance (Variables|Character|GetMesh) 1 "/Game/Models/Player/MAT_Player2.MAT_Player2" "None" :!class /Script/Engine.PrimitiveComponent))
      (bind _output_get (Variables|Default|SetDynamicMaterial _returnvalue))))
  (Rendering|Material|SetScalarParameterValue _output_get "HueShift" (Variables|NetworkVariables|GetHueShift) :!class /Script/Engine.MaterialInstanceDynamic)
  (Rendering|Material|SetScalarParameterValue _output_get "Brightness" (Variables|NetworkVariables|GetBrightness) :!class /Script/Engine.MaterialInstanceDynamic)
  (Rendering|Material|SetScalarParameterValue _output_get "Saturation" (Variables|NetworkVariables|GetSaturation) :!class /Script/Engine.MaterialInstanceDynamic))

(fn OnRepUsername
  (Rendering|Components|TextRender|SetText (Variables|Default|GetUsernameDisplay) (Utilities|Text|ToText(String) (Variables|NetworkVariables|GetUsername))))

(fn OnRepSaturation
  (Utilities|IsValid (Variables|Default|GetDynamicMaterial)
    (:Is%20Valid
      _)
    (:Is%20Not%20Valid
      (bind _returnvalue (Rendering|Material|CreateDynamicMaterialInstance (Variables|Character|GetMesh) 1 "/Game/Models/Player/MAT_Player2.MAT_Player2" "None" :!class /Script/Engine.PrimitiveComponent))
      (bind _output_get (Variables|Default|SetDynamicMaterial _returnvalue))))
  (Rendering|Material|SetScalarParameterValue _output_get "HueShift" (Variables|NetworkVariables|GetHueShift) :!class /Script/Engine.MaterialInstanceDynamic)
  (Rendering|Material|SetScalarParameterValue _output_get "Brightness" (Variables|NetworkVariables|GetBrightness) :!class /Script/Engine.MaterialInstanceDynamic)
  (Rendering|Material|SetScalarParameterValue _output_get "Saturation" (Variables|NetworkVariables|GetSaturation) :!class /Script/Engine.MaterialInstanceDynamic))

(fn OnRepBrightness
  (Utilities|IsValid (Variables|Default|GetDynamicMaterial)
    (:Is%20Valid
      _)
    (:Is%20Not%20Valid
      (bind _returnvalue (Rendering|Material|CreateDynamicMaterialInstance (Variables|Character|GetMesh) 1 "/Game/Models/Player/MAT_Player2.MAT_Player2" "None" :!class /Script/Engine.PrimitiveComponent))
      (bind _output_get (Variables|Default|SetDynamicMaterial _returnvalue))))
  (Rendering|Material|SetScalarParameterValue _output_get "HueShift" (Variables|NetworkVariables|GetHueShift) :!class /Script/Engine.MaterialInstanceDynamic)
  (Rendering|Material|SetScalarParameterValue _output_get "Brightness" (Variables|NetworkVariables|GetBrightness) :!class /Script/Engine.MaterialInstanceDynamic)
  (Rendering|Material|SetScalarParameterValue _output_get "Saturation" (Variables|NetworkVariables|GetSaturation) :!class /Script/Engine.MaterialInstanceDynamic))