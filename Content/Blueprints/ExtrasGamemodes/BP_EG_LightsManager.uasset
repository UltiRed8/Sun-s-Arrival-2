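; Manager actor that adjusts level lighting for the Exploration and Hardcore extra gamemodes.
; On BeginPlay it binds to BP_RoomManager's OnLoadingCompleted, then branches on the GameInstance's ExtraGamemode once loading finishes.
; Each mode sets every suspended and wall light to its own preset state.
; Hardcore also switches off all light posts, which Exploration leaves untouched.
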(event Custom|OnLoadingCompleted_Event
  (switch Utilities|FlowControl|Switch|SwitchonE_ExtrasGamemodes (Variables|/Game/BP_GameInstance.BP_GameInstance_C|GetExtraGamemode (Utilities|GameInstance))
    (:NewEnumerator1
      (CallFunction|SetupExploration))
    (:NewEnumerator2
      (CallFunction|SetupHardcore))))

(event Custom|SetupExploration
  (bind _outactors (Actor|GetAllActorsOfClass "/Game/Blueprints/GPE/Lights/BP_SuspendedLight.BP_SuspendedLight_C"))
  (for _array_element _outactors
    (Default|SetState _array_element "NewEnumerator2"))
  (bind _outactors_2 (Actor|GetAllActorsOfClass "/Game/Blueprints/GPE/Lights/BP_WallLight.BP_WallLight_C"))
  (for _array_element_2 _outactors_2
    (Default|SetState _array_element_2 "NewEnumerator2")))

(event Custom|SetupHardcore
  (bind _outactors (Actor|GetAllActorsOfClass "/Game/Blueprints/GPE/Lights/BP_SuspendedLight.BP_SuspendedLight_C"))
  (for _array_element _outactors
    (Default|SetState _array_element "NewEnumerator0"))
  (bind _outactors_2 (Actor|GetAllActorsOfClass "/Game/Blueprints/GPE/Lights/BP_WallLight.BP_WallLight_C"))
  (for _array_element_2 _outactors_2
    (Default|SetState _array_element_2 "NewEnumerator0"))
  (bind _outactors_3 (Actor|GetAllActorsOfClass "/Game/Blueprints/Decoratives/BP_LightPost.BP_LightPost_C"))
  (for _array_element_3 _outactors_3
    (Default|Off _array_element_3)))

(event EventBeginPlay
  (bind _returnvalue (Actor|GetActorOfClass "/Game/Blueprints/GPE/Rooms/BP_RoomManager.BP_RoomManager_C"))
  (EventDispatchers|AssignOnLoadingCompleted _returnvalue (delegate Custom|OnLoadingCompleted_Event)))

(fn ConstructionScript)