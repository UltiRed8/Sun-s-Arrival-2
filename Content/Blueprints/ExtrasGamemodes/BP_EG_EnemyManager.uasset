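; BP_EG_EnemyManager adjusts the level's Endo enemies at BeginPlay according to the extra gamemode stored on the GameInstance.
; Exploration destroys every BP_EndoBase and turns off attacking on BP_StandEndo actors.
; Chaos records and destroys all non-EndoBlock Endos, then spawns random classes from a list at the shuffled locations in their default state.
; Chaos also triggers any standing Endos flagged as attacking.
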(event Custom|SetupExploration
  (bind _outactors (Actor|GetAllActorsOfClass "/Game/Blueprints/Enemies/BP_EndoBase.BP_EndoBase_C"))
  (for _array_element _outactors
    (Actor|DestroyActor _array_element))
  (bind _outactors_2 (Actor|GetAllActorsOfClass "/Game/Blueprints/Enemies/BP_StandEndo.BP_StandEndo_C"))
  (for _array_element_2 _outactors_2
    (Variables|/Game/Blueprints/Enemies/BP_StandEndo.BP_StandEndo_C|SetIsAttacking _array_element_2 false)))

(event Custom|SetupChaos
  (bind _locations (Variables|Default|GetLocations))
  (bind _outactors (Actor|GetAllActorsOfClass "/Game/Blueprints/Enemies/BP_EndoBase.BP_EndoBase_C"))
  (for _array_element _outactors
    (Class|KismetSystemLibrary|IsObjectOfSoftClass _array_element "/Game/Blueprints/Enemies/BP_EndoBlock.BP_EndoBlock_C"
      (:False
        (Utilities|Array|Add (Variables|Default|GetLocations) (Transformation|GetActorLocation _array_element))
        (Actor|DestroyActor _array_element))))
  (Utilities|Array|Shuffle _locations)
  (for _array_element_2 _locations
    (bind _returnvalue (AI|SpawnAIFromClass (.OutItem (Utilities|Array|Random (Variables|Default|GetClasses))) 0 _array_element_2 "0, 0, 0" false 0))
    (bind _asbp_endo_base (Utilities|Casting|CastToBP_EndoBase _returnvalue))
    (Default|DefaultState _asbp_endo_base))
  (bind _outactors_2 (Actor|GetAllActorsOfClass "/Game/Blueprints/Enemies/BP_StandEndo.BP_StandEndo_C"))
  (for _array_element_3 _outactors_2
    (if (Variables|/Game/Blueprints/Enemies/BP_StandEndo.BP_StandEndo_C|GetIsAttacking _array_element_3)
      (Default|Trigger _array_element_3))))

(event EventBeginPlay
  (switch Utilities|FlowControl|Switch|SwitchonE_ExtrasGamemodes (Variables|/Game/BP_GameInstance.BP_GameInstance_C|GetExtraGamemode (Utilities|GameInstance))
    (:NewEnumerator1
      (CallFunction|SetupExploration))
    (:NewEnumerator3
      (CallFunction|SetupChaos))))

(fn ConstructionScript)