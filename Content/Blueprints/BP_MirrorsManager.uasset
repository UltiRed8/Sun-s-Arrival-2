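; BP_MirrorsManager applies the game's Mirrors setting to the level's planar reflections and mirror meshes.
; After a short tick delay on BeginPlay, it gathers all PlanarReflection actors, binds to the settings' update event and applies an initial update.
; Updates ignore the event's argument and read the setting, hiding reflections and swapping MirrorMeshes to a fake mirror material when off.
; It unbinds when destroyed.
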(event Custom|OnMirrorsUpdated_Event
  (params (Enabled :type Boolean))
  (bind _asbp_game_instance (Utilities|GameInstance))
  (bind _settings (Variables|/Game/BP_GameInstance.BP_GameInstance_C|GetSettings _asbp_game_instance))
  (bind _mirrors (Default|GetMirrors _settings))
  (for _array_element (Variables|Default|GetReflections)
    (Rendering|SetActorHiddenInGame _array_element (not _mirrors)))
  (for _array_element_2 (Variables|Default|GetMirrorMeshes)
    (Rendering|Material|SetMaterial (Variables|/Script/Engine.StaticMeshActor|GetStaticMeshComponent _array_element_2) 1 (select _mirrors "/Game/Materials/MAT_Mirror.MAT_Mirror" "/Game/Materials/MAT_FakeMirror.MAT_FakeMirror"))))

(event EventBeginPlay
  (Utilities|TickDelay 2)
  (bind _outactors (Actor|GetAllActorsOfClass "/Script/Engine.PlanarReflection"))
  (Variables|Default|SetReflections _outactors)
  (EventDispatchers|AssignOnMirrorsUpdated (Variables|/Game/BP_GameInstance.BP_GameInstance_C|GetSettings (Utilities|GameInstance)) (delegate Custom|OnMirrorsUpdated_Event))
  (CallFunction|OnMirrorsUpdatedEvent false))

(event EventDestroyed
  (EventDispatchers|UnbindEventfromOnMirrorsUpdated (Variables|/Game/BP_GameInstance.BP_GameInstance_C|GetSettings (Utilities|GameInstance)) (delegate Custom|OnMirrorsUpdated_Event)))

(fn ConstructionScript)