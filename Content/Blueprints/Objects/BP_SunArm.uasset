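; BP_SunArm is a sun arm object that glows blue while hovered, extending a parent class that provides the hover functions.
; On hover it saves each static mesh material into MaterialsObject and overrides every slot with MI_GlowBlue.
; On unhover it restores the saved materials by index and clears the array.
; Both functions then call the parent implementation, and the construction script only runs the parent's.
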(fn ConstructionScript
  (|CallParentFunction))

(fn Hovered
  (bind _staticmesh (Variables|Default|GetStaticMesh))
  (for (_array_element _array_index) (Rendering|Material|GetMaterials _staticmesh)
    (Utilities|Array|Add (Variables|Default|GetMaterialsObject) _array_element)
    (Rendering|Material|SetMaterial _staticmesh _array_index "/Game/Materials/Instances/MI_GlowBlue.MI_GlowBlue"))
  (|CallParentFunction))

(fn Unhovered
  (bind _materialsobject (Variables|Default|GetMaterialsObject))
  (for (_array_element _array_index) _materialsobject
    (Rendering|Material|SetMaterial (Variables|Default|GetStaticMesh) _array_index _array_element))
  (Utilities|Array|Clear _materialsobject)
  (|CallParentFunction))