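; BP_ObjectBase is a base world object that, when pickable, shows an interact cursor and can be collected into the inventory.
; The server interact event gives the item by ObjectID, calls the multi interact event and triggers an optional linked Node.
; The multi event plays the pickup sound, notifies BP_SunsPlaceSpotManager for Suns parts, and disables pickup, visibility and collision.
; The authority destroys the actor after a short delay; hover functions are empty stubs.
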(event Custom|Multi_Interact
  (Audio|PlaySoundatLocation (Variables|Default|GetPickupSound) (Transformation|GetActorLocation) "0, 0, 0" 1.0 1.0 0.0 0 0 0 0)
  (if (Variables|Default|GetIsSunsPart)
    (bind _returnvalue (Actor|GetActorOfClass "/Game/Blueprints/BP_SunsPlaceSpotManager.BP_SunsPlaceSpotManager_C"))
    (Default|ServerInteractwithSunsPlaceSpot _returnvalue))
  (Variables|Default|SetCanPickup false)
  (Rendering|SetVisibility (Variables|Default|GetDefaultSceneRoot) false true)
  (Collision|SetActorEnableCollision false)
  (Networking|SwitchHasAuthority
    (:Authority
      (Utilities|FlowControl|Delay 5.0)
      (Actor|DestroyActor))))

(event EventBeginPlay
  (if (Variables|Default|GetCanPickup)
    (Variables|/Game/Blueprints/Components/BP_CustomCursorComponent.BP_CustomCursorComponent_C|SetCursorTexture (Variables|Default|GetBP_CustomCursorComponent) "/Game/Textures/T_CursorInteract.T_CursorInteract")))

(event EventServerInteract
  (params (WhoInteracted :type Actor%20Object%20Reference))
  (bind _node (Variables|Default|GetNode))
  (if (Variables|Default|GetCanPickup)
    (Default|GiveItem (Utilities|Inventory) (Variables|Default|GetObjectID))
    (CallFunction|MultiInteract)
    (Utilities|IsValid _node
      (:Is%20Valid
        (Default|Trigger _node)))))

(fn ConstructionScript)

(fn Hovered)

(fn Unhovered)