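; Achievement manager that records unlocked achievement IDs in an SG_Achievements save game, loaded or created on BeginPlay.
; Single, batch and unlock-all events add new IDs, save, and queue popups; a clear event wipes the saved list.
; UpdatePopup shows UW_AchievementPopup widgets from the end of the queue, re-calling itself after a delay.
; Helpers check unlocks and compute completion percentage against DT_Achievements rows.
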(event Custom|Unlock
  (params (ID :type String))
  (bind _savereference (Variables|Default|GetSaveReference))
  (bind _unlockedids (Variables|/Game/Saves/SG_Achievements.SG_Achievements_C|GetUnlockedIDs _savereference))
  (if (not (Utilities|Array|ContainsItem _unlockedids ID))
    (Utilities|Array|Add _unlockedids ID)
    (Utilities|Array|Add (Variables|Default|GetQueuedPopups) ID)
    (CallFunction|Save)
    (CallFunction|UpdatePopup)))

(event Custom|UnlockMultiple
  (params (IDs :type Array%20of%20Strings))
  (bind _savereference (Variables|Default|GetSaveReference))
  (bind _unlockedids (Variables|/Game/Saves/SG_Achievements.SG_Achievements_C|GetUnlockedIDs _savereference))
  (for _array_element IDs
    (if (not (Utilities|Array|ContainsItem _unlockedids _array_element))
      (Utilities|Array|Add _unlockedids _array_element)
      (Utilities|Array|Add (Variables|Default|GetQueuedPopups) _array_element)))
  (CallFunction|Save)
  (CallFunction|UpdatePopup))

(event Custom|Load
  (bind _returnvalue (SaveGame|DoesSaveGameExist "Achievements"))
  (if _returnvalue
    (bind _returnvalue_2 (SaveGame|LoadGamefromSlot "Achievements"))
    (bind _assg_achievements (Utilities|Casting|CastToSG_Achievements _returnvalue_2))
    (Variables|Default|SetSaveReference _assg_achievements)
    (else
      (bind _returnvalue_3 (SaveGame|CreateSaveGameObject "/Game/Saves/SG_Achievements.SG_Achievements_C"))
      (Variables|Default|SetSaveReference _returnvalue_3))))

(event Custom|Save
  (SaveGame|SaveGametoSlot (Variables|Default|GetSaveReference) "Achievements"))

(event Custom|UpdatePopup
  (bind _queuedpopups (Variables|Default|GetQueuedPopups))
  (bind _returnvalue (Utilities|Array|Length _queuedpopups))
  (bind _returnvalue_2 (- _returnvalue 1))
  (if (not (Utilities|Array|IsEmpty _queuedpopups))
    (bind _returnvalue_3 (UserInterface|CreateWidget "/Game/Widgets/UW_AchievementPopup.UW_AchievementPopup_C" 0 (Utilities|Array|Get(acopy) _queuedpopups _returnvalue_2)))
    (UserInterface|Viewport|AddtoViewport _returnvalue_3 1)
    (Utilities|Array|RemoveIndex _queuedpopups _returnvalue_2)
    (Utilities|FlowControl|Delay 4.0)
    (CallFunction|UpdatePopup)))

(event Custom|UnlockAll
  (bind _outlist (CallFunction|GetListasString))
  (CallFunction|UnlockMultiple _outlist))

(event Custom|ClearAchievements
  (Variables|/Game/Saves/SG_Achievements.SG_Achievements_C|SetUnlockedIDs (Variables|Default|GetSaveReference) (Utilities|Array|MakeArray))
  (CallFunction|Save))

(event EventBeginPlay
  (CallFunction|Load))

(fn ConstructionScript)

(fn GetListasString
  (Utilities|Array|Clear (LocalVariables|GetList))
  (bind _outrownames (DataTable|GetDataTableRowNames "/Game/Achievements/DT_Achievements.DT_Achievements"))
  (for _array_element _outrownames
    (Utilities|Array|Add (LocalVariables|GetList) (Utilities|String|ToString(Name) _array_element)))
  (return (LocalVariables|GetList)))

(fn HasAchievement
  (params (ID :type Name))
  (return (Utilities|Array|ContainsItem (Variables|/Game/Saves/SG_Achievements.SG_Achievements_C|GetUnlockedIDs (Variables|Default|GetSaveReference)) (Utilities|String|ToString(Name) ID))))

(fn GetCompletionPercent
  (bind _outrownames (DataTable|GetDataTableRowNames "/Game/Achievements/DT_Achievements.DT_Achievements"))
  (return (Math|Float|Round (* (/ (Math|Conversions|ToFloat(Integer) (Utilities|Array|Length (Variables|/Game/Saves/SG_Achievements.SG_Achievements_C|GetUnlockedIDs (Variables|Default|GetSaveReference)))) (Math|Conversions|ToFloat(Integer) (Utilities|Array|Length _outrownames))) 1e+02))))