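; BP_TrailerCinematicLauncher is a trailer helper actor that plays a Level Sequence on level start for capturing cinematic footage.
; When enabled, BeginPlay waits a configurable delay, creates an auto-playing, repeatedly looping sequence player that disables player input and hides the HUD, then switches the player's view target to itself.
; It also hides the BP_Player InGame widget after a short tick delay, regardless of the enabled flag.
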(event EventBeginPlay
  (bind _returnvalue (Game|GetPlayerController 0))
  (if (Variables|Default|GetEnabled)
    (Utilities|FlowControl|Delay (Variables|Default|GetDelayBeforeStart))
    (Sequencer|Player|CreateLevelSequencePlayer (Variables|Default|GetLevel%20Sequence) (Utilities|Struct|MakeMovieSceneSequencePlaybackSettings true (Utilities|Struct|MakeMovieSceneSequenceLoopCount 20) "(TickIntervalSeconds=0.000000,EvaluationBudgetMicroseconds=0.000000,bTickWhenPaused=False,bAllowRounding=True)" 1.0 0.0 false true true false true))
    (Game|Player|SetViewTargetwithBlend _returnvalue self 0.0 "VTBlend_Linear" 0.0 false))
  (Utilities|TickDelay 5)
  (bind _asbp_player (Utilities|Casting|CastToBP_Player (Pawn|GetControlledPawn _returnvalue)))
  (Widget|SetVisibility (Variables|/Game/Blueprints/Player/BP_Player.BP_Player_C|GetInGame _asbp_player) "Collapsed"))

(fn ConstructionScript)