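; Director Blueprint for the trailer lockdown Level Sequence, holding event endpoints that script gameplay actors from Sequencer.
; Straight SAS actor events toggle its enabled state, open it or put it into lockdown, and a SAS node event triggers that node.
; Endo chase actor events force a chase or return it to its default state.
; Each event is a direct pass-through call on the actor passed in.
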(event Custom|BP_StraightSAS2_Event
  (params (BP_StraightSAS2 :type BP%20Security%20Door%20Object%20Reference) (IsEnabled :type Boolean))
  (Default|SetEnabled BP_StraightSAS2 IsEnabled))

(event Custom|BP_StraightSAS2_Event_0
  (params (BP_StraightSAS2 :type BP%20Security%20Door%20Object%20Reference))
  (Default|Open BP_StraightSAS2))

(event Custom|BP_EndoChase5_Event
  (params (BP_EndoChase5 :type BP%20Endo%20Chase%20Object%20Reference))
  (Default|DefaultState BP_EndoChase5))

(event Custom|BP_StraightSAS2_Event_1
  (params (BP_StraightSAS2 :type BP%20Security%20Door%20Object%20Reference))
  (Default|Lockdown BP_StraightSAS2))

(event Custom|BP_EndoChase5_Event_0
  (params (BP_EndoChase5 :type BP%20Endo%20Chase%20Object%20Reference))
  (Default|ForceChase BP_EndoChase5))

(event Custom|BP_SasNode13_Event
  (params (BP_SasNode13 :type BP%20Sas%20Node%20Object%20Reference))
  (Default|Trigger BP_SasNode13))

(event Custom|BP_EndoChase5_Event_1
  (params (BP_EndoChase5 :type BP%20Endo%20Chase%20Object%20Reference))
  (Default|DefaultState BP_EndoChase5))