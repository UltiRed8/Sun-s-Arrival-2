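; Triggerable conveyor that carries actors along its arrow's forward direction while running.
; Trigger toggles it on and off through Multi events that set the running state and sound, optionally reversing the arrow on each start.
; Tick offsets actors in ActorsToMove by speed and delta time without sweeping, dropping those being destroyed.
; The construction script flips the arrow when Direction is set.
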(event Custom|Multi_ReverseDirection
  (Transformation|AddRelativeRotation (Variables|Default|GetArrow) "-180.000000,0.000000,0.000000" false false))

(event Custom|Multi_SetRunning
  (params (IsRunning :type Boolean))
  (bind _running (Variables|Default|GetRunning))
  (bind _output_get (Variables|Default|SetIsRunning IsRunning))
  (if _output_get
    (Audio|Components|Audio|Play _running 0.0)
    (else
      (Audio|Components|Audio|Stop _running))))

(event EventTrigger
  (if (Variables|Default|GetIsRunning)
    (CallFunction|MultiSetRunning false)
    (else
      (if (Variables|Default|GetShouldSwitchDirections)
        (CallFunction|MultiReverseDirection))
      (CallFunction|MultiSetRunning true)))
  (|CallParentFunction))

(event EventTick
  (params (DeltaSeconds :type Float%20%28single-precision%29))
  (bind _actorstomove (Variables|Default|GetActorsToMove))
  (if (Variables|Default|GetIsRunning)
    (for _array_element _actorstomove
      (Utilities|IsValid _array_element
        (:Is%20Valid
          (if (Game|IsActorBeingDestroyed _array_element)
            (Utilities|Array|RemoveItem _actorstomove _array_element)
            (else
              (Transformation|AddActorWorldOffset _array_element (* (Math|Vector|GetForwardVector (Variables|Default|GetArrow)) (Variables|Default|GetSpeed) DeltaSeconds)))))))))

(fn ConstructionScript
  (if (Variables|Default|GetDirection)
    (Transformation|AddRelativeRotation (Variables|Default|GetArrow) "-180.000000,0.000000,0.000000" false false)))