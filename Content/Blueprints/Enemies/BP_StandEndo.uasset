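; BP_StandEndo is a standing endoskeleton enemy that, once triggered, stalks the player by vanishing and reappearing behind them.
; Trigger saves a "MasterEndo" checkpoint, which BeginPlay can restore for attacking instances.
; A dot-product poll hides it when the player faces away; random delays follow, lengthened every third cycle.
; Reappearance waits for a living player and a clear sphere trace behind them, then line-traces to the floor and turns toward the player.
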(event Custom|WantToDisappear
  (bind _player (Variables|Default|GetPlayer))
  (if (>= (Math|Vector|DotProduct (Transformation|GetActorForwardVector _player) (Math|Vector|Normalize (- (Transformation|GetActorLocation _player) (Transformation|GetActorLocation)) 0.0)) 0.3)
    (CallFunction|Disappear)
    (bind _result (Math|Integer|IncrementInt (Variables|Default|GetScore))
      (:%20%20
        (if (== _result 3)
          (Variables|Default|SetScore 0)
          (Utilities|FlowControl|Delay 1.2e+02))
        (Utilities|FlowControl|Delay (Math|Random|RandomFloatinRange 3e+01 6e+01))
        (CallFunction|WanttoAppear)))
    (else
      (Utilities|FlowControl|Delay 0.1)
      (CallFunction|WanttoDisappear))))

(event Custom|Disappear
  (Rendering|SetActorHiddenInGame true)
  (Physics|SetSimulatePhysics (Variables|Default|GetCapsule) false)
  (Collision|SetActorEnableCollision false)
  (Variables|Default|SetIsVisible false))

(event Custom|Appear
  (bind _returnvalue (Transformation|GetActorLocation))
  (Components|StaticMesh|SetStaticMesh (Variables|Default|GetStaticMesh) "/Game/Models/Endos/SM_MasterEndoPos3.SM_MasterEndoPos3")
  (Rendering|SetActorHiddenInGame false)
  (Collision|SetActorEnableCollision true)
  (Rendering|Material|SetMaterial (Variables|Default|GetStaticMesh) 6 "/Game/Models/EndoEnemy/MAT_RedGlow.MAT_RedGlow")
  (bind (_outhit _returnvalue_2) (Collision|LineTraceByChannel _returnvalue (+ _returnvalue "0.000000,0.000000,-500.000000") "TraceTypeQuery1" false 0 "None" true "(R=1.000000,G=0.000000,B=0.000000,A=1.000000)" "(R=0.000000,G=1.000000,B=0.000000,A=1.000000)" 1e+01))
  (if _returnvalue_2
    (Transformation|SetActorLocationAndRotation (- (.Location (Collision|BreakHitResult _outhit)) "0.000000,0.000000,8.000000") (Math|Rotator|MakeRotator 0.0 0.0 (+ (.yaw (Math|Rotator|FindLookatRotation _returnvalue (Transformation|GetActorLocation (Variables|Default|GetPlayer)))) -9e+01)))
    (Variables|Default|SetIsVisible true)
    (Utilities|FlowControl|Delay 1e+01)
    (CallFunction|WanttoDisappear)))

(event Custom|WantToAppear
  (bind _player (Variables|Default|GetPlayer))
  (bind _returnvalue (Transformation|GetActorForwardVector _player))
  (bind _returnvalue_2 (Transformation|GetActorLocation _player))
  (bind _returnvalue_3 (* _returnvalue -1e+02))
  (bind _returnvalue_4 (+ _returnvalue_2 _returnvalue_3))
  (if (Variables|/Game/Blueprints/Player/BP_Player.BP_Player_C|GetIsDead _player)
    (Utilities|FlowControl|Delay 15.0)
    (CallFunction|WanttoAppear)
    (else
      (bind _returnvalue_5 (Collision|SphereTraceByChannel _returnvalue_2 _returnvalue_4 6e+01 "TraceTypeQuery1" false 0 "None" true "(R=1.000000,G=0.000000,B=0.000000,A=1.000000)" "(R=0.000000,G=1.000000,B=0.000000,A=1.000000)" 1e+01))
      (if _returnvalue_5
        (Utilities|FlowControl|Delay 0.5)
        (CallFunction|WanttoAppear)
        (else
          (Transformation|SetActorLocation self _returnvalue_4 false true)
          (CallFunction|Appear))))))

(event EventTick
  (params (DeltaSeconds :type Float%20%28single-precision%29))
  (bind _returnvalue (Transformation|GetActorLocation))
  (Variables|Default|GetIsVisible
    (:then
      (bind (_outhit _returnvalue_2) (Collision|LineTraceByChannel (+ _returnvalue "0.000000,0.000000,100.000000") (+ _returnvalue "0.000000,0.000000,-100.000000") "TraceTypeQuery1" false 0 "None" true "(R=1.000000,G=0.000000,B=0.000000,A=1.000000)" "(R=0.000000,G=1.000000,B=0.000000,A=1.000000)" 1e+01))
      (if _returnvalue_2
        (Transformation|SetActorLocation (- (.Location (Collision|BreakHitResult _outhit)) "") false false)))
    (:else)))

(event EventTrigger
  (|CallParentFunction)
  (Utilities|CheckpointSaveBool "MasterEndo" true)
  (Rendering|Material|SetMaterial (Variables|Default|GetStaticMesh) 1 "/Game/Models/EndoEnemy/MAT_RedGlow.MAT_RedGlow")
  (CallFunction|WanttoDisappear))

(event EventBeginPlay
  (bind _asbp_player (Utilities|Casting|CastToBP_Player (Pawn|GetControlledPawn (Game|GetPlayerController 0))))
  (Variables|Default|SetPlayer _asbp_player)
  (if (Variables|Default|GetIsAttacking)
    (bind (_success _bool) (Utilities|CheckpointGetBool "MasterEndo"))
    (if _success
      (if _bool
        (CallFunction|Trigger :!label _label)
        (else
          (if (Variables|Default|GetActiveByDefault) :!label _label_2
            (goto _label))))
      (else
        (goto _label_2)))))

(fn ConstructionScript
  (if (Variables|Default|GetMissingHead)
    (Components|StaticMesh|SetStaticMesh (Variables|Default|GetStaticMesh) "/Game/Models/Endos/SM_MasterEndoPos2.SM_MasterEndoPos2")))