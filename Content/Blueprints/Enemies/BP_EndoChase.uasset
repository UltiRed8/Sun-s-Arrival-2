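; BP_EndoChase is an enemy that patrols, chases seen players and searches after losing them, with server-authoritative state logic in Blueprint.
; Idle alternates with random long-range patrols; PawnSensing starts chases on reachable, visible, living players, enabling door destruction.
; Lost chases fan three search points around the last seen direction before patrolling again, and a looping timer breaks stuck chases.
; A sphere overlap awards a stealth achievement when players get close undetected.
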(event OnComponentBeginOverlap(Sphere1)
  (params (OverlappedComponent :type Primitive%20Component%20Object%20Reference) (OtherActor :type Actor%20Object%20Reference) (OtherComp :type Primitive%20Component%20Object%20Reference) (OtherBodyIndex :type Integer) (bFromSweep :type Boolean) (SweepResult :type Hit%20Result%20Structure%20%28by%20ref%29))
  (bind _asbp_player (Utilities|Casting|CastToBP_Player OtherActor))
  (if (Math|Boolean|ANDBoolean (not (Variables|/Game/Blueprints/Player/BP_Player.BP_Player_C|GetIsDead _asbp_player)) (not (Variables|Default|GetIsChasing)) (Utilities|Array|IsEmpty (Variables|Default|GetSearchPoints)) (not (Variables|/Game/Blueprints/Player/BP_Player.BP_Player_C|GetIsHiding _asbp_player)))
    (Default|UnlockAchievement (Utilities|GameInstance) "ACH_Stealth")))

(event OnSeePawn(PawnSensing)
  (params (Pawn :type Pawn%20Object%20Reference))
  ;[0.15 0.15 0.15 0.5] Chasing
  (if (not (Variables|Default|GetIsWaitingForSAS))
    (Networking|SwitchHasAuthority
      (:Authority
        (if (not (Variables|Default|GetIsScreaming))
          (bind _asbp_player (Utilities|Casting|CastToBP_Player Pawn))
          (if (not (or (Variables|/Game/Blueprints/Player/BP_Player.BP_Player_C|GetIsDead _asbp_player) (Variables|/Game/Blueprints/Player/BP_Player.BP_Player_C|GetIsHiding _asbp_player)))
            (bind _returnvalue (CallFunction|IsReacheable (Transformation|GetActorLocation _asbp_player)))
            (if _returnvalue
              (Variables|Default|SetCanDestroyDoors true)
              (CallFunction|SetupDebug "(R=1.000000,G=0.000000,B=0.000000,A=1.000000)")
              (CallFunction|MultiUpdateValues 7e+02 true)
              (Utilities|IsValid (Variables|Default|GetMapDeviceTarget)
                (:Is%20Valid
                  _)
                (:Is%20Not%20Valid
                  (CallFunction|PlayAmbientSound)))
              (CallFunction|SetTarget _asbp_player)
              (bind _output_get (Variables|Default|SetLastKnownPlayerLocation (Transformation|GetActorLocation _asbp_player)))
              (Variables|Default|SetLastKnownPlayerDirection (Math|Rotator|FindLookatRotation (Transformation|GetActorLocation) (Transformation|GetActorLocation _asbp_player)))
              (bind _output_get_2 (Variables|Default|SetDestination _output_get))
              (bind _movementresult (AI|AIMoveTo self _output_get_2 0 5.0 false)
                (:OnSuccess
                  _)
                (:OnFail
                  _))
              (switch Utilities|FlowControl|Switch|SwitchonEPathFollowingResult _movementresult
                (:Success
                  _)
                (:Blocked
                  _)
                (:OffPath
                  _))
              (CallFunction|MultiUpdateValues 7e+02 false)
              (CallFunction|PrepareLookforLostPlayer))))))))

(event Custom|Patrol
  ;[0.15 0.15 0.15 0.5] Patrol
  (if (not (Variables|Default|GetIsWaitingForSAS))
    (Networking|SwitchHasAuthority
      (:Authority
        (Utilities|CanChangeState
          (:true
            (CallFunction|SetupDebug "(R=1.000000,G=1.000000,B=0.000000,A=1.000000)")
            (CallFunction|PlayAmbientSound)
            (CallFunction|MultiUpdateValues 4e+02 false)
            (bind _randomlocation (CallFunction|GetReachableLocation 10 2e+03 1e+04))
            (bind _output_get (Variables|Default|SetDestination _randomlocation))
            (AI|AIMoveTo self _output_get 0 5.0 false
              (:OnSuccess
                _)
              (:OnFail
                _))
            (CallFunction|Idle)))))))

(event Custom|Idle
  ;[0.15 0.15 0.15 0.5] Idle
  (if (not (Variables|Default|GetIsWaitingForSAS))
    (Networking|SwitchHasAuthority
      (:Authority
        (Utilities|CanChangeState
          (:true
            (CallFunction|SetTarget)
            (Variables|Default|SetCanDestroyDoors false)
            (CallFunction|SetupDebug "(R=0.000000,G=1.000000,B=0.000000,A=1.000000)")
            (CallFunction|StopAmbientSound)
            (CallFunction|MultiAmbientSound true)
            (Utilities|FlowControl|Delay 6.34)
            (CallFunction|MultiAmbientSound false)
            (if (Variables|Default|GetCanPatrol)
              (CallFunction|Patrol))))))))

(event Custom|LookForLostPlayer
  (bind _returnvalue (Transformation|GetActorForwardVector))
  (bind _searchpoints (Variables|Default|GetSearchPoints))
  (bind _searchpoints_2 (Variables|Default|GetSearchPoints))
  (bind _output (Utilities|Array|Get(acopy) _searchpoints))
  (bind _output_2 (Utilities|Array|Get(acopy) _searchpoints_2))
  (bind _returnvalue_2 (* _returnvalue -1e+02))
  (bind _returnvalue_3 (+ _output _returnvalue_2))
  ;[0.15 0.15 0.15 0.5] Look for lost player
  (if (not (Variables|Default|GetIsWaitingForSAS))
    (Networking|SwitchHasAuthority
      (:Authority
        (Utilities|CanChangeState
          (:true
            (if (Utilities|Array|IsEmpty (Variables|Default|GetSearchPoints))
              (CallFunction|Patrol)
              (else
                (CallFunction|SetupDebug "(R=0.000000,G=1.000000,B=1.000000,A=1.000000)")
                (CallFunction|PlayAmbientSound)
                (CallFunction|SetTarget)
                (bind _returnvalue_4 (CallFunction|IsReacheable _output_2))
                (if _returnvalue_4
                  (AI|AIMoveTo self _output_2 0 5.0 false
                    (:OnSuccess
                      _)
                    (:OnFail
                      _))
                  (Utilities|FlowControl|Delay 0.25))
                (if (not (Variables|Default|GetIsChasing))
                  (bind _returnvalue_5 (CallFunction|IsReacheable _returnvalue_3))
                  (if _returnvalue_5
                    (AI|AIMoveTo self _returnvalue_3 0 5.0 false
                      (:OnSuccess
                        _)
                      (:OnFail
                        _))
                    (Utilities|FlowControl|Delay 0.25))
                  (if (not (Variables|Default|GetIsChasing))
                    (Utilities|Array|RemoveIndex (Variables|Default|GetSearchPoints))
                    (CallFunction|LookforLostPlayer)))))))))))

(event Custom|PrepareLookForLostPlayer
  (bind _searchpoints (Variables|Default|GetSearchPoints))
  (bind _lastknownplayerlocation (Variables|Default|GetLastKnownPlayerLocation))
  (bind _lastknownplayerdirection (Variables|Default|GetLastKnownPlayerDirection))
  (bind _returnvalue (Math|Rotator|GetRotationXVector _lastknownplayerdirection))
  (bind _returnvalue_2 (* _returnvalue 1e+03))
  ;[0.15 0.15 0.15 0.5] Look for lost player
  (if (not (Variables|Default|GetIsWaitingForSAS))
    (Networking|SwitchHasAuthority
      (:Authority
        (Utilities|CanChangeState
          (:true
            (CallFunction|SetupDebug "(R=0.000000,G=0.000000,B=1.000000,A=1.000000)")
            (CallFunction|PlayAmbientSound)
            (CallFunction|SetTarget)
            (Utilities|Array|Clear (Variables|Default|GetSearchPoints))
            (Utilities|Array|Add _searchpoints (+ _lastknownplayerlocation _returnvalue_2))
            (Utilities|Array|Add _searchpoints (+ _lastknownplayerlocation (Math|Vector|RotateVector _returnvalue_2 "0.000000,45.000000,0.000000")))
            (Utilities|Array|Add _searchpoints (+ _lastknownplayerlocation (Math|Vector|RotateVector _returnvalue_2 "0.000000,-45.000000,0.000000")))
            (CallFunction|LookforLostPlayer)))))))

(event Custom|Multi_UpdateValues
  (params (Max%20Walk%20Speed :type Float%20%28single-precision%29) (IsChasing :type Boolean))
  (Variables|/Script/Engine.CharacterMovementComponent|SetMaxWalkSpeed (Variables|Character|GetCharacterMovement) (* Max%20Walk%20Speed (Math|Float|SelectFloat 1.5 (Variables|Default|GetNormalSpeedMultiplier) (Variables|Default|GetIsHardcore))))
  (Variables|Default|SetIsChasing IsChasing))

(event Custom|Multi_AmbientSound
  (params (Enabled :type Boolean))
  (bind _ambient (Variables|Default|GetAmbient))
  (if Enabled
    (Audio|Components|Audio|Play _ambient 0.0)
    (else
      (Audio|Components|Audio|Stop _ambient))))

(event Custom|Unstuck
  (if (not (Variables|Default|GetIsWaitingForSAS))
    (if (and (Variables|Default|GetIsChasing) (not (Variables|Default|GetIsScreaming)))
      (if (<= (Math|Vector|Distance(Vector) (Transformation|GetActorLocation) (Variables|Default|GetLastAILocation)) 5e+01)
        (bind _result (Math|Integer|DecrementInt (Variables|Default|GetTimedStuck))
          (:%20%20
            (if (<= _result 0)
              (Variables|Default|SetIsChasing false)
              (CallFunction|PrepareLookforLostPlayer)))))
      (else
        (Variables|Default|SetTimedStuck 2)))
    (Variables|Default|SetLastAILocation (Transformation|GetActorLocation))))

(event EventBeginPlay
  (|CallParentFunction)
  (Networking|SwitchHasAuthority
    (:Authority
      (Utilities|Time|SetTimerbyEvent (delegate Custom|Unstuck) 1.0 true)
      (if (Variables|Default|GetIsActiveByDefault)
        (CallFunction|DefaultState)))))

(event EventDefaultState
  (|CallParentFunction)
  (CallFunction|Idle)
  (Class|PawnSensingComponent|SetSensingUpdatesEnabled (Variables|Default|GetPawnSensing) true))

(fn ConstructionScript)

(fn GetReachableLocation
  (params (Tries :type Integer) (MinDistance :type Float%20%28double-precision%29) (MaxDistance :type Float%20%28double-precision%29))
  (bind _returnvalue (Transformation|GetActorLocation))
  (bind _output_get (LocalVariables|SetCurrentTries Tries))
  (bind _output_get_2 (LocalVariables|SetNewLocalVar (.RandomLocation (AI|Navigation|GetRandomReachablePointinRadius _returnvalue MaxDistance 0 0)) :!label _label))
  (if (< (Math|Vector|Distance(Vector) _output_get_2 _returnvalue) MinDistance)
    (bind _result (Math|Integer|DecrementInt _output_get)
      (:%20%20
        (if (<= _result 0)
          _
          (else
            (goto _label)))))
    (else
      (Variables|Default|SetDestination _output_get_2)))
  (return _output_get_2))