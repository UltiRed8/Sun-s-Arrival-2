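; BP_EndoSight is an endoskeleton enemy that chases players but freezes in place, animation included, while any player is looking at it.
; A looping timer targets the nearest living, unhidden player with a complete nav path, then checks each player's sight to toggle movement.
; Unseen, it can kill and pursues via AI MoveTo, faster in Hardcore.
; CheckForWall traces from a player's camera to several bones to test whether walls block the view.
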(event Custom|ChaseNearestPlayer
  (Variables|Default|GetIsActive
    (:then
      (Variables|Default|GetIsScreaming
        (:then)
        (:else
          (Variables|Default|GetCanKill
            (:then
              (bind _targetplayer (Variables|Default|GetTargetPlayer)
                (:then
                  (CallFunction|SetupDebug "(R=1.000000,G=0.000000,B=0.000000,A=1.000000)")
                  (Variables|Default|SetDestination (Transformation|GetActorLocation _targetplayer))
                  (AI|AIMoveTo self "0, 0, 0" _targetplayer 5.0 false
                    (:OnSuccess
                      _)
                    (:OnFail
                      _))
                  (CallFunction|ChaseNearestPlayer))
                (:else)))
            (:else)))))
    (:else)))

(event Custom|UpdateTarget
  (if (Variables|Default|GetIsActive)
    (bind _outclosestplayer (CallFunction|GetNearestPlayer))
    (Utilities|IsValid _outclosestplayer
      (:Is%20Valid
        (if (!= (Variables|Default|GetTargetPlayer) _outclosestplayer)
          (Variables|Default|SetTargetPlayer _outclosestplayer)
          (CallFunction|ChaseNearestPlayer)))
      (:Is%20Not%20Valid
        (Variables|Default|GetTargetPlayer
          (:then
            (Variables|Default|SetTargetPlayer 0)
            (CallFunction|SetupDebug "(R=0.000000,G=1.000000,B=0.000000,A=1.000000)"))
          (:else))))))

(event Custom|GlobalUpdate
  ;[0.15 0.15 0.15 0.5] TickUpdate
  (CallFunction|UpdateTarget)
  (CallFunction|UpdateTick))

(event Custom|UpdateTick
  ;[0.15 0.15 0.15 0.5] UpdateMovement
  (if (Variables|Default|GetIsActive)
    (Variables|Default|GetIsScreaming
      (:then)
      (:else
        (Variables|Default|SetCanMove true)
        (bind _array_element (Utilities|Array|ForEachLoopwithBreak (Variables|Default|GetAllPlayers) :!label _label)
          (:LoopBody
            (bind _returnvalue (Default|CheckIsSeeingSightEndo _array_element self))
            (if _returnvalue
              (Utilities|FlowControl|Sequence
                (:then_0
                  (Variables|Default|SetCanMove false))
                (:then_1
                  (goto _label Break)))))
          (:Completed
            (if (and (Variables|Default|GetCanMove) (Utilities|IsValid (Variables|Default|GetTargetPlayer)))
              (goto _label_2 InB)
              (else
                (Utilities|OnceGate :!label _label_2
                  (:OutA
                    (CallFunction|StopWalk)
                    (CallFunction|SetupDebug "(R=1.000000,G=1.000000,B=0.000000,A=1.000000)"))
                  (:OutB
                    (CallFunction|StartWalk)
                    (CallFunction|SetupDebug "(R=1.000000,G=0.000000,B=0.000000,A=1.000000)")))))))))))

(event Custom|Multi_StopAnim
  ;[0.15 0.15 0.15 0.5] Movement Anims
  (Audio|Components|Audio|Stop (Variables|Character|GetMesh)))

(event Custom|Multi_StartAnim
  ;[0.15 0.15 0.15 0.5] Movement Anims
  (Audio|Components|Audio|Play (Variables|Character|GetMesh) true))

(event Custom|StopWalk
  ;[0.15 0.15 0.15 0.5] Movement Setters
  (Variables|Default|SetCanKill false)
  (Variables|/Script/Engine.CharacterMovementComponent|SetMaxWalkSpeed (Variables|Character|GetCharacterMovement) 0.0)
  (AI|AIMoveTo self (Transformation|GetActorLocation) 0 5.0 false
    (:then
      (CallFunction|MultiStopAnim))))

(event Custom|StartWalk
  ;[0.15 0.15 0.15 0.5] Movement Setters
  (Variables|Default|SetCanKill true)
  (Variables|/Script/Engine.CharacterMovementComponent|SetMaxWalkSpeed (Variables|Character|GetCharacterMovement) (Math|Float|SelectFloat 3.6e+03 1.2e+03 (Variables|Default|GetIsHardcore)))
  (CallFunction|ChaseNearestPlayer)
  (CallFunction|MultiStartAnim)
  (CallFunction|CheckOverlaps))

(event EventDefaultState
  ;[0.15 0.15 0.15 0.5] DefaultState
  (for _array_element (Utilities|Array|MakeArray "bip_upperArm_L")
    (Components|SkinnedMesh|HideBonebyName (Variables|Character|GetMesh) _array_element "PBO_None"))
  (|CallParentFunction)
  (bind _outactors (Actor|GetAllActorsOfClass "/Game/Blueprints/Player/BP_Player.BP_Player_C"))
  (Variables|Default|SetAllPlayers _outactors)
  (Variables|Default|SetIsActive true))

(event EventScreamerStart
  ;[0.15 0.15 0.15 0.5] ScreamerAnim
  (Components|Animation|PlayAnimation (Variables|Character|GetMesh) "/Game/Animations/Endo/AS_Scream.AS_Scream" false))

(event EventScreamerEnd
  ;[0.15 0.15 0.15 0.5] ScreamerAnim
  (Components|Animation|SetAnimation (Variables|Character|GetMesh) "/Game/Animations/Endo/AS_Running.AS_Running"))

(event EventBeginPlay
  ;[0.15 0.15 0.15 0.5] BeginPlay
  (|CallParentFunction)
  (Utilities|Time|SetTimerbyEvent (delegate Custom|GlobalUpdate) 0.1 true)
  (Utilities|FlowControl|Sequence
    (:then_0
      (CallFunction|StopWalk))
    (:then_1
      (CallFunction|MultiStopAnim))))

(fn ConstructionScript)

(fn GetNearestPlayer
  (LocalVariables|SetClosestDistance 999999.0)
  (LocalVariables|SetClosestPlayer 0)
  (for _array_element (Variables|Default|GetAllPlayers)
    (if (not (Variables|/Game/Blueprints/Player/BP_Player.BP_Player_C|GetIsDead _array_element))
      (if (not (Variables|/Game/Blueprints/Player/BP_Player.BP_Player_C|GetIsHiding _array_element))
        (bind _returnvalue (Class|NavigationSystemV1|FindPathtoLocationSynchronously (Transformation|GetActorLocation) (Transformation|GetActorLocation _array_element) 0 0))
        (if (and (not (Class|NavigationPath|IsPartial _returnvalue)) (> (Utilities|Array|Length (Variables|/Script/NavigationSystem.NavigationPath|GetPathPoints _returnvalue)) 0))
          (if (< (Math|Vector|Distance(Vector) (Transformation|GetActorLocation _array_element) (Transformation|GetActorLocation)) (LocalVariables|GetClosestDistance))
            (LocalVariables|SetClosestDistance (Math|Vector|Distance(Vector) (Transformation|GetActorLocation _array_element) (Transformation|GetActorLocation)))
            (LocalVariables|SetClosestPlayer _array_element))))))
  (return (LocalVariables|GetClosestPlayer)))

(fn CheckforWall
  (params (Controller :type Controller%20Object%20Reference))
  (bind _asbp_player (Utilities|Casting|CastToBP_Player (Pawn|GetControlledPawn Controller)))
  (Utilities|FlowControl|Sequence
    (:then_0
      (goto _label_2 Open))
    (:then_1
      (bind _array_element (Utilities|Array|ForEachLoopwithBreak (Utilities|Array|MakeArray "bip_hand_L" "bip_hand_R" "bip_head" "bip_foot_L" "bip_foot_R") :!label _label)
        (:LoopBody
          (bind _returnvalue (Collision|LineTraceByChannel (Transformation|GetWorldLocation (select (Variables|/Game/Blueprints/Player/BP_Player.BP_Player_C|GetIsThirdPerson _asbp_player) (Variables|/Game/Blueprints/Player/BP_Player.BP_Player_C|GetThirdPersonCam _asbp_player) (Variables|/Game/Blueprints/Player/BP_Player.BP_Player_C|GetFirstPersonCam _asbp_player))) (Transformation|GetSocketLocation (Variables|Character|GetMesh) _array_element) "TraceTypeQuery1" false 0 "ForOneFrame"))
          (if (not _returnvalue)
            (Utilities|FlowControl|Sequence
              (:then_0
                (goto _label Break))
              (:then_1
                (goto _label_2 Close))
              (:then_2
                (return true)))))
        (:Completed
          (Utilities|FlowControl|Gate false :!label _label_2
            (:Exit
              (return false))))))))