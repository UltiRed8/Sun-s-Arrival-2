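; Endo enemy that patrols, chases sighted players and kills them on touch with a scream montage.
; Server-run event chains move between patrol, idle, chase and search using AIMoveTo and PawnSensing, gated by CanChangeState, with multicasts for speed, sound and animation.
; A lost player triggers a search of three points fanned around the last seen direction.
; A timer breaks stuck chases; touched closed, unlocked doors are opened, or smashed while chasing.
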(event OnComponentBeginOverlap(CapsuleComponent)
  (params (OverlappedComponent :type Primitive%20Component%20Object%20Reference) (OtherActor :type Actor%20Object%20Reference) (OtherComp :type Primitive%20Component%20Object%20Reference) (OtherBodyIndex :type Integer) (bFromSweep :type Boolean) (SweepResult :type Hit%20Result%20Structure%20%28by%20ref%29))
  ;[0.15 0.15 0.15 0.5] Interactions
  (Networking|SwitchHasAuthority
    (:Authority
      (bind _asbp_player (Utilities|Casting|CastToBP_Player OtherActor)
        (:then
          (if (not (or (Variables|/Game/Blueprints/Player/BP_Player.BP_Player_C|GetIsDead _asbp_player) (Variables|/Game/Blueprints/Player/BP_Player.BP_Player_C|GetIsHiding _asbp_player)))
            (if (not (Variables|Default|GetIsScreaming))
              (Variables|Default|SetIsScreaming true)
              (Default|ServerDeath _asbp_player self)
              (CallFunction|MultiScreamAnimation))))
        (:CastFailed
          (bind _asbp_classic_openable_door (Utilities|Casting|CastToBP_ClassicOpenableDoor OtherActor))
          (if (Math|Boolean|ANDBoolean (not (Variables|/Game/Blueprints/Doors/BP_DoorBase.BP_DoorBase_C|GetIsOpen _asbp_classic_openable_door)) (Variables|/Game/Blueprints/Doors/BP_DoorBase.BP_DoorBase_C|GetCanBeToggledByPlayer _asbp_classic_openable_door) (not (Variables|/Game/Blueprints/Doors/BP_DoorBase.BP_DoorBase_C|GetIsLocked _asbp_classic_openable_door)))
            (if (Variables|Default|GetIsChasing)
              (Default|MultiAIDestroy _asbp_classic_openable_door (Transformation|GetActorForwardVector))
              (else
                (Default|ServerToggleDoor _asbp_classic_openable_door)))))))))

(event OnSeePawn(PawnSensing)
  (params (Pawn :type Pawn%20Object%20Reference))
  ;[0.15 0.15 0.15 0.5] Chasing
  (Networking|SwitchHasAuthority
    (:Authority
      (if (not (Variables|Default|GetIsScreaming))
        (bind _asbp_player (Utilities|Casting|CastToBP_Player Pawn))
        (if (not (or (Variables|/Game/Blueprints/Player/BP_Player.BP_Player_C|GetIsDead _asbp_player) (Variables|/Game/Blueprints/Player/BP_Player.BP_Player_C|GetIsHiding _asbp_player)))
          (CallFunction|SetupDebug "(R=1.000000,G=0.000000,B=0.000000,A=1.000000)")
          (CallFunction|MultiUpdateValues 7e+02 true)
          (bind _output_get (Variables|Default|SetLastKnownPlayerLocation (Transformation|GetActorLocation _asbp_player)))
          (Variables|Default|SetLastKnownPlayerDirection (Math|Rotator|FindLookatRotation (Transformation|GetActorLocation) (Transformation|GetActorLocation _asbp_player)))
          (bind _movementresult (AI|AIMoveTo self _output_get 0 5.0 false)
            (:OnSuccess
              _)
            (:OnFail
              _))
          (switch Utilities|FlowControl|Switch|SwitchonEPathFollowingResult _movementresult
            (:Success
              _)
            (:Blocked
              _)
            (:OffPath
              _))
          (CallFunction|MultiUpdateValues 7e+02 false)
          (CallFunction|PrepareLookforLostPlayer))))))

(event Custom|Multi_ScreamAnimation
  ;[0.15 0.15 0.15 0.5] Interactions
  (bind _returnvalue (Animation|PlayAnimMontage "/Game/Animations/Endo/AM_Scream.AM_Scream" 1.0 "None"))
  (Networking|SwitchHasAuthority
    (:Authority
      (Utilities|FlowControl|Delay _returnvalue)
      (Variables|Default|SetIsScreaming false)
      (CallFunction|Patrol))))

(event Custom|Patrol
  ;[0.15 0.15 0.15 0.5] Patrol
  (Networking|SwitchHasAuthority
    (:Authority
      (Utilities|CanChangeState
        (:true
          (CallFunction|SetupDebug "(R=1.000000,G=1.000000,B=0.000000,A=1.000000)")
          (CallFunction|MultiUpdateValues 4e+02 false)
          (bind _randomlocation (CallFunction|GetReachableLocation 10 2e+03 1e+04))
          (AI|AIMoveTo self _randomlocation 0 5.0 false
            (:OnSuccess
              _)
            (:OnFail
              _))
          (CallFunction|Idle))))))

(event Custom|SetupDebug
  (params (Value :type Linear%20Color%20Structure))
  ;[0.15 0.15 0.15 0.5] Debugs
)

(event Custom|Idle
  ;[0.15 0.15 0.15 0.5] Idle
  (Networking|SwitchHasAuthority
    (:Authority
      (Utilities|CanChangeState
        (:true
          (CallFunction|SetupDebug "(R=0.000000,G=1.000000,B=0.000000,A=1.000000)")
          (CallFunction|MultiAmbientSound true)
          (Utilities|FlowControl|Delay 6.34)
          (CallFunction|MultiAmbientSound false)
          (CallFunction|Patrol))))))

(event Custom|LookForLostPlayer
  ;[0.15 0.15 0.15 0.5] Look for lost player
  (Networking|SwitchHasAuthority
    (:Authority
      (Utilities|CanChangeState
        (:true
          (if (Utilities|Array|IsEmpty (Variables|Default|GetSearchPoints))
            (CallFunction|Patrol)
            (else
              (CallFunction|SetupDebug "(R=0.000000,G=1.000000,B=1.000000,A=1.000000)")
              (AI|AIMoveTo self (Utilities|Array|Get(acopy) (Variables|Default|GetSearchPoints)) 0 5.0 false
                (:OnSuccess
                  _)
                (:OnFail
                  _))
              (Utilities|FlowControl|Delay 0.25)
              (if (not (Variables|Default|GetIsChasing))
                (AI|AIMoveTo self (+ (Utilities|Array|Get(acopy) (Variables|Default|GetSearchPoints)) (* (Transformation|GetActorForwardVector) -1e+02)) 0 5.0 false
                  (:OnSuccess
                    _)
                  (:OnFail
                    _))
                (Utilities|FlowControl|Delay 0.25)
                (if (not (Variables|Default|GetIsChasing))
                  (Utilities|Array|RemoveIndex (Variables|Default|GetSearchPoints))
                  (CallFunction|LookforLostPlayer))))))))))

(event Custom|PrepareLookForLostPlayer
  (bind _searchpoints (Variables|Default|GetSearchPoints))
  (bind _lastknownplayerlocation (Variables|Default|GetLastKnownPlayerLocation))
  (bind _lastknownplayerdirection (Variables|Default|GetLastKnownPlayerDirection))
  (bind _returnvalue (Math|Rotator|GetRotationXVector _lastknownplayerdirection))
  (bind _returnvalue_2 (* _returnvalue 1e+03))
  ;[0.15 0.15 0.15 0.5] Look for lost player
  (Networking|SwitchHasAuthority
    (:Authority
      (Utilities|CanChangeState
        (:true
          (CallFunction|SetupDebug "(R=0.000000,G=0.000000,B=1.000000,A=1.000000)")
          (Utilities|Array|Clear (Variables|Default|GetSearchPoints))
          (Utilities|Array|Add _searchpoints (+ _lastknownplayerlocation _returnvalue_2))
          (Utilities|Array|Add _searchpoints (+ _lastknownplayerlocation (Math|Vector|RotateVector _returnvalue_2 "0.000000,45.000000,0.000000")))
          (Utilities|Array|Add _searchpoints (+ _lastknownplayerlocation (Math|Vector|RotateVector _returnvalue_2 "0.000000,-45.000000,0.000000")))
          (CallFunction|LookforLostPlayer))))))

(event Custom|Multi_UpdateValues
  (params (Max%20Walk%20Speed :type Float%20%28single-precision%29) (IsChasing :type Boolean))
  (Variables|/Script/Engine.CharacterMovementComponent|SetMaxWalkSpeed (Variables|Character|GetCharacterMovement) Max%20Walk%20Speed)
  (Variables|Default|SetIsChasing IsChasing))

(event Custom|Multi_AmbientSound
  (params (Enabled :type Boolean))
  (bind _ambient (Variables|Default|GetAmbient))
  (if Enabled
    (Audio|Components|Audio|Play _ambient 0.0)
    (else
      (Audio|Components|Audio|Stop _ambient))))

(event Custom|Unstuck
  (if (and (Variables|Default|GetIsChasing) (not (Variables|Default|GetIsScreaming)))
    (if (<= (Math|Vector|Distance(Vector) (Transformation|GetActorLocation) (Variables|Default|GetLastAILocation)) 5e+01)
      (bind _result (Math|Integer|DecrementInt (Variables|Default|GetTimedStuck))
        (:%20%20
          (if (<= _result 0)
            (Variables|Default|SetIsChasing false)
            (CallFunction|PrepareLookforLostPlayer)))))
    (else
      (Variables|Default|SetTimedStuck 2)))
  (Variables|Default|SetLastAILocation (Transformation|GetActorLocation)))

(event EventBeginPlay
  (Networking|SwitchHasAuthority
    (:Authority
      (Utilities|Time|SetTimerbyEvent (delegate Custom|Unstuck) 1.0 true))))

(fn ConstructionScript)

(fn GetReachableLocation
  (params (Tries :type Integer) (MinDistance :type Float%20%28double-precision%29) (MaxDistance :type Float%20%28double-precision%29))
  (bind _returnvalue (Transformation|GetActorLocation))
  (bind _output_get (LocalVariables|SetCurrentTries Tries))
  (bind _output_get_2 (LocalVariables|SetNewLocalVar (.RandomLocation (AI|Navigation|GetRandomReachablePointinRadius _returnvalue MaxDistance 0 0)) :!label _label))
  (if (< (Math|Vector|Distance(Vector) _output_get_2 _returnvalue) MinDistance)
    (bind _result (Math|Integer|DecrementInt _output_get)
      (:%20%20
        (if (<= _result 0)
          _
          (else
            (goto _label))))))
  (return _output_get_2))