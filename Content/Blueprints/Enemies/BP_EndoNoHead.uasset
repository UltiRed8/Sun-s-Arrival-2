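; Headless Endo enemy variant that hides its neck bone and roams randomly, extending parent default-state and reset logic.
; Entering the default state enables pawn sensing and starts a server-side patrol loop, gated on not chasing or screaming.
; Each leg retries random reachable points for a minimum distance, then re-patrols whether the move succeeds or fails.
; A Multi update sets walk speed, boosted in hardcore mode, and chase state.
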(event Custom|Patrol
  ;[0.15 0.15 0.15 0.5] Patrol
  (Networking|SwitchHasAuthority
    (:Authority
      (Utilities|CanChangeState
        (:true
          (CallFunction|SetupDebug "(R=1.000000,G=1.000000,B=0.000000,A=1.000000)")
          (CallFunction|PlayAmbientSound)
          (CallFunction|MultiUpdateValues 7e+02 false)
          (bind _randomlocation (CallFunction|GetReachableLocation 10 2e+02 8e+02))
          (Variables|Default|SetDestination _randomlocation)
          (AI|AIMoveTo self _randomlocation 0 5.0 false
            (:OnSuccess
              _)
            (:OnFail
              _))
          (CallFunction|Patrol))))))

(event Custom|Multi_UpdateValues
  (params (Max%20Walk%20Speed :type Float%20%28single-precision%29) (IsChasing :type Boolean))
  (Variables|/Script/Engine.CharacterMovementComponent|SetMaxWalkSpeed (Variables|Character|GetCharacterMovement) (* Max%20Walk%20Speed (Math|Float|SelectFloat 1.5 1.0 (Variables|Default|GetIsHardcore))))
  (Variables|Default|SetIsChasing IsChasing))

(event EventReset
  ;[0.15 0.15 0.15 0.5] Reset
  (Variables|Default|SetIsChasing false)
  (Utilities|Array|Clear (Variables|Default|GetSearchPoints))
  (|CallParentFunction))

(event EventDefaultState
  (Components|SkinnedMesh|HideBonebyName (Variables|Character|GetMesh) "bip_neck" "PBO_None")
  (|CallParentFunction)
  (CallFunction|Patrol)
  (Class|PawnSensingComponent|SetSensingUpdatesEnabled (Variables|Default|GetPawnSensing) true))

(fn ConstructionScript)

(fn GetReachableLocation
  (params (Tries :type Integer) (MinDistance :type Float%20%28double-precision%29) (MaxDistance :type Float%20%28double-precision%29))
  (bind _returnvalue (Transformation|GetActorLocation))
  (bind _output_get (LocalVariables|SetCurrentTries Tries))
  (bind _output_get_2 (LocalVariables|SetNewLocalVar (.RandomLocation (AI|Navigation|GetRandomReachablePointinRadius _returnvalue MaxDistance 0 0)) :!label _label))
  (if (< (Math|Vector|Distance(Vector) _output_get_2 _returnvalue) MinDistance)
    (bind _result (Math|Integer|DecrementInt _output_get)
      (:%20%20
        (if (<= _result 0)
          _
          (else
            (goto _label)))))
    (else
      (Variables|Default|SetDestination _output_get_2)))
  (return _output_get_2))