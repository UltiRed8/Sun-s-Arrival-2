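; EndoBlock enemy with a fixed-arm PoseableMesh whose head tracks the player pawn every Tick, twitching harder as the player nears.
; Screamer events swap to the regular Mesh during the scare and back afterwards.
; Teleported saves rounded location and rotation as "A"-delimited checkpoint strings, which BeginPlay parses to restore the transform.
; GetReachableLocation retries random reachable points for a minimum distance, returning the last one when tries run out.
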(event Custom|Teleported
  (params (InVec :type Vector) (Rotation :type Rotator))
  (bind _returnvalue (Transformation|GetActorLocation))
  (bind _returnvalue_2 (Transformation|GetActorRotation))
  (bind _saveid (Variables|Default|GetSaveID))
  (bind (_x _y _z) (Math|Vector|BreakVector _returnvalue))
  (bind (_roll _pitch _yaw) (Math|Rotator|BreakRotator _returnvalue_2))
  (Utilities|CheckpointSaveString _saveid (Utilities|String|Append (Utilities|String|ToString(Integer) (Math|Float|Round _x)) "A" (Utilities|String|ToString(Integer) (Math|Float|Round _y)) "A" (Utilities|String|ToString(Integer) (Math|Float|Round _z))))
  (Utilities|CheckpointSaveString (Utilities|String|Append _saveid "_rotation") (Utilities|String|Append (Utilities|String|ToString(Integer) (Math|Float|Round _roll)) "A" (Utilities|String|ToString(Integer) (Math|Float|Round _pitch)) "A" (Utilities|String|ToString(Integer) (Math|Float|Round _yaw)))))

(event EventResettoDefaultPosition)

(event EventTick
  (params (DeltaSeconds :type Float%20%28single-precision%29))
  (bind _returnvalue (Transformation|GetActorLocation))
  (bind _returnvalue_2 (Game|GetPlayerController 0))
  (bind _poseablemesh (Variables|Default|GetPoseableMesh))
  (bind _returnvalue_3 (Pawn|GetControlledPawn _returnvalue_2))
  (bind _returnvalue_4 (Transformation|GetActorLocation _returnvalue_3))
  (bind _returnvalue_5 (+ _returnvalue_4 "0.000000,0.000000,90.000000"))
  (bind _returnvalue_6 (Math|Vector|Distance(Vector) _returnvalue _returnvalue_5))
  (bind _returnvalue_7 (Math|Float|Clamp(Float) _returnvalue_6 0.0 1e+03))
  (bind _returnvalue_8 (- 1e+03 _returnvalue_7))
  (bind _returnvalue_9 (Math|Float|Absolute(Float) _returnvalue_8))
  (bind _returnvalue_10 (/ _returnvalue_9 1e+03))
  (bind _returnvalue_11 (* _returnvalue_10 1e+01))
  (bind _returnvalue_12 (* _returnvalue_11 -1.0))
  (bind _returnvalue_13 (Class|PoseableMeshComponent|GetBoneLocationbyName _poseablemesh "bip_head" "WorldSpace"))
  (Utilities|IsValid _returnvalue_3
    (:Is%20Valid
      (Components|PoseableMesh|SetBoneRotationbyName _poseablemesh "bip_head" (Math|Rotator|CombineRotators (Math|Rotator|CombineRotators (Math|Rotator|MakeRotator 9e+01 0.0 -9e+01) (Math|Rotator|MakeRotator 1e+01 (.pitch (Math|Rotator|FindLookatRotation _returnvalue_13 _returnvalue_5)) (.yaw (Math|Rotator|FindLookatRotation _returnvalue_13 _returnvalue_5)))) (Math|Rotator|MakeRotator (Math|Random|RandomFloatinRange _returnvalue_12 _returnvalue_11) (Math|Random|RandomFloatinRange _returnvalue_12 _returnvalue_11) (Math|Random|RandomFloatinRange _returnvalue_12 _returnvalue_11))) "WorldSpace"))))

(event EventBeginPlay
  (bind _poseablemesh (Variables|Default|GetPoseableMesh))
  (Components|PoseableMesh|SetBoneRotationbyName _poseablemesh "bip_upperArm_L" "0.000000,-90.000000,-90.000000" "WorldSpace")
  (Components|PoseableMesh|SetBoneRotationbyName _poseablemesh "bip_upperArm_R" "0.000000,90.000000,-90.000000" "WorldSpace")
  (Components|PoseableMesh|SetBoneRotationbyName _poseablemesh "bip_thumb_0_L" "0.000000,180.000000,-90.000000" "WorldSpace")
  (Components|PoseableMesh|SetBoneRotationbyName _poseablemesh "bip_thumb_0_R" "0.000000,0.000000,-90.000000" "WorldSpace")
  (|CallParentFunction)
  (CallFunction|SetupDebug "(R=0.000000,G=0.000000,B=0.000000,A=1.000000)")
  (bind (_success _string) (Utilities|CheckpointGetString (Variables|Default|GetSaveID)))
  (if _success
    (bind (_success_2 _string_2) (Utilities|CheckpointGetString (Utilities|String|Append (Variables|Default|GetSaveID) "_rotation")))
    (if _success_2
      (Transformation|SetActorLocationAndRotation (Math|Vector|MakeVector (Math|Conversions|ToFloat(Integer) (Utilities|Array|Get(acopy) (Utilities|String|ParseIntoArray _string "A"))) (Math|Conversions|ToFloat(Integer) (Utilities|Array|Get(acopy) (Utilities|String|ParseIntoArray _string "A") 1)) (Math|Conversions|ToFloat(Integer) (Utilities|Array|Get(acopy) (Utilities|String|ParseIntoArray _string "A") 2))) (Math|Rotator|MakeRotator (Math|Conversions|ToFloat(Integer) (Utilities|Array|Get(acopy) (Utilities|String|ParseIntoArray _string_2 "A"))) (Math|Conversions|ToFloat(Integer) (Utilities|Array|Get(acopy) (Utilities|String|ParseIntoArray _string_2 "A") 1)) (Math|Conversions|ToFloat(Integer) (Utilities|Array|Get(acopy) (Utilities|String|ParseIntoArray _string_2 "A") 2)))))))

(event EventScreamerStart
  (Rendering|SetVisibility (Variables|Default|GetPoseableMesh) false false)
  (Rendering|SetVisibility (Variables|Character|GetMesh) true false))

(event EventScreamerEnd
  (Rendering|SetVisibility (Variables|Default|GetPoseableMesh) true false)
  (Rendering|SetVisibility (Variables|Character|GetMesh) false false))

(event EventStartDefaultVisibility
  (|CallParentFunction)
  (Rendering|SetVisibility (Variables|Character|GetMesh) false false)
  (Rendering|SetVisibility (Variables|Default|GetPoseableMesh) true false))

(fn ConstructionScript)

(fn GetReachableLocation
  (params (Tries :type Integer) (MinDistance :type Float%20%28double-precision%29) (MaxDistance :type Float%20%28double-precision%29))
  (bind _returnvalue (Transformation|GetActorLocation))
  (bind _output_get (LocalVariables|SetCurrentTries Tries))
  (bind _output_get_2 (LocalVariables|SetNewLocalVar (.RandomLocation (AI|Navigation|GetRandomReachablePointinRadius _returnvalue MaxDistance 0 0)) :!label _label))
  (if (< (Math|Vector|Distance(Vector) _output_get_2 _returnvalue) MinDistance)
    (bind _result (Math|Integer|DecrementInt _output_get)
      (:%20%20
        (if (<= _result 0)
          _
          (else
            (goto _label))))))
  (return _output_get_2))