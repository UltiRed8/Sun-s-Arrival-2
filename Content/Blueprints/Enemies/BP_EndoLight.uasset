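; BP_EndoLight is an enemy AI, an eyeless endoskeleton that hunts and kills only players with their flashlight on.
; The server tracks flashlight toggles in AllPlayers, and a looping timer picks the nearest one who is not hiding and has a complete nav path.
; That target triggers Chase with door breaking; otherwise it alternates Idle and random-point Patrol.
; Each moving state sets walk speed, scaled by hardcore mode.
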(event Custom|UpdateTarget
  (bind _outclosestplayer (CallFunction|GetNearestPlayer))
  (Utilities|IsValid _outclosestplayer
    (:Is%20Valid
      (if (!= _outclosestplayer (Variables|Default|GetClosePlayer))
        (Variables|Default|SetClosePlayer _outclosestplayer)
        (CallFunction|Chase)))
    (:Is%20Not%20Valid
      (Variables|Default|GetClosePlayer
        (:then
          (Variables|Default|SetClosePlayer 0)
          (CallFunction|Idle))
        (:else)))))

(event Custom|Patrol
  ;[0.15 0.15 0.15 0.5] Patrol
  (if (not (Variables|Default|GetIsWaitingForSAS))
    (if (Variables|Default|GetCanPatrol)
      (Variables|Default|SetCanPatrol false)
      (Networking|SwitchHasAuthority
        (:Authority
          (Variables|Default|SetCanDestroyDoors false)
          (CallFunction|SetupDebug "(R=1.000000,G=1.000000,B=0.000000,A=1.000000)")
          (CallFunction|PlayAmbientSound)
          (CallFunction|SetTarget)
          (CallFunction|MultiUpdateValues 4e+02)
          (bind _randomlocation (CallFunction|GetReachableLocation 10 2e+03 1e+04))
          (Variables|Default|SetDestination _randomlocation)
          (AI|AIMoveTo self _randomlocation 0 5.0 false
            (:OnSuccess
              _)
            (:OnFail
              _))
          (Variables|Default|GetClosePlayer
            (:then)
            (:else
              (CallFunction|Idle))))))))

(event Custom|Idle
  ;[0.15 0.15 0.15 0.5] Idle
  (if (not (Variables|Default|GetIsWaitingForSAS))
    (AI|AIMoveTo self (Transformation|GetActorLocation) 0 5.0 false
      (:then
        (Networking|SwitchHasAuthority
          (:Authority
            (Variables|Default|SetCanDestroyDoors false)
            (CallFunction|SetupDebug "(R=0.000000,G=1.000000,B=0.000000,A=1.000000)")
            (CallFunction|SetTarget)
            (CallFunction|StopAmbientSound)
            (Utilities|FlowControl|Delay 6.34)
            (Variables|Default|GetClosePlayer
              (:then)
              (:else
                (Variables|Default|SetCanPatrol true)
                (CallFunction|Patrol)))))))))

(event Custom|Server_OnFlashlightToggle
  (params (Player :type BP%20Player%20Object%20Reference) (Status :type Boolean))
  (bind _allplayers (Variables|Default|GetAllPlayers))
  (if Status
    (Utilities|Array|Add _allplayers Player)
    (Development|PrintString "+" true true "(R=0.000000,G=1.000000,B=0.140660,A=1.000000)")
    (else
      (Utilities|Array|RemoveItem _allplayers Player)
      (Development|PrintString "-" true true "(R=1.000000,G=0.060101,B=0.000000,A=1.000000)"))))

(event Custom|Chase
  (bind _closeplayer (Variables|Default|GetClosePlayer))
  (if (not (Variables|Default|GetIsWaitingForSAS))
    (Networking|SwitchHasAuthority
      (:Authority
        (Variables|Default|SetCanDestroyDoors true)
        (CallFunction|SetupDebug "(R=1.000000,G=0.000000,B=0.000000,A=1.000000)")
        (CallFunction|PlayAmbientSound)
        (CallFunction|MultiUpdateValues 1.2e+03)
        (Variables|Default|SetDestination (Transformation|GetActorLocation _closeplayer))
        (CallFunction|SetTarget _closeplayer)
        (AI|AIMoveTo self "0, 0, 0" _closeplayer 5.0 false
          (:OnSuccess
            _)
          (:OnFail
            _))
        (if (not (Utilities|Array|IsEmpty (Variables|Default|GetAllPlayers)))
          (Variables|Default|GetClosePlayer
            (:then
              (CallFunction|Chase))
            (:else)))))))

(event Custom|Multi_UpdateValues
  (params (Max%20Walk%20Speed :type Float%20%28single-precision%29))
  (Variables|/Script/Engine.CharacterMovementComponent|SetMaxWalkSpeed (Variables|Character|GetCharacterMovement) (* Max%20Walk%20Speed (Math|Float|SelectFloat 2.5 0.9 (Variables|Default|GetIsHardcore)))))

(event EventKillCondition
  (params (Player :type BP%20Player%20Object%20Reference))
  (if (Variables|/Game/Blueprints/Player/BP_Player.BP_Player_C|GetFlashlightStatus Player)
    (CallFunction|KillValidated Player)))

(event EventDefaultState
  (for _array_element (Utilities|Array|MakeArray "bip_eye_L" "bip_eye_R" "bip_eyelid_1_L" "bip_eyelid_1_L001" "endo01_Eyelids_001" "bip_eyelid_1_R" "bip_eyelid_1_R001" "endo01_Eyelids_002" "bip_upperArm_L" "bip_upperArm_R")
    (Components|SkinnedMesh|HideBonebyName (Variables|Character|GetMesh) _array_element "PBO_None"))
  (|CallParentFunction)
  (CallFunction|Idle)
  (Utilities|Authority
    (:Authority
      (bind _outactors (Actor|GetAllActorsOfClass "/Game/Blueprints/Player/BP_Player.BP_Player_C"))
      (for _array_element_2 _outactors
        (EventDispatchers|AssignOnFlashlightToggle _array_element_2 (delegate Custom|Server_OnFlashlightToggle))
        (CallFunction|ServeronFlashlightToggle _array_element_2 (Variables|/Game/Blueprints/Player/BP_Player.BP_Player_C|GetFlashlightStatus _array_element_2))))))

(event EventBeginPlay
  (|CallParentFunction)
  (Utilities|Time|SetTimerbyEvent (delegate Custom|UpdateTarget) 0.1 true))

(fn ConstructionScript
  (for _array_element (Utilities|Array|MakeArray "bip_eye_L" "bip_eye_R" "bip_eyelid_1_L" "bip_eyelid_1_L001" "endo01_Eyelids_001" "bip_eyelid_1_R" "bip_eyelid_1_R001" "endo01_Eyelids_002")
    (Components|SkinnedMesh|HideBonebyName (Variables|Character|GetMesh) _array_element "PBO_None")))

(fn GetNearestPlayer
  (LocalVariables|SetClosestPlayer 0)
  (LocalVariables|SetClosestDistance 999999.0)
  (for _array_element (Variables|Default|GetAllPlayers)
    (if (not (Variables|/Game/Blueprints/Player/BP_Player.BP_Player_C|GetIsHiding _array_element))
      (bind _returnvalue (Class|NavigationSystemV1|FindPathtoLocationSynchronously (Transformation|GetActorLocation) (Transformation|GetActorLocation _array_element) 0 0))
      (if (and (not (Class|NavigationPath|IsPartial _returnvalue)) (> (Utilities|Array|Length (Variables|/Script/NavigationSystem.NavigationPath|GetPathPoints _returnvalue)) 0))
        (if (< (Math|Vector|Distance(Vector) (Transformation|GetActorLocation _array_element) (Transformation|GetActorLocation)) (LocalVariables|GetClosestDistance))
          (LocalVariables|SetClosestDistance (Math|Vector|Distance(Vector) (Transformation|GetActorLocation _array_element) (Transformation|GetActorLocation)))
          (LocalVariables|SetClosestPlayer _array_element)))))
  (return (LocalVariables|GetClosestPlayer)))

(fn GetReachableLocation
  (params (Tries :type Integer) (MinDistance :type Float%20%28double-precision%29) (MaxDistance :type Float%20%28double-precision%29))
  (bind _returnvalue (Transformation|GetActorLocation))
  (bind _output_get (LocalVariables|SetCurrentTries Tries))
  (bind _output_get_2 (LocalVariables|SetNewLocalVar (.RandomLocation (AI|Navigation|GetRandomReachablePointinRadius _returnvalue MaxDistance 0 0)) :!label _label))
  (if (< (Math|Vector|Distance(Vector) _output_get_2 _returnvalue) MinDistance)
    (bind _result (Math|Integer|DecrementInt _output_get)
      (:%20%20
        (if (<= _result 0)
          _
          (else
            (goto _label))))))
  (return _output_get_2))