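; Base Endo enemy that kills players on contact and opens or destroys closed, unlocked doors in its path.
; Activation follows default state or, in Normal and Hardcore, checkpoints keyed by world location.
; Server-side overlaps optionally retry line traces past walls, skip dead or hiding players, then trigger death and a scream montage.
; It also handles ambient audio and map-device alerts, leaving empty screamer and reset events as hooks.
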(event OnComponentEndOverlap(InteractionCollision)
  (params (OverlappedComponent :type Primitive%20Component%20Object%20Reference) (OtherActor :type Actor%20Object%20Reference) (OtherComp :type Primitive%20Component%20Object%20Reference) (OtherBodyIndex :type Integer))
  ;[0.15 0.15 0.15 0.5] Interactions
  (Utilities|Casting|CastToBP_Player OtherActor)
  (Variables|Default|SetPlayerIsInRadius false))

(event OnComponentBeginOverlap(InteractionCollision)
  (params (OverlappedComponent :type Primitive%20Component%20Object%20Reference) (OtherActor :type Actor%20Object%20Reference) (OtherComp :type Primitive%20Component%20Object%20Reference) (OtherBodyIndex :type Integer) (bFromSweep :type Boolean) (SweepResult :type Hit%20Result%20Structure%20%28by%20ref%29))
  ;[0.15 0.15 0.15 0.5] Interactions
  (CallFunction|TriggeredOverlap OtherActor))

(event Custom|SetTarget
  (params (Target :type BP%20Player%20Object%20Reference))
  (if (!= Target (Variables|Default|GetMapDeviceTarget))
    (bind _output_get (Variables|Default|SetMapDeviceTarget Target))
    (Utilities|IsValid _output_get
      (:Is%20Valid
        (bind _asbp_map_device (Utilities|Casting|CastToBP_MapDevice (Variables|/Script/Engine.ChildActorComponent|GetChildActor (Variables|/Game/Blueprints/Player/BP_Player.BP_Player_C|GetMapDeviceActor _output_get))))
        (if (Variables|/Game/Blueprints/Player/BP_MapDevice.BP_MapDevice_C|GetIsOpened _asbp_map_device)
          (bind _asuw_map_device (Utilities|Casting|CastToUW_MapDevice (UserInterface|GetWidget (Variables|/Game/Blueprints/Player/BP_MapDevice.BP_MapDevice_C|GetWidget _asbp_map_device))))
          (Default|AlertDetected _asuw_map_device))))))

(event Custom|KillCondition
  (params (Player :type BP%20Player%20Object%20Reference))
  ;[0.15 0.15 0.15 0.5] Interactions
  (CallFunction|KillValidated Player))

(event Custom|DefaultState
  (Collision|SetCollisionEnabled (Variables|Default|GetInteractionCollision) "QueryOnly")
  (CallFunction|StartDefaultVisibility)
  (switch Utilities|FlowControl|Switch|SwitchonE_ExtrasGamemodes (Variables|/Game/BP_GameInstance.BP_GameInstance_C|GetExtraGamemode (Utilities|GameInstance))
    (:NewEnumerator0
      _)
    (:NewEnumerator2
      _))
  (Utilities|CheckpointSaveBool (Utilities|String|ToString(Vector) (Transformation|GetActorLocation)) true))

(event Custom|ScreamerStart)

(event Custom|ScreamerEnd)

(event Custom|StartDefaultVisibility
  (Rendering|SetVisibility (Variables|Default|GetDisabledStaticMesh) false true)
  (Rendering|SetVisibility (Variables|Character|GetMesh) true true))

(event Custom|Multi_ScreamAnimation
  ;[0.15 0.15 0.15 0.5] Interactions
  (bind _returnvalue (Animation|PlayAnimMontage "/Game/Animations/Endo/AM_Scream.AM_Scream" 1.0 "None"))
  (Networking|SwitchHasAuthority
    (:Authority
      (Utilities|FlowControl|Delay _returnvalue)
      (Variables|Default|SetIsScreaming false)
      (CallFunction|DefaultState)
      (CallFunction|ScreamerEnd))))

(event Custom|SetupDebug
  (params (Value :type Linear%20Color%20Structure))
  ;[0.15 0.15 0.15 0.5] Debugs
  (bind _returnvalue (Rendering|Material|CreateDynamicMaterialInstance (Variables|Default|GetSphere) 0 "/Game/Materials/MAT_GlowColor.MAT_GlowColor" "None" :!class /Script/Engine.PrimitiveComponent))
  (Rendering|Material|SetVectorParameterValue _returnvalue "Color" Value :!class /Script/Engine.MaterialInstanceDynamic))

(event Custom|KillValidated
  (params (Player :type BP%20Player%20Object%20Reference))
  ;[0.15 0.15 0.15 0.5] Interactions
  (Variables|Default|SetIsScreaming true)
  (Default|ServerDeath Player self)
  (CallFunction|MultiScreamAnimation)
  (CallFunction|ScreamerStart))

(event Custom|Reset)

(event Custom|ResetToDefaultPosition
  (Transformation|SetActorLocation (Variables|Default|GetDefaultLocation) false false))

(event Custom|TriggeredOverlap
  (params (Actor :type Actor%20Object%20Reference))
  ;[0.15 0.15 0.15 0.5] Interactions
  (Networking|SwitchHasAuthority
    (:Authority
      (bind _asbp_player (Utilities|Casting|CastToBP_Player Actor)
        (:then
          (Variables|Default|SetPlayerIsInRadius true)
          (if (Variables|Default|GetCheckForWalls)
            (bind _returnvalue (Collision|LineTraceByChannel (Transformation|GetActorLocation) (Transformation|GetActorLocation Actor) "TraceTypeQuery1" false (Utilities|Array|MakeArray Actor) "None" :!label _label))
            (if _returnvalue
              (Utilities|FlowControl|Delay 0.2)
              (if (Variables|Default|GetPlayerIsInRadius)
                (goto _label))
              (else
                (if (not (or (Variables|/Game/Blueprints/Player/BP_Player.BP_Player_C|GetIsDead _asbp_player) (Variables|/Game/Blueprints/Player/BP_Player.BP_Player_C|GetIsHiding _asbp_player))) :!label _label_2
                  (if (not (Variables|Default|GetIsScreaming))
                    (if (Variables|Default|GetCanKill)
                      (CallFunction|KillCondition _asbp_player))))))
            (else
              (goto _label_2))))
        (:CastFailed
          (bind _asbp_classic_openable_door (Utilities|Casting|CastToBP_ClassicOpenableDoor Actor))
          (if (Math|Boolean|ANDBoolean (not (Variables|/Game/Blueprints/GPE/Doors/BP_DoorBase.BP_DoorBase_C|GetIsOpen _asbp_classic_openable_door)) (Variables|/Game/Blueprints/GPE/Doors/BP_DoorBase.BP_DoorBase_C|GetCanBeToggledByPlayer _asbp_classic_openable_door) (not (Variables|/Game/Blueprints/GPE/Doors/BP_DoorBase.BP_DoorBase_C|GetIsLocked _asbp_classic_openable_door)))
            (if (Variables|Default|GetCanDestroyDoors)
              (Default|MultiAIDestroy _asbp_classic_openable_door (Transformation|GetActorForwardVector))
              (else
                (Default|ServerToggleDoor _asbp_classic_openable_door)))))))))

(event Custom|CheckOverlaps
  (for _array_element (Collision|GetOverlappingActors (Variables|Default|GetInteractionCollision) "/Game/Blueprints/Player/BP_Player.BP_Player_C" :!class /Script/Engine.PrimitiveComponent)
    (CallFunction|TriggeredOverlap _array_element)))

(event Custom|PlayAmbientSound
  (bind _audio (Variables|Default|GetAudio))
  (Audio|Components|Audio|SetSound _audio (select (Math|Random|RandomBool) "/Game/Audio/Sounds/SW_EndoAmbientB.SW_EndoAmbientB" "/Game/Audio/Sounds/SW_EndoAmbientA.SW_EndoAmbientA"))
  (Audio|Components|Audio|Play _audio 0.0))

(event Custom|StopAmbientSound
  (Audio|Components|Audio|Stop (Variables|Default|GetAudio)))

(event EventTick
  (params (DeltaSeconds :type Float%20%28single-precision%29)))

(event EventBeginPlay
  (Variables|Default|SetIsHardcore (Utilities|Enum|Equal(Enum) (Variables|/Game/BP_GameInstance.BP_GameInstance_C|GetExtraGamemode (Utilities|GameInstance)) "NewEnumerator2"))
  (Variables|Default|SetDefaultLocation (Transformation|GetActorLocation))
  (switch Utilities|FlowControl|Switch|SwitchonE_ExtrasGamemodes (Variables|/Game/BP_GameInstance.BP_GameInstance_C|GetExtraGamemode (Utilities|GameInstance))
    (:NewEnumerator0
      (bind (_success _bool) (Utilities|CheckpointGetBool (Utilities|String|ToString(Vector) (Transformation|GetActorLocation)) :!label _label))
      (if _success
        (if _bool
          (CallFunction|DefaultState :!label _label_2)
          (else
            (if (Variables|Default|GetIsActiveByDefault) :!label _label_3
              (goto _label_2))))
        (else
          (goto _label_3))))
    (:NewEnumerator1
      (goto _label_3))
    (:NewEnumerator2
      (goto _label))
    (:NewEnumerator3
      (goto _label_3))))

(fn ConstructionScript)