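; BP_Sun is the Sun enemy, a killer that walks along spline paths and can only kill or move in Normal, Hardcore and Chaos modes once loading completes.
; Tick advances it by a mode-dependent speed, using a downward trace to keep it on the ground.
; SetNextPath swaps the spline and resets progress.
; Overlapping a player stops it, kills them through ServerDeath and plays a lit screamer before returning to idle.
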(event OnComponentBeginOverlap(InteractionCollision)
  (params (OverlappedComponent :type Primitive%20Component%20Object%20Reference) (OtherActor :type Actor%20Object%20Reference) (OtherComp :type Primitive%20Component%20Object%20Reference) (OtherBodyIndex :type Integer) (bFromSweep :type Boolean) (SweepResult :type Hit%20Result%20Structure%20%28by%20ref%29))
  (if (Variables|Default|GetCanKill)
    (bind _asbp_player (Utilities|Casting|CastToBP_Player OtherActor))
    (CallFunction|PlayerScreamer _asbp_player)))

(event Custom|SetCanMove
  (if (Variables|Default|GetCanKill)
    (Variables|Default|SetSpeed (Utilities|Select :Index (Variables|/Game/BP_GameInstance.BP_GameInstance_C|GetExtraGamemode (Utilities|GameInstance)) :NewEnumerator0 5e+02 :NewEnumerator1 5e+02 :NewEnumerator2 6.5e+02 :NewEnumerator3 5e+02 :NewEnumerator4 0.0))
    (Variables|Default|SetCanMove true)
    (Components|Animation|PlayAnimation (Variables|Character|GetMesh) "/Game/Animations/Sun/SB_SunFullAnimations_Anim_RIG_Sunman_ao_SunMan_Walk.SB_SunFullAnimations_Anim_RIG_Sunman_ao_SunMan_Walk" true)))

(event Custom|PlayerScreamer
  (params (Player :type BP%20Player%20Object%20Reference))
  (bind _mesh (Variables|Character|GetMesh))
  (bind _mesh_2 (Variables|Character|GetMesh))
  (if (Variables|Default|GetCanKill)
    (Variables|Default|SetIsScreaming true)
    (Variables|Default|SetCanMove false)
    (Rendering|Components|Light|SetIntensity (Variables|Default|GetSpotLight) 5e+03)
    (Rendering|Components|Light|SetIntensity (Variables|Default|GetSpotLight1) 0.0)
    (Default|ServerDeath Player self)
    (Audio|Components|Audio|Stop _mesh)
    (Components|Animation|PlayAnimation _mesh "/Game/Animations/Sun/AS_SunScreamer.AS_SunScreamer" true)
    (Utilities|FlowControl|Delay 1.0)
    (Rendering|Components|Light|SetIntensity (Variables|Default|GetSpotLight) 0.0)
    (Rendering|Components|Light|SetIntensity (Variables|Default|GetSpotLight1) 1.5e+04)
    (Variables|Default|SetIsScreaming false)
    (Audio|Components|Audio|Stop _mesh_2)
    (Components|Animation|PlayAnimation _mesh_2 "/Game/Animations/Sun/SB_SunFullAnimations_Anim_RIG_Sunman_ao_SunMan_GatorGolf_Idle.SB_SunFullAnimations_Anim_RIG_Sunman_ao_SunMan_GatorGolf_Idle" true)))

(event Custom|SetNextPath
  (params (Path :type BP%20Sun%20Path%20Object%20Reference) (Normal :type Float%20%28double-precision%29) (Hardcore :type Float%20%28double-precision%29))
  (Variables|Default|SetPath Path)
  (Variables|Default|SetProgress 0.0)
  (Variables|Default|SetSpeed (Utilities|Select :Index (Variables|/Game/BP_GameInstance.BP_GameInstance_C|GetExtraGamemode (Utilities|GameInstance)) :NewEnumerator0 Normal :NewEnumerator1 Normal :NewEnumerator2 Hardcore :NewEnumerator3 Normal :NewEnumerator4 0.0)))

(event Custom|Init
  (Transformation|SetActorLocation (Spline|GetLocationatDistanceAlongSpline (Variables|/Game/Blueprints/Enemies/Sun/BP_SunPath.BP_SunPath_C|GetSpline (Variables|Default|GetPath)) 0.0 "World") false false))

(event Custom|OnLoadingCompleted_Event
  (bind _returnvalue (Actor|GetActorOfClass "/Game/Blueprints/GPE/Rooms/BP_RoomManager.BP_RoomManager_C"))
  (EventDispatchers|UnbindEventfromOnLoadingCompleted _returnvalue (delegate Custom|OnLoadingCompleted_Event))
  (switch Utilities|FlowControl|Switch|SwitchonE_ExtrasGamemodes (Variables|/Game/BP_GameInstance.BP_GameInstance_C|GetExtraGamemode (Utilities|GameInstance))
    (:NewEnumerator0
      _)
    (:NewEnumerator2
      _)
    (:NewEnumerator3
      _))
  (Variables|Default|SetCanKill true))

(event EventBeginPlay
  (bind _returnvalue (Actor|GetActorOfClass "/Game/Blueprints/GPE/Rooms/BP_RoomManager.BP_RoomManager_C"))
  (EventDispatchers|AssignOnLoadingCompleted _returnvalue (delegate Custom|OnLoadingCompleted_Event)))

(event EventTick
  (params (DeltaSeconds :type Float%20%28single-precision%29))
  (bind _path (Variables|Default|GetPath))
  (bind _spline (Variables|/Game/Blueprints/Enemies/Sun/BP_SunPath.BP_SunPath_C|GetSpline _path))
  (if (Variables|Default|GetCanKill)
    (if (Variables|Default|GetCanMove)
      (Variables|Default|SetProgress (+ (Variables|Default|GetProgress) (* DeltaSeconds (Variables|Default|GetSpeed))))
      (bind (_outhit _returnvalue) (Collision|LineTraceByChannel (Spline|GetLocationatDistanceAlongSpline _spline (Variables|Default|GetProgress) "World") (- (Spline|GetLocationatDistanceAlongSpline _spline (Variables|Default|GetProgress) "World") "0.000000,0.000000,1000.000000") "TraceTypeQuery1" false 0 "None"))
      (Transformation|SetActorLocationAndRotation (Math|Vector|SelectVector (+ (.Location (Collision|BreakHitResult _outhit)) "0.000000,0.000000,90.000000") (Spline|GetLocationatDistanceAlongSpline _spline (Variables|Default|GetProgress) "World") _returnvalue) (Math|Rotator|FindLookatRotation (Spline|GetLocationatDistanceAlongSpline _spline (Variables|Default|GetProgress) "World") (Spline|GetLocationatDistanceAlongSpline _spline (+ (Variables|Default|GetProgress) 1.0) "World"))))))

(fn ConstructionScript)