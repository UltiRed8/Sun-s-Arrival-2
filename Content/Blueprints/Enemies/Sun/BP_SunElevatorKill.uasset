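; Trigger volume actor that lets the Sun enemy catch the player at an elevator.
; When BP_Sun overlaps its box, it checks that the referenced elevator is not moving and sits below a fixed world height.
; If both hold, it calls the Sun's PlayerScreamer on the locally controlled player pawn, with no check on where that player is.
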(event OnComponentBeginOverlap(Box)
  (params (OverlappedComponent :type Primitive%20Component%20Object%20Reference) (OtherActor :type Actor%20Object%20Reference) (OtherComp :type Primitive%20Component%20Object%20Reference) (OtherBodyIndex :type Integer) (bFromSweep :type Boolean) (SweepResult :type Hit%20Result%20Structure%20%28by%20ref%29))
  (bind _elevator (Variables|Default|GetElevator))
  (bind _asbp_sun (Utilities|Casting|CastToBP_Sun OtherActor))
  (if (and (not (Variables|/Game/Blueprints/GPE/BP_Elevator.BP_Elevator_C|GetIsMoving _elevator)) (< (.z (Transformation|GetActorLocation _elevator)) 5e+02))
    (bind _asbp_player (Utilities|Casting|CastToBP_Player (Pawn|GetControlledPawn (Game|GetPlayerController 0))))
    (Default|PlayerScreamer _asbp_sun _asbp_player)))

(fn ConstructionScript)