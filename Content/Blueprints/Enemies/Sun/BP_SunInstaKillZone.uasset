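; BP_SunInstaKillZone is an enemy zone that triggers the Sun's screamer on the player when the Sun arrives while the player is inside.
; PlayerBox overlaps store or clear the player reference.
; When a BP_Sun begins overlapping SunTriggerKillBox and that reference is valid, the zone calls PlayerScreamer on its Sun reference, passing the player.
; The check runs only as the Sun enters, not when the player enters afterwards.
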(event OnComponentBeginOverlap(PlayerBox)
  (params (OverlappedComponent :type Primitive%20Component%20Object%20Reference) (OtherActor :type Actor%20Object%20Reference) (OtherComp :type Primitive%20Component%20Object%20Reference) (OtherBodyIndex :type Integer) (bFromSweep :type Boolean) (SweepResult :type Hit%20Result%20Structure%20%28by%20ref%29))
  (bind _asbp_player (Utilities|Casting|CastToBP_Player OtherActor))
  (Variables|Default|SetPlayerIn _asbp_player))

(event OnComponentEndOverlap(PlayerBox)
  (params (OverlappedComponent :type Primitive%20Component%20Object%20Reference) (OtherActor :type Actor%20Object%20Reference) (OtherComp :type Primitive%20Component%20Object%20Reference) (OtherBodyIndex :type Integer))
  (Utilities|Casting|CastToBP_Player OtherActor)
  (Variables|Default|SetPlayerIn 0))

(event OnComponentBeginOverlap(SunTriggerKillBox)
  (params (OverlappedComponent :type Primitive%20Component%20Object%20Reference) (OtherActor :type Actor%20Object%20Reference) (OtherComp :type Primitive%20Component%20Object%20Reference) (OtherBodyIndex :type Integer) (bFromSweep :type Boolean) (SweepResult :type Hit%20Result%20Structure%20%28by%20ref%29))
  (bind _playerin (Variables|Default|GetPlayerIn))
  (Utilities|Casting|CastToBP_Sun OtherActor)
  (Utilities|IsValid _playerin
    (:Is%20Valid
      (Default|PlayerScreamer (Variables|Default|GetSun) _playerin))))

(fn ConstructionScript)