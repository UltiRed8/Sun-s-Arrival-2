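; Spawner for the conveyor minigame that feeds chaos actors and a reward object onto a conveyor.
; Each Trigger calls the parent, then alternates between starting and clearing a looping timer that calls Spawn.
; Spawn creates a BP_ChaosActor at the Scene component's location and adds it to the conveyor's ActorsToMove list.
; Reward adds the existing RewardObject to that same list instead of spawning one.
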(event Custom|Spawn
  (bind _returnvalue (Game|SpawnActorfromClass "/Game/Chaos/BP_ChaosActor.BP_ChaosActor_C" (Math|Transform|MakeTransform (Transformation|GetWorldLocation (Variables|Default|GetScene)) "0, 0, 0" "1.000000,1.000000,1.000000") "AdjustIfPossibleButAlwaysSpawn" "MultiplyWithRoot" 0 0))
  (Utilities|IsValid _returnvalue
    (:Is%20Valid
      (Utilities|Array|Add (Variables|/Game/Blueprints/Decoratives/BP_Conveyor.BP_Conveyor_C|GetActorsToMove (Variables|Default|GetBP_Convoyer)) _returnvalue))))

(event Custom|Reward
  (Utilities|Array|Add (Variables|/Game/Blueprints/Decoratives/BP_Conveyor.BP_Conveyor_C|GetActorsToMove (Variables|Default|GetBP_Convoyer)) (Variables|Default|GetRewardObject)))

(event EventTrigger
  (|CallParentFunction)
  (Utilities|FlowControl|FlipFlop
    (:A
      (bind _returnvalue (Utilities|Time|SetTimerbyFunctionName 0 "Spawn" 2.5 true))
      (Variables|Default|SetTimerRef _returnvalue))
    (:B
      (if (Utilities|Time|IsValidTimerHandle (Variables|Default|GetTimerRef))
        (Utilities|Time|ClearandInvalidateTimerbyHandle (Variables|Default|GetTimerRef))))))

(fn ConstructionScript)