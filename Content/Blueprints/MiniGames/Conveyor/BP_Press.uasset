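; Conveyor minigame press that asks for random body part types on its screen and scores validated matches toward a victory reward.
; Each Trigger plays a timeline slam with camera shake; the first also starts the linked spawner and conveyor.
; The server picks types and destroys Chaos actors entering its box, while Multi events update screen, sound and progress.
; Results briefly toggle the conveyor; victory also clears its items and calls the spawner's Reward.
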(event OnComponentBeginOverlap(Box)
  (params (OverlappedComponent :type Primitive%20Component%20Object%20Reference) (OtherActor :type Actor%20Object%20Reference) (OtherComp :type Primitive%20Component%20Object%20Reference) (OtherBodyIndex :type Integer) (bFromSweep :type Boolean) (SweepResult :type Hit%20Result%20Structure%20%28by%20ref%29))
  (Networking|SwitchHasAuthority
    (:Authority
      (bind _asbp_chaos_actor (Utilities|Casting|CastToBP_ChaosActor OtherActor))
      (Default|PrepareDestroy _asbp_chaos_actor))))

(event Custom|Validated
  (params (Type :type E_GCType%20Enum :default "NewEnumerator0"))
  (if (Utilities|Enum|Equal(Enum) Type (Variables|Default|GetType))
    (bind _result (Math|Integer|IncrementInt (Variables|Default|GetScore))
      (:%20%20
        (CallFunction|MultiSetProgress _result)
        (if (>= _result (Variables|Default|GetMaxScore))
          (CallFunction|Victory)
          (else
            (CallFunction|MultiSuccess)))))
    (else
      (CallFunction|MultiError))))

(event Custom|SelectNextType
  (if (Math|Random|RandomBool)
    (if (Math|Random|RandomBool)
      (Variables|Default|SetType "NewEnumerator0")
      (else
        (Variables|Default|SetType "NewEnumerator1")))
    (elif (Math|Random|RandomBool)
      (Variables|Default|SetType "NewEnumerator2")
      (else
        (Variables|Default|SetType "NewEnumerator3"))))
  (CallFunction|MultiSetType (Variables|Default|GetType)))

(event Custom|Multi_Error
  (Audio|Components|Audio|Play (Variables|Default|GetErrorSound) 0.1)
  (Rendering|Material|SetMaterial (Variables|Default|GetDisplay) 1 "/Game/Materials/Instances/MI_KeycardReaderDenied.MI_KeycardReaderDenied")
  (Networking|SwitchHasAuthority
    (:Authority
      (Default|Trigger (Variables|Default|GetConveyorNode))
      (Utilities|FlowControl|Delay 1.0)
      (CallFunction|SelectNextType)
      (Default|Trigger (Variables|Default|GetConveyorNode)))))

(event Custom|Multi_Success
  (Audio|Components|Audio|Play (Variables|Default|GetSuccessSound) 0.1)
  (Rendering|Material|SetMaterial (Variables|Default|GetDisplay) 1 "/Game/Materials/Instances/MI_KeycardReaderSuccess.MI_KeycardReaderSuccess")
  (Networking|SwitchHasAuthority
    (:Authority
      (Default|Trigger (Variables|Default|GetConveyorNode))
      (Utilities|FlowControl|Delay 1.0)
      (CallFunction|SelectNextType)
      (Default|Trigger (Variables|Default|GetConveyorNode)))))

(event Custom|Multi_PressAnimation
  (bind _staticmesh (Variables|Default|GetStaticMesh))
  (bind _relativelocation (Variables|/Script/Engine.SceneComponent|GetRelativeLocation _staticmesh))
  (bind (_direction _newtrack_0) (Timeline|PressTimeline Play)
    (:Update
      (Transformation|SetRelativeLocation _staticmesh (Math|Vector|MakeVector (.x _relativelocation) (.y _relativelocation) (Math|Float|Lerp -8e+01 -1.4e+02 _newtrack_0)) false false))
    (:Finished
      (switch Utilities|FlowControl|Switch|SwitchonETimelineDirection _direction
        (:Forward
          (Default|CameraShake (Utilities|GameInstance) "/Game/Shakes/CS_Press.CS_Press_C" (Transformation|GetActorLocation) 8e+02 1.6e+03 1.0 false)
          (Audio|Components|Audio|Play (Variables|Default|GetPressed) 0.1)
          (Utilities|FlowControl|Delay 0.15)
          (|CallParentFunction)
          (Timeline|PressTimeline Reverse))))))

(event Custom|Multi_SetType
  (params (Type :type E_GCType%20Enum :default "NewEnumerator0"))
  (Variables|Default|SetType Type)
  (Rendering|Material|SetTextureParameterValue (Variables|Default|GetDynamicMaterial) "Texture" (Utilities|Select :Index (Variables|Default|GetType) :NewEnumerator0 "/Game/Textures/T_PressHead.T_PressHead" :NewEnumerator1 "/Game/Textures/T_PressArm.T_PressArm" :NewEnumerator2 "/Game/Textures/T_PressLeg.T_PressLeg" :NewEnumerator3 "/Game/Textures/T_PressBody.T_PressBody"))
  (Rendering|Material|SetMaterial (Variables|Default|GetDisplay) 1 (Variables|Default|GetDynamicMaterial)))

(event Custom|Victory
  (CallFunction|MultiVictory)
  (Default|Trigger (Variables|Default|GetSpawnerNode))
  (Utilities|FlowControl|Delay 2.0)
  (Default|Trigger (Variables|Default|GetConveyorNode))
  (Utilities|FlowControl|Delay 3.0)
  (Default|Trigger (Variables|Default|GetConveyorNode)))

(event Custom|Multi_Victory
  (bind _conveyornode (Variables|Default|GetConveyorNode))
  (Default|Trigger _conveyornode)
  (Audio|Components|Audio|Play (Variables|Default|GetSuccessSound) 0.1)
  (Rendering|Material|SetMaterial (Variables|Default|GetDisplay) 1 "/Game/Materials/Instances/MI_KeycardReaderSuccess.MI_KeycardReaderSuccess")
  (for _array_element (Variables|/Game/Blueprints/BP_Conveyor.BP_Conveyor_C|GetActorsToMove _conveyornode)
    (bind _asbp_chaos_actor (Utilities|Casting|CastToBP_ChaosActor _array_element))
    (Utilities|IsValid _asbp_chaos_actor
      (:Is%20Valid
        (Default|PrepareDestroy _asbp_chaos_actor))))
  (Utilities|FlowControl|Delay 2.0)
  (bind _asbp_press_object_spawner (Utilities|Casting|CastToBP_PressObjectSpawner (Variables|Default|GetSpawnerNode)))
  (Default|Reward _asbp_press_object_spawner))

(event Custom|Multi_SetProgress
  (params (Current :type Integer))
  (Rendering|Components|TextRender|SetText (Variables|Default|GetTextRender) (Utilities|Text|FormatText "{Current}/{Max}" Current (Variables|Default|GetMaxScore))))

(event EventBeginPlay
  (bind _returnvalue (Rendering|Material|CreateDynamicMaterialInstance (Variables|Default|GetDisplay) 1 "/Game/Materials/MAT_PressScreen.MAT_PressScreen" "None" :!class /Script/Engine.PrimitiveComponent))
  (Variables|Default|SetDynamicMaterial _returnvalue))

(event EventTrigger
  (Utilities|FlowControl|Sequence
    (:then_0
      (Utilities|FlowControl|DoOnce false
        (:Completed
          (Networking|SwitchHasAuthority
            (:Authority
              (Default|Trigger (Variables|Default|GetSpawnerNode))
              (Default|Trigger (Variables|Default|GetConveyorNode))
              (CallFunction|SelectNextType))))))
    (:then_1
      (CallFunction|MultiPressAnimation))))

(fn ConstructionScript)