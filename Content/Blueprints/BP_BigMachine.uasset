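; BP_BigMachine is the endgame machine that, when triggered with every BP_SunPlaceSpot completed, runs the victory sequence.
; The CheckingParts_2 macro gates on the spots gathered by the authority at BeginPlay, and an outer gate locks after success.
; A delayed chain removes BP_EndoChase enemies, toggles conveyors via parent Trigger, swaps in the fixed sun mesh and runs FinalConveyor.
; Multi events handle enemy removal, mesh swap and the win screen with achievement.
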(event Custom|Multi_Win
  (bind _returnvalue (Game|GetPlayerController 0))
  (bind _returnvalue_2 (UserInterface|CreateWidget "/Game/Widgets/UW_GameOver.UW_GameOver_C" _returnvalue true (Ability|HasAuthority _returnvalue)))
  (UserInterface|Viewport|AddtoViewport _returnvalue_2 0)
  (bind _returnvalue_3 (Actor|GetActorOfClass "/Game/Blueprints/BP_AchievementManager.BP_AchievementManager_C"))
  (Default|Unlock _returnvalue_3 "victory")
  (Audio|Components|Audio|Stop (Variables|Default|GetRunning)))

(event Custom|Multi_RemoveEnemies
  (bind _outactors (Actor|GetAllActorsOfClass "/Game/Blueprints/Enemies/BP_EndoChase.BP_EndoChase_C"))
  (for _array_element _outactors
    (Actor|DestroyActor _array_element))
  (Audio|Components|Audio|Play (Variables|Default|GetRunning) 0.0))

(event Custom|Multi_FixModel
  (Components|StaticMesh|SetStaticMesh (Variables|/Script/Engine.StaticMeshActor|GetStaticMeshComponent (Variables|Default|GetModelToReplace)) "/Game/Models/Sun/SM_SunBodyFixed.SM_SunBodyFixed"))

(event EventBeginPlay
  (Networking|SwitchHasAuthority
    (:Authority
      (bind _outactors (Actor|GetAllActorsOfClass "/Game/Blueprints/SunPlaceSpot/BP_SunPlaceSpot.BP_SunPlaceSpot_C"))
      (Variables|Default|SetAllSunPlaceSpot _outactors))))

(event EventTrigger
  (Utilities|FlowControl|Gate false :!label _label
    (:Exit
      (|CheckingParts_2
        (:Exit
          (Utilities|FlowControl|Sequence
            (:then_0
              (goto _label Close))
            (:then_1
              (CallFunction|MultiRemoveEnemies)
              ;[0.15 0.15 0.15 0.5] Enabling conveyors
              (|CallParentFunction)
              (Utilities|FlowControl|Delay 5.0)
              ;[0.15 0.15 0.15 0.5] Disabling conveyors
              (|CallParentFunction)
              (Utilities|FlowControl|Delay 1.0)
              (CallFunction|MultiFixModel)
              (bind _final_conveyor (Variables|Default|GetFinal%20Conveyor)
                (:then
                  (Default|Trigger _final_conveyor)
                  (Utilities|FlowControl|Delay 5.0)
                  (Default|Trigger _final_conveyor)
                  (Utilities|FlowControl|Delay 1.5)
                  (CallFunction|MultiWin))
                (:else)))))))))

(fn ConstructionScript)