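; Interactable keycard reader that has the player swipe a card with the mouse and checks the inventory for the required keycard.
; A first server interaction places the card; the next starts client mouse capture, accumulating one-directional vertical drag until it reports back to the server.
; The swipe animates, then either shows denial feedback with a notification or marks success, triggering its Node and syncing a connected reader without re-triggering.
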(event Custom|KeycardAnimation
  (bind (_direction _zposition _xposition _scale) (Timeline|SwipeAnimation PlayFromStart)
    (:Update
      (Transformation|SetRelativeTransform (Variables|Default|GetCard) (Math|Transform|MakeTransform (Math|Vector|MakeVector _xposition 8.5 _zposition) "0.000000,0.000000,90.100000" (Math|Vector|MakeVector (* _scale 0.045) (* _scale 0.045) (* _scale 0.045))) false false))
    (:Sound
      (Utilities|FlowControl|Delay 0.2)
      (Audio|Components|Audio|Play (Variables|Default|GetSwipe) 0.0))))

(event Custom|SuccessColor
  (Rendering|Material|SetMaterial (Variables|Default|GetReader) 1 "/Game/Materials/Instances/MI_KeycardReaderSuccess.MI_KeycardReaderSuccess")
  (Audio|Components|Audio|Play (Variables|Default|GetSuccess) 0.0)
  (Variables|Default|SetTexture2D "/Game/Textures/T_CursorNormal.T_CursorNormal"))

(event Custom|IdleColor
  (Rendering|Material|SetMaterial (Variables|Default|GetReader) 1 "/Game/Materials/Instances/MI_KeycardReaderIdle.MI_KeycardReaderIdle"))

(event Custom|OnMouseMovedDirection_Event
  (params (OffsetX :type Float%20%28double-precision%29) (OffsetY :type Float%20%28double-precision%29) (PositionOnScreen :type Vector%202D%20Structure) (Speed :type Float%20%28double-precision%29) (DirectionFromCenter :type Vector))
  (if (< OffsetY 0.0)
    (bind _output_get (Variables|Default|SetCardPositionY (+ OffsetY (Variables|Default|GetCardPositionY))))
    (if (<= _output_get 0.0)
      (bind _asbp_player (Utilities|Casting|CastToBP_Player (Pawn|GetControlledPawn (Game|GetPlayerController 0))))
      (Default|OntoServerInteractwith _asbp_player self)
      (Default|SoftStopCapturing (Variables|Default|GetBP_MouseMovementComponent)))))

(event Custom|ErrorColor
  (Rendering|Material|SetMaterial (Variables|Default|GetReader) 1 "/Game/Materials/Instances/MI_KeycardReaderDenied.MI_KeycardReaderDenied")
  (Audio|Components|Audio|Play (Variables|Default|GetDenied) 0.5)
  (bind _returnvalue (UserInterface|CreateWidget "/Game/Widgets/UW_Notification.UW_Notification_C" (Game|GetPlayerController 0) (Utilities|Text|FormatText "This keycard reader needs {value}!" (Variables|Default|GetKeycardID)) "(R=1.000000,G=0.000000,B=0.000000,A=1.000000)"))
  (UserInterface|Viewport|AddtoViewport _returnvalue 0)
  (Utilities|FlowControl|Delay 2.0)
  (CallFunction|IdleColor)
  (Variables|Default|SetTexture2D "/Game/Textures/T_CursorInteract.T_CursorInteract"))

(event Custom|OnMouseUncaptured_Event
  (Variables|Default|SetCardPositionY 2.5e+03))

(event Custom|SuccessEvent
  (params (IsOfficial :type Boolean))
  (Variables|Default|SetDidIt true)
  (CallFunction|SuccessColor)
  (if IsOfficial
    (bind _node (Variables|Default|GetNode)
      (:then
        (Default|Trigger _node)
        (bind _connectedkeycardreader (Variables|Default|GetConnectedKeycardReader)
          (:then
            (CallFunction|SuccessEvent _connectedkeycardreader false))
          (:else)))
      (:else))))

(event Custom|Multi_PlaceKeycard
  (bind (_direction _xposition _scale) (Timeline|Timeline PlayFromStart)
    (:Update
      (Transformation|SetRelativeTransform (Variables|Default|GetCard) (Math|Transform|MakeTransform (Math|Vector|MakeVector _xposition 8.5 35.0) "0.000000,0.000000,90.100000" (Math|Vector|MakeVector (* _scale 0.045) (* _scale 0.045) (* _scale 0.045))) false false)
      (Variables|Default|SetTexture2D "/Game/Textures/T_CursorMouseDown.T_CursorMouseDown"))))

(event EventServerInteract
  (params (WhoInteracted :type Actor%20Object%20Reference))
  (if (not (or (Variables|Default|GetDidIt) (Variables|Default|GetCooldown)))
    (if (Variables|Default|GetHasKeycard)
      (bind _asbp_player (Utilities|Casting|CastToBP_Player WhoInteracted))
      (Default|FromServerInteractwith _asbp_player self)
      (else
        (Variables|Default|SetCooldown true)
        (Variables|Default|SetHasKeycard true)
        (CallFunction|MultiPlaceKeycard)
        (Utilities|FlowControl|Delay 0.3)
        (Variables|Default|SetCooldown false)))))

(event EventBeginPlay
  (bind _bp_mousemovementcomponent (Variables|Default|GetBP_MouseMovementComponent))
  (EventDispatchers|AssignOnMouseMovedDirection _bp_mousemovementcomponent (delegate Custom|OnMouseMovedDirection_Event))
  (EventDispatchers|AssignOnMouseUncaptured _bp_mousemovementcomponent (delegate Custom|OnMouseUncaptured_Event))
  (if (Variables|Default|GetDidIt)
    (Variables|Default|SetTexture2D "/Game/Textures/T_CursorNormal.T_CursorNormal")))

(event EventOntoServerInteract
  (params (MethodName :type String))
  (Variables|Default|SetCooldown true)
  (CallFunction|KeycardAnimation)
  (Utilities|FlowControl|Delay 1.2)
  (bind _returnvalue (Default|HasItem (Utilities|Inventory) (Variables|Default|GetKeycardID)))
  (if _returnvalue
    (CallFunction|SuccessEvent true)
    (else
      (CallFunction|ErrorColor)
      (Variables|Default|SetCooldown false)
      (Variables|Default|SetHasKeycard false))))

(event EventClientInteract
  (Default|StartCapturing (Variables|Default|GetBP_MouseMovementComponent)))

(fn ConstructionScript)