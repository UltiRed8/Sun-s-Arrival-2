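; BP_MapManager tells the in-game map where the player is, reporting the current floor and room.
; GetFloor returns a boolean for whether the controlled pawn's Z is at or below a fixed height threshold.
; GetRoom line-traces down along the pawn's negative up vector on a custom object type to find a BP_MapRoom actor.
; It caches that actor's Room in LastRoom, which is returned whenever the trace finds no room.
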(fn ConstructionScript)

(fn GetFloor
  (return (<= (.z (Transformation|GetActorLocation (Pawn|GetControlledPawn (Game|GetPlayerController 0)))) 6e+02)))

(fn GetRoom
  (bind _returnvalue (Game|GetPlayerController 0))
  (bind _returnvalue_2 (Pawn|GetControlledPawn _returnvalue))
  (bind _returnvalue_3 (Transformation|GetActorLocation _returnvalue_2))
  (bind (_outhit _returnvalue_4) (Collision|LineTraceForObjects _returnvalue_3 (+ _returnvalue_3 (* (Transformation|GetActorUpVector _returnvalue_2) -5e+03)) (Utilities|Array|MakeArray "ObjectTypeQuery10") false 0 "None"))
  (if _returnvalue_4
    (bind _asbp_map_room (Utilities|Casting|CastToBP_MapRoom (.HitActor (Collision|BreakHitResult _outhit)))
      (:then
        (bind _output_get (Variables|Default|SetLastRoom (Variables|/Game/Blueprints/InGameMap/BP_MapRoom.BP_MapRoom_C|GetRoom _asbp_map_room)))
        (return _output_get))
      (:CastFailed
        _)))
  (return (Variables|Default|GetLastRoom)))