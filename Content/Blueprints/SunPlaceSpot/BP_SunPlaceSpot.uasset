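; BP_SunPlaceSpot is an interactable spot where a Sun part, head or arm, is placed from the inventory.
; The construction script uses IsHead to pick the mesh and required item ID, and the model starts hidden.
; On the first server interaction with that item, it removes the item, reveals the model and plays a sound through a multicast, then triggers an optional linked Node.
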(event Custom|Multi_Validate
  (Rendering|SetVisibility (Variables|Default|GetModel) true false)
  (Audio|Components|Audio|Play (Variables|Default|GetPlaced) 0.0))

(event EventServerInteract
  (params (WhoInteracted :type Actor%20Object%20Reference))
  (bind _inventory (Utilities|Inventory))
  (bind _sunpartid (Variables|Default|GetSunPartID))
  (bind _node (Variables|Default|GetNode))
  (if (not (Variables|Default|GetDidIt))
    (bind _returnvalue (Default|HasItem _inventory _sunpartid))
    (if _returnvalue
      (Default|RemoveItem _inventory _sunpartid)
      (CallFunction|MultiValidate)
      (Variables|Default|SetDidIt true)
      (Utilities|IsValid _node
        (:Is%20Valid
          (Default|Trigger _node))))))

(event EventBeginPlay
  (Rendering|SetVisibility (Variables|Default|GetModel) false false))

(fn ConstructionScript
  (bind _ishead (Variables|Default|GetIsHead))
  (Components|StaticMesh|SetStaticMesh (Variables|Default|GetModel) (select _ishead "/Game/Models/Sun/SM_SunHead.SM_SunHead" "/Game/Models/Sun/SM_SunArm.SM_SunArm"))
  (Variables|Default|SetSunPartID (Utilities|String|SelectString "Sun's Head" "Sun's Arm" _ishead)))