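; A falling note or mine for the BeatBox arcade rhythm game.
; The note component starts at an offset on local Y and slides each tick at constant speed, reaching zero after TimeToEnd.
; Once it passes half the offset beyond zero, it destroys itself, first reporting a missed note to the arcade unless it is a mine.
; Mines receive a distinct material in the construction script.
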(event EventBeginPlay
  (Transformation|AddRelativeLocation (Variables|Default|GetNote) (Math|Vector|MakeVector 0.0 (Variables|Default|GetDefaultOffset) 0.0) false false))

(event EventTick
  (params (DeltaSeconds :type Float%20%28single-precision%29))
  (bind _defaultoffset (Variables|Default|GetDefaultOffset))
  (bind _returnvalue (* _defaultoffset -1.0))
  (Transformation|AddRelativeLocation (Variables|Default|GetNote) (Math|Vector|MakeVector 0.0 (* DeltaSeconds _returnvalue (/ 1.0 (Variables|Default|GetTimeToEnd))) 0.0) false false)
  (if (< (.y (Variables|/Script/Engine.SceneComponent|GetRelativeLocation (Variables|Default|GetNote))) (/ _returnvalue 2.0))
    (if (Variables|Default|GetIsMine)
      _
      (else
        (Default|UpdateScore (Variables|Default|GetBeatBoxArcade) true false)))
    (Actor|DestroyActor)))

(fn ConstructionScript
  (if (Variables|Default|GetIsMine)
    (Rendering|Material|SetMaterial (Variables|Default|GetNote) 0 "/Game/Textures/Arcades/M_Mine.M_Mine")))