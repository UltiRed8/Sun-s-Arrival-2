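; Component for the BeatBox arcade arrows that animates a vertical, horizontal and rotational offset into a Result transform.
; SetMovement retargets each changed channel from its current value with its own duration and ease strengths, and Reset eases all back to zero.
; Tick advances each lerp and rebuilds the transform.
; A custom ease-in-out curve blends from linear through cubic to back overshoot as strength rises.
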(event Custom|Reset
  (CallFunction|SetMovement 0.0 0.1 0.1 0.1 0.0 0.1 0.1 0.1 0.0 0.1 0.1 0.1))

(event Custom|SetMovement
  (params (V_Target :type Float%20%28double-precision%29) (V_InTransition :type Float%20%28double-precision%29) (V_OutTransition :type Float%20%28double-precision%29) (V_TransitionTime :type Float%20%28double-precision%29) (H_Target :type Float%20%28double-precision%29) (H_InTransition :type Float%20%28double-precision%29) (H_OutTransition :type Float%20%28double-precision%29) (H_TransitionTime :type Float%20%28double-precision%29) (R_Target :type Float%20%28double-precision%29) (R_InTransition :type Float%20%28double-precision%29) (R_OutTransition :type Float%20%28double-precision%29) (R_TransitionTime :type Float%20%28double-precision%29))
  ;[0 1 0.002238 0.25] Set Shake
  (if (!= V_Target (Variables|VOffset|GetV_Target))
    (Variables|VOffset|SetV_Current (Variables|Default|GetResultV))
    (Variables|VOffset|SetV_Target V_Target)
    (Variables|VOffset|SetV_InTransition V_InTransition)
    (Variables|VOffset|SetV_OutTransition V_OutTransition)
    (Variables|VOffset|SetV_TransitionTime V_TransitionTime)
    (Variables|VOffset|SetV_CurrentTime 0.0))
  (if (!= H_Target (Variables|HOffset|GetH_Target))
    (Variables|HOffset|SetH_Current (Variables|Default|GetResultH))
    (Variables|HOffset|SetH_Target H_Target)
    (Variables|HOffset|SetH_InTransition H_InTransition)
    (Variables|HOffset|SetH_OutTransition H_OutTransition)
    (Variables|HOffset|SetH_TransitionTime H_TransitionTime)
    (Variables|HOffset|SetH_CurrentTime 0.0))
  (if (!= R_Target (Variables|ROffset|GetR_Target))
    (Variables|ROffset|SetR_Current (Variables|Default|GetResultR))
    (Variables|ROffset|SetR_Target R_Target)
    (Variables|ROffset|SetR_InTransition R_InTransition)
    (Variables|ROffset|SetR_OutTransition R_OutTransition)
    (Variables|ROffset|SetR_TransitionTime R_TransitionTime)
    (Variables|ROffset|SetR_CurrentTime 0.0)))

(event Custom|ComputeVOffset
  (params (Deltatime :type Float%20%28double-precision%29))
  ;[0.15 0.15 0.15 0.5] Compute V Offset
  (if (< (Variables|VOffset|GetV_CurrentTime) 1.0)
    (bind _output_get (Variables|VOffset|SetV_CurrentTime (+ (Variables|VOffset|GetV_CurrentTime) (* (/ 1.0 (Variables|VOffset|GetV_TransitionTime)) Deltatime))))
    (Variables|Default|SetResultV (Math|Float|Lerp (Variables|VOffset|GetV_Current) (Variables|VOffset|GetV_Target) (Utilities|CubicEaseinOutAdvanced _output_get (Variables|VOffset|GetV_InTransition) (Variables|VOffset|GetV_OutTransition))))))

(event Custom|ComputeHOffset
  (params (Deltatime :type Float%20%28double-precision%29))
  ;[0.15 0.15 0.15 0.5] Compute H Offset
  (if (< (Variables|HOffset|GetH_CurrentTime) 1.0)
    (bind _output_get (Variables|HOffset|SetH_CurrentTime (+ (Variables|HOffset|GetH_CurrentTime) (* (/ 1.0 (Variables|HOffset|GetH_TransitionTime)) Deltatime))))
    (Variables|Default|SetResultH (Math|Float|Lerp (Variables|HOffset|GetH_Current) (Variables|HOffset|GetH_Target) (Utilities|CubicEaseinOutAdvanced _output_get (Variables|HOffset|GetH_InTransition) (Variables|HOffset|GetH_OutTransition))))))

(event Custom|ComputeROffset
  (params (Deltatime :type Float%20%28double-precision%29))
  ;[0.15 0.15 0.15 0.5] Compute R Offset
  (if (< (Variables|ROffset|GetR_CurrentTime) 1.0)
    (bind _output_get (Variables|ROffset|SetR_CurrentTime (+ (Variables|ROffset|GetR_CurrentTime) (* (/ 1.0 (Variables|ROffset|GetR_TransitionTime)) Deltatime))))
    (Variables|Default|SetResultR (Math|Float|Lerp (Variables|ROffset|GetR_Current) (Variables|ROffset|GetR_Target) (Utilities|CubicEaseinOutAdvanced _output_get (Variables|ROffset|GetR_InTransition) (Variables|ROffset|GetR_OutTransition))))))

(event EventTick
  (params (DeltaSeconds :type Float%20%28single-precision%29))
  ;[1 1 0 0.25] Tick
  (CallFunction|ComputeVOffset DeltaSeconds)
  (CallFunction|ComputeHOffset DeltaSeconds)
  (CallFunction|ComputeROffset DeltaSeconds)
  (Variables|Default|SetResult (Math|Transform|MakeTransform (Math|Vector|MakeVector 0.0 (Variables|Default|GetResultV) (Variables|Default|GetResultH)) (Math|Rotator|MakeRotator (Variables|Default|GetResultR) 0.0 0.0) "1.000000,1.000000,1.000000")))