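; Component for the BeatBox arcade arrows that computes a shake offset transform for other code to read.
; SetShake supplies time, strength, frequency and phase offset for three channels: vertical Z, horizontal Y and roll.
; Each tick it counts the timers down, resets Result to identity, then adds a game-time cosine wave per channel.
; Remaining time clamped to one scales each wave, fading it out over its final second.
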(event Custom|DecreaseShakeTimes
  (params (Deltatime :type Float%20%28double-precision%29))
  ;[0.15 0.15 0.15 0.5] Decrease Shake Times
  (Variables|VShake|SetV_ShakeTime (Math|Float|Clamp(Float) (- (Variables|VShake|GetV_ShakeTime) Deltatime) 0.0 1e+02))
  (Variables|HShake|SetH_ShakeTime (Math|Float|Clamp(Float) (- (Variables|HShake|GetH_ShakeTime) Deltatime) 0.0 1e+02))
  (Variables|RShake|SetR_ShakeTime (Math|Float|Clamp(Float) (- (Variables|RShake|GetR_ShakeTime) Deltatime) 0.0 1e+02)))

(event Custom|SetShake
  (params (V_ShakeTime :type Float%20%28double-precision%29) (V_ShakeStrength :type Float%20%28double-precision%29) (V_ShakeFrequency :type Float%20%28double-precision%29) (V_Offset :type Float%20%28double-precision%29) (H_ShakeTime :type Float%20%28double-precision%29) (H_ShakeStrength :type Float%20%28double-precision%29) (H_ShakeFrequency :type Float%20%28double-precision%29) (H_Offset :type Float%20%28double-precision%29) (R_ShakeTime :type Float%20%28double-precision%29) (R_ShakeStrength :type Float%20%28double-precision%29) (R_ShakeFrequency :type Float%20%28double-precision%29) (R_Offset :type Float%20%28double-precision%29))
  ;[0 1 0.002238 0.25] Set Shake
  (Variables|VShake|SetV_ShakeTime V_ShakeTime)
  (Variables|VShake|SetV_ShakeStrength V_ShakeStrength)
  (Variables|VShake|SetV_ShakeFrequency V_ShakeFrequency)
  (Variables|VShake|SetV_Offset V_Offset)
  (Variables|HShake|SetH_ShakeTime H_ShakeTime)
  (Variables|HShake|SetH_ShakeStrength H_ShakeStrength)
  (Variables|HShake|SetH_ShakeFrequency H_ShakeFrequency)
  (Variables|HShake|SetH_Offset H_Offset)
  (Variables|RShake|SetR_ShakeTime R_ShakeTime)
  (Variables|RShake|SetR_ShakeStrength R_ShakeStrength)
  (Variables|RShake|SetR_ShakeFrequency R_ShakeFrequency)
  (Variables|RShake|SetR_Offset R_Offset))

(event Custom|ComputeRShake
  ;[0.15 0.15 0.15 0.5] Compute R Shake
  (Variables|Default|SetResult (Math|Transform|MakeTransform (.location (Variables|Default|GetResult)) (Math|Rotator|MakeRotator (+ (.roll (.rotation (Variables|Default|GetResult))) (* (* (Math|Trig|Cos(Radians) (* (+ (Utilities|Time|GetGameTimeinSeconds) (Variables|RShake|GetR_Offset)) (Variables|RShake|GetR_ShakeFrequency))) (Variables|RShake|GetR_ShakeStrength)) (Math|Float|Clamp(Float) (Variables|RShake|GetR_ShakeTime)))) (.pitch (.rotation (Variables|Default|GetResult))) (.yaw (.rotation (Variables|Default|GetResult)))) (.scale (Variables|Default|GetResult)))))

(event Custom|ComputeVShake
  ;[0.15 0.15 0.15 0.5] Compute V Shake
  (Variables|Default|SetResult (Math|Transform|MakeTransform (Math|Vector|MakeVector (.x (.location (Variables|Default|GetResult))) (.y (.location (Variables|Default|GetResult))) (+ (.z (.location (Variables|Default|GetResult))) (* (* (Math|Trig|Cos(Radians) (* (+ (Utilities|Time|GetGameTimeinSeconds) (Variables|VShake|GetV_Offset)) (Variables|VShake|GetV_ShakeFrequency))) (Variables|VShake|GetV_ShakeStrength)) (Math|Float|Clamp(Float) (Variables|VShake|GetV_ShakeTime))))) (.rotation (Variables|Default|GetResult)) (.scale (Variables|Default|GetResult)))))

(event Custom|ComputeHShake
  ;[0.15 0.15 0.15 0.5] Compute H Shake
  (Variables|Default|SetResult (Math|Transform|MakeTransform (Math|Vector|MakeVector (.x (.location (Variables|Default|GetResult))) (+ (.y (.location (Variables|Default|GetResult))) (* (* (Math|Trig|Cos(Radians) (* (+ (Utilities|Time|GetGameTimeinSeconds) (Variables|HShake|GetH_Offset)) (Variables|HShake|GetH_ShakeFrequency))) (Variables|HShake|GetH_ShakeStrength)) (Math|Float|Clamp(Float) (Variables|HShake|GetH_ShakeTime)))) (.z (.location (Variables|Default|GetResult)))) (.rotation (Variables|Default|GetResult)) (.scale (Variables|Default|GetResult)))))

(event EventTick
  (params (DeltaSeconds :type Float%20%28single-precision%29))
  ;[1 1 0 0.25] Tick
  (CallFunction|DecreaseShakeTimes DeltaSeconds)
  (Variables|Default|SetResult (Math|Transform|MakeTransform "0, 0, 0" "0, 0, 0" "1.000000,1.000000,1.000000"))
  (CallFunction|ComputeVShake)
  (CallFunction|ComputeHShake)
  (CallFunction|ComputeRShake))