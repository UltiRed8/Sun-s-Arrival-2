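; BP_BeatBoxArrowLine is an arrow lane for the BeatBox arcade interactive.
; Its Arrow component takes its yaw from the Rotation variable, set in the construction script and again one tick after BeginPlay.
; The Spawn event creates a BP_BeatBoxNote, passing through an IsMine flag, and attaches it to the lane's root with relative transforms.
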(event Custom|Spawn
  (params (IsMine :type Boolean))
  (bind _returnvalue (Game|SpawnActorfromClass "/Game/Blueprints/Interactives/Arcades/BeatBox/BP_BeatBoxNote.BP_BeatBoxNote_C" (Math|Transform|MakeTransform "0, 0, 0" "0, 0, 0" "1.000000,1.000000,1.000000") "Undefined" "MultiplyWithRoot" 0 IsMine 0))
  (Transformation|AttachComponentToComponent _returnvalue (Variables|Transformation|GetRootComponent) "None" "KeepRelative" "KeepRelative" "KeepRelative" true))

(event EventBeginPlay
  (Utilities|FlowControl|DelayUntilNextTick)
  (Transformation|SetRelativeRotation (Variables|Default|GetArrow) (Math|Rotator|MakeRotator 0.0 0.0 (Variables|Default|GetRotation)) false false))

(fn ConstructionScript
  (Transformation|SetRelativeRotation (Variables|Default|GetArrow) (Math|Rotator|MakeRotator 0.0 0.0 (Variables|Default|GetRotation)) false false))