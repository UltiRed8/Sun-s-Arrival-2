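; Networked interactable handcrank box that takes a handcrank item from the inventory, then can be cranked once to trigger a linked Node.
; Server interaction either places the crank through multicast or hands off to BP_Player, while client interaction routes back through the player to the server trigger.
; Triggering plays a timeline handle rotation and fires the Node after a delay.
; The circular mouse-gesture cranking logic is disconnected and never runs.
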(event Custom|HandcrankAnimation
  (Variables|/Game/Blueprints/Components/BP_CustomCursorComponent.BP_CustomCursorComponent_C|SetCursorTexture (Variables|Default|GetBP_CustomCursorComponent) "/Game/Textures/T_CursorNormal.T_CursorNormal")
  (bind _rotation (Timeline|DoorOpening Play)
    (:Update
      (Transformation|SetRelativeRotation (Variables|Default|GetHandlePivot) (Math|Rotator|MakeRotator _rotation 0.0 0.0) false false))))

(event Custom|Multi_PlaceHandcrank
  (Rendering|SetVisibility (Variables|Default|GetHandlePivot) true true)
  (Audio|Components|Audio|Play (Variables|Default|GetPlaced) 0.0)
  (Variables|/Game/Blueprints/Components/BP_CustomCursorComponent.BP_CustomCursorComponent_C|SetCursorTexture (Variables|Default|GetBP_CustomCursorComponent) "/Game/Textures/T_CursorMouseCircle.T_CursorMouseCircle"))

(event Custom|CheckInventory
  (bind _inventory (Utilities|Inventory))
  (bind _handcrankid (Variables|Default|GetHandcrankID))
  (bind _returnvalue (Utilities|String|MakeLiteralString _handcrankid))
  (bind _returnvalue_2 (Default|HasItem _inventory _returnvalue))
  (if _returnvalue_2
    (Default|RemoveItem _inventory _returnvalue)
    (Variables|Default|SetHasHandcrank true)
    (CallFunction|MultiPlaceHandcrank)))

(event Custom|Multi_SetRotation
  (params (RotationX :type Float%20%28single-precision%29))
  (Transformation|SetRelativeRotation (Variables|Default|GetHandlePivot) (Math|Rotator|MakeRotator RotationX 0.0 0.0) false false))

(event Custom|OnMouseMovedDirection_Event
  (params (Offset :type Vector%202D%20Structure) (PositionOnScreen :type Vector%202D%20Structure) (Speed :type Float%20%28double-precision%29) (Direction :type Vector)))

(event Custom|Trigger
  (Variables|Default|SetDidIt true)
  (CallFunction|HandcrankAnimation)
  (Utilities|FlowControl|Delay 2.0)
  (bind _node (Variables|Default|GetNode)
    (:then
      (Default|Trigger _node))
    (:else)))

(event Custom|Server_SetRotation
  (params (RotationX :type Float%20%28single-precision%29))
  (CallFunction|MultiSetRotation RotationX))

(event EventBeginPlay
  (bind _bp_customcursorcomponent (Variables|Default|GetBP_CustomCursorComponent))
  (EventDispatchers|AssignOnMouseMovedDirection (Variables|Default|GetBP_MouseMovementComponent) (delegate Custom|OnMouseMovedDirection_Event))
  (if (Variables|Default|GetHasHandcrank)
    (Variables|/Game/Blueprints/Components/BP_CustomCursorComponent.BP_CustomCursorComponent_C|SetCursorTexture _bp_customcursorcomponent "/Game/Textures/T_CursorMouseCircle.T_CursorMouseCircle")
    (else
      (Variables|/Game/Blueprints/Components/BP_CustomCursorComponent.BP_CustomCursorComponent_C|SetCursorTexture _bp_customcursorcomponent "/Game/Textures/T_CursorInteract.T_CursorInteract"))))

(event EventOntoServerInteract
  (params (MethodName :type String))
  (CallFunction|Trigger))

(event EventServerInteract
  (params (WhoInteracted :type Actor%20Object%20Reference))
  (Actor|SetOwner WhoInteracted)
  (if (not (Variables|Default|GetDidIt))
    (if (Variables|Default|GetHasHandcrank)
      (bind _asbp_player (Utilities|Casting|CastToBP_Player WhoInteracted))
      (Default|FromServerInteractwith _asbp_player self)
      (else
        (CallFunction|CheckInventory)))))

(event EventClientInteract
  (bind _asbp_player (Utilities|Casting|CastToBP_Player (Pawn|GetControlledPawn (Game|GetPlayerController 0))))
  (Default|OntoServerInteractwith _asbp_player self))

(fn ConstructionScript
  (Rendering|SetVisibility (Variables|Default|GetHandlePivot) (Variables|Default|GetHasHandcrank) true))