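; Elevator press button interactive that requests a floor and shows a configurable text label.
; On server interaction it broadcasts OnTriggered with its Floor, plays a sound through a multicast event, and triggers its Node.
; The construction script writes the Text variable into the TextRender component.
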(event Custom|Multi_PlaySound
  (Audio|Components|Audio|Play (Variables|Default|GetLeverDownEnd) 0.0))

(event EventServerInteract
  (params (WhoInteracted :type Actor%20Object%20Reference))
  (Default|CallOnTriggered (Variables|Default|GetFloor))
  (CallFunction|MultiPlaySound)
  (Default|Trigger (Variables|Default|GetNode)))

(fn ConstructionScript
  (Rendering|Components|TextRender|SetText (Variables|Default|GetTextRender) (Utilities|Text|ToText(String) (Variables|Default|GetText))))