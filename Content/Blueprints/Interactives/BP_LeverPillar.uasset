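; BP_LeverPillar is an interactive lever that players pull with a mouse drag to trigger an optional linked Node.
; Client interaction starts mouse capture, accumulating negative vertical movement until a threshold sends a server interaction through BP_Player, followed by a short cooldown.
; OntoServerInteract animates the handle with sounds, calls OnTriggered and triggers the Node after a brief delay.
; DidIt blocks further server interactions until the handle returns.
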(event Custom|FuseboxAnimation
  (Audio|Components|Audio|Play (Variables|Default|GetLeverDown) 0.0)
  (bind _rotation (Timeline|HandleAnimation PlayFromStart)
    (:Update
      (Transformation|SetRelativeRotation (Variables|Default|GetHandlePivot) (Math|Rotator|MakeRotator 0.0 _rotation 0.0) false false))
    (:Finished
      (Audio|Components|Audio|Play (Variables|Default|GetLeverDownEnd) 0.0)
      (Utilities|FlowControl|Delay 0.2)
      (bind _rotation_2 (Timeline|Timeline ReverseFromEnd)
        (:Update
          (Transformation|SetRelativeRotation (Variables|Default|GetHandlePivot) (Math|Rotator|MakeRotator 0.0 _rotation_2 0.0) false false))
        (:Finished
          (Variables|Default|SetDidIt false))))))

(event Custom|OnMouseMovedDirection_Event
  (params (OffsetX :type Float%20%28double-precision%29) (OffsetY :type Float%20%28double-precision%29) (PositionOnScreen :type Vector%202D%20Structure) (Speed :type Float%20%28double-precision%29) (DirectionFromCenter :type Vector))
  (if (not (Variables|Default|GetCooldown))
    (if (< OffsetY 0.0)
      (bind _output_get (Variables|Default|SetLeverPositionY (+ OffsetY (Variables|Default|GetLeverPositionY))))
      (if (<= _output_get 0.0)
        (bind _asbp_player (Utilities|Casting|CastToBP_Player (Pawn|GetControlledPawn (Game|GetPlayerController 0))))
        (Default|OntoServerInteractwith _asbp_player self)
        (Variables|Default|SetLeverPositionY 2.5e+03)
        (Variables|Default|SetCooldown true)
        (Utilities|FlowControl|Delay 0.5)
        (Variables|Default|SetCooldown false)))))

(event Custom|OnMouseUncaptured_Event
  (Variables|Default|SetLeverPositionY 2.5e+03))

(event EventBeginPlay
  (bind _bp_mousemovementcomponent (Variables|Default|GetBP_MouseMovementComponent))
  (EventDispatchers|AssignOnMouseMovedDirection _bp_mousemovementcomponent (delegate Custom|OnMouseMovedDirection_Event))
  (EventDispatchers|AssignOnMouseUncaptured _bp_mousemovementcomponent (delegate Custom|OnMouseUncaptured_Event)))

(event EventServerInteract
  (params (WhoInteracted :type Actor%20Object%20Reference))
  (if (not (Variables|Default|GetDidIt))
    (bind _asbp_player (Utilities|Casting|CastToBP_Player WhoInteracted))
    (Default|FromServerInteractwith _asbp_player self)))

(event EventOntoServerInteract
  (params (MethodName :type String))
  (Variables|Default|SetDidIt true)
  (CallFunction|FuseboxAnimation)
  (Default|CallOnTriggered)
  (Utilities|FlowControl|Delay 0.15)
  (bind _node (Variables|Default|GetNode)
    (:then
      (Default|Trigger _node))
    (:else)))

(event EventClientInteract
  (Default|StartCapturing (Variables|Default|GetBP_MouseMovementComponent)))

(fn ConstructionScript)