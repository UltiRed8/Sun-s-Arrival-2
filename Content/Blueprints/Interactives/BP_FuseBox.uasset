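; Interactive, single-use fuse box that players open, then operate by pulling its lever with the mouse to trigger a linked Node.
; The first server interaction multicasts the door opening; the next hands back to the player's client to start mouse capture.
; Accumulated negative Y movement drives a lever counter, reset on release, that notifies the server at zero.
; This sets DidIt, plays handle and door-closing timelines with sounds and camera shake, and triggers Node.
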(event Custom|FuseboxAnimation
  (Variables|Default|SetTexture2D "/Game/Textures/T_CursorNormal.T_CursorNormal")
  (Audio|Components|Audio|Play (Variables|Default|GetLeverDown) 0.0)
  (bind _rotation (Timeline|HandleAnimation PlayFromStart)
    (:Update
      (Transformation|SetRelativeRotation (Variables|Default|GetHandlePivot) (Math|Rotator|MakeRotator 0.0 _rotation 0.0) false false))
    (:Finished
      (Audio|Components|Audio|Play (Variables|Default|GetSW_FuseBox) 0.0)
      (Audio|Components|Audio|Play (Variables|Default|GetLeverDownEnd) 0.0)
      (Utilities|FlowControl|Delay 0.1)
      (bind _rotation_2 (Timeline|DoorClosing PlayFromStart)
        (:Update
          (Transformation|SetRelativeRotation (Variables|Default|GetDoorPivot) (Math|Rotator|MakeRotator 0.0 0.0 _rotation_2) false false))
        (:Sound
          (Audio|Components|Audio|Play (Variables|Default|GetCloseDoor) 0.5)
          (Default|CameraShake (Utilities|GameInstance) "/Game/Shakes/CS_FuseBox.CS_FuseBox_C" (Transformation|GetActorLocation) 6e+02 8e+02 1.0 false))))))

(event Custom|OnMouseMovedDirection_Event
  (params (OffsetX :type Float%20%28double-precision%29) (OffsetY :type Float%20%28double-precision%29) (PositionOnScreen :type Vector%202D%20Structure) (Speed :type Float%20%28double-precision%29) (DirectionFromCenter :type Vector))
  (if (< OffsetY 0.0)
    (bind _output_get (Variables|Default|SetLeverPositionY (+ OffsetY (Variables|Default|GetLeverPositionY))))
    (if (<= _output_get 0.0)
      (bind _asbp_player (Utilities|Casting|CastToBP_Player (Pawn|GetControlledPawn (Game|GetPlayerController 0))))
      (Default|OntoServerInteractwith _asbp_player self)
      (Default|SoftStopCapturing (Variables|Default|GetBP_MouseMovementComponent)))))

(event Custom|OnMouseUncaptured_Event
  (Variables|Default|SetLeverPositionY 2.5e+03))

(event Custom|Multi_OpenDoor
  (Variables|Default|SetIsOpened true)
  (Variables|Default|SetTexture2D "/Game/Textures/T_CursorMouseDown.T_CursorMouseDown")
  (Audio|Components|Audio|Play (Variables|Default|GetOpenDoor) 0.0)
  (bind _rotation (Timeline|Timeline PlayFromStart)
    (:Update
      (Transformation|SetRelativeRotation (Variables|Default|GetDoorPivot) (Math|Rotator|MakeRotator 0.0 0.0 _rotation) false false))))

(event EventBeginPlay
  (bind _bp_mousemovementcomponent (Variables|Default|GetBP_MouseMovementComponent))
  (EventDispatchers|AssignOnMouseMovedDirection _bp_mousemovementcomponent (delegate Custom|OnMouseMovedDirection_Event))
  (EventDispatchers|AssignOnMouseUncaptured _bp_mousemovementcomponent (delegate Custom|OnMouseUncaptured_Event))
  (if (Variables|Default|GetDidIt)
    (Variables|Default|SetTexture2D "/Game/Textures/T_CursorNormal.T_CursorNormal")))

(event EventServerInteract
  (params (WhoInteracted :type Actor%20Object%20Reference))
  (if (not (Variables|Default|GetDidIt))
    (if (Variables|Default|GetIsOpened)
      (bind _asbp_player (Utilities|Casting|CastToBP_Player WhoInteracted))
      (Default|FromServerInteractwith _asbp_player self)
      (else
        (CallFunction|MultiOpenDoor)))))

(event EventOntoServerInteract
  (params (MethodName :type String))
  (Variables|Default|SetDidIt true)
  (CallFunction|FuseboxAnimation)
  (Utilities|FlowControl|Delay 0.15)
  (bind _node (Variables|Default|GetNode)
    (:then
      (Default|Trigger _node))
    (:else)))

(event EventClientInteract
  (Default|StartCapturing (Variables|Default|GetBP_MouseMovementComponent)))

(fn ConstructionScript)