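; Post-process manager that applies the player's gamma and contrast settings to the level's PostProcessVolume.
; After a short delay on BeginPlay it finds the volume, binds to the GameInstance settings update and applies once; it unbinds on Destroyed.
; Each update rereads stored values, offset by 0.5, with contrast driving Saturation rather than Contrast.
; It rebuilds the whole settings struct, resetting drunk and focus materials to zero weight and keeping outline on.
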(event Custom|OnGammaContrastUpdated_Event
  (params (Gamma :type Float%20%28double-precision%29) (Contrast :type Float%20%28double-precision%29))
  (Variables|/Script/Engine.PostProcessVolume|SetSettings (Variables|Default|GetPostProcessVolume) (Utilities|Struct|MakePostProcessSettings (Math|Vector4|MakeVector4 (+ (Default|GetContrast (Variables|/Game/BP_GameInstance.BP_GameInstance_C|GetSettings (Utilities|GameInstance))) 0.5) (+ (Default|GetContrast (Variables|/Game/BP_GameInstance.BP_GameInstance_C|GetSettings (Utilities|GameInstance))) 0.5) (+ (Default|GetContrast (Variables|/Game/BP_GameInstance.BP_GameInstance_C|GetSettings (Utilities|GameInstance))) 0.5) 1.0) (Math|Vector4|MakeVector4 (+ (Default|GetGamma (Variables|/Game/BP_GameInstance.BP_GameInstance_C|GetSettings (Utilities|GameInstance))) 0.5) (+ (Default|GetGamma (Variables|/Game/BP_GameInstance.BP_GameInstance_C|GetSettings (Utilities|GameInstance))) 0.5) (+ (Default|GetGamma (Variables|/Game/BP_GameInstance.BP_GameInstance_C|GetSettings (Utilities|GameInstance))) 0.5) 1.0) (Utilities|Struct|MakeWeightedBlendables (Utilities|Array|MakeArray (Utilities|Struct|MakeWeightedBlendable 0.0 "/Game/Materials/PostProcess/MAT_DrunkPostProcess.MAT_DrunkPostProcess") (Utilities|Struct|MakeWeightedBlendable 0.0 "/Game/Materials/PostProcess/MAT_FocusPostProcess.MAT_FocusPostProcess") (Utilities|Struct|MakeWeightedBlendable 1.0 "/Game/Materials/PostProcess/MAT_Outline.MAT_Outline"))))))

(event EventBeginPlay
  (Utilities|TickDelay 2)
  (bind _returnvalue (Actor|GetActorOfClass "/Script/Engine.PostProcessVolume"))
  (Variables|Default|SetPostProcessVolume _returnvalue)
  (EventDispatchers|AssignOnGammaContrastUpdated (Variables|/Game/BP_GameInstance.BP_GameInstance_C|GetSettings (Utilities|GameInstance)) (delegate Custom|OnGammaContrastUpdated_Event))
  (CallFunction|OnGammaContrastUpdatedEvent 0.0 0.0))

(event EventDestroyed
  (EventDispatchers|UnbindEventfromOnGammaContrastUpdated (Variables|/Game/BP_GameInstance.BP_GameInstance_C|GetSettings (Utilities|GameInstance)) (delegate Custom|OnGammaContrastUpdated_Event)))

(fn ConstructionScript)