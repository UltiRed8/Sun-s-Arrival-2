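; BP_SunsPlaceSpotManager manages a set of sun place spots where sun parts belong.
; A server interaction event, gated on authority, loops over the spots and checks the inventory for each spot's sun part ID.
; For each part found, EnableEffect activates that spot's Niagara indicator by index.
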(event Custom|EnableEffect
  (params (Index :type Integer))
  (Components|Activation|Activate (Variables|/Game/Blueprints/GPE/BP_SunPlaceSpot.BP_SunPlaceSpot_C|GetNS_SunsPlaceSpotIndicator (Utilities|Array|Get(acopy) (Variables|Default|GetSunsPlacesSpot) Index)) false))

(event Custom|Server_InteractWithSunsPlaceSpot
  (Networking|SwitchHasAuthority
    (:Authority
      (for (_array_element _array_index) (Variables|Default|GetSunsPlacesSpot)
        (bind _returnvalue (Default|HasItem (Utilities|Inventory) (Variables|/Game/Blueprints/GPE/BP_SunPlaceSpot.BP_SunPlaceSpot_C|GetSunPartID _array_element)))
        (if _returnvalue
          (CallFunction|EnableEffect _array_index))))))

(fn ConstructionScript)