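; BP_HandcrankBox is a networked interactable crank box that needs a Handcrank item from inventory unless one is already fitted.
; Interacting captures mouse movement, using a sphere and dot-product test to accept one circling direction, turning the handle and counting down RotationNeeded.
; At zero, the client notifies the server through BP_Player, and Trigger plays the DoorOpening handle animation, then fires the linked Node after a delay.
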(event Custom|HandcrankAnimation
  (Variables|Default|SetTexture2D "/Game/Textures/T_CursorNormal.T_CursorNormal")
  (bind _rotation (Timeline|DoorOpening PlayFromStart)
    (:Update
      (Transformation|SetRelativeRotation (Variables|Default|GetHandlePivot) (Math|Rotator|MakeRotator _rotation 0.0 0.0) false false))
    (:Finished
      (Audio|Components|Audio|Stop (Variables|Default|GetRotated)))))

(event Custom|Multi_PlaceHandcrank
  (Rendering|SetVisibility (Variables|Default|GetHandlePivot) true true)
  (Audio|Components|Audio|Play (Variables|Default|GetPlaced) 0.0)
  (Variables|Default|SetTexture2D "/Game/Textures/T_CursorMouseCircle.T_CursorMouseCircle"))

(event Custom|CheckInventory
  (bind _returnvalue (Utilities|String|MakeLiteralString "Handcrank"))
  (bind _inventory (Utilities|Inventory))
  (bind _returnvalue_2 (Default|HasItem _inventory _returnvalue))
  (if _returnvalue_2
    (Default|RemoveItem _inventory _returnvalue)
    (Variables|Default|SetHasHandcrank true)
    (CallFunction|MultiPlaceHandcrank)))

(event Custom|OnMouseMovedDirection_Event
  (params (OffsetX :type Float%20%28double-precision%29) (OffsetY :type Float%20%28double-precision%29) (PositionOnScreen :type Vector%202D%20Structure) (Speed :type Float%20%28double-precision%29) (DirectionFromCenter :type Vector))
  (bind _returnvalue (Math|Float|Clamp(Float) Speed 0.0 2e+01))
  (bind _sphere (Variables|Default|GetSphere))
  (bind _rotated (Variables|Default|GetRotated))
  (bind _sphere_2 (Variables|Default|GetSphere))
  (bind _returnvalue_2 (Transformation|GetWorldLocation _sphere_2))
  (bind _returnvalue_3 (* _returnvalue -1.0))
  (Utilities|FlowControl|Sequence
    (:then_0
      (if (!= Speed 0.0)
        (Utilities|FlowControl|DoOnce false :!label _label
          (:Completed
            (Utilities|FlowControl|Sequence
              (:then_0
                (goto _label_2 Reset))
              (:then_1
                (Audio|Components|Audio|Play _rotated 0.0)))))
        (else
          (Utilities|FlowControl|DoOnce true :!label _label_2
            (:Completed
              (Utilities|FlowControl|Sequence
                (:then_0
                  (goto _label Reset))
                (:then_1
                  (Audio|Components|Audio|Stop _rotated))))))))
    (:then_1
      (Variables|Default|SetLastLocation (Transformation|GetWorldLocation _sphere))
      (Transformation|SetWorldLocation _sphere (+ (Transformation|GetActorLocation) (* DirectionFromCenter 1e+02)) false false)
      (if (> (Math|Vector|DotProduct (Math|Vector|RotateVector (- _returnvalue_2 (Transformation|GetActorLocation)) "90.000000,0.000000,0.000000") (- _returnvalue_2 (Variables|Default|GetLastLocation))) 0.8)
        (Transformation|AddRelativeRotation (Variables|Default|GetHandlePivot) (Math|Rotator|MakeRotator _returnvalue_3 0.0 0.0) false false)
        (Variables|Default|SetRotationNeeded (- (Variables|Default|GetRotationNeeded) (Math|Float|Absolute(Float) _returnvalue_3)))
        (if (<= (Variables|Default|GetRotationNeeded) 0.0)
          (bind _asbp_player (Utilities|Casting|CastToBP_Player (Pawn|GetControlledPawn (Game|GetPlayerController 0))))
          (Default|OntoServerInteractwith _asbp_player self)
          (Default|SoftStopCapturing (Variables|Default|GetBP_MouseMovementComponent))
          (Audio|Components|Audio|Play (Variables|Default|GetRotated) 0.0))))))

(event Custom|Trigger
  (Variables|Default|SetDidIt true)
  (CallFunction|HandcrankAnimation)
  (Utilities|FlowControl|Delay 2.0)
  (bind _node (Variables|Default|GetNode)
    (:then
      (Default|Trigger _node))
    (:else)))

(event EventBeginPlay
  (EventDispatchers|AssignOnMouseMovedDirection (Variables|Default|GetBP_MouseMovementComponent) (delegate Custom|OnMouseMovedDirection_Event))
  (if (Variables|Default|GetHasHandcrank)
    (Variables|Default|SetTexture2D "/Game/Textures/T_CursorMouseCircle.T_CursorMouseCircle")))

(event EventOntoServerInteract
  (params (MethodName :type String))
  (CallFunction|Trigger))

(event EventServerInteract
  (params (WhoInteracted :type Actor%20Object%20Reference))
  (if (not (Variables|Default|GetDidIt))
    (if (Variables|Default|GetHasHandcrank)
      (bind _asbp_player (Utilities|Casting|CastToBP_Player WhoInteracted))
      (Default|FromServerInteractwith _asbp_player self)
      (else
        (CallFunction|CheckInventory)))))

(event EventClientInteract
  (Default|StartCapturing (Variables|Default|GetBP_MouseMovementComponent)))

(fn ConstructionScript
  (Rendering|SetVisibility (Variables|Default|GetHandlePivot) (Variables|Default|GetHasHandcrank) true))