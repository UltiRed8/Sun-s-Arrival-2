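; BP_BigMachineLeak is a decorative machine leak that emits a short burst of steam or fire with sound when triggered.
; Trigger uses IsSteam to pick the effect, activates it, then switches it off after a delay.
; A gate blocks overlapping triggers and reopens after steam, but the fire branch closes it again, so it stays shut after fire.
; The fire branch plays both steam and fire audio, stopping only the fire audio.
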(event Custom|Trigger
  (params (IsSteam :type Boolean))
  (bind _steam (Variables|Default|GetSteam))
  (bind _fire (Variables|Default|GetFire))
  (Utilities|FlowControl|Gate false :!label _label
    (:Exit
      (Utilities|FlowControl|Sequence
        (:then_0
          (goto _label Close))
        (:then_1
          (if IsSteam
            (Components|Activation|SetActive _steam true true)
            (Audio|Components|Audio|Play (Variables|Default|GetSteamAudio) 0.0)
            (Utilities|FlowControl|Delay 0.5)
            (Components|Activation|SetActive _steam false false)
            (Utilities|FlowControl|Delay 0.2)
            (goto _label Open)
            (else
              (Components|Activation|SetActive _fire true false)
              (Audio|Components|Audio|Play (Variables|Default|GetSteamAudio) 0.0)
              (Utilities|FlowControl|Delay 1.0)
              (Components|Activation|SetActive _fire false false)
              (Audio|Components|Audio|Stop (Variables|Default|GetFireAudio))
              (Utilities|FlowControl|Delay 0.5)
              (goto _label Close))))))))

(fn ConstructionScript)