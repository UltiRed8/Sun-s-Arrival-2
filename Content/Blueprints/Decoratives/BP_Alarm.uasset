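; BP_Alarm is a decorative alarm beacon with rotating spotlights and sound.
; SetActive, gated by CanBeActivated and also called on BeginPlay when IsActive is preset, starts both sounds, brightens the two spotlights and gives the base a red glow material.
; While active, Tick spins the base at a constant, frame-rate-independent yaw rate; the file has no deactivation path.
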(event Custom|SetActive
  (bind _sound (Variables|Default|GetSound))
  (if (Variables|Default|GetCanBeActivated)
    (Variables|Default|SetIsActive true)
    (Audio|Components|Audio|SetSound _sound (Variables|Default|GetAlarm))
    (Audio|Components|Audio|Play _sound 0.0)
    (Rendering|Components|Light|SetIntensity (Variables|Default|GetSpotLight) 1e+04)
    (Rendering|Material|SetMaterial (Variables|Default|GetBase) 0 "/Game/Models/EndoEnemy/MAT_RedGlow.MAT_RedGlow")))

(event EventTick
  (params (DeltaSeconds :type Float%20%28single-precision%29))
  (if (Variables|Default|GetIsActive)
    (Transformation|AddRelativeRotation (Variables|Default|GetBase) (Math|Rotator|MakeRotator 0.0 0.0 (* DeltaSeconds 4.5e+02)) false false)))

(event EventBeginPlay
  (if (Variables|Default|GetIsActive)
    (CallFunction|SetActive)))

(fn ConstructionScript)