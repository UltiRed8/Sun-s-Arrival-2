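; BP_ControlPanelA is a decorative control panel whose two screens switch to a static material when triggered.
; Trigger calls the parent implementation, saves a true checkpoint bool keyed by the actor's location string, then applies MAT_Static to material slot 1 of both screens.
; BeginPlay reads that bool and reapplies the static material if set, so the triggered look persists through checkpoints.
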(event EventTrigger
  (|CallParentFunction)
  (Utilities|CheckpointSaveBool (Utilities|String|ToString(Vector) (Transformation|GetActorLocation)) true)
  (Rendering|Material|SetMaterial (Variables|Default|GetScreen) 1 "/Game/Materials/MAT_Static.MAT_Static"))

(event EventBeginPlay
  (bind (_success _bool) (Utilities|CheckpointGetBool (Utilities|String|ToString(Vector) (Transformation|GetActorLocation))))
  (if _success
    (if _bool
      (Rendering|Material|SetMaterial (Variables|Default|GetScreen) 1 "/Game/Materials/MAT_Static.MAT_Static"))))

(fn ConstructionScript)