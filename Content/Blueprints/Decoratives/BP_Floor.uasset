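; BP_Floor is a decorative floor actor that wraps a BP_CameraVisibleActor in a child actor component and gives it a configurable default material.
; The construction script copies DefaultMaterial into the child's variable of the same name.
; At BeginPlay it also applies that material directly to the first slot of the child's Plane.
; Both steps do nothing if the child is not a BP_CameraVisibleActor.
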(event EventBeginPlay
  (bind _asbp_camera_visible_actor (Utilities|Casting|CastToBP_CameraVisibleActor (Variables|/Script/Engine.ChildActorComponent|GetChildActor (Variables|Default|GetChildActor))))
  (Rendering|Material|SetMaterial (Variables|/Game/Blueprints/Player/BP_CameraVisibleActor.BP_CameraVisibleActor_C|GetPlane _asbp_camera_visible_actor) 0 (Variables|Default|GetDefault%20Material)))

(fn ConstructionScript
  (bind _asbp_camera_visible_actor (Utilities|Casting|CastToBP_CameraVisibleActor (Variables|/Script/Engine.ChildActorComponent|GetChildActor (Variables|Default|GetChildActor))))
  (Variables|/Game/Blueprints/Player/BP_CameraVisibleActor.BP_CameraVisibleActor_C|SetDefaultMaterial _asbp_camera_visible_actor (Variables|Default|GetDefault%20Material)))