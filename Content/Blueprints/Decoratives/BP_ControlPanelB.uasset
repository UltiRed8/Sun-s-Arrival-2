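; BP_ControlPanelB is a decorative control panel with a screen and twelve child-actor press buttons that powers on when triggered.
; Trigger calls the parent, saves a checkpoint bool keyed by the actor's location, then applies lit button materials and a static screen material.
; BeginPlay restores that state from the checkpoint, or blacks out the buttons when none is saved or it is false.
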(event EventTrigger
  (|CallParentFunction)
  (Utilities|CheckpointSaveBool (Utilities|String|ToString(Vector) (Transformation|GetActorLocation)) true)
  (for _array_element (Utilities|Array|MakeArray (Variables|Default|GetChildActor1) (Variables|Default|GetChildActor2) (Variables|Default|GetChildActor3) (Variables|Default|GetChildActor4) (Variables|Default|GetChildActor5) (Variables|Default|GetChildActor6) (Variables|Default|GetChildActor7) (Variables|Default|GetChildActor8) (Variables|Default|GetChildActor9) (Variables|Default|GetChildActor10) (Variables|Default|GetChildActor11) (Variables|Default|GetChildActor12))
    (bind _asbp_press_button (Utilities|Casting|CastToBP_PressButton (Variables|/Script/Engine.ChildActorComponent|GetChildActor _array_element)))
    (Rendering|Material|SetMaterial (Variables|/Game/Blueprints/GPE/BP_PressButton.BP_PressButton_C|GetCylinder _asbp_press_button) 0 "/Game/Materials/Instances/MI_PressButton.MI_PressButton"))
  (Rendering|Material|SetMaterial (Variables|Default|GetScreen) 1 "/Game/Materials/MAT_Static.MAT_Static"))

(event EventBeginPlay
  (bind _childactor10 (Variables|Default|GetChildActor10))
  (bind _childactor5 (Variables|Default|GetChildActor5))
  (bind _childactor4 (Variables|Default|GetChildActor4))
  (bind _childactor11 (Variables|Default|GetChildActor11))
  (bind _childactor3 (Variables|Default|GetChildActor3))
  (bind _childactor1 (Variables|Default|GetChildActor1))
  (bind _childactor6 (Variables|Default|GetChildActor6))
  (bind _childactor12 (Variables|Default|GetChildActor12))
  (bind _childactor2 (Variables|Default|GetChildActor2))
  (bind _childactor8 (Variables|Default|GetChildActor8))
  (bind _childactor7 (Variables|Default|GetChildActor7))
  (bind _childactor9 (Variables|Default|GetChildActor9))
  (bind _array (Utilities|Array|MakeArray _childactor1 _childactor2 _childactor3 _childactor4 _childactor5 _childactor6 _childactor7 _childactor8 _childactor9 _childactor10 _childactor11 _childactor12))
  (bind (_success _bool) (Utilities|CheckpointGetBool (Utilities|String|ToString(Vector) (Transformation|GetActorLocation))))
  (if _success
    (if _bool
      (for _array_element _array
        (bind _asbp_press_button (Utilities|Casting|CastToBP_PressButton (Variables|/Script/Engine.ChildActorComponent|GetChildActor _array_element)))
        (Rendering|Material|SetMaterial (Variables|/Game/Blueprints/GPE/BP_PressButton.BP_PressButton_C|GetCylinder _asbp_press_button) 0 "/Game/Materials/Instances/MI_PressButton.MI_PressButton"))
      (Rendering|Material|SetMaterial (Variables|Default|GetScreen) 1 "/Game/Materials/MAT_Static.MAT_Static")
      (else
        (for _array_element_2 _array :!label _label
          (bind _asbp_press_button_2 (Utilities|Casting|CastToBP_PressButton (Variables|/Script/Engine.ChildActorComponent|GetChildActor _array_element_2)))
          (Rendering|Material|SetMaterial (Variables|/Game/Blueprints/GPE/BP_PressButton.BP_PressButton_C|GetCylinder _asbp_press_button_2) 0 "/Game/Materials/Instances/MI_Black.MI_Black"))))
    (else
      (goto _label))))

(fn ConstructionScript)