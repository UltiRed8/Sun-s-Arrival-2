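; BP_SunPlaceSpot is an interactable spot where a player places a Sun part: head, arm or leg.
; The construction script derives the required item ID from the assigned mesh, which stays hidden until placed.
; Server interaction consumes the item, multicasts the reveal, removes the indicator and triggers an optional Node.
; Completion is saved as a checkpoint bool keyed by actor location and restored by the authority on BeginPlay.
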(event Custom|Multi_Validate
  (Rendering|SetVisibility (Variables|Default|GetModel) true false)
  (Audio|Components|Audio|Play (Variables|Default|GetPlaced) 0.0)
  (Components|DestroyComponent (Variables|Default|GetNS_SunsPlaceSpotIndicator))
  (Variables|/Game/Blueprints/Components/BP_CustomCursorComponent.BP_CustomCursorComponent_C|SetCursorTexture (Variables|Default|GetBP_CustomCursorComponent) "/Game/Textures/T_CursorNormal.T_CursorNormal"))

(event EventBeginPlay
  (Utilities|RegisterInteractable)
  (Rendering|SetVisibility (Variables|Default|GetModel) false false)
  (Networking|SwitchHasAuthority
    (:Authority
      (if (Variables|Default|GetDidIt)
        (CallFunction|MultiValidate))
      (bind (_success _bool) (Utilities|CheckpointGetBool (Utilities|String|ToString(Vector) (Transformation|GetActorLocation))))
      (if _success
        (if _bool
          (CallFunction|MultiValidate)
          (Variables|Default|SetDidIt true))))))

(event EventServerInteract
  (params (WhoInteracted :type Actor%20Object%20Reference))
  (bind _inventory (Utilities|Inventory))
  (bind _sunpartid (Variables|Default|GetSunPartID))
  (bind _node (Variables|Default|GetNode))
  (if (not (Variables|Default|GetDidIt))
    (bind _returnvalue (Default|HasItem _inventory _sunpartid))
    (if _returnvalue
      (Default|RemoveItem _inventory _sunpartid)
      (CallFunction|MultiValidate)
      (Variables|Default|SetDidIt true)
      (Utilities|IsValid _node
        (:Is%20Valid
          (Default|Trigger _node))
        (:Is%20Not%20Valid
          _))
      (Utilities|CheckpointSaveBool (Utilities|String|ToString(Vector) (Transformation|GetActorLocation)) true))))

(event EventDestroyed
  (Utilities|UnregisterInteractable))

(fn ConstructionScript
  (bind _mesh (Variables|Default|GetMesh))
  (Components|StaticMesh|SetStaticMesh (Variables|Default|GetModel) _mesh)
  (Variables|Default|SetSunPartID (Utilities|String|SelectString "Sun's Head" (Utilities|String|SelectString "Sun's Arm" "Sun's Leg" (== _mesh "/Game/Models/Sun/SM_SunArm.SM_SunArm")) (== _mesh "/Game/Models/Sun/SM_SunHead.SM_SunHead"))))