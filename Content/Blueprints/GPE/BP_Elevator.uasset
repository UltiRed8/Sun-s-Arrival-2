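; Multiplayer elevator actor that carries players vertically between linked Floor actors.
; GoTo, also triggered by per-floor buttons spawned once on its first authority call, toggles floor doors and closes the cabin.
; The reversed door timeline's finish starts an authority-gated Move, which lerps height on a second timeline, then reopens doors on arrival.
; Start/loop/stop sounds, music, a red/green indicator and camera shake for the local rider accompany the cycle.
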(event OnAudioFinished(InElevatorSounds)
  (bind _inelevatorsounds (Variables|Default|GetInElevatorSounds))
  (if (== (Variables|/Script/Engine.AudioComponent|GetSound _inelevatorsounds) "/Game/Audio/Sounds/SW_InElevatorStart.SW_InElevatorStart")
    (Audio|Components|Audio|SetSound _inelevatorsounds "/Game/Audio/Sounds/SW_InElevatorLoop.SW_InElevatorLoop")
    (Audio|Components|Audio|Play _inelevatorsounds 0.0)))

(event OnComponentBeginOverlap(Box)
  (params (OverlappedComponent :type Primitive%20Component%20Object%20Reference) (OtherActor :type Actor%20Object%20Reference) (OtherComp :type Primitive%20Component%20Object%20Reference) (OtherBodyIndex :type Integer) (bFromSweep :type Boolean) (SweepResult :type Hit%20Result%20Structure%20%28by%20ref%29))
  (bind _asbp_player (Utilities|Casting|CastToBP_Player OtherActor))
  (if (== _asbp_player (Pawn|GetControlledPawn (Game|GetPlayerController 0)))
    (Variables|Default|SetIsPlayerIn true)))

(event OnComponentEndOverlap(Box)
  (params (OverlappedComponent :type Primitive%20Component%20Object%20Reference) (OtherActor :type Actor%20Object%20Reference) (OtherComp :type Primitive%20Component%20Object%20Reference) (OtherBodyIndex :type Integer))
  (bind _asbp_player (Utilities|Casting|CastToBP_Player OtherActor))
  (if (== _asbp_player (Pawn|GetControlledPawn (Game|GetPlayerController 0)))
    (Variables|Default|SetIsPlayerIn false)))

(event Custom|GoTo
  (params (Floor :type BP%20Elevator%20Door%20Object%20Reference))
  (bind _inelevatorsounds (Variables|Default|GetInElevatorSounds))
  (Networking|SwitchHasAuthority
    (:Authority
      (CallFunction|GenerateButtons))
    (:Remote
      _))
  (if (!= Floor (Variables|Default|GetFloor))
    (Default|CallMoving)
    (Audio|Components|Audio|SetSound _inelevatorsounds "/Game/Audio/Sounds/SW_InElevatorStart.SW_InElevatorStart")
    (Audio|Components|Audio|Play _inelevatorsounds 0.0)
    (Variables|Default|GetIsMoving
      (:then)
      (:else
        (Variables|Default|SetIsMoving true)
        (Variables|Default|SetTargetZ (.z (Transformation|GetActorLocation Floor)))
        (Variables|Default|SetStartingZ (.z (Transformation|GetActorLocation)))
        (bind _floor (Variables|Default|GetFloor)
          (:then
            (Default|ToggleDoor _floor))
          (:else
            _))
        (Variables|Default|SetFloor Floor)
        (CallFunction|CloseDoor)))))

(event Custom|CloseDoor
  (Default|CallClosingDoors)
  (bind _asbp_camera_visible_actor (Utilities|Casting|CastToBP_CameraVisibleActor (Variables|/Script/Engine.ChildActorComponent|GetChildActor (Variables|Default|GetChildActor4))))
  (Rendering|Material|SetMaterial (Variables|/Game/Blueprints/Player/BP_CameraVisibleActor.BP_CameraVisibleActor_C|GetPlane _asbp_camera_visible_actor) 0 "/Game/Materials/Instances/MI_Red.MI_Red")
  (bind (_direction _dooropening) (Timeline|Timeline Reverse)
    (:Update
      (Transformation|SetRelativeLocation (Variables|Default|GetDoorA) (Math|Vector|MakeVector -6e+02 _dooropening 2e+02) false false)
      (Transformation|SetRelativeLocation (Variables|Default|GetDoorB) (Math|Vector|MakeVector -6e+02 (* _dooropening -1.0) 2e+02) false false))
    (:Finished
      (switch Utilities|FlowControl|Switch|SwitchonETimelineDirection _direction
        (:Backward
          (Networking|SwitchHasAuthority
            (:Authority
              (CallFunction|Move (Variables|Default|GetTargetZ)))))))))

(event Custom|OpenDoor
  (Default|CallOpeningDoors)
  (bind _asbp_camera_visible_actor (Utilities|Casting|CastToBP_CameraVisibleActor (Variables|/Script/Engine.ChildActorComponent|GetChildActor (Variables|Default|GetChildActor4))))
  (Rendering|Material|SetMaterial (Variables|/Game/Blueprints/Player/BP_CameraVisibleActor.BP_CameraVisibleActor_C|GetPlane _asbp_camera_visible_actor) 0 "/Game/Materials/Instances/MI_Green.MI_Green")
  (bind (_direction _dooropening) (Timeline|Timeline Play)
    (:Update
      (Transformation|SetRelativeLocation (Variables|Default|GetDoorA) (Math|Vector|MakeVector -6e+02 _dooropening 2e+02) false false)
      (Transformation|SetRelativeLocation (Variables|Default|GetDoorB) (Math|Vector|MakeVector -6e+02 (* _dooropening -1.0) 2e+02) false false))
    (:Finished
      (switch Utilities|FlowControl|Switch|SwitchonETimelineDirection _direction
        (:Backward
          (Networking|SwitchHasAuthority
            (:Authority
              (CallFunction|Move (Variables|Default|GetTargetZ)))))))))

(event Custom|Move
  (params (TargetZ :type Float%20%28double-precision%29))
  (bind _returnvalue (Transformation|GetActorLocation))
  (bind _inelevatorsounds (Variables|Default|GetInElevatorSounds))
  (if (Variables|Default|GetIsPlayerIn)
    (Default|CameraShake (Utilities|GameInstance) "/Game/Shakes/CS_Elevator.CS_Elevator_C" (Transformation|GetActorLocation) 1e+03 1e+03 0.0 false))
  (Audio|Components|Audio|Play (Variables|Default|GetSW_ElevatorMusic) 0.0)
  (Variables|Default|SetTargetZ TargetZ)
  (bind _progress (Timeline|Elevator PlayFromStart)
    (:Update
      (Transformation|SetActorLocation (Math|Vector|MakeVector (.x _returnvalue) (.y _returnvalue) (Math|Float|Lerp (Variables|Default|GetStartingZ) (Variables|Default|GetTargetZ) _progress)) false false))
    (:Finished
      (Default|CallStopping)
      (Audio|Components|Audio|SetSound _inelevatorsounds "/Game/Audio/Sounds/SW_InElevatorStop.SW_InElevatorStop")
      (Audio|Components|Audio|Play _inelevatorsounds 0.0)
      (Utilities|FlowControl|Delay 1.0)
      (Networking|SwitchHasAuthority
        (:Authority
          (Default|ToggleDoor (Variables|Default|GetFloor))
          (CallFunction|OpenDoor)
          (Variables|Default|SetIsMoving false))))))

(event Custom|GenerateButtons
  (Utilities|FlowControl|DoOnce false
    (:Completed
      (for (_array_element _array_index) (Variables|Default|GetFloors)
        (bind _returnvalue (AddComponent|AddChildActorComponent false (Math|Transform|MakeTransform (+ (Variables|/Script/Engine.SceneComponent|GetRelativeLocation (Variables|Default|GetScene)) (* "0.000000,0.000000,-50.000000" _array_index)) "0.000000,90.000000,0.000000" "1.000000,1.000000,1.000000")))
        (bind _asbp_elevator_press_button (Utilities|Casting|CastToBP_ElevatorPressButton (Variables|/Script/Engine.ChildActorComponent|GetChildActor _returnvalue)))
        (Default|SetText _asbp_elevator_press_button (Variables|/Game/Blueprints/GPE/Doors/BP_ElevatorDoor.BP_ElevatorDoor_C|GetDoorLabel _array_element))
        (Variables|/Game/Blueprints/GPE/BP_ElevatorPressButton.BP_ElevatorPressButton_C|SetFloor _asbp_elevator_press_button _array_element)
        (EventDispatchers|AssignOnTriggered _asbp_elevator_press_button (delegate Custom|OnTriggered_Event))))))

(event Custom|OnTriggered_Event
  (params (Floor :type BP%20Elevator%20Door%20Object%20Reference))
  (CallFunction|Goto Floor))

(event EventBeginPlay
  (for _array_element (Variables|Default|GetFloors)
    (Variables|/Game/Blueprints/GPE/Doors/BP_ElevatorDoor.BP_ElevatorDoor_C|SetConnectedElevator _array_element self)))

(fn ConstructionScript)