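; BP_Vent is a ventilation fan actor with a spinning Fan component and a ventilation sound.
; Tick rotates the fan around yaw at RotationSpeed, scaled by delta time.
; The construction script derives the sound's pitch and volume multipliers from the absolute RotationSpeed, normalized and clamped between zero and one, so audio follows the configured speed in either direction.
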(event EventTick
  (params (DeltaSeconds :type Float%20%28single-precision%29))
  (Transformation|AddRelativeRotation (Variables|Default|GetFan) (Math|Rotator|MakeRotator 0.0 0.0 (* DeltaSeconds (Variables|Default|GetRotationSpeed))) false false))

(fn ConstructionScript
  (bind _sw_ventilationfan (Variables|Default|GetSW_VentilationFan))
  (bind _rotationspeed (Variables|Default|GetRotationSpeed))
  (bind _returnvalue (Math|Float|Absolute(Float) _rotationspeed))
  (bind _returnvalue_2 (/ _returnvalue 2e+02))
  (bind _returnvalue_3 (Math|Float|Clamp(Float) _returnvalue_2))
  (Audio|Components|Audio|SetPitchMultiplier _sw_ventilationfan _returnvalue_3)
  (Audio|Components|Audio|SetVolumeMultiplier _sw_ventilationfan _returnvalue_3 :!class /Script/Engine.AudioComponent))