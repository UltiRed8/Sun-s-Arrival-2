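; Interactable boombox gameplay element that plays a random track from its music list when interacted with.
; It extends an interactable parent, calling its BeginPlay and Interaction logic, and only triggers playback while CanBeInteract is true.
; Each trigger stops the current audio, then picks a random entry from MusicsList and plays it from the start, staying silent if the list is empty.
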(event Custom|PlaySound
  (bind _musicslist (Variables|Default|GetMusicsList))
  (Audio|Components|Audio|Stop (Variables|Default|GetAudio))
  (if (Utilities|Array|IsNotEmpty _musicslist)
    (Audio|Components|Audio|SetSound (Variables|Default|GetAudio) (Utilities|Array|Get(acopy) _musicslist (Math|Random|RandomInteger (Utilities|Array|Length (Variables|Default|GetMusicsList)))))
    (Audio|Components|Audio|Play (Variables|Default|GetAudio) 0.0)))

(event EventBeginPlay
  (|CallParentFunction))

(event EventInteraction
  (|CallParentFunction)
  (if (Variables|Default|GetCanBeInteract)
    (CallFunction|PlaySound)))

(fn ConstructionScript)