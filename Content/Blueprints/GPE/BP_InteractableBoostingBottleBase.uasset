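; Base interactable bottle that gives the interacting player a timed boost, one effect at a time, with an invalid sound if one is active.
; Interaction fires once: it multicasts sound and hiding, unlocks the drink achievement, then calls Boost, left empty here, and ResetBoost after BoostingTime.
; The reset goes through server and multicast events to clear the player's effect flag, then authority destroys the bottle.
; Hovering toggles custom depth on the mesh.
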(event Custom|Boost
  (params (Player :type BP%20Player%20Object%20Reference)))

(event Custom|ResetBoost
  (params (Player :type BP%20Player%20Object%20Reference))
  (CallFunction|ServerResetinEffect Player))

(event Custom|Multi_Used
  (Audio|Components|Audio|Play (Variables|Default|GetAudio) 0.0)
  (CallFunction|SetCanInteract false)
  (Rendering|SetActorHiddenInGame true)
  (Collision|SetActorEnableCollision false))

(event Custom|Multi_ResetInEffect
  (params (Player :type BP%20Player%20Object%20Reference))
  (Variables|/Game/Blueprints/Player/BP_Player.BP_Player_C|SetIsInEffect Player false)
  (Utilities|Authority
    (:Authority
      (Utilities|FlowControl|Delay 0.2)
      (Actor|DestroyActor))))

(event Custom|Server_ResetInEffect
  (params (Player :type BP%20Player%20Object%20Reference))
  (CallFunction|MultiResetinEffect Player))

(event EventInteracted
  (params (HitComponent :type Actor%20Component%20Object%20Reference%20%28by%20ref%29) (WhoInteracted :type Actor%20Object%20Reference) (HasMouseMovements :type Boolean))
  (bind _asbp_player (Utilities|Casting|CastToBP_Player WhoInteracted))
  (if (Variables|/Game/Blueprints/Player/BP_Player.BP_Player_C|GetIsInEffect _asbp_player)
    (CallFunction|PlayInvalidSound WhoInteracted)
    (else
      (Variables|/Game/Blueprints/Player/BP_Player.BP_Player_C|SetIsInEffect _asbp_player true)
      (Actor|SetOwner _asbp_player)
      (Utilities|FlowControl|DoOnce false
        (:Completed
          (CallFunction|MultiUsed)
          (Default|UnlockAchievement (Utilities|GameInstance) "ACH_DRINK")
          (CallFunction|Boost _asbp_player)
          (Utilities|FlowControl|RetriggerableDelay (Variables|Default|GetBoostingTime))
          (CallFunction|ResetBoost _asbp_player))))))

(fn ConstructionScript)

(fn Unhovered
  (Rendering|SetRenderCustomDepth (Variables|Default|GetStaticMesh) false))

(fn Hovered
  (Rendering|SetRenderCustomDepth (Variables|Default|GetStaticMesh) true))