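; Boosting bottle interactable that gives the player a focus effect, highlighting interactables through custom depth.
; It extends the parent's Boost and ResetBoost events to toggle the player's focus flag and the Game Instance's focus post-process, with the drunk effect off.
; Both events loop over every valid interactable in the Game Instance's list, switching custom depth rendering on all its static mesh components on or off.
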(event EventBoost
  (params (Player :type BP%20Player%20Object%20Reference))
  (Variables|/Game/Blueprints/Player/BP_Player.BP_Player_C|SetHasFocusEffect Player true)
  (|CallParentFunction Player)
  (Default|UpdatePostProcess (Utilities|GameInstance) false true)
  (for _array_element (Variables|/Game/BP_GameInstance.BP_GameInstance_C|GetAllInteractables (Utilities|GameInstance))
    (Utilities|IsValid _array_element
      (:Is%20Valid
        (for _array_element_2 (Actor|GetComponentsByClass _array_element "/Script/Engine.StaticMeshComponent")
          (Rendering|SetRenderCustomDepth _array_element_2 true))))))

(event EventResetBoost
  (params (Player :type BP%20Player%20Object%20Reference))
  (bind _asbp_game_instance (Utilities|GameInstance))
  (Variables|/Game/Blueprints/Player/BP_Player.BP_Player_C|SetHasFocusEffect Player false)
  (|CallParentFunction Player)
  (Default|UpdatePostProcess _asbp_game_instance false false)
  (for _array_element (Variables|/Game/BP_GameInstance.BP_GameInstance_C|GetAllInteractables _asbp_game_instance)
    (Utilities|IsValid _array_element
      (:Is%20Valid
        (for _array_element_2 (Actor|GetComponentsByClass _array_element "/Script/Engine.StaticMeshComponent")
          (Rendering|SetRenderCustomDepth _array_element_2 false))))))

(fn ConstructionScript
  (|CallParentFunction))