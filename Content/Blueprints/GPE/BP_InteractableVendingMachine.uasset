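; Interactable vending machine that takes a coin from BP_GlobalInventory and dispenses bottles from its child actors.
; Timelines animate coin and bottle, which then drops with physics and becomes pickable if a boosting bottle.
; After the first purchase, bottles randomly jam until the player rocks the machine by mouse movement, or repeated interaction when that setting is off.
; Use count saves to a checkpoint keyed by location, removing dispensed bottles on BeginPlay.
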(event Custom|OnMouseCapture_Event
  (Variables|/Game/Blueprints/Components/BP_CustomCursorComponent.BP_CustomCursorComponent_C|SetCursorTexture (Variables|Default|GetBP_CustomCursorComponent) "/Game/Textures/T_CursorMouseLR.T_CursorMouseLR"))

(event Custom|OnMouseUncaptured_Event
  (Variables|/Game/Blueprints/Components/BP_CustomCursorComponent.BP_CustomCursorComponent_C|SetCursorTexture (Variables|Default|GetBP_CustomCursorComponent) (select (Variables|Default|GetCanBeInteract) "/Game/Textures/T_CursorInteract.T_CursorInteract" "/Game/Textures/T_CursorNormal.T_CursorNormal")))

(event Custom|OnMouseMoved_Event
  (params (Angle :type Float%20%28double-precision%29) (Direction :type Vector%202D%20Structure))
  (bind _allrewards (Variables|Default|GetAllRewards))
  (bind _defaultsceneroot (Variables|Default|GetDefaultSceneRoot))
  (bind _rectlight1 (Variables|Default|GetRectLight1))
  (bind _sw_vendingmachineidle (Variables|Default|GetSW_VendingMachineIdle))
  (bind _relativerotation (Variables|/Script/Engine.SceneComponent|GetRelativeRotation _defaultsceneroot))
  (if (> (Variables|Default|GetStuckAmount) 0)
    (Utilities|FlowControl|Sequence
      (:then_0
        (if (> (.x Direction) 0.0)
          (Utilities|FlowControl|Sequence
            (:then_0
              (bind _tilt (Timeline|TiltLeft Stop)
                (:Update
                  (Transformation|SetRelativeRotation _defaultsceneroot (Math|Rotator|MakeRotator _tilt (.pitch _relativerotation) (.yaw _relativerotation)) false false))))
            (:then_1
              (bind _tilt_2 (Timeline|TiltRight PlayFromStart)
                (:Update
                  (Transformation|SetRelativeRotation _defaultsceneroot (Math|Rotator|MakeRotator _tilt_2 (.pitch _relativerotation) (.yaw _relativerotation)) false false))))
            (:then_2
              (Audio|Components|Audio|Play (Variables|Default|GetAudio) 0.0 :!label _label)
              (Default|CameraShake (Utilities|GameInstance) "/Game/Shakes/CS_ClassicDoor.CS_ClassicDoor_C" (Transformation|GetActorLocation) 6e+02 1.2e+03 1.0 false))
            (:then_3
              (Components|Activation|Activate (Variables|Default|GetNS_Right) true)))
          (else
            (Utilities|FlowControl|Sequence
              (:then_0
                (Timeline|TiltRight Stop))
              (:then_1
                (Timeline|TiltLeft PlayFromStart))
              (:then_2
                (goto _label))
              (:then_3
                (Components|Activation|Activate (Variables|Default|GetNS_Left) true))))))
      (:then_1
        (bind _result (Math|Integer|DecrementInt (Variables|Default|GetStuckAmount))
          (:%20%20
            (if (<= _result 0)
              (Default|SoftStopCapturing (Variables|Default|GetBP_MouseMovementComponent))
              (Utilities|FlowControl|Sequence
                (:then_0
                  (Utilities|FlowControl|Sequence
                    (:then_0
                      (bind _height (Timeline|UnStuckReward PlayFromStart)
                        (:Update
                          (Transformation|SetRelativeLocation (Variables|Default|GetActualReward) (Math|Vector|MakeVector (.x (Variables|/Script/Engine.SceneComponent|GetRelativeLocation (Variables|Default|GetActualReward))) (.y (Variables|/Script/Engine.SceneComponent|GetRelativeLocation (Variables|Default|GetActualReward))) (Math|Float|Lerp (.z (Variables|/Script/Engine.SceneComponent|GetRelativeLocation (Variables|Default|GetActualReward))) 6e+01 _height)) false false))
                        (:Finished
                          (Variables|Default|SetIsRewardStuck false)
                          (Utilities|IsValid (Actor|GetComponentbyClass (Variables|/Script/Engine.ChildActorComponent|GetChildActor (Variables|Default|GetActualReward)) "/Script/Engine.StaticMeshComponent")
                            (:Is%20Valid
                              (Physics|SetSimulatePhysics (Actor|GetComponentbyClass (Variables|/Script/Engine.ChildActorComponent|GetChildActor (Variables|Default|GetActualReward)) "/Script/Engine.StaticMeshComponent") true)
                              (Collision|SetCollisionResponsetoAllChannels (Actor|GetComponentbyClass (Variables|/Script/Engine.ChildActorComponent|GetChildActor (Variables|Default|GetActualReward)) "/Script/Engine.StaticMeshComponent") "ECR_Ignore")
                              (Collision|SetCollisionResponsetoChannel (Actor|GetComponentbyClass (Variables|/Script/Engine.ChildActorComponent|GetChildActor (Variables|Default|GetActualReward)) "/Script/Engine.StaticMeshComponent") "ECC_WorldDynamic" "ECR_Block")
                              (Collision|SetCollisionResponsetoChannel (Actor|GetComponentbyClass (Variables|/Script/Engine.ChildActorComponent|GetChildActor (Variables|Default|GetActualReward)) "/Script/Engine.StaticMeshComponent") "ECC_WorldStatic" "ECR_Block")
                              (Collision|SetCollisionResponsetoChannel (Actor|GetComponentbyClass (Variables|/Script/Engine.ChildActorComponent|GetChildActor (Variables|Default|GetActualReward)) "/Script/Engine.StaticMeshComponent") "ECC_Visibility" "ECR_Block")
                              (Variables|Default|SetCanBeInteract true)
                              (bind _asbp_interactable_boosting_bottle_base (Utilities|Casting|CastToBP_InteractableBoostingBottleBase (Variables|/Script/Engine.ChildActorComponent|GetChildActor (Variables|Default|GetActualReward))))
                              (Utilities|IsValid _asbp_interactable_boosting_bottle_base
                                (:Is%20Valid
                                  (Variables|/Game/Blueprints/GPE/Objects/BP_ObjectBase.BP_ObjectBase_C|SetCanPickup _asbp_interactable_boosting_bottle_base true))
                                (:Is%20Not%20Valid
                                  _)))
                            (:Is%20Not%20Valid
                              _))
                          (Variables|Default|SetActualReward 0)
                          (Utilities|Array|RemoveIndex _allrewards)
                          (if (Utilities|Array|IsEmpty _allrewards)
                            (Variables|Default|SetCanBeInteract false)
                            (Variables|/Game/Blueprints/Components/BP_CustomCursorComponent.BP_CustomCursorComponent_C|SetCursorTexture (Variables|Default|GetBP_CustomCursorComponent) "/Game/Textures/T_CursorNormal.T_CursorNormal")))))
                    (:then_1
                      (Utilities|FlowControl|Delay 0.3)
                      (Transformation|SetRelativeRotation (Variables|Default|GetActualReward) (Math|Rotator|MakeRotator -9e+01 (.pitch (Variables|/Script/Engine.SceneComponent|GetRelativeRotation (Variables|Default|GetActualReward))) (.yaw (Variables|/Script/Engine.SceneComponent|GetRelativeRotation (Variables|Default|GetActualReward)))) false false))))
                (:then_1
                  (Rendering|Components|Light|SetIntensity (Variables|Default|GetRectLight1) 0.0)
                  (Audio|Components|Audio|Stop (Variables|Default|GetSW_VendingMachineIdle))
                  (Utilities|FlowControl|Delay 1.0)
                  (Audio|Components|Audio|Play (Variables|Default|GetBlinkLight) 0.0)
                  (Rendering|Components|Light|SetIntensity _rectlight1 1e+04)
                  (Audio|Components|Audio|Play (Variables|Default|GetSW_VendingMachineIdle) 0.0)
                  (Utilities|FlowControl|Delay 0.1)
                  (Rendering|Components|Light|SetIntensity _rectlight1 0.0)
                  (Audio|Components|Audio|Stop _sw_vendingmachineidle)
                  (Utilities|FlowControl|Delay 0.1)
                  (Rendering|Components|Light|SetIntensity _rectlight1 1e+04)
                  (Audio|Components|Audio|Play _sw_vendingmachineidle 0.0))
                (:then_2
                  (Audio|Components|Audio|Play (Variables|Default|GetVendingDrop) 2.0))))))))))

(event EventInteraction
  (bind _allrewards (Variables|Default|GetAllRewards))
  (bind _coin (Variables|Default|GetCoin))
  (bind _coin_2 (Variables|Default|GetCoin))
  (bind _relativelocation (Variables|/Script/Engine.SceneComponent|GetRelativeLocation _coin_2))
  (|CallParentFunction)
  (if (Variables|Default|GetIsEnabled)
    (if (Variables|Default|GetCanBeInteract)
      (if (Utilities|Array|IsEmpty (Variables|Default|GetAllRewards))
        (Audio|PlaySound2D "/Game/Audio/Sounds/SW_InteractionError.SW_InteractionError" 1.0 1.0 0.0 0 0)
        (Variables|Default|SetCanBeInteract false)
        (Variables|/Game/Blueprints/Components/BP_CustomCursorComponent.BP_CustomCursorComponent_C|SetCursorTexture (Variables|Default|GetBP_CustomCursorComponent) "/Game/Textures/T_CursorNormal.T_CursorNormal")
        (else
          (Utilities|IsValid (Variables|Default|GetGlobalInventory)
            (:Is%20Valid
              (if (Variables|Default|GetIsRewardStuck)
                (if (> (Variables|Default|GetStuckAmount) 0)
                  (if (Variables|/Game/Saves/SG_Settings.SG_Settings_C|GetMouseInteractions (Variables|/Game/BP_GameInstance.BP_GameInstance_C|GetSettings (Utilities|GameInstance)))
                    (Default|StartCapturing (Variables|Default|GetBP_MouseMovementComponent))
                    (else
                      (bind _isa (Utilities|FlowControl|FlipFlop)
                        (:A
                          _)
                        (:B
                          _))
                      (CallFunction|OnMouseMovedEvent 0.0 (Math|Vector2D|MakeVector2D (Math|Float|SelectFloat 1.0 -1.0 _isa) 0.0)))))
                (else
                  (Variables|Default|SetActualReward (Utilities|Array|Get(acopy) (Variables|Default|GetAllRewards)))
                  (if (>= (Variables|/Game/Blueprints/Inventory/BP_GlobalInventory.BP_GlobalInventory_C|GetCoinsBalance (Variables|Default|GetGlobalInventory)) 1)
                    (Math|Integer|DecrementInt (Variables|/Game/Blueprints/Inventory/BP_GlobalInventory.BP_GlobalInventory_C|GetCoinsBalance (Variables|Default|GetGlobalInventory))
                      (:%20%20
                        (bind _result (Math|Integer|IncrementInt (Variables|Default|GetAmountUsed))
                          (:%20%20
                            (Utilities|CheckpointSaveInt (Utilities|String|ToString(Vector) (Transformation|GetActorLocation)) _result)
                            (Audio|Components|Audio|Play (Variables|Default|GetVendingDrop) 0.0)
                            (Variables|Default|SetCanBeInteract false)
                            (Rendering|SetVisibility (Variables|Default|GetCoin) true false)
                            (Audio|PlaySoundatLocation (Variables|Default|GetInteractSound) (Transformation|GetActorLocation) "0, 0, 0" 1.0 1.0 0.0 0 0 0 0)
                            (bind _movement (Timeline|CoinMovement PlayFromStart)
                              (:Update
                                (Transformation|SetRelativeLocation _coin_2 (Math|Vector|MakeVector _movement (.y _relativelocation) (.z _relativelocation)) false false))
                              (:Finished
                                (Rendering|SetVisibility _coin false false)
                                (Transformation|SetRelativeLocation _coin (Variables|Default|GetBaseCoinLocation) false false)
                                (Utilities|IsValid (Variables|Default|GetActualReward)
                                  (:Is%20Valid
                                    (Utilities|FlowControl|Delay 1.0)
                                    (Variables|Default|SetStartZ (.z (Variables|/Script/Engine.SceneComponent|GetRelativeLocation (Variables|Default|GetActualReward))))
                                    (if (Variables|Default|GetIsFirstInteraction)
                                      (Variables|Default|SetIsFirstInteraction false)
                                      (bind (_direction _move _height) (Timeline|PushCan PlayFromStart)
                                        (:Update
                                          (Transformation|SetRelativeLocation (Variables|Default|GetActualReward) (Math|Vector|MakeVector _move (.y (Variables|/Script/Engine.SceneComponent|GetRelativeLocation (Variables|Default|GetActualReward))) (Math|Float|SelectFloat (Variables|Default|GetStartZ) (Math|Float|Lerp (Variables|Default|GetStartZ) 6e+01 _height) (Variables|Default|GetIsRewardStuck))) false false))
                                        (:Finished
                                          (if (Variables|Default|GetIsRewardStuck)
                                            (Variables|Default|SetCanBeInteract true)
                                            (else
                                              (Utilities|IsValid (Actor|GetComponentbyClass (Variables|/Script/Engine.ChildActorComponent|GetChildActor (Variables|Default|GetActualReward)) "/Script/Engine.StaticMeshComponent")
                                                (:Is%20Valid
                                                  (Physics|SetSimulatePhysics (Actor|GetComponentbyClass (Variables|/Script/Engine.ChildActorComponent|GetChildActor (Variables|Default|GetActualReward)) "/Script/Engine.StaticMeshComponent") true)
                                                  (Collision|SetCollisionResponsetoAllChannels (Actor|GetComponentbyClass (Variables|/Script/Engine.ChildActorComponent|GetChildActor (Variables|Default|GetActualReward)) "/Script/Engine.StaticMeshComponent") "ECR_Ignore")
                                                  (Collision|SetCollisionResponsetoChannel (Actor|GetComponentbyClass (Variables|/Script/Engine.ChildActorComponent|GetChildActor (Variables|Default|GetActualReward)) "/Script/Engine.StaticMeshComponent") "ECC_WorldDynamic" "ECR_Block")
                                                  (Collision|SetCollisionResponsetoChannel (Actor|GetComponentbyClass (Variables|/Script/Engine.ChildActorComponent|GetChildActor (Variables|Default|GetActualReward)) "/Script/Engine.StaticMeshComponent") "ECC_WorldStatic" "ECR_Block")
                                                  (Collision|SetCollisionResponsetoChannel (Actor|GetComponentbyClass (Variables|/Script/Engine.ChildActorComponent|GetChildActor (Variables|Default|GetActualReward)) "/Script/Engine.StaticMeshComponent") "ECC_Visibility" "ECR_Block")
                                                  (Variables|Default|SetCanBeInteract true)
                                                  (bind _asbp_interactable_boosting_bottle_base (Utilities|Casting|CastToBP_InteractableBoostingBottleBase (Variables|/Script/Engine.ChildActorComponent|GetChildActor (Variables|Default|GetActualReward))))
                                                  (Utilities|IsValid _asbp_interactable_boosting_bottle_base
                                                    (:Is%20Valid
                                                      (Variables|/Game/Blueprints/GPE/Objects/BP_ObjectBase.BP_ObjectBase_C|SetCanPickup _asbp_interactable_boosting_bottle_base true))
                                                    (:Is%20Not%20Valid
                                                      _)))
                                                (:Is%20Not%20Valid
                                                  _))
                                              (Variables|Default|SetActualReward 0)
                                              (Utilities|Array|RemoveIndex _allrewards)
                                              (if (Utilities|Array|IsEmpty _allrewards)
                                                (Variables|Default|SetCanBeInteract false)
                                                (Variables|/Game/Blueprints/Components/BP_CustomCursorComponent.BP_CustomCursorComponent_C|SetCursorTexture (Variables|Default|GetBP_CustomCursorComponent) "/Game/Textures/T_CursorNormal.T_CursorNormal")))))
                                        (:Rotate
                                          (if (not (stale _output_get))
                                            (Transformation|SetRelativeRotation (Variables|Default|GetActualReward) (Math|Rotator|MakeRotator -9e+01 (.pitch (Variables|/Script/Engine.SceneComponent|GetRelativeRotation (Variables|Default|GetActualReward))) (.yaw (Variables|/Script/Engine.SceneComponent|GetRelativeRotation (Variables|Default|GetActualReward)))) false false))))
                                      (elif (== (Math|Random|RandomIntegerinRange 0 2) 1)
                                        (bind _output_get (Variables|Default|SetIsRewardStuck true))
                                        (Utilities|FlowControl|Sequence
                                          (:then_0
                                            (Variables|Default|SetStuckAmount 10)
                                            (Timeline|PushCan PlayFromStart))
                                          (:then_1
                                            (Utilities|FlowControl|Delay 0.4)
                                            (Audio|Components|Audio|Stop (Variables|Default|GetVendingDrop))))
                                        (else
                                          (Timeline|PushCan PlayFromStart)))))
                                  (:Is%20Not%20Valid
                                    (Development|PrintString "Reward not valid")))))))))
                    (else
                      (Audio|PlaySound2D "/Game/Audio/Sounds/SW_InteractionError.SW_InteractionError" 1.0 1.0 0.0 0 0))))))))))))

(event EventBeginPlay
  (bind _bp_mousemovementcomponent (Variables|Default|GetBP_MouseMovementComponent))
  (bind _allrewards (Variables|Default|GetAllRewards))
  (Utilities|RegisterInteractable)
  (|CallParentFunction)
  (EventDispatchers|AssignOnMouseCapture _bp_mousemovementcomponent (delegate Custom|OnMouseCapture_Event))
  (EventDispatchers|AssignOnMouseUncaptured _bp_mousemovementcomponent (delegate Custom|OnMouseUncaptured_Event))
  (EventDispatchers|AssignOnMouseMoved _bp_mousemovementcomponent (delegate Custom|OnMouseMoved_Event))
  (bind _returnvalue (Actor|GetActorOfClass "/Game/Blueprints/Inventory/BP_GlobalInventory.BP_GlobalInventory_C"))
  (Variables|Default|SetGlobalInventory _returnvalue)
  (Variables|Default|SetBaseCoinLocation (Variables|/Script/Engine.SceneComponent|GetRelativeLocation (Variables|Default|GetCoin)))
  (if (Variables|Default|GetIsEnabled)
    _
    (else
      (Variables|/Game/Blueprints/Components/BP_CustomCursorComponent.BP_CustomCursorComponent_C|SetCursorTexture (Variables|Default|GetBP_CustomCursorComponent) "/Game/Textures/T_CursorNormal.T_CursorNormal")))
  (for _array_element (Components|GetChildrenComponents (Variables|Default|GetDefaultSceneRoot) false)
    (bind _aschild_actor_component (Utilities|Casting|CastToChildActorComponent _array_element))
    (Utilities|Array|Add (Variables|Default|GetAllRewards) _aschild_actor_component))
  (bind (_success _int) (Utilities|CheckpointGetInt (Utilities|String|ToString(Vector) (Transformation|GetActorLocation))))
  (if _success
    (bind _output_get (Variables|Default|SetAmountUsed _int))
    (for _index (range 0 (- _output_get 1))
      (Components|DestroyComponent (Utilities|Array|Get(acopy) _allrewards))
      (Utilities|Array|RemoveIndex _allrewards))
    (if (Utilities|Array|IsEmpty _allrewards)
      (Variables|Default|SetCanBeInteract false)
      (Variables|/Game/Blueprints/Components/BP_CustomCursorComponent.BP_CustomCursorComponent_C|SetCursorTexture (Variables|Default|GetBP_CustomCursorComponent) "/Game/Textures/T_CursorNormal.T_CursorNormal"))))

(event EventDestroyed
  (Utilities|UnregisterInteractable))

(fn ConstructionScript
  (|CallParentFunction)
  (if (Variables|Default|GetIsEnabled)
    _
    (else
      (Rendering|SetCustomDepthStencilValue (Variables|Default|GetMainGlass) 0)
      (Components|DestroyComponent (Variables|Default|GetRectLight1))
      (Rendering|Material|SetMaterial (Variables|Default|GetVendingMachine) 3 "/Game/Materials/Instances/MI_UnlitBlack.MI_UnlitBlack")))
  (for _array_element (Utilities|Array|MakeArray (Variables|Default|GetChildActor) (Variables|Default|GetChildActor1) (Variables|Default|GetChildActor2) (Variables|Default|GetChildActor3) (Variables|Default|GetChildActor4) (Variables|Default|GetChildActor5) (Variables|Default|GetChildActor6) (Variables|Default|GetChildActor7))
    (ChildActorComponent|SetChildActorClass _array_element (Variables|Default|GetInteractableBottleClass))))