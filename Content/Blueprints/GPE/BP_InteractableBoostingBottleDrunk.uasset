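; Boosting bottle interactable that makes the player drunk for the duration of the boost.
; Boost sets the drunk flag, intensifies both cameras' post-process, overrides the master submix with EQ and tap delay, and triggers a server drunk ragdoll.
; It also enables custom depth on every BP_EndoBase actor's primitives and the GameInstance drunk effect.
; ResetBoost reverts these effects, reusing the cached actor list, and both events call their parent versions.
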(event EventBoost
  (params (Player :type BP%20Player%20Object%20Reference))
  (bind _firstpersoncam (Variables|/Game/Blueprints/Player/BP_Player.BP_Player_C|GetFirstPersonCam Player))
  (Variables|/Game/Blueprints/Player/BP_Player.BP_Player_C|SetLastMouseDirection Player "")
  (Variables|/Game/Blueprints/Player/BP_Player.BP_Player_C|SetIsDrunk Player true)
  (bind _structout (Utilities|Struct|SetmembersinPostProcessSettings (Variables|/Script/Engine.CameraComponent|GetPostProcessSettings _firstpersoncam) 3e+01))
  (Variables|/Script/Engine.CameraComponent|SetPostProcessSettings _firstpersoncam _structout)
  (Variables|/Script/Engine.CameraComponent|SetPostProcessSettings (Variables|/Game/Blueprints/Player/BP_Player.BP_Player_C|GetThirdPersonCam Player) _structout)
  (bind _outactors (Actor|GetAllActorsOfClass "/Game/Blueprints/Enemies/BP_EndoBase.BP_EndoBase_C"))
  (for _array_element _outactors
    (for _array_element_2 (Actor|GetComponentsByClass _array_element "/Script/Engine.PrimitiveComponent")
      (Rendering|SetRenderCustomDepth _array_element_2 true)))
  (Class|AudioMixerBlueprintLibrary|SetSubmixEffectChainOverride "/Game/Audio/Filters/SS_Master.SS_Master" (Utilities|Array|MakeArray "/Game/Audio/Filters/SME_EQ.SME_EQ" "/Game/Audio/Filters/SME_TapDelay.SME_TapDelay") 0.0)
  (|CallParentFunction Player)
  (Default|ServerDrunkRagdoll Player (Variables|Default|GetBoostingTime))
  (Default|UpdatePostProcess (Utilities|GameInstance) true false))

(event EventResetBoost
  (params (Player :type BP%20Player%20Object%20Reference))
  (bind _firstpersoncam (Variables|/Game/Blueprints/Player/BP_Player.BP_Player_C|GetFirstPersonCam Player))
  (Variables|/Game/Blueprints/Player/BP_Player.BP_Player_C|SetIsDrunk Player false)
  (bind _structout (Utilities|Struct|SetmembersinPostProcessSettings (Variables|/Script/Engine.CameraComponent|GetPostProcessSettings _firstpersoncam) 0.675))
  (Variables|/Script/Engine.CameraComponent|SetPostProcessSettings _firstpersoncam _structout)
  (Variables|/Script/Engine.CameraComponent|SetPostProcessSettings (Variables|/Game/Blueprints/Player/BP_Player.BP_Player_C|GetThirdPersonCam Player) _structout)
  (for _array_element (stale EventBoost _outactors)
    (for _array_element_2 (Actor|GetComponentsByClass _array_element "/Script/Engine.PrimitiveComponent")
      (Rendering|SetRenderCustomDepth _array_element_2 false)))
  (|CallParentFunction Player)
  (Default|UpdatePostProcess (Utilities|GameInstance) false false)
  (Class|AudioMixerBlueprintLibrary|ClearSubmixEffects "/Game/Audio/Filters/SS_Master.SS_Master"))

(fn ConstructionScript
  (|CallParentFunction))