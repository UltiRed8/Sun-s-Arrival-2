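; Big machine puzzle element that runs once, when triggered after every BP_SunPlaceSpot in the level is completed.
; A gate-based check of all spots starts a timed sequence toggling conveyors, playing the Running effect and triggering the start and final nodes.
; Completion is saved to a checkpoint keyed by actor location.
; On authority BeginPlay, a saved completion marks it done and replays only part of the conveyor sequence.
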(event EventBeginPlay
  (bind _modelconveyor (Variables|Default|GetModelConveyor))
  (Networking|SwitchHasAuthority
    (:Authority
      (bind _outactors (Actor|GetAllActorsOfClass "/Game/Blueprints/GPE/BP_SunPlaceSpot.BP_SunPlaceSpot_C"))
      (Variables|Default|SetAllSunPlaceSpot _outactors)
      (bind (_success _bool) (Utilities|CheckpointGetBool (Utilities|String|ToString(Vector) (Transformation|GetActorLocation))))
      (if _success
        (if _bool
          (Utilities|FlowControl|Sequence
            (:then_0
              ;[0.15 0.15 0.15 0.5] Enabling conveyors
              (|CallParentFunction)
              (Utilities|FlowControl|Delay 12.5)
              ;[0.15 0.15 0.15 0.5] Disabling conveyors
              (|CallParentFunction))
            (:then_1
              (Variables|Default|SetConditionsMet true))
            (:then_2
              (Default|Trigger _modelconveyor)
              (Utilities|FlowControl|Delay 3.5)
              (Default|Trigger _modelconveyor))))))))

(event EventTrigger
  (bind _modelconveyor (Variables|Default|GetModelConveyor))
  (bind _final_conveyor (Variables|Default|GetFinal%20Conveyor))
  (if (not (Variables|Default|GetConditionsMet))
    (Utilities|FlowControl|Gate false :!label _label
      (:Exit
        (|CheckingParts_2
          (:Exit
            (Utilities|FlowControl|Sequence
              (:then_0
                (goto _label Close))
              (:then_1
                ;[0.15 0.15 0.15 0.5] Enabling conveyors
                (|CallParentFunction)
                (Utilities|FlowControl|Delay 12.5)
                ;[0.15 0.15 0.15 0.5] Disabling conveyors
                (|CallParentFunction)
                (Audio|Components|Audio|Play (Variables|Default|GetRunning) 0.0)
                (Utilities|FlowControl|Delay 2.0)
                (Default|Trigger _final_conveyor)
                (Utilities|FlowControl|Delay 2.0)
                (Default|Trigger _final_conveyor)
                (Utilities|FlowControl|Delay 3.0)
                (Default|Trigger _modelconveyor)
                (Utilities|FlowControl|Delay 3.5)
                (Default|Trigger _modelconveyor)
                (Utilities|FlowControl|Delay 1.5)
                (Audio|Components|Audio|Stop (Variables|Default|GetRunning))
                (Default|Trigger (Variables|Default|GetFinalNode))
                (Variables|Default|SetConditionsMet true)
                (Utilities|CheckpointSaveBool (Utilities|String|ToString(Vector) (Transformation|GetActorLocation)) true))
              (:then_2
                (Default|Trigger (Variables|Default|GetStartNode))))))))))

(fn ConstructionScript)