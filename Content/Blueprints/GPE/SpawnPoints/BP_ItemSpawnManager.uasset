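; Manager actor that places an existing item (ItemToPlace) at a random spawn point from its SpawnPoints list on BeginPlay.
; The construction script adds a child actor component and previews the item at the point chosen by DebugSpawnPointIndex.
; TeleportNodeToObject does the reverse, snapping that indexed point to the item's transform for authoring.
; EditorTick draws debug arrows from the manager to every spawn point.
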(event Custom|Init
  (bind _spawnpoints (Variables|Default|GetSpawnPoints))
  (bind _spawnpoints_2 (Variables|Default|GetSpawnPoints))
  (bind _returnvalue (Utilities|Array|Length _spawnpoints))
  (bind _returnvalue_2 (- _returnvalue 1))
  (bind _returnvalue_3 (Math|Random|RandomIntegerinRange 0 _returnvalue_2))
  (bind _output (Utilities|Array|Get(acopy) _spawnpoints_2 _returnvalue_3))
  (if (Utilities|Array|IsNotEmpty (Variables|Default|GetSpawnPoints))
    (Utilities|IsValid (Variables|Default|GetItemToPlace)
      (:Is%20Valid
        (Transformation|SetActorLocationAndRotation (Variables|Default|GetItemToPlace) (Transformation|GetActorLocation _output) (Transformation|GetActorRotation _output))))))

(event Custom|TeleportNodeToObject
  (bind _itemtoplace (Variables|Default|GetItemToPlace))
  (Utilities|IsValid _itemtoplace
    (:Is%20Valid
      (Transformation|SetActorLocationAndRotation (Utilities|Array|Get(acopy) (Variables|Default|GetSpawnPoints) (Math|Integer|Clamp(Integer) (Variables|Default|GetDebugSpawnPointIndex) 0 (- (Utilities|Array|Length (Variables|Default|GetSpawnPoints)) 1))) (Transformation|GetActorLocation _itemtoplace) (Transformation|GetActorRotation _itemtoplace)))))

(event EventBeginPlay
  (CallFunction|Init))

(event Collision|EventActorBeginOverlap
  (params (OtherActor :type Actor%20Object%20Reference)))

(event EventTick
  (params (DeltaSeconds :type Float%20%28single-precision%29)))

(event EventEditorTick
  (if (Utilities|Array|IsNotEmpty (Variables|Default|GetSpawnPoints))
    (for _array_element (Variables|Default|GetSpawnPoints)
      (Rendering|Debug|DrawDebugArrow (Transformation|GetActorLocation) (Transformation|GetActorLocation _array_element) 5e+03 "(R=0.000000,G=0.439009,B=1.000000,A=1.000000)" 0.0 5.0))))

(fn ConstructionScript
  (bind _spawnpoints (Variables|Default|GetSpawnPoints))
  (bind _spawnpoints_2 (Variables|Default|GetSpawnPoints))
  (bind _debugspawnpointindex (Variables|Default|GetDebugSpawnPointIndex))
  (bind _returnvalue (Utilities|Array|Length _spawnpoints_2))
  (bind _returnvalue_2 (- _returnvalue 1))
  (bind _returnvalue_3 (Math|Integer|Clamp(Integer) _debugspawnpointindex 0 _returnvalue_2))
  (bind _output (Utilities|Array|Get(acopy) _spawnpoints _returnvalue_3))
  (AddComponent|AddChildActorComponent false)
  (Utilities|IsValid (Variables|Default|GetItemToPlace)
    (:Is%20Valid
      (Transformation|SetActorLocationAndRotation (Variables|Default|GetItemToPlace) (Transformation|GetActorLocation _output) (Transformation|GetActorRotation _output)))))