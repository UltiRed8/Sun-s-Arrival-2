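; BeatBox arcade cabinet: a four-arrow rhythm game with song selection, scoring, combos and achievements.
; Input drives a Startup, Main Menu, In Level and Scores state machine, with a timeout returning to Startup.
; Each song pairs music with a Level Sequence; spawn events feed child arrow-line actors, and difficulty thins notes but never mines.
; The Konami code toggles EventMode, which gates arrow shake and movement effects.
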(event Custom|Spawn
  (params (Direction :type String) (IsMine :type Boolean))
  (if IsMine
    (switch string Direction :!label _label
      (:Left
        (bind _asbp_beat_box_arrow_line (Utilities|Casting|CastToBP_BeatBoxArrowLine (Variables|/Script/Engine.ChildActorComponent|GetChildActor (Variables|Default|GetArrowLeft))))
        (Default|Spawn _asbp_beat_box_arrow_line IsMine))
      (:Down
        (bind _asbp_beat_box_arrow_line_2 (Utilities|Casting|CastToBP_BeatBoxArrowLine (Variables|/Script/Engine.ChildActorComponent|GetChildActor (Variables|Default|GetArrowDown))))
        (Default|Spawn _asbp_beat_box_arrow_line_2 IsMine))
      (:Up
        (bind _asbp_beat_box_arrow_line_3 (Utilities|Casting|CastToBP_BeatBoxArrowLine (Variables|/Script/Engine.ChildActorComponent|GetChildActor (Variables|Default|GetArrowUp))))
        (Default|Spawn _asbp_beat_box_arrow_line_3 IsMine))
      (:Right
        (bind _asbp_beat_box_arrow_line_4 (Utilities|Casting|CastToBP_BeatBoxArrowLine (Variables|/Script/Engine.ChildActorComponent|GetChildActor (Variables|Default|GetArrowRight))))
        (Default|Spawn _asbp_beat_box_arrow_line_4 IsMine)))
    (else
      (bind _continue (CallFunction|TrySpawn))
      (if _continue
        (goto _label)))))

(event Custom|MainMenu
  (CallFunction|ResetTimeout)
  (Variables|Default|SetState "NewEnumerator1")
  (Default|DisplayMainMenu (Variables|Default|GetBeatBoxWidget))
  (Audio|Components|Audio|SetSound (Variables|Default|GetIdle) "/Game/Audio/Musics/BeatBox/SW_BBSelectionMenu.SW_BBSelectionMenu"))

(event Custom|UpdateScore
  (params (IsNote :type Boolean) (Success :type Boolean) (IsEmpty :type Boolean))
  (bind _beatboxwidget (Variables|Default|GetBeatBoxWidget))
  (if IsEmpty
    (Variables|Default|SetScore (- (Variables|Default|GetScore) 2))
    (Variables|Default|SetCombo 0 :!label _label)
    (if (< (Variables|Default|GetScore) 0) :!label _label_2
      (Variables|Default|SetScore 0))
    (elif IsNote
      (Variables|Default|SetMaxScore (+ (Variables|Default|GetMaxScore) 10))
      (if Success
        (Variables|Default|SetScore (+ (Variables|Default|GetScore) 10))
        (Math|Integer|IncrementInt (Variables|Default|GetCombo)
          (:%20%20
            (goto _label_2)))
        (else
          (goto _label)))
      (else
        (Variables|Default|SetScore (- (Variables|Default|GetScore) 4))
        (Variables|Default|SetCombo 0))))
  (Default|UpdateScores _beatboxwidget (Variables|Default|GetScore) (Variables|Default|GetMaxScore) (Math|Float|Round (* (/ (Math|Conversions|ToFloat(Integer) (Variables|Default|GetScore)) (Math|Conversions|ToFloat(Integer) (Variables|Default|GetMaxScore))) 1e+02)))
  (Default|SetCombo _beatboxwidget (Variables|Default|GetCombo))
  (if (> (Variables|Default|GetCombo) (Variables|Default|GetMaxCombo))
    (Variables|Default|SetMaxCombo (Variables|Default|GetCombo))))

(event Custom|ResetTimeout
  (Variables|Default|SetTimeout 1e+01))

(event Custom|End
  (bind _asbp_game_instance (Utilities|GameInstance))
  (bind _idle (Variables|Default|GetIdle))
  (bind _score (Variables|Default|GetScore))
  (bind _maxscore (Variables|Default|GetMaxScore))
  (bind _outactors (Actor|GetAllActorsOfClass "/Game/Blueprints/GPE/Arcades/BeatBox/BP_BeatBoxNote.BP_BeatBoxNote_C"))
  (for _array_element _outactors
    (Actor|DestroyActor _array_element))
  (Rendering|SetVisibility (Variables|Default|GetArrowUp) false true)
  (Default|DisplayScores (Variables|Default|GetBeatBoxWidget) (Utilities|String|Append (Utilities|Array|Get(acopy) (Variables|Default|GetSongNameList) (Variables|Default|GetSelectedIndex)) (Utilities|Select :Index (Variables|Default|GetDifficulty) :Option%200 " 
Easy" :Option%201 " 
Normal" :Option%202 " 
Hard") (Utilities|String|SelectString " EventCore" "" (Variables|Default|GetEventMode))) _score _maxscore (Math|Float|Round (* (/ (Math|Conversions|ToFloat(Integer) _score) (Math|Conversions|ToFloat(Integer) _maxscore)) 1e+02)) (Variables|Default|GetMaxCombo) (Variables|Default|GetForceEnded))
  (Utilities|FlowControl|Sequence
    (:then_0
      (Audio|Components|Audio|SetSound _idle "/Game/Audio/Musics/BeatBox/SW_BBScores.SW_BBScores")
      (Audio|Components|Audio|Play _idle 0.0)
      (Variables|Default|SetTimeout 2e+01)
      (bind _levelsequenceactor (Variables|Default|GetLevelSequenceActor)
        (:then
          (Sequencer|Player|Stop (Variables|/Script/LevelSequence.LevelSequenceActor|GetSequencePlayer _levelsequenceactor) :!class /Script/MovieScene.MovieSceneSequencePlayer))
        (:else
          _))
      (Variables|Default|SetState "NewEnumerator3")
      (Default|StopBeats (Variables|Default|GetBeatBoxWidget)))
    (:then_1
      (if (Variables|Default|GetEventMode)
        (Default|UnlockAchievement _asbp_game_instance "ACH_BEATBOXTRYHARD")
        (else
          (Default|UnlockAchievement _asbp_game_instance "ACH_BEATBOXBEGINNER"))))))

(event Custom|ToggleDifficulty
  (CallFunction|ResetTimeout)
  (bind _result (Math|Integer|IncrementInt (Variables|Default|GetDifficulty))
    (:%20%20
      (if (>= _result 3)
        (Variables|Default|SetDifficulty 0))
      (Default|SetDifficulty (Variables|Default|GetBeatBoxWidget) (Utilities|String|Append (Utilities|Select :Index (Variables|Default|GetDifficulty) :Option%200 "Easy" :Option%201 "Normal" :Option%202 "Hard") (Utilities|String|SelectString " 
EventCore" "" (stale Custom|ToggleEventMode _output_get)))))))

(event Custom|ToggleEventMode
  (CallFunction|ResetTimeout)
  (bind _output_get (Variables|Default|SetEventMode (not (Variables|Default|GetEventMode))))
  (Default|SetDifficulty (Variables|Default|GetBeatBoxWidget) (Utilities|String|Append (Utilities|Select :Index (Variables|Default|GetDifficulty) :Option%200 "Easy" :Option%201 "Normal" :Option%202 "Hard") (Utilities|String|SelectString " 
EventCore" "" _output_get))))

(event Custom|MoveArrows
  (params (Arrows :type Array%20of%20Booleans) (V_Target :type Float%20%28double-precision%29) (V_InTransition :type Float%20%28double-precision%29) (V_OutTransition :type Float%20%28double-precision%29) (V_TransitionTime :type Float%20%28double-precision%29) (H_Target :type Float%20%28double-precision%29) (H_InTransition :type Float%20%28double-precision%29) (H_OutTransition :type Float%20%28double-precision%29) (H_TransitionTime :type Float%20%28double-precision%29) (R_Target :type Float%20%28double-precision%29) (R_InTransition :type Float%20%28double-precision%29) (R_OutTransition :type Float%20%28double-precision%29) (R_TransitionTime :type Float%20%28double-precision%29))
  (Utilities|CanEvent)
  (for (_array_element _array_index) Arrows
    (if _array_element
      (Default|SetMovement (Variables|/Game/Blueprints/GPE/Arcades/BeatBox/BP_BeatBoxArrowLine.BP_BeatBoxArrowLine_C|GetBP_BeatBoxArrowMoveComponent (Utilities|Array|Get(acopy) (Variables|Default|GetArrows) _array_index)) V_Target V_InTransition V_OutTransition V_TransitionTime H_Target H_InTransition H_OutTransition H_TransitionTime R_Target R_InTransition R_OutTransition R_TransitionTime))))

(event Custom|ShakeArrows
  (params (Arrows :type Array%20of%20Booleans) (V_ShakeTime :type Float%20%28double-precision%29) (V_ShakeStrength :type Float%20%28double-precision%29) (V_ShakeFrequency :type Float%20%28double-precision%29) (V_Offset :type Float%20%28double-precision%29) (H_ShakeTime :type Float%20%28double-precision%29) (H_ShakeStrength :type Float%20%28double-precision%29) (H_ShakeFrequency :type Float%20%28double-precision%29) (H_Offset :type Float%20%28double-precision%29) (R_ShakeTime :type Float%20%28double-precision%29) (R_ShakeStrength :type Float%20%28double-precision%29) (R_ShakeFrequency :type Float%20%28double-precision%29) (R_Offset :type Float%20%28double-precision%29))
  (Utilities|CanEvent)
  (for (_array_element _array_index) Arrows
    (if _array_element
      (Default|SetShake (Variables|/Game/Blueprints/GPE/Arcades/BeatBox/BP_BeatBoxArrowLine.BP_BeatBoxArrowLine_C|GetBP_BeatBoxArrowShakeComponent (Utilities|Array|Get(acopy) (Variables|Default|GetArrows) _array_index)) V_ShakeTime V_ShakeStrength V_ShakeFrequency V_Offset H_ShakeTime H_ShakeStrength H_ShakeFrequency H_Offset R_ShakeTime R_ShakeStrength R_ShakeFrequency R_Offset))))

(event Custom|Startup
  (Variables|Default|SetState "NewEnumerator0")
  (Default|DisplayStartup (Variables|Default|GetBeatBoxWidget))
  (Audio|Components|Audio|SetSound (Variables|Default|GetIdle) "/Game/Audio/Musics/BeatBox/SW_BBIdle.SW_BBIdle"))

(event Custom|SelectMusicUp
  (CallFunction|ResetTimeout)
  (bind _result (Math|Integer|DecrementInt (Variables|Default|GetSelectedIndex))
    (:%20%20
      (if (< _result 0)
        (Variables|Default|SetSelectedIndex (- (Utilities|Array|Length (Variables|Default|GetSongNameList)) 1)))
      (Default|SetSelectedIndex (Variables|Default|GetBeatBoxWidget) (Variables|Default|GetSelectedIndex)))))

(event Custom|SelectMusicDown
  (CallFunction|ResetTimeout)
  (bind _result (Math|Integer|IncrementInt (Variables|Default|GetSelectedIndex))
    (:%20%20
      (if (>= _result (Utilities|Array|Length (Variables|Default|GetSongNameList)))
        (Variables|Default|SetSelectedIndex 0))
      (Default|SetSelectedIndex (Variables|Default|GetBeatBoxWidget) (Variables|Default|GetSelectedIndex)))))

(event Custom|ConfirmSelection
  (bind _levelsequenceactor (Variables|Default|GetLevelSequenceActor))
  (bind _beatboxwidget (Variables|Default|GetBeatBoxWidget))
  (bind _selectedindex (Variables|Default|GetSelectedIndex))
  (bind _idle (Variables|Default|GetIdle))
  (Variables|Default|SetStarted false)
  (for _array_element (Utilities|Array|MakeArray (Variables|/Script/Engine.ChildActorComponent|GetChildActor (Variables|Default|GetArrowUp)) (Variables|/Script/Engine.ChildActorComponent|GetChildActor (Variables|Default|GetArrowDown)) (Variables|/Script/Engine.ChildActorComponent|GetChildActor (Variables|Default|GetArrowLeft)) (Variables|/Script/Engine.ChildActorComponent|GetChildActor (Variables|Default|GetArrowRight)))
    (bind _asbp_beat_box_arrow_line (Utilities|Casting|CastToBP_BeatBoxArrowLine _array_element))
    (Default|Reset (Variables|/Game/Blueprints/GPE/Arcades/BeatBox/BP_BeatBoxArrowLine.BP_BeatBoxArrowLine_C|GetBP_BeatBoxArrowShakeComponent _asbp_beat_box_arrow_line))
    (Default|Reset (Variables|/Game/Blueprints/GPE/Arcades/BeatBox/BP_BeatBoxArrowLine.BP_BeatBoxArrowLine_C|GetBP_BeatBoxArrowMoveComponent _asbp_beat_box_arrow_line)))
  (Variables|Default|SetState "NewEnumerator2")
  (Variables|Default|SetForceEnded false)
  (Rendering|SetVisibility (Variables|Default|GetArrowUp) true true)
  (Default|UpdateScores _beatboxwidget 0 0 100)
  (Default|SetCombo _beatboxwidget)
  (Default|DisplayinGame _beatboxwidget)
  (Audio|Components|Audio|SetSound _idle (Utilities|Array|Get(acopy) (Variables|Default|GetMusics) _selectedindex))
  (Audio|Components|Audio|Stop _idle)
  (Variables|Default|SetTimeout -1.0)
  (Class|LevelSequenceActor|SetSequence _levelsequenceactor (Utilities|Array|Get(acopy) (Variables|Default|GetLevelSequences) _selectedindex))
  (Utilities|FlowControl|Delay 1.0)
  (Sequencer|Player|Play (Variables|/Script/LevelSequence.LevelSequenceActor|GetSequencePlayer _levelsequenceactor) :!class /Script/MovieScene.MovieSceneSequencePlayer)
  (Variables|Default|SetMaxCombo 0)
  (Variables|Default|SetCombo 0)
  (Variables|Default|SetMaxScore 0)
  (Variables|Default|SetScore 0)
  (Utilities|FlowControl|Delay 1.0)
  (Audio|Components|Audio|Play _idle 0.0)
  (Default|SetupBeatDelay (Variables|Default|GetBeatBoxWidget) (Utilities|Array|Get(acopy) (Variables|Default|GetBeatDelays) (Variables|Default|GetSelectedIndex)))
  (Utilities|FlowControl|Delay 1.0)
  (Variables|Default|SetStarted true))

(event Custom|InteractUp
  (bind _asbp_beat_box_arrow_line (Utilities|Casting|CastToBP_BeatBoxArrowLine (Variables|/Script/Engine.ChildActorComponent|GetChildActor (Variables|Default|GetArrowUp))))
  (Default|Press _asbp_beat_box_arrow_line))

(event Custom|InteractDown
  (bind _asbp_beat_box_arrow_line (Utilities|Casting|CastToBP_BeatBoxArrowLine (Variables|/Script/Engine.ChildActorComponent|GetChildActor (Variables|Default|GetArrowDown))))
  (Default|Press _asbp_beat_box_arrow_line))

(event Custom|InteractRight
  (bind _asbp_beat_box_arrow_line (Utilities|Casting|CastToBP_BeatBoxArrowLine (Variables|/Script/Engine.ChildActorComponent|GetChildActor (Variables|Default|GetArrowRight))))
  (Default|Press _asbp_beat_box_arrow_line))

(event Custom|InteractLeft
  (bind _asbp_beat_box_arrow_line (Utilities|Casting|CastToBP_BeatBoxArrowLine (Variables|/Script/Engine.ChildActorComponent|GetChildActor (Variables|Default|GetArrowLeft))))
  (Default|Press _asbp_beat_box_arrow_line))

(event EventBeginPlay
  (bind _arrows (Variables|Default|GetArrows))
  (|CallParentFunction)
  (bind _asuw_arcade_beat_box (Utilities|Casting|CastToUW_ArcadeBeatBox (UserInterface|GetWidget (Variables|Default|GetWidget))))
  (Variables|Default|SetBeatBoxWidget _asuw_arcade_beat_box)
  (bind _asbp_beat_box_arrow_line (Utilities|Casting|CastToBP_BeatBoxArrowLine (Variables|/Script/Engine.ChildActorComponent|GetChildActor (Variables|Default|GetArrowLeft))))
  (Variables|/Game/Blueprints/GPE/Arcades/BeatBox/BP_BeatBoxArrowLine.BP_BeatBoxArrowLine_C|SetRotation _asbp_beat_box_arrow_line -9e+01)
  (Utilities|Array|Add _arrows _asbp_beat_box_arrow_line)
  (bind _asbp_beat_box_arrow_line_2 (Utilities|Casting|CastToBP_BeatBoxArrowLine (Variables|/Script/Engine.ChildActorComponent|GetChildActor (Variables|Default|GetArrowDown))))
  (Variables|/Game/Blueprints/GPE/Arcades/BeatBox/BP_BeatBoxArrowLine.BP_BeatBoxArrowLine_C|SetRotation _asbp_beat_box_arrow_line_2 1.8e+02)
  (Utilities|Array|Add _arrows _asbp_beat_box_arrow_line_2)
  (bind _asbp_beat_box_arrow_line_3 (Utilities|Casting|CastToBP_BeatBoxArrowLine (Variables|/Script/Engine.ChildActorComponent|GetChildActor (Variables|Default|GetArrowUp))))
  (Variables|/Game/Blueprints/GPE/Arcades/BeatBox/BP_BeatBoxArrowLine.BP_BeatBoxArrowLine_C|SetRotation _asbp_beat_box_arrow_line_3 0.0)
  (Utilities|Array|Add _arrows _asbp_beat_box_arrow_line_3)
  (bind _asbp_beat_box_arrow_line_4 (Utilities|Casting|CastToBP_BeatBoxArrowLine (Variables|/Script/Engine.ChildActorComponent|GetChildActor (Variables|Default|GetArrowRight))))
  (Variables|/Game/Blueprints/GPE/Arcades/BeatBox/BP_BeatBoxArrowLine.BP_BeatBoxArrowLine_C|SetRotation _asbp_beat_box_arrow_line_4 9e+01)
  (Utilities|Array|Add _arrows _asbp_beat_box_arrow_line_4)
  (Rendering|SetVisibility (Variables|Default|GetArrowUp) false false)
  (bind _returnvalue (Game|SpawnActorfromClass :Class "/Script/LevelSequence.LevelSequenceActor" :CollisionHandlingOverride "Undefined" :TransformScaleMethod "MultiplyWithRoot" :LevelSequenceAsset 0 :Instigator 0))
  (Variables|Default|SetLevelSequenceActor _returnvalue))

(event EventTick
  (params (DeltaSeconds :type Float%20%28single-precision%29))
  (|CallParentFunction DeltaSeconds)
  (if (not (== (Variables|Default|GetTimeout) -1.0))
    (if (>= (Variables|Default|GetTimeout) 0.0)
      (Variables|Default|SetTimeout (- (Variables|Default|GetTimeout) DeltaSeconds))
      (goto _label Reset)
      (else
        (Utilities|FlowControl|DoOnce false :!label _label
          (:Completed
            (CallFunction|Startup)))))))

(event EventKonamiCodeTriggered
  (|CallParentFunction)
  (CallFunction|ToggleEventMode))

(event EventEnteredInputWithoutKonami
  (params (Input :type String))
  (|CallParentFunction Input)
  (switch Utilities|FlowControl|Switch|SwitchonE_BeatBoxState (Variables|Default|GetState)
    (:NewEnumerator0
      (switch string Input
        (:E
          (CallFunction|MainMenu))))
    (:NewEnumerator1
      (switch string Input
        (:E
          (CallFunction|ConfirmSelection))
        (:U
          (CallFunction|SelectMusicUp))
        (:D
          (CallFunction|SelectMusicDown))
        (:X
          (CallFunction|ToggleDifficulty))))
    (:NewEnumerator2
      (switch string Input
        (:U
          (CallFunction|InteractUp))
        (:D
          (CallFunction|InteractDown))
        (:L
          (CallFunction|InteractLeft))
        (:R
          (CallFunction|InteractRight))
        (:A
          (if (Variables|Default|GetStarted)
            (Variables|Default|SetForceEnded true)
            (CallFunction|End)))))
    (:NewEnumerator3
      (switch string Input
        (:E
          (CallFunction|MainMenu))))))

(fn ConstructionScript
  (|CallParentFunction))

(fn TrySpawn
  (bind _result (Math|Integer|IncrementInt (Variables|Default|GetCurrentCount))
    (:%20%20
      (if (>= _result (Utilities|Select :Index (Variables|Default|GetDifficulty) :Option%200 3 :Option%201 2 :Option%202 1))
        (Variables|Default|SetCurrentCount 0)
        (return true)
        (else
          (return false))))))