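; One arrow lane of the BeatBox arcade rhythm game, spawning notes or mines attached to itself.
; A box overlap tracks notes in range; Press consumes one, favoring regular notes over mines, and reports hit, mine or empty press to BP_BeatBox.
; Timelines animate the arrow's material color and scale on each press.
; Tick rebuilds the lane transform from its cached default plus Shake and Move component offsets.
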(event OnComponentBeginOverlap(Box)
  (params (OverlappedComponent :type Primitive%20Component%20Object%20Reference) (OtherActor :type Actor%20Object%20Reference) (OtherComp :type Primitive%20Component%20Object%20Reference) (OtherBodyIndex :type Integer) (bFromSweep :type Boolean) (SweepResult :type Hit%20Result%20Structure%20%28by%20ref%29))
  (bind _asbp_beat_box_note (Utilities|Casting|CastToBP_BeatBoxNote OtherActor))
  (Utilities|Array|Add (Variables|Default|GetTargetArrows) _asbp_beat_box_note))

(event OnComponentEndOverlap(Box)
  (params (OverlappedComponent :type Primitive%20Component%20Object%20Reference) (OtherActor :type Actor%20Object%20Reference) (OtherComp :type Primitive%20Component%20Object%20Reference) (OtherBodyIndex :type Integer))
  (bind _asbp_beat_box_note (Utilities|Casting|CastToBP_BeatBoxNote OtherActor))
  (Utilities|Array|RemoveItem (Variables|Default|GetTargetArrows) _asbp_beat_box_note))

(event Custom|Spawn
  (params (IsMine :type Boolean))
  (bind _returnvalue (Game|SpawnActorfromClass "/Game/Blueprints/GPE/Arcades/BeatBox/BP_BeatBoxNote.BP_BeatBoxNote_C" (Math|Transform|MakeTransform "0, 0, 0" "0, 0, 0" "1.000000,1.000000,1.000000") "Undefined" "MultiplyWithRoot" 0 IsMine (Variables|Default|GetBeatBoxArcade) 0))
  (Transformation|AttachComponentToComponent _returnvalue (Variables|Default|GetDefaultSceneRoot) "None" "KeepRelative" "KeepRelative" "KeepRelative" true))

(event Custom|Press
  (bind _beatboxarcade (Variables|Default|GetBeatBoxArcade))
  (bind _closest (CallFunction|GetClosestNote))
  (Utilities|IsValid _closest
    (:Is%20Valid
      (Default|UpdateScore _beatboxarcade (not (Variables|/Game/Blueprints/GPE/Arcades/BeatBox/BP_BeatBoxNote.BP_BeatBoxNote_C|GetIsMine _closest)) true false)
      (if (Variables|/Game/Blueprints/GPE/Arcades/BeatBox/BP_BeatBoxNote.BP_BeatBoxNote_C|GetIsMine _closest)
        (Actor|DestroyActor _closest)
        (Utilities|FlowControl|Sequence
          (:then_0
            (bind _red (Timeline|PressAnimation PlayFromStart)
              (:Update
                (Rendering|Material|SetVectorParameterValue (Variables|Default|GetMaterial) "Color" (Math|Color|MakeColor _red 1.0 1.0) :!class /Script/Engine.MaterialInstanceDynamic))))
          (:then_1
            (bind _scale (Timeline|ArrowScale PlayFromStart)
              (:Update
                (Transformation|SetRelativeScale3D (Variables|Default|GetArrow) (Math|Vector|MakeVector _scale _scale _scale))))))
        (else
          (Actor|DestroyActor _closest)
          (Utilities|FlowControl|Sequence
            (:then_0
              (bind _green (Timeline|Timeline PlayFromStart)
                (:Update
                  (Rendering|Material|SetVectorParameterValue (Variables|Default|GetMaterial) "Color" (Math|Color|MakeColor 1.0 _green 1.0) :!class /Script/Engine.MaterialInstanceDynamic))))
            (:then_1
              (Timeline|ArrowScale PlayFromStart))))))
    (:Is%20Not%20Valid
      (Default|UpdateScore _beatboxarcade true false true)
      (Utilities|FlowControl|Sequence
        (:then_0
          (Timeline|PressAnimation PlayFromStart))
        (:then_1
          (Timeline|ArrowScale PlayFromStart))))))

(event EventBeginPlay
  (Variables|Default|SetDefaultTransform (Transformation|GetWorldTransform (Variables|Default|GetDefaultSceneRoot)))
  (Utilities|FlowControl|DelayUntilNextTick)
  (Transformation|SetRelativeRotation (Variables|Default|GetArrow) (Math|Rotator|MakeRotator 0.0 0.0 (Variables|Default|GetRotation)) false false)
  (bind _returnvalue (Rendering|Material|CreateDynamicMaterialInstance (Variables|Default|GetArrow) 0 "/Game/Textures/Arcades/MAT_Arrow.MAT_Arrow" "None" :!class /Script/Engine.PrimitiveComponent))
  (Variables|Default|SetMaterial _returnvalue)
  (bind _returnvalue_2 (Actor|GetActorOfClass "/Game/Blueprints/GPE/Arcades/BeatBox/BP_BeatBox.BP_BeatBox_C"))
  (Variables|Default|SetBeatBoxArcade _returnvalue_2))

(event EventTick
  (params (DeltaSeconds :type Float%20%28single-precision%29))
  (bind _bp_beatboxarrowshakecomponent (Variables|Default|GetBP_BeatBoxArrowShakeComponent))
  (bind _bp_beatboxarrowmovecomponent (Variables|Default|GetBP_BeatBoxArrowMoveComponent))
  (bind _defaulttransform (Variables|Default|GetDefaultTransform))
  (bind _result (Variables|/Game/Blueprints/GPE/Arcades/BeatBox/BP_BeatBoxArrowShakeComponent.BP_BeatBoxArrowShakeComponent_C|GetResult _bp_beatboxarrowshakecomponent))
  (bind _result_2 (Variables|/Game/Blueprints/GPE/Arcades/BeatBox/BP_BeatBoxArrowMoveComponent.BP_BeatBoxArrowMoveComponent_C|GetResult _bp_beatboxarrowmovecomponent))
  (Transformation|SetWorldTransform (Variables|Default|GetDefaultSceneRoot) (Math|Transform|MakeTransform (+ (+ (.location _defaulttransform) (* (Transformation|GetActorForwardVector) (.y (.location _result))) (* (Transformation|GetActorRightVector) (.z (.location _result)))) (* (Transformation|GetActorForwardVector) (.z (.location _result_2))) (* (Transformation|GetActorRightVector) (.y (.location _result_2)))) (Math|Rotator|MakeRotator (.roll (.rotation _defaulttransform)) (.pitch (.rotation _defaulttransform)) (.yaw (.rotation _defaulttransform))) (.scale _defaulttransform)) false false)
  (Class|Actor|AddActorWorldRotation (Math|Rotator|CombineRotators (Math|Vector|RotatorfromAxisandAngle (Transformation|GetActorUpVector) (.roll (.rotation _result))) (Math|Vector|RotatorfromAxisandAngle (Transformation|GetActorUpVector) (.roll (.rotation _result_2))))))

(fn ConstructionScript
  (Transformation|SetRelativeRotation (Variables|Default|GetArrow) (Math|Rotator|MakeRotator 0.0 0.0 (Variables|Default|GetRotation)) false false))

(fn GetClosestNote
  (LocalVariables|SetClosestNote 0)
  (bind _array_element (Utilities|Array|ForEachLoopwithBreak (Variables|Default|GetTargetArrows) :!label _label)
    (:LoopBody
      (if (Variables|/Game/Blueprints/GPE/Arcades/BeatBox/BP_BeatBoxNote.BP_BeatBoxNote_C|GetIsMine _array_element)
        (LocalVariables|SetClosestNote _array_element)
        (else
          (LocalVariables|SetClosestNote _array_element)
          (goto _label Break))))
    (:Completed
      (return (LocalVariables|GetClosestNote)))))