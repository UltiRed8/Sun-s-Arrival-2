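; Music manager for the Darkventure arcade game that tracks the current music state: exterior, interior, unknown presence or one of two battle variants.
; On BeginPlay or a state change, it selects the matching sound and broadcasts it through OnMusicChanged rather than playing it directly.
; It then sets a per-track rhythm on registered actors and recolors wall torches blue for battle music, warm otherwise.
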(event Custom|Update
  (bind _music (Variables|Default|GetMusic))
  (bind _returnvalue (Utilities|Select :Index _music :NewEnumerator0 "/Game/Audio/Musics/Darkventure/SW_DVExterior.SW_DVExterior" :NewEnumerator1 "/Game/Audio/Musics/Darkventure/SW_DVInterior.SW_DVInterior" :NewEnumerator2 "/Game/Audio/Musics/Darkventure/SW_DVUnknownPresence.SW_DVUnknownPresence" :NewEnumerator3 "/Game/Audio/Musics/Darkventure/SW_DVBattle.SW_DVBattle" :NewEnumerator4 "/Game/Audio/Musics/Darkventure/SW_DVBattleAlternative.SW_DVBattleAlternative"))
  (Variables|Default|SetCurrentMusic _returnvalue)
  (Default|CallOnMusicChanged _returnvalue)
  (for _array_element (Variables|Default|GetRhythmActors)
    (Utilities|IsValid _array_element
      (:Is%20Valid
        (Default|SetRhythm _array_element (Utilities|Select :Index _music :NewEnumerator0 1.375 :NewEnumerator1 1.375 :NewEnumerator2 0.6875 :NewEnumerator3 2.75 :NewEnumerator4 2.75))
        (bind _asbp_dvwall_torch (Utilities|Casting|CastToBP_DVWallTorch _array_element))
        (switch Utilities|FlowControl|Switch|SwitchonE_DVMusic _music
          (:NewEnumerator0
            (Default|SetColor _asbp_dvwall_torch "(R=1.000000,G=1.000000,B=1.000000,A=1.000000)" "(R=1.000000,G=0.545725,B=0.000000,A=1.000000)" :!label _label))
          (:NewEnumerator1
            (goto _label))
          (:NewEnumerator2
            (goto _label))
          (:NewEnumerator3
            (Default|SetColor _asbp_dvwall_torch "(R=0.000000,G=0.817369,B=1.000000,A=1.000000)" "(R=0.002827,G=0.398694,B=1.000000,A=1.000000)" :!label _label_2))
          (:NewEnumerator4
            (goto _label_2)))))))

(event Custom|SetMusic
  (params (Music :type E_DVMusic%20Enum :default "NewEnumerator0"))
  (if (Utilities|Enum|NotEqual(Enum) Music (Variables|Default|GetMusic))
    (Variables|Default|SetMusic Music)
    (CallFunction|Update)))

(event Custom|RegisterActor
  (params (NewItem :type BP%20DV%20Rhythmed%20Actor%20Object%20Reference%20%28by%20ref%29))
  (Utilities|Array|AddUnique (Variables|Default|GetRhythmActors) NewItem))

(event Custom|UnregisterActor
  (params (Item :type BP%20DV%20Rhythmed%20Actor%20Object%20Reference%20%28by%20ref%29))
  (Utilities|Array|RemoveItem (Variables|Default|GetRhythmActors) Item))

(event EventBeginPlay
  (CallFunction|Update))

(fn ConstructionScript)