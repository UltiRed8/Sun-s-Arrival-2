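; Arcade cabinet for the Darkventure minigame, switching between an idle startup screen and in-level play, with an inactivity timeout back to startup.
; It streams in LVL_Darkventure, retries to find and link its character, and forwards cabinet inputs as movement, attack and interact.
; A spawned music manager drives level music, and an in-game widget shows health.
; Game end shows defeat or victory, unlocks an achievement on a win, then reloads the level.
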(event Custom|Event_OnMusicChanged
  (params (Music :type Sound%20Base%20Object%20Reference))
  (bind _idle (Variables|Default|GetIdle))
  (switch Utilities|FlowControl|Switch|SwitchonE_BeatBoxState (Variables|Default|GetState)
    (:NewEnumerator2
      (Audio|Components|Audio|SetSound _idle Music)
      (Audio|Components|Audio|Play _idle 0.0))))

(event Custom|ResetTimeout
  (Variables|Default|SetTimeout 1e+01))

(event Custom|Startup
  (Development|SetHiddeninGame (Variables|Default|GetPlane) true false)
  (CallFunction|EventonMusicChanged "/Game/Audio/Musics/Darkventure/SW_DVIdle.SW_DVIdle")
  (Variables|Default|SetState "NewEnumerator0")
  (Rendering|SetVisibility (Variables|Default|GetWidgetInGame) false false))

(event Custom|EndGame
  (Variables|Default|SetTimeout -1.0)
  (bind _asuw_dv_in_game (Utilities|Casting|CastToUW_DV_InGame (UserInterface|GetWidget (Variables|Default|GetWidgetInGame))))
  (Default|GameOver _asuw_dv_in_game (<= (Variables|/Game/Blueprints/GPE/Arcades/Darkventure/BP_DVCharacter.BP_DVCharacter_C|GetLife (Variables|Default|GetCharacter)) 0))
  (CallFunction|PlaySound (select (<= (Variables|/Game/Blueprints/GPE/Arcades/Darkventure/BP_DVCharacter.BP_DVCharacter_C|GetLife (Variables|Default|GetCharacter)) 0) "/Game/Audio/Sounds/SW_DVGameOver.SW_DVGameOver" "/Game/Audio/Sounds/SW_DVVictory.SW_DVVictory") 1.0 0.0)
  (Audio|Components|Audio|SetVolumeMultiplier (Variables|Default|GetIdle) 0.0 :!class /Script/Engine.AudioComponent)
  (if (>= (Variables|/Game/Blueprints/GPE/Arcades/Darkventure/BP_DVCharacter.BP_DVCharacter_C|GetLife (Variables|Default|GetCharacter)) 1)
    (Default|UnlockAchievement (Utilities|GameInstance) "ACH_DARKVENTURE"))
  (Utilities|FlowControl|Delay 3.0)
  (Default|Reset _asuw_dv_in_game)
  (Variables|Default|SetCharacter 0)
  (Default|SetMusic (Variables|Default|GetMusicManager) "NewEnumerator0")
  (CallFunction|ResetLevel)
  (Audio|Components|Audio|SetVolumeMultiplier (Variables|Default|GetIdle) 1.0 :!class /Script/Engine.AudioComponent)
  (CallFunction|Startup))

(event Custom|UpdateLifeUI
  (params (NewHealth :type Integer))
  (bind _asuw_dv_in_game (Utilities|Casting|CastToUW_DV_InGame (UserInterface|GetWidget (Variables|Default|GetWidgetInGame))))
  (Default|UpdateHealth (Variables|/Game/Widgets/Arcades/UW_DV_InGame.UW_DV_InGame_C|GetUW_DV_LifePart _asuw_dv_in_game) NewHealth)
  (if (== NewHealth 0)
    (CallFunction|EndGame)))

(event Custom|Reset%20Level
  (Class|GameplayStatics|UnloadStreamLevelbySoftObjectPtr "/Game/Levels/LVL_Darkventure.LVL_Darkventure" true)
  (Class|GameplayStatics|LoadStreamLevelbySoftObjectPtr "/Game/Levels/LVL_Darkventure.LVL_Darkventure" true true)
  (Default|Update (Variables|Default|GetMusicManager))
  (Utilities|WhileInvalid (Variables|Default|GetCharacter) 0.1 15
    (:Valid
      (bind _asuw_dv_in_game (Utilities|Casting|CastToUW_DV_InGame (UserInterface|GetWidget (Variables|Default|GetWidgetInGame)))
        (:then
          (Variables|/Game/Blueprints/GPE/Arcades/Darkventure/BP_DVCharacter.BP_DVCharacter_C|SetArcadeWidget (Variables|Default|GetCharacter) _asuw_dv_in_game))
        (:CastFailed
          _))
      (Variables|/Game/Blueprints/GPE/Arcades/Darkventure/BP_DVCharacter.BP_DVCharacter_C|SetArcade (Variables|Default|GetCharacter) self)
      (Variables|Default|SetFirstStart true))
    (:Getter
      (bind _returnvalue (Actor|GetActorOfClass "/Game/Blueprints/GPE/Arcades/Darkventure/BP_DVCharacter.BP_DVCharacter_C"))
      (Variables|Default|SetCharacter _returnvalue))))

(event Custom|PlaySound
  (params (NewSound :type Sound%20Base%20Object%20Reference) (NewPitchMultiplier :type Float%20%28single-precision%29) (StartTime :type Float%20%28single-precision%29))
  (bind _sound (Variables|Default|GetSound))
  (Audio|Components|Audio|SetSound _sound NewSound)
  (Audio|Components|Audio|SetPitchMultiplier _sound NewPitchMultiplier)
  (Audio|Components|Audio|Play _sound StartTime))

(event EventTick
  (params (DeltaSeconds :type Float%20%28single-precision%29))
  (|CallParentFunction DeltaSeconds)
  (if (not (== (Variables|Default|GetTimeout) -1.0))
    (if (>= (Variables|Default|GetTimeout) 0.0)
      (Variables|Default|SetTimeout (- (Variables|Default|GetTimeout) DeltaSeconds))
      (goto _label Reset)
      (else
        (Utilities|FlowControl|DoOnce false :!label _label
          (:Completed
            (CallFunction|Startup)))))))

(event EventBeginPlay
  (bind _returnvalue (Game|SpawnActorfromClass "/Game/Blueprints/GPE/Arcades/Darkventure/BP_DVMusicManager.BP_DVMusicManager_C" (Math|Transform|MakeTransform "0, 0, 0" "0, 0, 0" "1.000000,1.000000,1.000000") "Undefined" "MultiplyWithRoot" 0 0))
  (bind _output_get (Variables|Default|SetMusicManager _returnvalue))
  (EventDispatchers|AssignOnMusicChanged _output_get (delegate Custom|Event_OnMusicChanged))
  (CallFunction|ResetLevel))

(event EventUpPressed
  (Utilities|DoOnceGate
    (:OutA
      (|CallParentFunction)
      (switch Utilities|FlowControl|Switch|SwitchonE_BeatBoxState (Variables|Default|GetState)
        (:NewEnumerator2
          (bind _character (Variables|Default|GetCharacter)
            (:then
              (Default|UpdateDirection _character "1.000000,0.000000,0.000000")
              (CallFunction|ResetTimeout))
            (:else)))))
    (:OutB
      (|CallParentFunction)
      (switch Utilities|FlowControl|Switch|SwitchonE_BeatBoxState (Variables|Default|GetState)
        (:NewEnumerator2
          (bind _character_2 (Variables|Default|GetCharacter)
            (:then
              (Default|UpdateDirection _character_2 "-1.000000,0.000000,0.000000")
              (CallFunction|ResetTimeout))
            (:else)))))))

(event EventUpReleased
  (Utilities|DoOnceGate) ; enters at InB
)

(event EventAPressed
  (|CallParentFunction)
  (switch Utilities|FlowControl|Switch|SwitchonE_BeatBoxState (Variables|Default|GetState)
    (:NewEnumerator2
      (Default|Attack (Variables|Default|GetCharacter))
      (CallFunction|ResetTimeout))))

(event EventBPressed
  (|CallParentFunction)
  (switch Utilities|FlowControl|Switch|SwitchonE_BeatBoxState (Variables|Default|GetState)
    (:NewEnumerator2
      (Default|Interact (Variables|Default|GetCharacter))
      (CallFunction|ResetTimeout))))

(event EventDownPressed
  (Utilities|DoOnceGate
    (:OutA
      (|CallParentFunction)
      (switch Utilities|FlowControl|Switch|SwitchonE_BeatBoxState (Variables|Default|GetState)
        (:NewEnumerator2
          (bind _character (Variables|Default|GetCharacter)
            (:then
              (Default|UpdateDirection _character "-1.000000,0.000000,0.000000")
              (CallFunction|ResetTimeout))
            (:else)))))
    (:OutB
      (|CallParentFunction)
      (switch Utilities|FlowControl|Switch|SwitchonE_BeatBoxState (Variables|Default|GetState)
        (:NewEnumerator2
          (bind _character_2 (Variables|Default|GetCharacter)
            (:then
              (Default|UpdateDirection _character_2 "1.000000,0.000000,0.000000")
              (CallFunction|ResetTimeout))
            (:else)))))))

(event EventEnteredInputWithoutKonami
  (params (Input :type String))
  (|CallParentFunction Input)
  (if (Utilities|Enum|Equal(Enum) Input "E")
    (switch Utilities|FlowControl|Switch|SwitchonE_BeatBoxState (Variables|Default|GetState)
      (:NewEnumerator0
        (Development|SetHiddeninGame (Variables|Default|GetPlane) false false)
        (Rendering|SetVisibility (Variables|Default|GetWidgetInGame) true false)
        (Variables|Default|SetState "NewEnumerator2")
        (bind _musicmanager (Variables|Default|GetMusicManager)
          (:then
            (CallFunction|EventonMusicChanged (Variables|/Game/Blueprints/GPE/Arcades/Darkventure/BP_DVMusicManager.BP_DVMusicManager_C|GetCurrentMusic _musicmanager))
            (CallFunction|ResetTimeout)
            (if (Variables|Default|GetFirstStart)
              (Variables|Default|SetFirstStart false)
              (CallFunction|PlaySound "/Game/Audio/Sounds/SW_DVGameStart.SW_DVGameStart" 2.0 0.0)))
          (:else))))))

(event EventDownReleased
  (Utilities|DoOnceGate) ; enters at InB
)

(event EventLeftPressed
  (Utilities|DoOnceGate
    (:OutA
      (|CallParentFunction)
      (switch Utilities|FlowControl|Switch|SwitchonE_BeatBoxState (Variables|Default|GetState)
        (:NewEnumerator2
          (bind _character (Variables|Default|GetCharacter)
            (:then
              (Default|UpdateDirection _character "0.000000,-1.000000,0.000000")
              (CallFunction|ResetTimeout))
            (:else)))))
    (:OutB
      (|CallParentFunction)
      (switch Utilities|FlowControl|Switch|SwitchonE_BeatBoxState (Variables|Default|GetState)
        (:NewEnumerator2
          (bind _character_2 (Variables|Default|GetCharacter)
            (:then
              (Default|UpdateDirection _character_2 "0.000000,1.000000,0.000000")
              (CallFunction|ResetTimeout))
            (:else)))))))

(event EventLeftReleased
  (Utilities|DoOnceGate) ; enters at InB
)

(event EventRightPressed
  (Utilities|DoOnceGate
    (:OutA
      (|CallParentFunction)
      (switch Utilities|FlowControl|Switch|SwitchonE_BeatBoxState (Variables|Default|GetState)
        (:NewEnumerator2
          (bind _character (Variables|Default|GetCharacter)
            (:then
              (Default|UpdateDirection _character "0.000000,1.000000,0.000000")
              (CallFunction|ResetTimeout))
            (:else)))))
    (:OutB
      (|CallParentFunction)
      (switch Utilities|FlowControl|Switch|SwitchonE_BeatBoxState (Variables|Default|GetState)
        (:NewEnumerator2
          (bind _character_2 (Variables|Default|GetCharacter)
            (:then
              (Default|UpdateDirection _character_2 "0.000000,-1.000000,0.000000")
              (CallFunction|ResetTimeout))
            (:else)))))))

(event EventRightReleased
  (Utilities|DoOnceGate) ; enters at InB
)

(fn ConstructionScript
  (|CallParentFunction))