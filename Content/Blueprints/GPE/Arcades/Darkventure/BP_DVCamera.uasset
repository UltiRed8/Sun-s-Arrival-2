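; BP_DVCamera is a follow actor for the Darkventure arcade game that tracks the player character.
; On BeginPlay it finds the BP_DVCharacter, then each tick snaps itself to that character's location with a fixed upward offset.
; Each tick it also draws colored debug lines from itself to its North, South, West and East target components.
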(event EventBeginPlay
  (bind _returnvalue (Actor|GetActorOfClass "/Game/Blueprints/GPE/Arcades/Darkventure/BP_DVCharacter.BP_DVCharacter_C"))
  (Variables|Default|SetCharacter _returnvalue))

(event EventTick
  (params (DeltaSeconds :type Float%20%28single-precision%29))
  (bind _returnvalue (Transformation|GetActorLocation))
  (Utilities|FlowControl|Sequence
    (:then_0
      (bind _character (Variables|Default|GetCharacter)
        (:then
          (Transformation|SetActorLocation (+ (Transformation|GetActorLocation _character) "0.000000,0.000000,50.000000") false false))
        (:else)))
    (:then_1
      (Rendering|Debug|DrawDebugLine _returnvalue (Transformation|GetWorldLocation (Variables|Default|GetNorthTarget)) "(R=1.000000,G=0.000000,B=0.000000,A=1.000000)" 0.0 0.0)
      (Rendering|Debug|DrawDebugLine _returnvalue (Transformation|GetWorldLocation (Variables|Default|GetSouthTarget)) "(R=0.000000,G=0.000000,B=1.000000,A=1.000000)" 0.0 0.0)
      (Rendering|Debug|DrawDebugLine _returnvalue (Transformation|GetWorldLocation (Variables|Default|GetWestTarget)) "(R=0.000000,G=1.000000,B=0.000000,A=1.000000)" 0.0 0.0)
      (Rendering|Debug|DrawDebugLine _returnvalue (Transformation|GetWorldLocation (Variables|Default|GetEastTarget)) "(R=1.000000,G=0.000000,B=1.000000,A=1.000000)" 0.0 0.0))))

(fn ConstructionScript)