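; Enemy for the Darkventure arcade game that chases the player and costs them life on contact.
; On BeginPlay it registers with the room found by a downward trace; a player entering its sphere makes that room activate its enemies.
; Once activated it shows its plane and builds velocity toward the player each tick, accelerating harder when farther away and stopping when a box trace is blocked.
; A gate throttles contact damage, reopening shortly after hitting the player.
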(event OnComponentBeginOverlap(Sphere)
  (params (OverlappedComponent :type Primitive%20Component%20Object%20Reference) (OtherActor :type Actor%20Object%20Reference) (OtherComp :type Primitive%20Component%20Object%20Reference) (OtherBodyIndex :type Integer) (bFromSweep :type Boolean) (SweepResult :type Hit%20Result%20Structure%20%28by%20ref%29))
  (Utilities|Casting|CastToBP_DVCharacter OtherActor)
  (bind _room (Variables|Default|GetRoom)
    (:then
      (Default|ActivateEnemies _room))
    (:else)))

(event OnComponentBeginOverlap(Box)
  (params (OverlappedComponent :type Primitive%20Component%20Object%20Reference) (OtherActor :type Actor%20Object%20Reference) (OtherComp :type Primitive%20Component%20Object%20Reference) (OtherBodyIndex :type Integer) (bFromSweep :type Boolean) (SweepResult :type Hit%20Result%20Structure%20%28by%20ref%29))
  (bind _playerref (Variables|Default|GetPlayerRef))
  (Utilities|FlowControl|Gate false :!label _label
    (:Exit
      (Utilities|FlowControl|Sequence
        (:then_0
          (goto _label Close))
        (:then_1
          (if (== _playerref OtherActor)
            (Default|UpdateLife _playerref -1)
            (Utilities|FlowControl|Delay 0.5)
            (goto _label Open)))))))

(event Custom|Activate
  (CallFunction|Chase)
  (Development|SetHiddeninGame (Variables|Default|GetPlane) false false))

(event Custom|Chase
  (bind _returnvalue (Transformation|GetActorLocation))
  (bind _returnvalue_2 (Transformation|GetActorLocation))
  (bind _playerref (Variables|Default|GetPlayerRef))
  (bind _returnvalue_3 (Transformation|GetActorLocation _playerref))
  (if (Utilities|IsValid (Variables|Default|GetPlayerRef))
    (Variables|Default|SetIs%20Chasing true)
    (bind _output_get (Variables|Default|SetCurrentVelocity (Math|Vector|ClampVectorSize (+ (Variables|Default|GetCurrentVelocity) (* (/ (Math|Vector|Normalize (- _returnvalue_3 _returnvalue)) 25) (+ (* (/ (- (Math|Float|Clamp(Float) (Math|Vector|Distance(Vector) _returnvalue _returnvalue_3) 1e+02 1e+03) 1e+02) 9e+02) 1e+01) 1.0))) -1e+03 1e+03)))
    (bind _returnvalue_4 (Collision|BoxTraceByChannel (+ _returnvalue_2 "0.000000,0.000000,1.000000") (+ _returnvalue_2 (Math|Vector|MakeVector (.x _output_get) (.y _output_get) 0.0) "0.000000,0.000000,1.000000") "64.000000,64.000000,0.000000" "0, 0, 0" "TraceTypeQuery1" false 0 "ForDuration"))
    (if _returnvalue_4
      (Variables|Default|SetCurrentVelocity "0, 0, 0")
      (else
        (Transformation|AddActorWorldOffset (Math|Vector|MakeVector (.x _output_get) (.y _output_get) 0.0))))))

(event EventTick
  (params (DeltaSeconds :type Float%20%28single-precision%29))
  (if (Variables|Default|GetIs%20Chasing)
    (CallFunction|Chase)))

(event EventBeginPlay
  (bind _returnvalue (Transformation|GetActorLocation))
  (bind (_outhit _returnvalue_2) (Collision|LineTraceByChannel _returnvalue (+ _returnvalue "0.000000,0.000000,-50.000000") "TraceTypeQuery1" false 0 "None"))
  (if _returnvalue_2
    (bind _asbp_dvroom (Utilities|Casting|CastToBP_DVRoom (.HitActor (Collision|BreakHitResult _outhit))))
    (Default|RegisterEnemy _asbp_dvroom self)
    (Variables|Default|SetRoom _asbp_dvroom)
    (bind _returnvalue_3 (Actor|GetActorOfClass "/Game/Blueprints/GPE/Arcades/Darkventure/BP_DVCharacter.BP_DVCharacter_C"))
    (Variables|Default|SetPlayerRef _returnvalue_3)))

(fn ConstructionScript)