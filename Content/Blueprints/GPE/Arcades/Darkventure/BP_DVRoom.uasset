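; Room actor for the Darkventure arcade game that tracks its enemies and the music status matching their state.
; Enemies register into a list, then are activated together, picking one of two music statuses at random and telling BP_DVManager to update player music.
; When the list empties after kills, the room deactivates and sets its status by whether it is exterior.
; The construction script gives exterior rooms a grass material.
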(event Custom|RegisterEnemy
  (params (Enemy :type BP%20DV%20Enemy%20Object%20Reference%20%28by%20ref%29))
  (Utilities|Array|Add (Variables|Default|GetEnemyList) Enemy)
  (Variables|Default|SetMusicStatus "NewEnumerator2"))

(event Custom|KilledEnemy
  (Utilities|Array|RemoveItem (Variables|Default|GetEnemyList) 0)
  (CallFunction|CheckEnemies))

(event Custom|CheckEnemies
  (if (Utilities|Array|IsEmpty (Variables|Default|GetEnemyList))
    (Variables|Default|SetMusicStatus (select (Variables|Default|GetIsExterior) "NewEnumerator0" "NewEnumerator1"))
    (Variables|Default|SetEnemiesActive false)))

(event Custom|ActivateEnemies
  (if (not (Variables|Default|GetEnemiesActive))
    (Variables|Default|SetEnemiesActive true)
    (for _array_element (Variables|Default|GetEnemyList)
      (Default|Activate _array_element)
      (Variables|Default|SetMusicStatus (select (Math|Random|RandomBool) "NewEnumerator4" "NewEnumerator3"))
      (bind _manager (Variables|Default|GetManager)
        (:then
          (Default|UpdatePlayerMusic _manager))
        (:else)))))

(event EventBeginPlay
  (bind _returnvalue (Actor|GetActorOfClass "/Game/Blueprints/GPE/Arcades/Darkventure/BP_DVMusicManager.BP_DVMusicManager_C"))
  (Variables|Default|SetMusicManager _returnvalue)
  (bind _returnvalue_2 (Actor|GetActorOfClass "/Game/Blueprints/GPE/Arcades/Darkventure/BP_DVManager.BP_DVManager_C"))
  (Variables|Default|SetManager _returnvalue_2))

(fn ConstructionScript
  (if (Variables|Default|GetIsExterior)
    (Rendering|Material|SetMaterial (Variables|Default|GetCube) 0 "/Game/Materials/Instances/MI_Grass.MI_Grass")))