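; A door in the Darkventure arcade minigame that teleports the player character between its two gates, optionally requiring a key.
; On BeginPlay it caches the character and registers itself with the Darkventure manager.
; On interact, a locked door consumes the player's key, unlocks and hides the HUD key icon.
; It then sends the character to whichever gate is farther away and has the manager update the player music.
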(event EventInteract
  (bind _gatea (Variables|Default|GetGateA))
  (bind _gateb (Variables|Default|GetGateB))
  (bind _character (Variables|Default|GetCharacter))
  (bind _character_2 (Variables|Default|GetCharacter))
  (bind _character_3 (Variables|Default|GetCharacter))
  (bind _returnvalue (Transformation|GetActorLocation _character_2))
  (bind _returnvalue_2 (Transformation|GetWorldLocation _gateb))
  (bind _returnvalue_3 (Transformation|GetWorldLocation _gatea))
  (if (Variables|Default|GetCanInteract)
    (if (Variables|Default|GetNeedKey)
      (if (Variables|/Game/Blueprints/GPE/Arcades/Darkventure/BP_DVCharacter.BP_DVCharacter_C|GetHasKey _character_3)
        (Variables|/Game/Blueprints/GPE/Arcades/Darkventure/BP_DVCharacter.BP_DVCharacter_C|SetHasKey _character_3 false)
        (Variables|Default|SetNeedKey false)
        (bind _asuw_dv_in_game (Utilities|Casting|CastToUW_DV_InGame (UserInterface|GetWidget (Variables|/Game/Blueprints/GPE/Arcades/Darkventure/BP_Darkventure.BP_Darkventure_C|GetWidgetInGame (Variables|/Game/Blueprints/GPE/Arcades/Darkventure/BP_DVManager.BP_DVManager_C|GetArcade (Variables|Default|GetManager))))))
        (Widget|SetVisibility (Variables|/Game/Widgets/Arcades/UW_DV_InGame.UW_DV_InGame_C|GetKeyImg _asuw_dv_in_game) "Hidden")
        (if (< (Math|Vector|Distance(Vector) _returnvalue _returnvalue_3) (Math|Vector|Distance(Vector) _returnvalue _returnvalue_2)) :!label _label
          (Transformation|Teleport _character _returnvalue_2 "0, 0, 0")
          (else
            (Transformation|Teleport _character _returnvalue_3 "0, 0, 0")))
        (Default|UpdatePlayerMusic (Variables|Default|GetManager)))
      (else
        (goto _label)))))

(event EventBeginPlay
  (bind _returnvalue (Actor|GetActorOfClass "/Game/Blueprints/GPE/Arcades/Darkventure/BP_DVCharacter.BP_DVCharacter_C"))
  (Variables|Default|SetCharacter _returnvalue)
  (bind _returnvalue_2 (Actor|GetActorOfClass "/Game/Blueprints/GPE/Arcades/Darkventure/BP_DVManager.BP_DVManager_C"))
  (Default|Register _returnvalue_2 self)
  (Variables|Default|SetManager _returnvalue_2))

(fn ConstructionScript)