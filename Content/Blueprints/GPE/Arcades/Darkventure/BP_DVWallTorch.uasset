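; Animated wall torch for the Darkventure arcade, pairing a Paper2D flipbook flame with a flickering point light.
; SetRhythm scales the flipbook play rate, restarts it, resets the light intensity and replaces any running looping timer with one whose period is inversely proportional to the rhythm.
; Each timer tick randomizes the light's intensity and slightly jitters its horizontal position, so the flicker keeps pace with the animation.
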(event Custom|DelayLight
  (bind _pointlight (Variables|Default|GetPointLight))
  (Rendering|Components|Light|SetIntensity _pointlight (Math|Random|RandomFloatinRange 7.5e+03 1e+04))
  (Transformation|SetRelativeLocation _pointlight (Math|Vector|MakeVector (Math|Random|RandomFloatinRange -2.0 2.0) (Math|Random|RandomFloatinRange -2.0 2.0) 0.0) false false))

(event EventSetRhythm
  (params (Rhytm :type Float%20%28double-precision%29))
  (bind _paperflipbook (Variables|Default|GetPaperFlipbook))
  (Components|Timeline|SetPlayRate _paperflipbook Rhytm)
  (Components|Timeline|PlayfromStart _paperflipbook)
  (Rendering|Components|Light|SetIntensity (Variables|Default|GetPointLight) 1e+04)
  (if (Utilities|Time|IsValidTimerHandle (Variables|Default|GetTimer))
    (Utilities|Time|ClearandInvalidateTimerbyHandle (Variables|Default|GetTimer)))
  (bind _returnvalue (Utilities|Time|SetTimerbyEvent (delegate Custom|DelayLight) (/ 0.25 Rhytm) true))
  (Variables|Default|SetTimer _returnvalue))

(fn ConstructionScript
  (|CallParentFunction))