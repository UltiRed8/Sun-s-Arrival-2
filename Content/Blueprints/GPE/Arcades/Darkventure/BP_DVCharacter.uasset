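; Player character of the Darkventure arcade minigame, a flipbook sprite with life, interaction and a flashlight attack.
; Accumulated direction input aims the flashlight and drives Tick movement, blocked by a box trace.
; Attack, allowed only while moving, flashes the light and deals distance-scaled damage to enemies that were chasing upon entering its cone, then recharges.
; Life changes update the arcade UI, with damage feedback and a death animation at zero.
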(event OnComponentBeginOverlap(Cone)
  (params (OverlappedComponent :type Primitive%20Component%20Object%20Reference) (OtherActor :type Actor%20Object%20Reference) (OtherComp :type Primitive%20Component%20Object%20Reference) (OtherBodyIndex :type Integer) (bFromSweep :type Boolean) (SweepResult :type Hit%20Result%20Structure%20%28by%20ref%29))
  (bind _asbp_dvenemy (Utilities|Casting|CastToBP_DVEnemy OtherActor))
  (if (Variables|/Game/Blueprints/GPE/Arcades/Darkventure/BP_DVEnemy.BP_DVEnemy_C|GetIs%20Chasing _asbp_dvenemy)
    (Utilities|Array|Add (Variables|Default|GetEnemies) _asbp_dvenemy)))

(event OnComponentEndOverlap(Cone)
  (params (OverlappedComponent :type Primitive%20Component%20Object%20Reference) (OtherActor :type Actor%20Object%20Reference) (OtherComp :type Primitive%20Component%20Object%20Reference) (OtherBodyIndex :type Integer))
  (bind _asbp_dvenemy (Utilities|Casting|CastToBP_DVEnemy OtherActor))
  (Utilities|Array|RemoveItem (Variables|Default|GetEnemies) _asbp_dvenemy))

(event Custom|UpdateDirection
  (params (Additive :type Vector))
  (bind _pf_dvplayerspritesheet_s_dvplayerdeath (Variables|Default|GetPF_DVPlayerSpriteSheet_S_DVPlayerDeath))
  (Variables|Default|SetDirection (Utilities|Struct|MakeIntPoint (+ (.x Additive) (.x (Variables|Default|GetDirection))) (+ (.y Additive) (.y (Variables|Default|GetDirection)))))
  (Transformation|SetRelativeRotation (Variables|Default|GetFlashlightAxis) (Math|Rotator|MakeRotator 0.0 0.0 (Math|Trig|RadiansToDegrees (Math|Trig|Atan2(Radians) (Math|Conversions|ToFloat(Integer) (.y (Variables|Default|GetDirection))) (Math|Conversions|ToFloat(Integer) (.x (Variables|Default|GetDirection)))))) false false)
  (if (not (Variables|Default|GetIsDead))
    (if (== (.y (Variables|Default|GetDirection)) 0)
      _
      (else
        (Transformation|SetRelativeRotation (Variables|Default|GetPF_DVPlayerSpriteSheet_S_DVPlayerDeath) (Math|Rotator|MakeRotator 9e+01 (Math|Float|SelectFloat 1.8e+02 0.0 (>= (.y (Variables|Default|GetDirection)) 0)) -9e+01) false false)))
    (if (== (+ (Math|Integer|Absolute(Integer) (.x (Variables|Default|GetDirection))) (Math|Integer|Absolute(Integer) (.y (Variables|Default|GetDirection)))) 0)
      (Utilities|OnceGate true :!label _label
        (:OutA
          (Sprite|SetFlipbook _pf_dvplayerspritesheet_s_dvplayerdeath "/Game/Textures/Arcades/DV/Player/PF_DVPlayerIdle.PF_DVPlayerIdle"))
        (:OutB
          (Sprite|SetFlipbook _pf_dvplayerspritesheet_s_dvplayerdeath "/Game/Textures/Arcades/DV/Player/PF_DVPlayerMoving.PF_DVPlayerMoving")))
      (else
        (goto _label InB)))))

(event Custom|Interact
  (if (not (Variables|Default|GetIsDead))
    (bind _manager (Variables|Default|GetManager)
      (:then
        (bind _interactable1 (Default|GetClosestInteractable _manager))
        (Utilities|IsValid _interactable1
          (:Is%20Valid
            (Default|Interact _interactable1))))
      (:else))))

(event Custom|Attack
  (if (not (or (Variables|Default|GetIsDead) (Class|KismetMathLibrary|EqualIntPointIntPoint (Variables|Default|GetDirection))))
    (Utilities|FlowControl|Gate false :!label _label
      (:Exit
        (Utilities|FlowControl|Sequence
          (:then_0
            (goto _label Close))
          (:then_1
            (bind _intensity (Timeline|Timeline PlayFromStart)
              (:Update
                (Rendering|Components|Light|SetIntensity (Variables|Default|GetFlashlight) _intensity))))
          (:then_2
            (Default|FlashlightUse (Variables|Default|GetArcadeWidget))
            (Utilities|FlowControl|Delay 2.0)
            (Default|PlaySound (Variables|Default|GetArcade) "/Game/Audio/Sounds/SW_DV_FlashlightReloaded.SW_DV_FlashlightReloaded" 1.0 0.0)
            (Sprite|SetSpriteColor (Variables|Default|GetPF_DVPlayerSpriteSheet_S_DVPlayerDeath) "(R=1.000000,G=1.000000,B=1.000000,A=1.000000)")
            (goto _label Open))
          (:then_3
            (Default|PlaySound (Variables|Default|GetArcade) "/Game/Audio/Sounds/SW_DV_FlashlightUse.SW_DV_FlashlightUse" 1.0 0.0))
          (:then_4
            (for _array_element (Variables|Default|GetEnemies)
              (Default|ApplyDamage _array_element (Math|Conversions|ToFloat(Integer) (Math|Float|Round (Math|Float|SelectFloat 1e+04 (Math|Float|Absolute(Float) (Math|Float|Max(Float) (- 1e+04 (+ (* (/ (- (Transformation|GetDistanceTo _array_element self) 2e+02) 6e+02) 9e+03) 1e+03)) 1e+03)) (<= (Transformation|GetDistanceTo _array_element self) 2e+02)))))))
          (:then_5
            (Sprite|SetSpriteColor (Variables|Default|GetPF_DVPlayerSpriteSheet_S_DVPlayerDeath) "(R=0.536417,G=0.000000,B=1.000000,A=1.000000)")))))))

(event Custom|UpdateLife
  (params (Value :type Integer))
  (bind _pf_dvplayerspritesheet_s_dvplayerdeath (Variables|Default|GetPF_DVPlayerSpriteSheet_S_DVPlayerDeath))
  (Utilities|FlowControl|Sequence
    (:then_0
      (if (not (Variables|Default|GetIsDead))
        (bind _output_get (Variables|Default|SetLife (Math|Integer|Clamp(Integer) (+ (Variables|Default|GetLife) Value) 0 3)))
        (Default|UpdateLifeUI (Variables|/Game/Blueprints/GPE/Arcades/Darkventure/BP_DVManager.BP_DVManager_C|GetArcade (Variables|Default|GetManager)) _output_get)
        (Variables|Default|SetIsDead (<= _output_get 0))
        (if (< Value 0)
          (Default|DamagePlayer (Variables|Default|GetArcadeWidget))
          (Default|PlaySound (Variables|Default|GetArcade) "/Game/Audio/Sounds/SW_DVPlayerDamage.SW_DVPlayerDamage" 1.0 0.0)
          (if (Variables|Default|GetIsDead)
            (Sprite|SetFlipbook _pf_dvplayerspritesheet_s_dvplayerdeath "/Game/Textures/Arcades/DV/Player/PF_DVPlayerrDeath.PF_DVPlayerrDeath")
            (Components|Timeline|SetLooping _pf_dvplayerspritesheet_s_dvplayerdeath false)
            (Utilities|FlowControl|Delay 0.8)
            (Development|SetHiddeninGame _pf_dvplayerspritesheet_s_dvplayerdeath true false)))))
    (:then_1
      (if (< Value 0)
        (Variables|Default|SetNoHit false)))))

(event EventBeginPlay
  (bind _returnvalue (Actor|GetActorOfClass "/Game/Blueprints/GPE/Arcades/Darkventure/BP_DVManager.BP_DVManager_C"))
  (Variables|Default|SetManager _returnvalue))

(event EventTick
  (params (DeltaSeconds :type Float%20%28single-precision%29))
  (bind _returnvalue (Transformation|GetActorLocation))
  (bind _direction (Variables|Default|GetDirection))
  (bind _returnvalue_2 (Math|Conversions|ToFloat(Integer) (.x _direction)))
  (bind _returnvalue_3 (Math|Conversions|ToFloat(Integer) (.y _direction)))
  (bind _returnvalue_4 (Math|Vector|MakeVector _returnvalue_2 _returnvalue_3 0.0))
  (if (not (Variables|Default|GetIsDead))
    (bind _returnvalue_5 (Collision|BoxTraceByChannel (+ _returnvalue "0.000000,0.000000,1.000000") (+ _returnvalue (* _returnvalue_4 5.0 DeltaSeconds (Variables|Default|GetWalkSpeed)) "0.000000,0.000000,1.000000") "32.000000,32.000000,0.000000" "0, 0, 0" "TraceTypeQuery1" false 0 "ForOneFrame"))
    (if (not _returnvalue_5)
      (Transformation|AddActorWorldOffset (* _returnvalue_4 4.0 DeltaSeconds (Variables|Default|GetWalkSpeed))))))

(fn ConstructionScript)