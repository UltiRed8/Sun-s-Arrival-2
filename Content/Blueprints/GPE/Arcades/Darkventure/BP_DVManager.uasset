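; BP_DVManager is the manager for the Darkventure arcade game, linking the player character to interactables and music.
; It caches the character and music manager on BeginPlay and keeps a list of registered interactables.
; GetClosestInteractable returns the nearest one whose own interaction range contains the character.
; UpdatePlayerMusic traces down from the character to find the room underneath and passes its music status to the music manager.
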(event Custom|Register
  (params (Interactable :type BP%20DV%20Interactable%20Object%20Reference%20%28by%20ref%29))
  (Utilities|Array|Add (Variables|Default|GetInteractives) Interactable))

(event Custom|UpdatePlayerMusic
  (bind _character (Variables|Default|GetCharacter))
  (bind _returnvalue (Transformation|GetActorLocation _character))
  (bind (_outhit _returnvalue_2) (Collision|LineTraceByChannel _returnvalue (+ _returnvalue "0.000000,0.000000,-50.000000") "TraceTypeQuery1" false 0 "None"))
  (if _returnvalue_2
    (bind _asbp_dvroom (Utilities|Casting|CastToBP_DVRoom (.HitActor (Collision|BreakHitResult _outhit))))
    (bind _musicmanager (Variables|Default|GetMusicManager)
      (:then
        (Default|SetMusic _musicmanager (Variables|/Game/Blueprints/GPE/Arcades/Darkventure/BP_DVRoom.BP_DVRoom_C|GetMusicStatus _asbp_dvroom)))
      (:else))))

(event EventBeginPlay
  (bind _returnvalue (Actor|GetActorOfClass "/Game/Blueprints/GPE/Arcades/Darkventure/BP_DVCharacter.BP_DVCharacter_C"))
  (Variables|Default|SetCharacter _returnvalue)
  (bind _returnvalue_2 (Actor|GetActorOfClass "/Game/Blueprints/GPE/Arcades/Darkventure/BP_DVMusicManager.BP_DVMusicManager_C"))
  (Variables|Default|SetMusicManager _returnvalue_2))

(fn ConstructionScript)

(fn GetClosestInteractable
  (bind _interactives (Variables|Default|GetInteractives))
  (LocalVariables|SetInteractable 0)
  (LocalVariables|SetDistance 999999.0)
  (Development|PrintString (Utilities|String|ToString(Integer) (Utilities|Array|Length _interactives)))
  (for _array_element _interactives
    (if (<= (Transformation|GetDistanceTo _array_element (Variables|Default|GetCharacter)) (Variables|/Game/Blueprints/GPE/Arcades/Darkventure/BP_DVInteractable.BP_DVInteractable_C|GetInteractionDistance _array_element))
      (Utilities|IsValid (LocalVariables|GetInteractable)
        (:Is%20Valid
          (if (< (Transformation|GetDistanceTo _array_element (Variables|Default|GetCharacter)) (LocalVariables|GetDistance))
            (LocalVariables|SetInteractable _array_element :!label _label)
            (LocalVariables|SetDistance (Transformation|GetDistanceTo _array_element (Variables|Default|GetCharacter)))))
        (:Is%20Not%20Valid
          (goto _label)))))
  (return (LocalVariables|GetInteractable)))