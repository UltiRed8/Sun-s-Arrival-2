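; Elevator press button that players interact with to send a floor value to its listeners.
; It registers as an interactable on begin play, sets an interact cursor texture, and unregisters on destruction.
; Server interaction fires the OnTriggered dispatcher with its Floor, multicasts the LeverDownEnd sound and triggers an optional linked Node.
; A text render shows the button label, set at construction or through SetText.
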(event Custom|SetText
  (params (InString :type String))
  (Rendering|Components|TextRender|SetText (Variables|Default|GetTextRender) (Utilities|Text|ToText(String) InString)))

(event Custom|Multi_PlaySound
  (Audio|Components|Audio|Play (Variables|Default|GetLeverDownEnd) 0.0))

(event EventBeginPlay
  (Utilities|RegisterInteractable)
  (Variables|/Game/Blueprints/Components/BP_CustomCursorComponent.BP_CustomCursorComponent_C|SetCursorTexture (Variables|Default|GetBP_CustomCursorComponent) "/Game/Textures/T_CursorInteract.T_CursorInteract"))

(event EventServerInteract
  (params (WhoInteracted :type Actor%20Object%20Reference))
  (Default|CallOnTriggered (Variables|Default|GetFloor))
  (CallFunction|MultiPlaySound)
  (bind _node (Variables|Default|GetNode)
    (:then
      (Default|Trigger _node))
    (:else)))

(event EventDestroyed
  (Utilities|UnregisterInteractable))

(fn ConstructionScript
  (Rendering|Components|TextRender|SetText (Variables|Default|GetTextRender) (Utilities|Text|ToText(String) (Variables|Default|GetText))))