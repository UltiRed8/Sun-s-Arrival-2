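; Interactable water dispenser that plays a sound and a short water effect when used, registering as an interactable on BeginPlay and unregistering on destruction.
; Interaction runs the parent logic, then triggers MultiToggleFX if CanBeInteract is set, otherwise just re-arms that flag.
; MultiToggleFX plays the sound, activates one of two water effects at random after a delay, then deactivates both.
; A valid sound re-enables interaction immediately, before the effect finishes.
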(event Custom|PlayWaterSound
  (Utilities|IsValid (Variables|Default|GetInteractSound)
    (:Is%20Valid
      (Audio|PlaySoundatLocation (Variables|Default|GetInteractSound) (Transformation|GetActorLocation) "0, 0, 0" 1.0 1.0 0.0 0 0 0 0)
      (Variables|Default|SetCanBeInteract true))))

(event Custom|MultiToggleFX
  (Variables|Default|SetCanBeInteract false)
  (CallFunction|PlayWaterSound)
  (Utilities|FlowControl|Delay 1.0)
  (Components|Activation|Activate (select (Math|Random|RandomBool) (Variables|Default|GetWaterFX) (Variables|Default|GetNS_WaterDispenser)) false)
  (Utilities|FlowControl|Delay 3.0)
  (Components|Activation|Deactivate (Variables|Default|GetNS_WaterDispenser)))

(event EventBeginPlay
  (Utilities|RegisterInteractable)
  (|CallParentFunction))

(event EventInteraction
  (|CallParentFunction)
  (if (Variables|Default|GetCanBeInteract)
    (CallFunction|MultiToggleFX)
    (else
      (Variables|Default|SetCanBeInteract true))))

(event EventDestroyed
  (Utilities|UnregisterInteractable))

(fn ConstructionScript)