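; Interactable computer that toggles its linked screens on and off when used.
; Interaction calls Multi_ToggleScreen, whose flip-flop switches every valid linked screen and plays the computer sound on switch-on, or on each toggle if none are linked.
; The toggle state is saved to a checkpoint keyed by the actor's location string; on BeginPlay, the authority re-runs the toggle if the saved state is true.
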(event Custom|PlayComputerSound
  (Audio|Components|Audio|Play (Variables|Default|GetSW_Computer) 0.0))

(event Custom|Multi_ToggleScreen
  (if (Utilities|Array|IsNotEmpty (Variables|Default|GetAllScreensLinked))
    (bind _isa (Utilities|FlowControl|FlipFlop)
      (:A
        (for _array_element (Variables|Default|GetAllScreensLinked)
          (Utilities|IsValid _array_element
            (:Is%20Valid
              (Default|TurnScreenon _array_element))))
        (CallFunction|PlayComputerSound :!label _label))
      (:B
        (for _array_element_2 (Variables|Default|GetAllScreensLinked)
          (Utilities|IsValid _array_element_2
            (:Is%20Valid
              (Default|TurnScreenOff _array_element_2))))))
    (else
      (goto _label)))
  (Utilities|CheckpointSaveBool (Utilities|String|ToString(Vector) (Transformation|GetActorLocation)) _isa))

(event EventBeginPlay
  (|CallParentFunction)
  (Utilities|Authority
    (:Authority
      (bind (_success _bool) (Utilities|CheckpointGetBool (Utilities|String|ToString(Vector) (Transformation|GetActorLocation))))
      (if _success
        (if _bool
          (CallFunction|MultiToggleScreen))))))

(event EventInteracted
  (params (HitComponent :type Actor%20Component%20Object%20Reference%20%28by%20ref%29) (WhoInteracted :type Actor%20Object%20Reference) (HasMouseMovements :type Boolean))
  (CallFunction|MultiToggleScreen))

(fn ConstructionScript)