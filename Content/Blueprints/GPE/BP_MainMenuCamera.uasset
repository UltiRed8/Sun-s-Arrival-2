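; Main menu camera actor that can make itself the player's view target on BeginPlay through an ActiveByDefault flag.
; Two timelines at different slowed play rates define a subtle sway around the starting location.
; Horizontal stores an X offset, while Vertical's update applies both offsets along the camera's right and up vectors.
; The graph never calls Play on either timeline, so any motion depends on autoplay or an external trigger.
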(event EventBeginPlay
  (Variables|Default|SetDefaultLocation (Transformation|GetActorLocation))
  (Components|Timeline|SetPlayRate (Variables|Default|GetVertical) 0.25)
  (Components|Timeline|SetPlayRate (Variables|Default|GetHorizontal) 0.5)
  (if (Variables|Default|GetActiveByDefault)
    (Game|Player|SetViewTargetwithBlend (Game|GetPlayerController 0) self 0.0 "VTBlend_Linear" 0.0 false)))

(fn ConstructionScript)