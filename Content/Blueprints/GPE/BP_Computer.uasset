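; BP_Computer is an interactable computer that unlocks the player's map device.
; A server interaction event fires its triggered call, then runs an unlock event, apparently multicast.
; The unlock reaches the BP_MapDevice child actor on player 0's pawn, flags it unlocked and hides its static screen.
; It also switches the computer's cursor from interact to normal and swaps materials to a black screen plane and red glow.
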(event Custom|Multi_Unlock
  (bind _asbp_player (Utilities|Casting|CastToBP_Player (Game|Player|GetPlayerPawn 0)))
  (bind _asbp_map_device (Utilities|Casting|CastToBP_MapDevice (Variables|/Script/Engine.ChildActorComponent|GetChildActor (Variables|/Game/Blueprints/Player/BP_Player.BP_Player_C|GetMapDeviceActor _asbp_player))))
  (Variables|/Game/Blueprints/Player/BP_MapDevice.BP_MapDevice_C|SetIsUnlock _asbp_map_device true)
  (Development|SetHiddeninGame (Variables|/Game/Blueprints/Player/BP_MapDevice.BP_MapDevice_C|GetScreenStatic _asbp_map_device) true false)
  (Variables|/Game/Blueprints/Components/BP_CustomCursorComponent.BP_CustomCursorComponent_C|SetCursorTexture (Variables|Default|GetBP_CustomCursorComponent) "/Game/Textures/T_CursorNormal.T_CursorNormal")
  (Rendering|Material|SetMaterial (Variables|Default|GetPlane) 0 "/Game/Materials/Instances/MI_Black.MI_Black")
  (Rendering|Material|SetMaterial (Variables|Default|GetStaticMesh) 4 "/Game/Models/EndoEnemy/MAT_RedGlow.MAT_RedGlow"))

(event EventBeginPlay
  (Variables|/Game/Blueprints/Components/BP_CustomCursorComponent.BP_CustomCursorComponent_C|SetCursorTexture (Variables|Default|GetBP_CustomCursorComponent) "/Game/Textures/T_CursorInteract.T_CursorInteract"))

(event EventServerInteract
  (params (WhoInteracted :type Actor%20Object%20Reference))
  (Default|CallOnTriggered)
  (CallFunction|MultiUnlock))

(fn ConstructionScript)