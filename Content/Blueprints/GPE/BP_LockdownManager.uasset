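; Manager that tracks how many security doors are on lockdown at once to award the lockdown achievement.
; On BeginPlay it binds to the lockdown state event of each door in its SecurityDoors array.
; Each event raises or lowers a running count, and the GameInstance unlocks the achievement when a new lockdown brings that count to three or more.
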(event Custom|OnLockdownStateUpdated_Event
  (params (IsOnLockdown :type Boolean))
  (bind _currentlylockeddown (Variables|Default|GetCurrentlyLockedDown))
  (if IsOnLockdown
    (Math|Integer|IncrementInt _currentlylockeddown
      (:%20%20
        (if (>= _currentlylockeddown 3)
          (Default|UnlockAchievement (Utilities|GameInstance) "ACH_Lockdown"))))
    (else
      (Math|Integer|DecrementInt _currentlylockeddown))))

(event EventBeginPlay
  (for _array_element (Variables|Default|GetSecurityDoors)
    (EventDispatchers|AssignOnLockdownStateUpdated _array_element (delegate Custom|OnLockdownStateUpdated_Event))))

(fn ConstructionScript)