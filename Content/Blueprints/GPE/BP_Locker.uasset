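; BP_Locker is an interactable locker that players can hide in behind a closing door.
; A trigger tracks players inside; closing sets their IsHiding, while opening or leaving clears it.
; Interaction alternates Multi open and close events, which rotate the door by timeline with sounds, a cooldown and a camera shake on closing.
; Door state saves to checkpoints keyed by world location, and BeginPlay replays Interacted when the saved value is true.
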(event OnComponentBeginOverlap(Trigger)
  (params (OverlappedComponent :type Primitive%20Component%20Object%20Reference) (OtherActor :type Actor%20Object%20Reference) (OtherComp :type Primitive%20Component%20Object%20Reference) (OtherBodyIndex :type Integer) (bFromSweep :type Boolean) (SweepResult :type Hit%20Result%20Structure%20%28by%20ref%29))
  (if (Variables|Default|GetIsEffective)
    (bind _asbp_player (Utilities|Casting|CastToBP_Player OtherActor))
    (Utilities|Array|Add (Variables|Default|GetPlayers) _asbp_player)))

(event OnComponentEndOverlap(Trigger)
  (params (OverlappedComponent :type Primitive%20Component%20Object%20Reference) (OtherActor :type Actor%20Object%20Reference) (OtherComp :type Primitive%20Component%20Object%20Reference) (OtherBodyIndex :type Integer))
  (if (Variables|Default|GetIsEffective)
    (bind _asbp_player (Utilities|Casting|CastToBP_Player OtherActor))
    (Variables|/Game/Blueprints/Player/BP_Player.BP_Player_C|SetIsHiding _asbp_player false)
    (Utilities|Array|RemoveItem (Variables|Default|GetPlayers) _asbp_player)))

(event Custom|Multi_Open
  (if (not (Variables|Default|GetCooldown))
    (Variables|Default|SetCooldown true)
    (for _array_element (Variables|Default|GetPlayers)
      (Variables|/Game/Blueprints/Player/BP_Player.BP_Player_C|SetIsHiding _array_element false))
    (Audio|Components|Audio|Play (Variables|Default|GetOpenDoor) 0.0)
    (bind _doorangle (Timeline|OpenAnimation PlayFromStart)
      (:Update
        (Transformation|SetRelativeRotation (Variables|Default|GetAxis) (Math|Rotator|MakeRotator 0.0 0.0 (* _doorangle -1.0)) false false))
      (:Finished
        (Variables|Default|SetCooldown false)))))

(event Custom|Multi_Close
  (if (not (Variables|Default|GetCooldown))
    (Variables|Default|SetCooldown true)
    (bind _doorangle (Timeline|CloseAnimation PlayFromStart)
      (:Update
        (Transformation|SetRelativeRotation (Variables|Default|GetAxis) (Math|Rotator|MakeRotator 0.0 0.0 (* _doorangle -1.0)) false false))
      (:Finished
        (Default|CameraShake (Utilities|GameInstance) "/Game/Shakes/CS_Locker.CS_Locker_C" (Transformation|GetActorLocation) 3e+02 5e+02 1.0 false)
        (Audio|Components|Audio|Play (Variables|Default|GetCloseDoor) 0.0)
        (for _array_element (Variables|Default|GetPlayers)
          (Variables|/Game/Blueprints/Player/BP_Player.BP_Player_C|SetIsHiding _array_element true))
        (Variables|Default|SetCooldown false)))))

(event EventBeginPlay
  (|CallParentFunction)
  (bind (_success _bool) (Utilities|CheckpointGetBool (Utilities|String|ToString(Vector) (Transformation|GetActorLocation))))
  (if _success
    (if _bool
      (CallFunction|Interacted 0 0 false false))))

(event EventInteracted
  (params (HitComponent :type Actor%20Component%20Object%20Reference%20%28by%20ref%29) (WhoInteracted :type Actor%20Object%20Reference) (HasMouseMovements :type Boolean) (IsServer :type Boolean))
  (if (not (Variables|Default|GetCooldown))
    (bind _isa (Utilities|FlowControl|FlipFlop)
      (:A
        (CallFunction|MultiOpen))
      (:B
        (CallFunction|MultiClose)))
    (Utilities|CheckpointSaveBool (Utilities|String|ToString(Vector) (Transformation|GetActorLocation)) _isa)))

(fn ConstructionScript)