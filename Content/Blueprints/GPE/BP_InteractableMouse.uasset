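; Interactable mouse gameplay element that plays a sound when the player interacts with it.
; It registers itself as an interactable on BeginPlay, after which it runs the parent BeginPlay, and unregisters when destroyed.
; Interaction calls the parent logic, then plays its Audio component from the start if CanBeInteract is set and the component is valid.
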(event Custom|PlaySound
  (Utilities|IsValid (Variables|Default|GetAudio)
    (:Is%20Valid
      (Audio|Components|Audio|Play (Variables|Default|GetAudio) 0.0))))

(event EventInteraction
  (|CallParentFunction)
  (if (Variables|Default|GetCanBeInteract)
    (CallFunction|PlaySound)))

(event EventDestroyed
  (Utilities|UnregisterInteractable))

(event EventBeginPlay
  (Utilities|RegisterInteractable)
  (|CallParentFunction))

(fn ConstructionScript)