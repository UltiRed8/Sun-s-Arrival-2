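; Interactable screen that unlocks the player's map device (minimap) and grants the map device achievement.
; Interacting fires OnTriggered, runs Multi_Unlock, then triggers an optional linked Node after a short delay.
; Unlocking enables the map on the player's child-actor device, switches the screen off, removes its audio and highlight, and saves HasMap to the checkpoint.
; BeginPlay restores that used state when the checkpoint already has the map.
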(event Custom|Multi_Unlock
  (Utilities|IsValid (Variables|Default|GetAudio)
    (:Is%20Valid
      (bind _asbp_player (Utilities|Casting|CastToBP_Player (Game|Player|GetPlayerPawn 0)))
      (bind _asbp_map_device (Utilities|Casting|CastToBP_MapDevice (Variables|/Script/Engine.ChildActorComponent|GetChildActor (Variables|/Game/Blueprints/Player/BP_Player.BP_Player_C|GetMapDeviceActor _asbp_player))))
      (Default|Unlock _asbp_map_device true)
      (if (Variables|/Game/Blueprints/Player/BP_MapDevice.BP_MapDevice_C|GetIsOpened _asbp_map_device)
        (Rendering|Material|SetMaterial (Variables|/Game/Blueprints/Player/BP_MapDevice.BP_MapDevice_C|GetDevice _asbp_map_device) 1 "/Game/Textures/MAT_RT_Map.MAT_RT_Map"))
      (Variables|/Game/Blueprints/Components/BP_CustomCursorComponent.BP_CustomCursorComponent_C|SetCursorTexture (Variables|Default|GetBP_CustomCursorComponent) "/Game/Textures/T_CursorNormal.T_CursorNormal")
      (Rendering|SetVisibility (Variables|Default|GetWidget) false false)
      (Rendering|Material|SetMaterial (Variables|Default|GetStaticMesh) 4 "/Game/Materials/Instances/MI_ScreenOffLed.MI_ScreenOffLed")
      (Components|DestroyComponent (Variables|Default|GetAudio))
      (Rendering|SetCustomDepthStencilValue (Variables|Default|GetStaticMesh) 0)
      (Variables|/Game/Saves/SG_Checkpoint.SG_Checkpoint_C|SetHasMap (Utilities|GetCheckpoint) true))))

(event EventInteracted
  (params (HitComponent :type Actor%20Component%20Object%20Reference%20%28by%20ref%29) (WhoInteracted :type Actor%20Object%20Reference) (HasMouseMovements :type Boolean))
  (bind _node (Variables|Default|GetNode))
  (Default|CallOnTriggered)
  (Default|UnlockAchievement (Utilities|GameInstance) "ACH_MAPDEVICE")
  (CallFunction|MultiUnlock)
  (Utilities|FlowControl|Delay 0.5)
  (Utilities|IsValid _node
    (:Is%20Valid
      (Default|Trigger _node))))

(event EventBeginPlay
  (|CallParentFunction)
  (if (Variables|/Game/Saves/SG_Checkpoint.SG_Checkpoint_C|GetHasMap (Utilities|GetCheckpoint))
    (bind _asbp_player (Utilities|Casting|CastToBP_Player (Game|Player|GetPlayerPawn 0)))
    (bind _asbp_map_device (Utilities|Casting|CastToBP_MapDevice (Variables|/Script/Engine.ChildActorComponent|GetChildActor (Variables|/Game/Blueprints/Player/BP_Player.BP_Player_C|GetMapDeviceActor _asbp_player))))
    (Default|Unlock _asbp_map_device false)
    (if (Variables|/Game/Blueprints/Player/BP_MapDevice.BP_MapDevice_C|GetIsOpened _asbp_map_device)
      (Rendering|Material|SetMaterial (Variables|/Game/Blueprints/Player/BP_MapDevice.BP_MapDevice_C|GetDevice _asbp_map_device) 1 "/Game/Textures/MAT_RT_Map.MAT_RT_Map"))
    (Variables|/Game/Blueprints/Components/BP_CustomCursorComponent.BP_CustomCursorComponent_C|SetCursorTexture (Variables|Default|GetBP_CustomCursorComponent) "/Game/Textures/T_CursorNormal.T_CursorNormal")
    (Rendering|SetVisibility (Variables|Default|GetWidget) false false)
    (Rendering|Material|SetMaterial (Variables|Default|GetStaticMesh) 4 "/Game/Materials/Instances/MI_ScreenOffLed.MI_ScreenOffLed")
    (Components|DestroyComponent (Variables|Default|GetAudio))
    (Rendering|SetCustomDepthStencilValue (Variables|Default|GetStaticMesh) 0)))

(fn ConstructionScript)