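; Elevator call button that players interact with to signal its floor, with an indicator showing whether the elevator is going up or down.
; It registers as an interactable on BeginPlay with an interact cursor, and unregisters when destroyed.
; Server interaction broadcasts OnTriggered with its Floor, multicasts a lever sound and triggers an optional linked Node.
; Events toggle GoingUp and GoingDown scalar parameters on the indicator plane's dynamic material.
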(event Custom|GoingUpMaterial
  (Rendering|Material|SetScalarParameterValue (Variables|Default|GetMaterial) "GoingUp" 1.0 :!class /Script/Engine.MaterialInstanceDynamic))

(event Custom|GoingDownMaterial
  (Rendering|Material|SetScalarParameterValue (Variables|Default|GetMaterial) "GoingDown" 1.0 :!class /Script/Engine.MaterialInstanceDynamic))

(event Custom|Multi_PlaySound
  (Audio|Components|Audio|Play (Variables|Default|GetLeverDownEnd) 0.0))

(event Custom|ResetMaterial
  (bind _material (Variables|Default|GetMaterial))
  (Rendering|Material|SetScalarParameterValue _material "GoingUp" 0.0 :!class /Script/Engine.MaterialInstanceDynamic)
  (Rendering|Material|SetScalarParameterValue _material "GoingDown" 0.0 :!class /Script/Engine.MaterialInstanceDynamic))

(event EventBeginPlay
  (Utilities|RegisterInteractable)
  (Variables|/Game/Blueprints/Components/BP_CustomCursorComponent.BP_CustomCursorComponent_C|SetCursorTexture (Variables|Default|GetBP_CustomCursorComponent) "/Game/Textures/T_CursorInteract.T_CursorInteract")
  (bind _returnvalue (Rendering|Material|CreateDynamicMaterialInstance (Variables|Default|GetPlane) 0 "/Game/Materials/MAT_ElevatorIndicator.MAT_ElevatorIndicator" "None" :!class /Script/Engine.PrimitiveComponent))
  (Variables|Default|SetMaterial _returnvalue))

(event EventServerInteract
  (params (WhoInteracted :type Actor%20Object%20Reference))
  (Default|CallOnTriggered (Variables|Default|GetFloor))
  (CallFunction|MultiPlaySound)
  (bind _node (Variables|Default|GetNode)
    (:then
      (Default|Trigger _node))
    (:else)))

(event EventDestroyed
  (Utilities|UnregisterInteractable))

(fn ConstructionScript)