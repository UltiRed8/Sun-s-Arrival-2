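; BP_SunLeg is a Sun Leg gameplay object that highlights itself when hovered, extending a parent Blueprint's hover events.
; Hovered and Unhovered toggle custom depth rendering on the static mesh, which suggests a post-process outline.
; An older highlight that swaps materials to a blue glow and restores the cached originals is left disconnected, along with both parent hover calls.
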(fn ConstructionScript
  (|CallParentFunction))

(fn Hovered
  (Rendering|SetRenderCustomDepth (Variables|Default|GetStaticMesh) true))

(fn Unhovered
  (Rendering|SetRenderCustomDepth (Variables|Default|GetStaticMesh) false))