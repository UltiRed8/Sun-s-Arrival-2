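; Interactable coin pickup that adds to the global inventory's coin count and persists its collected state through checkpoints.
; Its world location string serves as the checkpoint ID, so a coin already saved as collected destroys itself on BeginPlay.
; A one-shot server interaction saves, hides and moves the coin away, plays audio, increments coins, then destroys it after a delay.
; Hovering toggles custom depth highlighting; an older glow-material swap is left disconnected.
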(event EventBeginPlay
  (Utilities|RegisterInteractable)
  (bind _returnvalue (Actor|GetActorOfClass "/Game/Blueprints/Inventory/BP_GlobalInventory.BP_GlobalInventory_C"))
  (Variables|Default|SetInventory _returnvalue)
  (bind (_success _bool) (Utilities|CheckpointGetBool (Utilities|String|ToString(Vector) (Transformation|GetActorLocation))))
  (if _success
    (if _bool
      (Actor|DestroyActor)
      (else
        (Development|PrintString "Hello")))))

(event EventServerInteract
  (params (WhoInteracted :type Actor%20Object%20Reference))
  (Utilities|FlowControl|DoOnce false
    (:Completed
      (Utilities|CheckpointSaveBool (Utilities|String|ToString(Vector) (Transformation|GetActorLocation)) "true")
      (Rendering|SetActorHiddenInGame true)
      (Collision|SetActorEnableCollision false)
      (Transformation|Teleport "0.000000,0.000000,-1000.000000" "0, 0, 0")
      (Audio|Components|Audio|Play (Variables|Default|GetAudio) 0.0)
      (Default|IncrementCoins (Variables|Default|GetInventory))
      (Utilities|FlowControl|Delay 1.0)
      (Actor|DestroyActor))))

(event EventDestroyed
  (Utilities|UnregisterInteractable))

(fn ConstructionScript)

(fn Unhovered
  (Rendering|SetRenderCustomDepth (Variables|Default|GetStaticMesh) false))

(fn Hovered
  (Rendering|SetRenderCustomDepth (Variables|Default|GetStaticMesh) true))