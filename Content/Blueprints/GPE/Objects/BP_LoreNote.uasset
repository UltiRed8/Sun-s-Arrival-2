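; BP_LoreNote is an interactable note object that shows a readable lore page when a player interacts with it.
; Server interaction makes the interactor its owner, then Owning_OpenNote creates a UW_LoreNote widget with the note's text, typography and texture.
; The construction script applies that texture to the mesh through a dynamic material.
; Hovering toggles custom depth for highlighting, leaving an older glow-material swap unreachable.
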(event Custom|Owning_OpenNote
  (bind _returnvalue (UserInterface|CreateWidget "/Game/Widgets/Lore/UW_LoreNote.UW_LoreNote_C" (Game|GetPlayerController 0) (Variables|Default|GetTitle) (Variables|Default|GetText) (Variables|Default|GetAuthor) (Variables|Default|GetLine%20Height%20Percentage) (Variables|Default|GetFont) (Variables|Default|GetTitle%20Size) (Variables|Default|GetText%20Size) (Variables|Default|GetAuthor%20Size) (Variables|Default|GetTitle%20Space) (Variables|Default|GetText%20Space) (Variables|Default|GetAuthor%20Space) (Variables|Default|GetTexture)))
  (UserInterface|Viewport|AddtoViewport _returnvalue 0))

(event EventServerInteract
  (params (WhoInteracted :type Actor%20Object%20Reference))
  (Actor|SetOwner WhoInteracted)
  (CallFunction|OwningOpenNote))

(fn ConstructionScript
  (|CallParentFunction)
  (bind _returnvalue (Rendering|Material|CreateDynamicMaterialInstance (Variables|Default|GetStaticMesh) 0 0 "None" :!class /Script/Engine.PrimitiveComponent))
  (Rendering|Material|SetTextureParameterValue _returnvalue "Texture" (Variables|Default|GetTexture)))

(fn Hovered
  (Rendering|SetRenderCustomDepth (Variables|Default|GetStaticMesh) true))

(fn Unhovered
  (Rendering|SetRenderCustomDepth (Variables|Default|GetStaticMesh) false))