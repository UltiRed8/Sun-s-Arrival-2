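; Short-lived visual actor that animates a pickup flying to a target actor, then destroys itself.
; BeginPlay applies the supplied mesh, scale, rotation and materials, setting the start transform and activating inside the materials loop, so an empty list leaves it inactive.
; Tick lerps toward the target's current location over a set movement time while shrinking the actor to zero.
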(event EventBeginPlay
  (bind _staticmesh (Variables|Default|GetStaticMesh))
  (Components|StaticMesh|SetStaticMesh _staticmesh (Variables|Default|GetMesh))
  (Transformation|SetRelativeScale3D _staticmesh (Variables|Default|GetMeshScale))
  (Transformation|SetRelativeRotation _staticmesh (Variables|Default|GetMeshRotation) false false)
  (for (_array_element _array_index) (Variables|Default|GetMaterials)
    (Rendering|Material|SetMaterial _staticmesh _array_index _array_element)
    (Transformation|SetActorLocationAndRotation (Variables|Default|GetDefaultLocation) (Variables|Default|GetDefaultRotation))
    (Variables|Default|SetActive true)))

(event EventTick
  (params (DeltaSeconds :type Float%20%28single-precision%29))
  (if (Variables|Default|GetActive)
    (bind _output_get (Variables|Default|SetProgress (Math|Float|Clamp(Float) (+ (/ DeltaSeconds (Variables|Default|GetMovementTime)) (Variables|Default|GetProgress)))))
    (Transformation|SetActorLocation (Math|Vector|Lerp(Vector) (Variables|Default|GetDefaultLocation) (Transformation|GetActorLocation (Variables|Default|GetTargetActor)) _output_get) false false)
    (Transformation|SetActorScale3D (* (Variables|Default|GetActorScale) (- 1.0 _output_get)))
    (if (>= _output_get 1.0)
      (Actor|DestroyActor))))

(fn ConstructionScript)