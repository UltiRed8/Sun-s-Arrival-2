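; Base interactive gameplay Blueprint that completes after the player makes enough successful mouse movements.
; Capture requests pass from server to multicast, setting the interactor as owner on authority and starting BPMouseMovementComponent capture only for the local player's pawn.
; Component callbacks count successes, reset the count on uncapture, and fire MovementCompleted at the threshold, optionally soft-stopping capture.
; The completion events are empty in this base.
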(event Custom|MouseMovementSuccess
  (params (Angle :type Float%20%28double-precision%29) (Direction :type Vector%202D%20Structure))
  (bind _result (Math|Integer|IncrementInt (Variables|Default|GetCurrentMovementSuccess))
    (:%20%20
      (if (>= _result (Variables|Default|GetNeededMovementSuccess))
        (CallFunction|MovementCompleted true)
        (if (Variables|Default|GetStopMouseCaptureAtSucceess)
          (Default|SoftStopCapturing (Variables|Default|GetBP_MouseMovementComponent)))))))

(event Custom|OnMouseUncaptured
  (Variables|Default|SetCurrentMovementSuccess 0))

(event Custom|Server_StartCapture
  (params (Interactor :type Actor%20Object%20Reference))
  (CallFunction|MultiStartCapture Interactor))

(event Custom|MovementCompleted
  (params (FromMouseMovement :type Boolean)))

(event Custom|Multi_StartCapture
  (params (Interactor :type Actor%20Object%20Reference))
  (Utilities|Authority
    (:Authority
      (Actor|SetOwner Interactor))
    (:Remote
      _))
  (if (== Interactor (Pawn|GetControlledPawn (Game|GetPlayerController 0)))
    (Default|StartCapturing (Variables|Default|GetBP_MouseMovementComponent))))

(event Custom|Owning_MovementCompleted)

(event EventBeginPlay
  (bind _bp_mousemovementcomponent (Variables|Default|GetBP_MouseMovementComponent))
  (|CallParentFunction)
  (EventDispatchers|AssignOnMouseMoved _bp_mousemovementcomponent (delegate Custom|MouseMovementSuccess))
  (EventDispatchers|AssignOnMouseUncaptured _bp_mousemovementcomponent (delegate Custom|OnMouseUncaptured)))

(fn ConstructionScript)