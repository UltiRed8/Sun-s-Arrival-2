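; BP_MusicListenerAch is a trigger volume that unlocks the music listener achievement when the player stays inside it long enough.
; Entering the box starts a countdown on Tick, and reaching zero stops it and calls UnlockAchievement on the game instance.
; Leaving before completion pauses and resets the countdown, so the stay must be continuous.
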(event OnComponentBeginOverlap(Box)
  (params (OverlappedComponent :type Primitive%20Component%20Object%20Reference) (OtherActor :type Actor%20Object%20Reference) (OtherComp :type Primitive%20Component%20Object%20Reference) (OtherBodyIndex :type Integer) (bFromSweep :type Boolean) (SweepResult :type Hit%20Result%20Structure%20%28by%20ref%29))
  (Utilities|Casting|CastToBP_Player OtherActor)
  (Variables|Default|SetIsActive true))

(event OnComponentEndOverlap(Box)
  (params (OverlappedComponent :type Primitive%20Component%20Object%20Reference) (OtherActor :type Actor%20Object%20Reference) (OtherComp :type Primitive%20Component%20Object%20Reference) (OtherBodyIndex :type Integer))
  (if (!= (Variables|Default|GetTimeRemaining) 0.0)
    (Utilities|Casting|CastToBP_Player OtherActor)
    (Variables|Default|SetIsActive false)
    (Variables|Default|SetTimeRemaining 3e+01)))

(event EventTick
  (params (DeltaSeconds :type Float%20%28single-precision%29))
  (if (Variables|Default|GetIsActive)
    (bind _output_get (Variables|Default|SetTimeRemaining (- (Variables|Default|GetTimeRemaining) DeltaSeconds)))
    (if (<= _output_get 0.0)
      (Variables|Default|SetIsActive false)
      (Variables|Default|SetTimeRemaining 0.0)
      (Default|UnlockAchievement (Utilities|GameInstance) "ACH_MusicListener"))))

(fn ConstructionScript)