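; BP_MainMenuManager is a level actor that opens the main menu and switches between menu cameras.
; On BeginPlay it shows UW_Startup on first launch or UW_MainMenu afterward, using the GameInstance FirstStart flag, which it then clears.
; It also shows the mouse cursor and sets Game and UI input.
; Two events blend the player view to the main menu or customisation camera with eased transitions.
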(event Custom|SetMainMenuCamera
  (Game|Player|SetViewTargetwithBlend (Game|GetPlayerController 0) (Variables|Default|GetMainMenuCamera) 1.0 "VTBlend_EaseInOut" 2.0 false))

(event Custom|SetCustomisationCamera
  (Game|Player|SetViewTargetwithBlend (Game|GetPlayerController 0) (Variables|Default|GetCustomisationCamera) 1.0 "VTBlend_EaseInOut" 2.0 false))

(event EventBeginPlay
  (bind _returnvalue (Game|GetPlayerController 0))
  (bind _asbp_game_instance (Utilities|GameInstance))
  (bind _returnvalue_2 (UserInterface|CreateWidget (select (Variables|/Game/BP_GameInstance.BP_GameInstance_C|GetFirstStart _asbp_game_instance) "/Game/Widgets/UW_Startup.UW_Startup_C" "/Game/Widgets/UW_MainMenu.UW_MainMenu_C") (Game|GetPlayerController 0)))
  (UserInterface|Viewport|AddtoViewport _returnvalue_2 (Math|Integer|SelectInt 30 0 (Variables|/Game/BP_GameInstance.BP_GameInstance_C|GetFirstStart _asbp_game_instance)))
  (Variables|/Game/BP_GameInstance.BP_GameInstance_C|SetFirstStart _asbp_game_instance false)
  (Variables|/Script/Engine.PlayerController|SetbShowMouseCursor _returnvalue true)
  (Input|SetInputModeGameandUI _returnvalue 0 "DoNotLock" true false))

(fn ConstructionScript)