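; Panel door, a child of a parent door Blueprint, that slides open and closed with a sound and a red/green status indicator.
; Server open and close events play timelines driving the door's Y position, then call the parent logic and save state to checkpoints.
; BeginPlay restores that state using the actor's location as ID.
; Opening turns the cylinder and camera-visible child plane green, also applied at construction for open or player-toggleable doors.
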(event Custom|Multi_Sound
  (Audio|Components|Audio|Play (Variables|Default|GetOpenDoor) 0.0))

(event Custom|Multi_Open
  (Rendering|Material|SetMaterial (Variables|Default|GetCylinder) 0 "/Game/Models/EndoEnemy/MAT_GreenGlow.MAT_GreenGlow")
  (bind _asbp_camera_visible_actor (Utilities|Casting|CastToBP_CameraVisibleActor (Variables|/Script/Engine.ChildActorComponent|GetChildActor (Variables|Default|GetChildActor))))
  (Rendering|Material|SetMaterial (Variables|/Game/Blueprints/Player/BP_CameraVisibleActor.BP_CameraVisibleActor_C|GetPlane _asbp_camera_visible_actor) 0 "/Game/Materials/Instances/MI_Green.MI_Green"))

(event EventBeginPlay
  (|CallParentFunction)
  (Variables|Default|SetID (Utilities|String|ToString(Vector) (Transformation|GetActorLocation)))
  (bind _asbp_camera_visible_actor (Utilities|Casting|CastToBP_CameraVisibleActor (Variables|/Script/Engine.ChildActorComponent|GetChildActor (Variables|Default|GetChildActor)))
    (:then
      (Rendering|Material|SetMaterial (Variables|/Game/Blueprints/Player/BP_CameraVisibleActor.BP_CameraVisibleActor_C|GetPlane _asbp_camera_visible_actor) 0 "/Game/Materials/Instances/MI_Red.MI_Red"))
    (:CastFailed
      _))
  (bind (_success _bool) (Utilities|CheckpointGetBool (Variables|Default|GetID)))
  (if _success
    (if _bool
      (CallFunction|ServerOpenDoor)
      (else
        (CallFunction|ServerCloseDoor)))))

(event EventServerOpenDoor
  (CallFunction|MultiOpen)
  (CallFunction|MultiSound)
  (Utilities|CheckpointSaveBool (Variables|Default|GetID) true)
  (bind _position (Timeline|OpenDoorAnim PlayFromStart)
    (:Update
      (CallFunction|UpdateDoorData (Math|Vector|MakeVector 0.0 _position 0.0) "0, 0, 0"))
    (:Finished
      (|CallParentFunction))))

(event EventServerCloseDoor
  (CallFunction|MultiSound)
  (Utilities|CheckpointSaveBool (Variables|Default|GetID) false)
  (bind _position (Timeline|CloseDoorAnim PlayFromStart)
    (:Update
      (CallFunction|UpdateDoorData (Math|Vector|MakeVector 0.0 _position 0.0) "0, 0, 0"))
    (:Finished
      (|CallParentFunction))))

(fn ConstructionScript
  (if (or (Variables|Default|GetIsOpen) (Variables|Default|GetCanBeToggledByPlayer))
    (CallFunction|MultiOpen))
  (|CallParentFunction))