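; BP_ElevatorDoor is a floor's elevator landing door that calls the connected elevator and plays its motion sounds.
; On the server, it binds its child call button to send the elevator here with an up/down indicator, and relays the elevator's closing and stopping events to multicast start/stop sounds that chain into loops.
; A timeline slides both panels, swapping a green/red indicator, dinging, and saving the floor to the checkpoint on opening.
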(event OnAudioFinished(Audio)
  (bind _audio (Variables|Default|GetAudio))
  (if (== (Variables|/Script/Engine.AudioComponent|GetSound _audio) "/Game/Audio/Sounds/SW_ElevatorMotorStart.SW_ElevatorMotorStart")
    (Audio|Components|Audio|SetSound _audio "/Game/Audio/Sounds/SW_ElevatorMotorLoop.SW_ElevatorMotorLoop")
    (Audio|Components|Audio|Play _audio 0.0)))

(event OnAudioFinished(ElevatorOut)
  (bind _elevatorout (Variables|Default|GetElevatorOut))
  (if (== (Variables|/Script/Engine.AudioComponent|GetSound _elevatorout) "/Game/Audio/Sounds/SW_OutElevatorStart.SW_OutElevatorStart")
    (Audio|Components|Audio|SetSound _elevatorout "/Game/Audio/Sounds/SW_OutElevatorLoop.SW_OutElevatorLoop")
    (Audio|Components|Audio|Play _elevatorout 0.0)))

(event Custom|ToggleDoor
  (Utilities|FlowControl|FlipFlop
    (:A
      (CallFunction|OpenDoor)
      (bind _asbp_elevator_call_button (Utilities|Casting|CastToBP_ElevatorCallButton (Variables|/Script/Engine.ChildActorComponent|GetChildActor (Variables|Default|GetChildActor))))
      (Default|ResetMaterial _asbp_elevator_call_button))
    (:B
      (CallFunction|CloseDoor))))

(event Custom|Multi_StoppingSoundEffect
  (bind _audio (Variables|Default|GetAudio))
  (bind _elevatorout (Variables|Default|GetElevatorOut))
  (Audio|Components|Audio|SetSound _audio "/Game/Audio/Sounds/SW_ElevatorMotorStop.SW_ElevatorMotorStop")
  (Audio|Components|Audio|Play _audio 0.0)
  (Audio|Components|Audio|SetSound _elevatorout "/Game/Audio/Sounds/SW_OutElevatorStop.SW_OutElevatorStop")
  (Audio|Components|Audio|Play _elevatorout 0.0))

(event Custom|OpenDoor
  (bind _asbp_camera_visible_actor (Utilities|Casting|CastToBP_CameraVisibleActor (Variables|/Script/Engine.ChildActorComponent|GetChildActor (Variables|Default|GetChildActor4))))
  (Rendering|Material|SetMaterial (Variables|/Game/Blueprints/Player/BP_CameraVisibleActor.BP_CameraVisibleActor_C|GetPlane _asbp_camera_visible_actor) 0 "/Game/Materials/Instances/MI_Green.MI_Green")
  (Utilities|FlowControl|Sequence
    (:then_0
      (Audio|Components|Audio|Play (Variables|Default|GetElevatorDoor) 0.0)
      (bind _dooropening (Timeline|Timeline Play)
        (:Update
          (Transformation|SetRelativeLocation (Variables|Default|GetDoorA) (Math|Vector|MakeVector -6.3e+02 _dooropening 2e+02) false false)
          (Transformation|SetRelativeLocation (Variables|Default|GetDoorB) (Math|Vector|MakeVector -6.3e+02 (* _dooropening -1.0) 2e+02) false false))))
    (:then_1
      (Utilities|FlowControl|Delay 0.5)
      (Audio|Components|Audio|Play (Variables|Default|GetSW_ElevatorDing) 0.0))
    (:then_2
      (Variables|/Game/Saves/SG_Checkpoint.SG_Checkpoint_C|SetElevatorFloor (Variables|/Game/BP_GameInstance.BP_GameInstance_C|GetCheckpoint (Utilities|GameInstance)) (Variables|Default|GetElevator%20Floor)))))

(event Custom|CloseDoor
  (bind _asbp_camera_visible_actor (Utilities|Casting|CastToBP_CameraVisibleActor (Variables|/Script/Engine.ChildActorComponent|GetChildActor (Variables|Default|GetChildActor4))))
  (Rendering|Material|SetMaterial (Variables|/Game/Blueprints/Player/BP_CameraVisibleActor.BP_CameraVisibleActor_C|GetPlane _asbp_camera_visible_actor) 0 "/Game/Materials/Instances/MI_Red.MI_Red")
  (Audio|Components|Audio|Play (Variables|Default|GetElevatorDoor) 0.0)
  (bind _dooropening (Timeline|Timeline Reverse)
    (:Update
      (Transformation|SetRelativeLocation (Variables|Default|GetDoorA) (Math|Vector|MakeVector -6.3e+02 _dooropening 2e+02) false false)
      (Transformation|SetRelativeLocation (Variables|Default|GetDoorB) (Math|Vector|MakeVector -6.3e+02 (* _dooropening -1.0) 2e+02) false false))))

(event Custom|Multi_ClosingDoorsSoundEffect
  (bind _audio (Variables|Default|GetAudio))
  (bind _elevatorout (Variables|Default|GetElevatorOut))
  (Audio|Components|Audio|SetSound _audio "/Game/Audio/Sounds/SW_ElevatorMotorStart.SW_ElevatorMotorStart")
  (Audio|Components|Audio|Play _audio 0.0)
  (Audio|Components|Audio|SetSound _elevatorout "/Game/Audio/Sounds/SW_OutElevatorStart.SW_OutElevatorStart")
  (Audio|Components|Audio|Play _elevatorout 0.0))

(event Custom|CallElevator
  (params (Floor :type BP%20Elevator%20Door%20Object%20Reference))
  (bind _returnvalue (Transformation|GetActorLocation))
  (bind _connectedelevator (Variables|Default|GetConnectedElevator)
    (:then
      (Default|Goto _connectedelevator self)
      (bind _asbp_elevator_call_button (Utilities|Casting|CastToBP_ElevatorCallButton (Variables|/Script/Engine.ChildActorComponent|GetChildActor (Variables|Default|GetChildActor))))
      (if (< (.z (Transformation|GetActorLocation _connectedelevator)) (.z _returnvalue))
        (Default|GoingUpMaterial _asbp_elevator_call_button)
        (elif (> (.z (Transformation|GetActorLocation _connectedelevator)) (.z _returnvalue))
          (Default|GoingDownMaterial _asbp_elevator_call_button))))
    (:else)))

(event Custom|Stopping_Event
  (CallFunction|MultiStoppingSoundEffect))

(event Custom|ClosingDoors_Event
  (CallFunction|MultiClosingDoorsSoundEffect))

(event EventBeginPlay
  (bind _connectedelevator (Variables|Default|GetConnectedElevator))
  (Audio|Components|Audio|SetVolumeMultiplier (Variables|Default|GetAudio) (Math|Float|SelectFloat 3.0 0.0 (Variables|Default|GetIsTopHasSounds)) :!class /Script/Engine.AudioComponent)
  (Utilities|Authority
    (:Authority
      (bind _asbp_elevator_call_button (Utilities|Casting|CastToBP_ElevatorCallButton (Variables|/Script/Engine.ChildActorComponent|GetChildActor (Variables|Default|GetChildActor))))
      (EventDispatchers|AssignOnTriggered _asbp_elevator_call_button (delegate Custom|CallElevator))
      (Utilities|FlowControl|DelayUntilNextTick)
      (Utilities|IsValid _connectedelevator
        (:Is%20Valid
          (EventDispatchers|AssignClosingDoors _connectedelevator (delegate Custom|ClosingDoors_Event))
          (EventDispatchers|AssignStopping _connectedelevator (delegate Custom|Stopping_Event)))))))

(fn ConstructionScript)