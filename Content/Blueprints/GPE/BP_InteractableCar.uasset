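; Interactable car prop that flashes its lights and plays a sound when interacted with.
; It registers as an interactable on BeginPlay, unregisters on Destroyed, and starts the Multi blinking and sound events when interaction is allowed.
; A looping timeline toggles two spotlights and the car's yellow and red glow materials.
; A retriggerable delay clears the blinking flag, so the lights switch off after the current cycle finishes.
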(event Custom|Multi_PlaySound
  (Audio|Components|Audio|Play (Variables|Default|GetAudio) 0.0))

(event Custom|On
  (bind _car (Variables|Default|GetCar))
  (Rendering|Components|Light|SetIntensity (Variables|Default|GetSpotLight1) 5e+04)
  (Rendering|Material|SetMaterial _car 2 "/Game/Models/EndoEnemy/MAT_YellowGlow.MAT_YellowGlow")
  (Rendering|Material|SetMaterial _car 3 "/Game/Models/EndoEnemy/MAT_RedGlow.MAT_RedGlow"))

(event Custom|Off
  (bind _car (Variables|Default|GetCar))
  (Rendering|Components|Light|SetIntensity (Variables|Default|GetSpotLight1) 0.0)
  (Rendering|Material|SetMaterial _car 2 "/Game/Materials/Instances/MI_Yellow.MI_Yellow")
  (Rendering|Material|SetMaterial _car 3 "/Game/Materials/Instances/MI_Red.MI_Red"))

(event Custom|Multi_Blinking
  (CallFunction|MultiPlaySound)
  (Utilities|FlowControl|Sequence
    (:then_0
      (Variables|Default|SetIsBlinking true))
    (:then_1
      (bind _blinking (Timeline|Blinking PlayFromStart)
        (:Update
          (if (> _blinking 0.5)
            (CallFunction|On)
            (else
              (CallFunction|Off))))
        (:Finished
          (if (Variables|Default|GetIsBlinking)
            (Timeline|Blinking PlayFromStart)
            (else
              (CallFunction|Off))))))
    (:then_2
      (Utilities|FlowControl|RetriggerableDelay 2.0)
      (Variables|Default|SetIsBlinking false))))

(event EventBeginPlay
  (Utilities|RegisterInteractable))

(event EventInteraction
  (|CallParentFunction)
  (if (Variables|Default|GetCanBeInteract)
    (CallFunction|MultiBlinking)))

(event EventDestroyed
  (Utilities|UnregisterInteractable))

(fn ConstructionScript)