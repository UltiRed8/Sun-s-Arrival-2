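; Interactable keyboard gameplay element that plays a sound when the player interacts with it.
; It registers itself as an interactable on BeginPlay, before running the parent BeginPlay, and unregisters when destroyed.
; Interaction runs the parent logic first, then triggers PlaySound if CanBeInteract is true, which plays the Audio component from the start when it is valid.
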(event Custom|PlaySound
  (Utilities|IsValid (Variables|Default|GetAudio)
    (:Is%20Valid
      (Audio|Components|Audio|Play (Variables|Default|GetAudio) 0.0))))

(event EventBeginPlay
  (Utilities|RegisterInteractable)
  (|CallParentFunction))

(event EventInteraction
  (|CallParentFunction)
  (if (Variables|Default|GetCanBeInteract)
    (CallFunction|PlaySound)))

(event EventDestroyed
  (Utilities|UnregisterInteractable))

(fn ConstructionScript)