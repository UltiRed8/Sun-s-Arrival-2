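; Night ambience manager actor that switches audio between exterior and interior as the locally controlled player overlaps its interior or exterior trigger box.
; Triggers set a target volume that Tick interpolates at constant speed for the Night and Wind sounds, while registered windows' audio switches instantly to the opposite level.
; The inside/outside state saves to a checkpoint keyed by actor location, and BeginPlay reapplies a saved interior state.
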(event OnComponentBeginOverlap(InteriorBox)
  (params (OverlappedComponent :type Primitive%20Component%20Object%20Reference) (OtherActor :type Actor%20Object%20Reference) (OtherComp :type Primitive%20Component%20Object%20Reference) (OtherBodyIndex :type Integer) (bFromSweep :type Boolean) (SweepResult :type Hit%20Result%20Structure%20%28by%20ref%29))
  (bind _asbp_player (Utilities|Casting|CastToBP_Player OtherActor))
  (if (Pawn|IsLocallyControlled _asbp_player)
    (Variables|Default|SetTargetExteriorVolume 0.0)
    (for _array_element (Variables|Default|GetAllWindows)
      (Audio|Components|Audio|SetVolumeMultiplier (Variables|/Game/Blueprints/GPE/BP_Window.BP_Window_C|GetAudio _array_element) 1.0 :!class /Script/Engine.AudioComponent)
      (Utilities|CheckpointSaveBool (Utilities|String|ToString(Vector) (Transformation|GetActorLocation)) true))))

(event OnComponentBeginOverlap(ExteriorBox)
  (params (OverlappedComponent :type Primitive%20Component%20Object%20Reference) (OtherActor :type Actor%20Object%20Reference) (OtherComp :type Primitive%20Component%20Object%20Reference) (OtherBodyIndex :type Integer) (bFromSweep :type Boolean) (SweepResult :type Hit%20Result%20Structure%20%28by%20ref%29))
  (bind _asbp_player (Utilities|Casting|CastToBP_Player OtherActor))
  (if (Pawn|IsLocallyControlled _asbp_player)
    (Variables|Default|SetTargetExteriorVolume 1.0)
    (for _array_element (Variables|Default|GetAllWindows)
      (Audio|Components|Audio|SetVolumeMultiplier (Variables|/Game/Blueprints/GPE/BP_Window.BP_Window_C|GetAudio _array_element) 0.0 :!class /Script/Engine.AudioComponent)
      (Utilities|CheckpointSaveBool (Utilities|String|ToString(Vector) (Transformation|GetActorLocation)) false))))

(event Custom|RegisterWindow
  (params (Window :type BP%20Window%20Object%20Reference%20%28by%20ref%29))
  (Utilities|Array|Add (Variables|Default|GetAllWindows) Window))

(event EventBeginPlay
  (bind _returnvalue (Transformation|GetActorLocation))
  (bind _returnvalue_2 (Utilities|String|ToString(Vector) _returnvalue))
  (bind (_success _bool) (Utilities|CheckpointGetBool _returnvalue_2))
  (if _success
    (if _bool
      (Variables|Default|SetTargetExteriorVolume 0.0)
      (for _array_element (Variables|Default|GetAllWindows)
        (Audio|Components|Audio|SetVolumeMultiplier (Variables|/Game/Blueprints/GPE/BP_Window.BP_Window_C|GetAudio _array_element) 1.0 :!class /Script/Engine.AudioComponent)
        (Utilities|CheckpointSaveBool _returnvalue_2 true)))))

(event EventTick
  (params (DeltaSeconds :type Float%20%28single-precision%29))
  (bind _targetexteriorvolume (Variables|Default|GetTargetExteriorVolume))
  (if (not (== (Variables|Default|GetCurrentVolume) _targetexteriorvolume))
    (bind _output_get (Variables|Default|SetCurrentVolume (Math|Interpolation|FInterptoConstant (Variables|Default|GetCurrentVolume) _targetexteriorvolume DeltaSeconds 1.0)))
    (Audio|Components|Audio|SetVolumeMultiplier (Variables|Default|GetNight) _output_get :!class /Script/Engine.AudioComponent)))

(fn ConstructionScript)