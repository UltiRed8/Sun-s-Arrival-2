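; Suspended disco light whose point light color shifts while disco mode is active.
; Three timelines (ColorR, ColorG, ColorB) get different play rates on BeginPlay and each feeds one color channel, though the graph never calls Play on them.
; Tick applies the combined color while active.
; ToggleDisco flips that state and resets the light to white when switched off.
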(event Custom|ToggleDisco
  (bind _output_get (Variables|Default|SetIsActive (not (Variables|Default|GetIsActive))))
  (if (not _output_get)
    (Rendering|Components|Light|SetLightColor (Variables|Default|GetPointLight) (Utilities|Struct|MakeLinearColor 1.0 1.0 1.0 1.0) true)))

(event EventBeginPlay
  (Components|Timeline|SetPlayRate (Variables|Default|GetColorR) 0.5)
  (Components|Timeline|SetPlayRate (Variables|Default|GetColorG) 0.3)
  (Components|Timeline|SetPlayRate (Variables|Default|GetColorB) 0.1))

(event EventTick
  (params (DeltaSeconds :type Float%20%28single-precision%29))
  (if (Variables|Default|GetIsActive)
    (Rendering|Components|Light|SetLightColor (Variables|Default|GetPointLight) (Utilities|Struct|MakeLinearColor (Variables|Default|GetRed) (Variables|Default|GetGreen) (Variables|Default|GetBlue) 1.0) true)))

(fn ConstructionScript)