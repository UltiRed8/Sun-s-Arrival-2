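; BP_SuspendedLight is a light prop with Off, Blinking and On states that drive its point light and sounds.
; SetState applies the initial state on BeginPlay, then reruns only when the state changes, clearing any blink timer.
; On and Off toggle light visibility alongside the Ambient and PowerOn audio.
; Blinking uses a looping timer with randomized delays for irregular flicker, switching off again only while still Blinking.
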(event Custom|SetState
  (params (NewState :type E_LightState%20Enum :default "NewEnumerator0"))
  (bind _blinkingtimer (Variables|Default|GetBlinkingTimer))
  (Utilities|FlowControl|Sequence
    (:then_0
      (Utilities|FlowControl|DoOnce false
        (:Completed
          (bind _output_get (Variables|Default|SetLightState NewState :!label _label))
          (if (Utilities|Time|IsValidTimerHandle _blinkingtimer)
            (Utilities|Time|ClearandInvalidateTimerbyHandle _blinkingtimer))
          (switch Utilities|FlowControl|Switch|SwitchonE_LightState _output_get
            (:NewEnumerator0
              (CallFunction|Off))
            (:NewEnumerator1
              (CallFunction|Blinking))
            (:NewEnumerator2
              (CallFunction|On))))))
    (:then_1
      (if (Utilities|Enum|NotEqual(Enum) NewState (Variables|Default|GetLightState))
        (goto _label)))))

(event Custom|Off
  (Rendering|SetVisibility (Variables|Default|GetPointLight) false false)
  (Audio|Components|Audio|Stop (Variables|Default|GetAmbient))
  (Audio|Components|Audio|Stop (Variables|Default|GetPowerOn)))

(event Custom|On
  (Rendering|SetVisibility (Variables|Default|GetPointLight) true false)
  (Audio|Components|Audio|Play (Variables|Default|GetAmbient) 0.0)
  (Audio|Components|Audio|Play (Variables|Default|GetPowerOn) 0.0))

(event Custom|Blinking
  (bind _returnvalue (Utilities|Time|SetTimerbyFunctionName 0 "DoBlink" 2.0 true false 0.0 1.0))
  (Variables|Default|SetBlinkingTimer _returnvalue))

(event Custom|DoBlink
  (Utilities|FlowControl|Delay (Math|Random|RandomFloatinRange 0.5 1.5))
  (CallFunction|On)
  (Utilities|FlowControl|Delay (Math|Random|RandomFloatinRange 0.1 0.8))
  (switch Utilities|FlowControl|Switch|SwitchonE_LightState (Variables|Default|GetLightState)
    (:NewEnumerator1
      (CallFunction|Off))))

(event EventBeginPlay
  (CallFunction|SetState (Variables|Default|GetLightState)))

(fn ConstructionScript)