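; Interactable desk light Blueprint that switches its point light between two intensities when the player interacts with it.
; Interaction runs the parent logic, then, if interaction is allowed, toggles the intensity and plays the interact sound at the actor's location.
; The toggle picks the target by comparing the current intensity to the second value.
; On BeginPlay, a light that is not enabled toggles once without sound.
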(event Custom|PlayLightSound
  (Utilities|IsValid (Variables|Default|GetInteractSound)
    (:Is%20Valid
      (Audio|PlaySoundatLocation (Variables|Default|GetInteractSound) (Transformation|GetActorLocation) "0, 0, 0" 1.0 1.0 0.0 0 0 0 0))))

(event Custom|MultiToggleLight
  (params (WithSound :type Boolean))
  (bind _pointlight (Variables|Default|GetPointLight))
  (if (== (Variables|/Script/Engine.LightComponentBase|GetIntensity (Variables|Default|GetPointLight)) (Variables|Default|GetSecondIntensity))
    (Rendering|Components|Light|SetIntensity _pointlight (Variables|Default|GetFirstIntensity))
    (else
      (Rendering|Components|Light|SetIntensity _pointlight (Variables|Default|GetSecondIntensity))))
  (if WithSound
    (CallFunction|PlayLightSound)))

(event EventBeginPlay
  (|CallParentFunction)
  (if (not (Variables|Default|GetIsEnabled))
    (CallFunction|MultiToggleLight false)))

(event EventInteraction
  (|CallParentFunction)
  (if (Variables|Default|GetCanBeInteract)
    (CallFunction|MultiToggleLight true)))

(fn ConstructionScript)