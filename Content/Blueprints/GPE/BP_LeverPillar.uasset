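; BP_LeverPillar is an interactable lever that fires its trigger callback and, after a short delay, triggers a linked Node.
; Client interaction starts mouse capture and swaps the cursor texture; server interaction is routed through BP_Player.
; Activation animates the handle down with sounds, then reverses it, with a DidIt flag blocking reuse until the lever resets.
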(event Custom|FuseboxAnimation
  (Audio|Components|Audio|Play (Variables|Default|GetLeverDown) 0.0)
  (bind _rotation (Timeline|HandleAnimation PlayFromStart)
    (:Update
      (Transformation|SetRelativeRotation (Variables|Default|GetHandlePivot) (Math|Rotator|MakeRotator 0.0 _rotation 0.0) false false))
    (:Finished
      (Audio|Components|Audio|Play (Variables|Default|GetLeverDownEnd) 0.0)
      (Utilities|FlowControl|Delay 0.2)
      (bind _rotation_2 (Timeline|Timeline ReverseFromEnd)
        (:Update
          (Transformation|SetRelativeRotation (Variables|Default|GetHandlePivot) (Math|Rotator|MakeRotator 0.0 _rotation_2 0.0) false false))
        (:Finished
          (Variables|Default|SetDidIt false))))))

(event Custom|OnMouseCapture_Event_0
  (Variables|/Game/Blueprints/Components/BP_CustomCursorComponent.BP_CustomCursorComponent_C|SetCursorTexture (Variables|Default|GetBP_CustomCursorComponent) "/Game/Textures/T_CursorMouseDown.T_CursorMouseDown"))

(event Custom|OnMouseUncaptured_Event
  (Variables|/Game/Blueprints/Components/BP_CustomCursorComponent.BP_CustomCursorComponent_C|SetCursorTexture (Variables|Default|GetBP_CustomCursorComponent) "/Game/Textures/T_CursorInteract.T_CursorInteract"))

(event EventServerInteract
  (params (WhoInteracted :type Actor%20Object%20Reference))
  (if (not (Variables|Default|GetDidIt))
    (bind _asbp_player (Utilities|Casting|CastToBP_Player WhoInteracted))
    (Default|FromServerInteractwith _asbp_player self)))

(event EventOntoServerInteract
  (params (MethodName :type String))
  (if (not (Variables|Default|GetDidIt))
    (Variables|Default|SetDidIt true)
    (CallFunction|FuseboxAnimation)
    (Default|CallOnTriggered)
    (Utilities|FlowControl|Delay 0.15)
    (bind _node (Variables|Default|GetNode)
      (:then
        (Default|Trigger _node))
      (:else))))

(event EventDestroyed
  (Utilities|UnregisterInteractable))

(event EventBeginPlay
  (bind _bp_mousemovementcomponent (Variables|Default|GetBP_MouseMovementComponent))
  (Utilities|RegisterInteractable)
  (|CallParentFunction)
  (EventDispatchers|AssignOnMouseCapture _bp_mousemovementcomponent (delegate Custom|OnMouseCapture_Event_0))
  (EventDispatchers|AssignOnMouseUncaptured _bp_mousemovementcomponent (delegate Custom|OnMouseUncaptured_Event))
  (Variables|/Game/Blueprints/Components/BP_CustomCursorComponent.BP_CustomCursorComponent_C|SetCursorTexture (Variables|Default|GetBP_CustomCursorComponent) "/Game/Textures/T_CursorInteract.T_CursorInteract"))

(event EventClientInteract
  (Default|StartCapturing (Variables|Default|GetBP_MouseMovementComponent))
  (Variables|/Game/Blueprints/Components/BP_CustomCursorComponent.BP_CustomCursorComponent_C|SetCursorTexture (Variables|Default|GetBP_CustomCursorComponent) "/Game/Textures/T_CursorMouseDown.T_CursorMouseDown"))

(fn ConstructionScript)