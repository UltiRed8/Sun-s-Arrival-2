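; Keycard reader interactable that triggers a linked Node when the swiped card's ID is in the inventory.
; Interacting animates the card into place, then runs a mouse-capture swipe or completes directly, leading to success or temporary denied feedback.
; Success saves a checkpoint bool keyed by actor location, restored on BeginPlay, and can auto-reset.
; The construction script labels the reader from KeycardID.
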(event Custom|KeycardAnimation
  (bind (_direction _zposition _xposition _scale) (Timeline|SwipeAnimation PlayFromStart)
    (:Update
      (Transformation|SetRelativeTransform (Variables|Default|GetCard) (Math|Transform|MakeTransform (Math|Vector|MakeVector (+ _xposition 37.5) 8.5 _zposition) "0.000000,0.000000,90.100000" (Math|Vector|MakeVector (* _scale 0.045) (* _scale 0.045) (* _scale 0.045))) false false))
    (:Sound
      (Utilities|FlowControl|Delay 0.1)
      (Audio|Components|Audio|Play (Variables|Default|GetSwipe) 0.0))))

(event Custom|SuccessColor
  (Rendering|Material|SetMaterial (Variables|Default|GetReader) 1 "/Game/Materials/Instances/MI_KeycardReaderSuccess.MI_KeycardReaderSuccess")
  (Audio|Components|Audio|Play (Variables|Default|GetSuccess) 0.0)
  (Variables|/Game/Blueprints/Components/BP_CustomCursorComponent.BP_CustomCursorComponent_C|SetCursorTexture (Variables|Default|GetBP_CustomCursorComponent) "/Game/Textures/T_CursorNormal.T_CursorNormal")
  (Rendering|SetVisibility (Variables|Default|GetIDText1) false false))

(event Custom|OnMouseCapture_Event
  (Variables|/Game/Blueprints/Components/BP_CustomCursorComponent.BP_CustomCursorComponent_C|SetCursorTexture (Variables|Default|GetBP_CustomCursorComponent) "/Game/Textures/T_CursorMouseDown.T_CursorMouseDown"))

(event Custom|TryInteract
  (params (Interactor :type Actor%20Object%20Reference) (Condition :type Boolean))
  (if Condition
    (CallFunction|ServerStartCapture Interactor)
    (else
      (CallFunction|MovementCompleted false))))

(event Custom|IdleColor
  (Rendering|Material|SetMaterial (Variables|Default|GetReader) 1 "/Game/Materials/Instances/MI_KeycardReaderIdle.MI_KeycardReaderIdle")
  (Rendering|SetVisibility (Variables|Default|GetIDText1) true false))

(event Custom|Reset
  (CallFunction|IdleColor)
  (Variables|Default|SetDidIt false)
  (Variables|Default|SetHasKeycard false)
  (Variables|/Game/Blueprints/Components/BP_CustomCursorComponent.BP_CustomCursorComponent_C|SetCursorTexture (Variables|Default|GetBP_CustomCursorComponent) "/Game/Textures/T_CursorInteract.T_CursorInteract")
  (Variables|Default|SetCooldown false))

(event Custom|ErrorColor
  (Rendering|Material|SetMaterial (Variables|Default|GetReader) 1 "/Game/Materials/Instances/MI_KeycardReaderDenied.MI_KeycardReaderDenied")
  (Audio|Components|Audio|Play (Variables|Default|GetDenied) 0.5)
  (Rendering|SetVisibility (Variables|Default|GetIDText1) false false)
  (Utilities|FlowControl|Delay 2.0)
  (CallFunction|IdleColor)
  (Variables|/Game/Blueprints/Components/BP_CustomCursorComponent.BP_CustomCursorComponent_C|SetCursorTexture (Variables|Default|GetBP_CustomCursorComponent) "/Game/Textures/T_CursorInteract.T_CursorInteract"))

(event Custom|SuccessEvent
  (params (IsOfficial :type Boolean))
  (Variables|Default|SetDidIt true)
  (Default|CallOnTriggered)
  (CallFunction|SuccessColor)
  (if IsOfficial
    (bind _node (Variables|Default|GetNode)
      (:then
        (Default|Trigger _node)
        (Utilities|CheckpointSaveBool (Utilities|String|ToString(Vector) (Transformation|GetActorLocation)) true)
        (if (Variables|Default|GetAutoReset)
          (Utilities|FlowControl|Delay 1.0)
          (CallFunction|Reset)))
      (:else))))

(event Custom|Multi_PlaceKeycard
  (bind (_direction _xposition _scale) (Timeline|Timeline PlayFromStart)
    (:Update
      (Transformation|SetRelativeTransform (Variables|Default|GetCard) (Math|Transform|MakeTransform (Math|Vector|MakeVector (+ _xposition 37.5) 8.5 35.0) "0.000000,0.000000,90.100000" (Math|Vector|MakeVector (* _scale 0.045) (* _scale 0.045) (* _scale 0.045))) false false))))

(event Custom|OnMouseUncaptured_Event
  (Variables|/Game/Blueprints/Components/BP_CustomCursorComponent.BP_CustomCursorComponent_C|SetCursorTexture (Variables|Default|GetBP_CustomCursorComponent) (select (Variables|Default|GetDidIt) "/Game/Textures/T_CursorNormal.T_CursorNormal" "/Game/Textures/T_CursorInteract.T_CursorInteract")))

(event EventInteracted
  (params (HitComponent :type Actor%20Component%20Object%20Reference%20%28by%20ref%29) (WhoInteracted :type Actor%20Object%20Reference) (HasMouseMovements :type Boolean) (IsServer :type Boolean))
  (if (not (or (Variables|Default|GetDidIt) (Variables|Default|GetCooldown)))
    (if (Variables|Default|GetHasKeycard)
      (bind _asbp_player (Utilities|Casting|CastToBP_Player WhoInteracted :!label _label))
      (CallFunction|TryInteract _asbp_player HasMouseMovements)
      (else
        (Variables|Default|SetCooldown true)
        (Variables|Default|SetHasKeycard true)
        (CallFunction|MultiPlaceKeycard)
        (Utilities|FlowControl|Sequence
          (:then_0
            (goto _label))
          (:then_1
            (Utilities|FlowControl|Delay 0.3)
            (Variables|Default|SetCooldown false)))))))

(event EventBeginPlay
  (bind _bp_mousemovementcomponent (Variables|Default|GetBP_MouseMovementComponent))
  (|CallParentFunction)
  (EventDispatchers|AssignOnMouseCapture _bp_mousemovementcomponent (delegate Custom|OnMouseCapture_Event))
  (EventDispatchers|AssignOnMouseUncaptured _bp_mousemovementcomponent (delegate Custom|OnMouseUncaptured_Event))
  (bind (_success _bool) (Utilities|CheckpointGetBool (Utilities|String|ToString(Vector) (Transformation|GetActorLocation))))
  (if _success
    (if _bool
      (CallFunction|SuccessEvent true))))

(event EventMovementCompleted
  (params (FromMouseMovement :type Boolean))
  (Variables|Default|SetCooldown true)
  (CallFunction|KeycardAnimation)
  (Utilities|FlowControl|Delay 0.4)
  (bind _returnvalue (Default|HasItem (Utilities|Inventory) (Variables|Default|GetKeycardID)))
  (if _returnvalue
    (CallFunction|SuccessEvent true)
    (else
      (CallFunction|ErrorColor)
      (Variables|Default|SetCooldown false)
      (Variables|Default|SetHasKeycard false))))

(fn ConstructionScript
  (bind _keycardid (Variables|Default|GetKeycardID))
  (if (Utilities|String|Contains _keycardid "Master")
    (Rendering|Components|TextRender|SetText (Variables|Default|GetIDText) (Utilities|Text|MakeLiteralText "M"))
    (else
      (Rendering|Components|TextRender|SetText (Variables|Default|GetIDText) (Utilities|Text|ToText(String) (Utilities|String|Right _keycardid 1))))))