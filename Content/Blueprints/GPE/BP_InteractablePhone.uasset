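; Interactable phone prop that dials a preset key sequence, stepping through one key per interaction.
; Key characters come from the SimpleKeys string when it is set.
; Each press runs Multi_PlaySound, which plays that key's dial tone, appends it to a short scrolling text display and briefly flashes one of nine visibility targets.
; A retriggerable delay clears the display and resets the index after three idle seconds.
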(event Custom|Multi_PlaySound
  (bind _keys (Variables|Default|GetKeys))
  (bind _textrender (Variables|Default|GetTextRender))
  (bind _result (Math|Integer|IncrementInt (Variables|Default|GetCurrentIndex))
    (:%20%20
      (if (>= _result (Utilities|Array|Length _keys))
        (Variables|Default|SetCurrentIndex 0))
      (Audio|PlaySoundatLocation (.Value (Utilities|Map|Find (Utilities|Map|MakeMap "0" "/Game/Audio/Sounds/Phones/SW_PhoneDialKey0.SW_PhoneDialKey0" "1" "/Game/Audio/Sounds/Phones/SW_PhoneDialKey1.SW_PhoneDialKey1" "2" "/Game/Audio/Sounds/Phones/SW_PhoneDialKey2.SW_PhoneDialKey2" "3" "/Game/Audio/Sounds/Phones/SW_PhoneDialKey3.SW_PhoneDialKey3" "4" "/Game/Audio/Sounds/Phones/SW_PhoneDialKey4.SW_PhoneDialKey4" "5" "/Game/Audio/Sounds/Phones/SW_PhoneDialKey5.SW_PhoneDialKey5" "6" "/Game/Audio/Sounds/Phones/SW_PhoneDialKey6.SW_PhoneDialKey6" "7" "/Game/Audio/Sounds/Phones/SW_PhoneDialKey7.SW_PhoneDialKey7" "8" "/Game/Audio/Sounds/Phones/SW_PhoneDialKey8.SW_PhoneDialKey8" "9" "/Game/Audio/Sounds/Phones/SW_PhoneDialKey9.SW_PhoneDialKey9" "*" "/Game/Audio/Sounds/Phones/SW_PhoneDialKeyStar.SW_PhoneDialKeyStar" "#" "/Game/Audio/Sounds/Phones/SW_PhoneDialKeyHash.SW_PhoneDialKeyHash") (Utilities|Array|Get(acopy) _keys (Variables|Default|GetCurrentIndex)))) "0, 0, 0" "0, 0, 0" 1e+01 1.0 0.0 0 0 0 0)
      (if (Utilities|Enum|Equal(Enum) (Utilities|Array|Get(acopy) _keys (Variables|Default|GetCurrentIndex)) " ")
        _
        (else
          (if (>= (Utilities|String|Len (Utilities|String|Append (Utilities|String|ToString(Text) (Variables|/Script/Engine.TextRenderComponent|GetText (Variables|Default|GetTextRender))) (Utilities|Array|Get(acopy) _keys (Variables|Default|GetCurrentIndex)))) 8)
            (Rendering|Components|TextRender|SetText _textrender (Utilities|Text|ToText(String) (Utilities|String|RightChop (Utilities|String|Append (Utilities|String|ToString(Text) (Variables|/Script/Engine.TextRenderComponent|GetText (Variables|Default|GetTextRender))) (Utilities|Array|Get(acopy) _keys (Variables|Default|GetCurrentIndex))) 1)))
            (else
              (Rendering|Components|TextRender|SetText _textrender (Utilities|Text|ToText(String) (Utilities|String|Append (Utilities|String|ToString(Text) (Variables|/Script/Engine.TextRenderComponent|GetText (Variables|Default|GetTextRender))) (Utilities|Array|Get(acopy) _keys (Variables|Default|GetCurrentIndex)))))))
          (Utilities|ToggleVisibility (Utilities|Array|Get(acopy) (Utilities|Array|MakeArray (Variables|Default|Get1) (Variables|Default|Get2) (Variables|Default|Get3) (Variables|Default|Get4) (Variables|Default|Get5) (Variables|Default|Get6) (Variables|Default|Get7) (Variables|Default|Get8) (Variables|Default|Get9)) (- (Math|Conversions|ToInteger(Byte) (Utilities|String|Replace (Utilities|String|Replace (Utilities|String|Replace (Utilities|Array|Get(acopy) _keys (Variables|Default|GetCurrentIndex)) "0" "1") "*" "2") "#" "3")) 1)))))
      (Utilities|FlowControl|RetriggerableDelay 3.0)
      (Rendering|Components|TextRender|SetText _textrender (Utilities|Text|MakeLiteralText ""))
      (Variables|Default|SetCurrentIndex 0))))

(event EventBeginPlay
  (Utilities|RegisterInteractable)
  (|CallParentFunction)
  (if (not (Utilities|Array|IsEmpty (Variables|Default|GetSimpleKeys)))
    (Variables|Default|SetKeys (Utilities|String|GetCharacterArrayfromString (Variables|Default|GetSimpleKeys)))))

(event EventInteraction
  (|CallParentFunction)
  (if (Variables|Default|GetCanBeInteract)
    (CallFunction|MultiPlaySound)))

(event EventDestroyed
  (Utilities|UnregisterInteractable))

(fn ConstructionScript)