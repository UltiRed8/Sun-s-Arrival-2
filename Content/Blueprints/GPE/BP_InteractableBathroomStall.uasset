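; Interactable bathroom stall whose door toggles open and closed with a sound.
; Interaction relays through server and multicast events, then a FlipFlop plays open or close timelines that rotate the Axis component, blocking re-interaction until finished.
; The open state is saved as a checkpoint bool keyed by the actor's location, and BeginPlay replays the opening if saved open.
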(event Custom|Multi_OpenDoor
  (Variables|Default|SetCanBeInteract false)
  (if (== (Variables|Default|GetInteractComponent) (Variables|Default|GetDoor))
    (CallFunction|PlaySounds)
    (Utilities|FlowControl|Sequence
      (:then_0
        (Utilities|FlowControl|FlipFlop
          (:A
            (Variables|Default|SetIsOpen true)
            (bind _opendoortrack (Timeline|OpenDoor PlayFromStart)
              (:Update
                (Transformation|SetRelativeRotation (Variables|Default|GetAxis) (Math|Rotator|MakeRotator 0.0 0.0 _opendoortrack) false false))
              (:Finished
                (Variables|Default|SetCanBeInteract true :!label _label))))
          (:B
            (Variables|Default|SetIsOpen false)
            (bind _opendoortrack_2 (Timeline|CloseDoor PlayFromStart)
              (:Update
                (Transformation|SetRelativeRotation (Variables|Default|GetAxis) (Math|Rotator|MakeRotator 0.0 0.0 _opendoortrack_2) false false))
              (:Finished
                (goto _label))))))
      (:then_1
        (Utilities|CheckpointSaveBool (Utilities|String|ToString(Vector) (Transformation|GetActorLocation)) (Variables|Default|GetIsOpen))))
    (else
      (goto _label))))

(event Custom|Server_OpenDoor
  (CallFunction|MultiOpenDoor))

(event Custom|PlaySounds
  (bind _isopen (Variables|Default|GetIsOpen))
  (bind _interactsound (Variables|Default|GetInteractSound))
  (bind _closesound (Variables|Default|GetCloseSound))
  (bind _returnvalue (select _isopen _closesound _interactsound))
  (Utilities|IsValid _returnvalue
    (:Is%20Valid
      (Audio|PlaySoundatLocation _returnvalue (Transformation|GetActorLocation) "0, 0, 0" 1.0 1.0 0.0 0 0 0 0))))

(event EventInteraction
  (|CallParentFunction)
  (if (Variables|Default|GetCanBeInteract)
    (CallFunction|ServerOpenDoor)))

(event EventBeginPlay
  (Utilities|RegisterInteractable)
  (|CallParentFunction)
  (bind (_success _bool) (Utilities|CheckpointGetBool (Utilities|String|ToString(Vector) (Transformation|GetActorLocation))))
  (if _success
    (if _bool
      (Variables|Default|SetCanBeInteract false)
      (Utilities|FlowControl|FlipFlop
        (:A
          (Variables|Default|SetIsOpen true)
          (bind _opendoortrack (Timeline|OpenDoor PlayFromStart)
            (:Update
              (Transformation|SetRelativeRotation (Variables|Default|GetAxis) (Math|Rotator|MakeRotator 0.0 0.0 _opendoortrack) false false))
            (:Finished
              (Variables|Default|SetCanBeInteract true :!label _label))))
        (:B
          (Variables|Default|SetIsOpen false)
          (bind _opendoortrack_2 (Timeline|CloseDoor PlayFromStart)
            (:Update
              (Transformation|SetRelativeRotation (Variables|Default|GetAxis) (Math|Rotator|MakeRotator 0.0 0.0 _opendoortrack_2) false false))
            (:Finished
              (goto _label))))))))

(event EventDestroyed
  (Utilities|UnregisterInteractable))

(fn ConstructionScript)