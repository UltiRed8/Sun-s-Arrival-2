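; BP_InteractableCoin is an interactable coin pickup that adds to a shared coin balance.
; On BeginPlay it caches the BP_GlobalInventory actor; ServerInteract plays audio, increments CoinsBalance on that actor and destroys the coin.
; Hover and unhover toggle custom depth rendering on the mesh as a highlight.
; An older glow-material swap, along with the parent hover calls, remains in both functions but is disconnected.
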(event EventBeginPlay
  (bind _returnvalue (Actor|GetActorOfClass "/Game/Blueprints/Inventory/BP_GlobalInventory.BP_GlobalInventory_C"))
  (Variables|Default|SetInventory _returnvalue))

(event EventServerInteract
  (params (WhoInteracted :type Actor%20Object%20Reference))
  (Audio|Components|Audio|Play (Variables|Default|GetAudio) 0.0)
  (Math|Integer|IncrementInt (Variables|/Game/Blueprints/Inventory/BP_GlobalInventory.BP_GlobalInventory_C|GetCoinsBalance (Variables|Default|GetInventory))
    (:%20%20
      (Actor|DestroyActor))))

(fn ConstructionScript)

(fn Unhovered
  (Rendering|SetRenderCustomDepth (Variables|Default|GetStaticMesh) false))

(fn Hovered
  (Rendering|SetRenderCustomDepth (Variables|Default|GetStaticMesh) true))