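; BP_InteractableCoffeeMachine is an interactable coffee machine that the player toggles on and off.
; Interaction calls the parent and, if allowed, flip-flops between turning the screen on and off.
; Turning on plays audio, swaps the screen plane to unlit white, then after a short delay runs two coffee effects for a timed pour.
; Turning off sets the screen to black and stops both effects without cancelling pending delays.
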(event Custom|TurnScreenOn
  (bind _ns_coffee (Variables|Default|GetNS_Coffee))
  (CallFunction|PlaySound)
  (Rendering|Material|SetMaterial (Variables|Default|GetPlane) 0 "/Game/Materials/Instances/MI_UnlitWhite.MI_UnlitWhite")
  (Utilities|FlowControl|Delay 1.5)
  (Components|Activation|Activate _ns_coffee false)
  (Utilities|FlowControl|Delay 1e+01)
  (Components|Activation|Deactivate _ns_coffee))

(event Custom|TurnScreenOff
  (Rendering|Material|SetMaterial (Variables|Default|GetPlane) 0 "/Game/Materials/Instances/MI_UnlitBlack.MI_UnlitBlack")
  (Components|Activation|Deactivate (Variables|Default|GetNS_Coffee)))

(event Custom|PlaySound
  (Audio|Components|Audio|Play (Variables|Default|GetAudio) 0.0))

(event EventInteraction
  (|CallParentFunction)
  (if (Variables|Default|GetCanBeInteract)
    (Utilities|FlowControl|FlipFlop
      (:A
        (CallFunction|TurnScreenon))
      (:B
        (CallFunction|TurnScreenOff)))))

(fn ConstructionScript)