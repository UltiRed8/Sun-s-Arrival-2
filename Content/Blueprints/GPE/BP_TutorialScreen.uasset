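; Tutorial screen actor that asks the player to press a given key a set number of times, then triggers its linked nodes.
; Construction shows the key name or override text, plus a counter that is hidden for single presses.
; AnyKey and Mouse2D inputs match the key by display name and decrement the counter.
; At zero, it disables its input, swaps to a success material, plays a sound and calls Trigger on each node.
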(event Custom|Success
  (Input|DisableInput (Game|GetPlayerController 0))
  (Rendering|Material|SetMaterial (Variables|Default|GetPlane) 0 "/Game/Materials/Instances/MI_KeycardReaderSuccess.MI_KeycardReaderSuccess")
  (Audio|PlaySoundatLocation "/Game/Audio/Sounds/SW_KeycardSuccess.SW_KeycardSuccess" (Transformation|GetActorLocation) "0, 0, 0" 1.0 1.0 0.0 0 0 0 0)
  (for _array_element (Variables|Default|GetNodes)
    (Default|Trigger _array_element)))

(event EventBeginPlay
  (Input|EnableInput (Game|GetPlayerController 0)))

(event Input|MouseEvents|Mouse2D
  (params (Key :type Key%20Structure :default "None"))
  (:Pressed
    (if (Utilities|Enum|Equal(Enum) (Class|KismetInputLibrary|KeyGetDisplayName Key false) (Class|KismetInputLibrary|KeyGetDisplayName (Variables|Default|GetKeyToPress) false))
      (bind _result (Math|Integer|DecrementInt (Variables|Default|GetAmountToPress))
        (:%20%20
          (if (< _result 0)
            (Variables|Default|SetAmountToPress 0))
          (Rendering|Components|TextRender|SetText (Variables|Default|GetTextRender1) (Utilities|Text|ToText(Integer) (Variables|Default|GetAmountToPress)))
          (if (== _result 0)
            (CallFunction|Success)))))))

(event Input|KeyboardEvents|AnyKey
  (params (Key :type Key%20Structure :default "None"))
  (:Pressed
    (if (Utilities|Enum|Equal(Enum) (Class|KismetInputLibrary|KeyGetDisplayName (Variables|Default|GetKeyToPress) false) (Class|KismetInputLibrary|KeyGetDisplayName Key false))
      (bind _result (Math|Integer|DecrementInt (Variables|Default|GetAmountToPress))
        (:%20%20
          (if (< _result 0)
            (Variables|Default|SetAmountToPress 0))
          (Rendering|Components|TextRender|SetText (Variables|Default|GetTextRender1) (Utilities|Text|ToText(Integer) (Variables|Default|GetAmountToPress)))
          (if (== _result 0)
            (CallFunction|Success)))))))

(fn ConstructionScript
  (bind _textrender (Variables|Default|GetTextRender))
  (bind _amounttopress (Variables|Default|GetAmountToPress))
  (bind _overridetext (Variables|Default|GetOverrideText))
  (if (Utilities|Text|TextIsEmpty _overridetext)
    (Rendering|Components|TextRender|SetText _textrender (Class|KismetInputLibrary|KeyGetDisplayName (Variables|Default|GetKeyToPress) true))
    (else
      (Rendering|Components|TextRender|SetText _textrender _overridetext)))
  (Rendering|Components|TextRender|SetText (Variables|Default|GetTextRender1) (Utilities|Text|ToText(Integer) _amounttopress))
  (if (<= _amounttopress 1)
    (Rendering|SetVisibility (Variables|Default|GetTextRender1) false false)
    (Transformation|SetRelativeLocation (Variables|Default|GetTextRender) "8.200000,0.000000,0.000000" false false)))