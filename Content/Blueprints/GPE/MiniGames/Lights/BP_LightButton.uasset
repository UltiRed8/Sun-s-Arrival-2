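; BP_LightButton is one light in a Lights minigame, toggled between green (on) and red (off) by its child BP_LightInnerButton.
; A press toggles the light and its Adjacents, without propagating further, and only on lights marked Available.
; Active buttons mark themselves and neighbours Available; unavailable ones can be shown white.
; SetActive changes the inner button's interactability and, after a random delay, rotates it by timeline with pitch-varied audio.
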(event Custom|Toggle
  (params (IsMain :type Boolean))
  (if (Variables|Default|GetAvailable)
    (if (Variables|Default|GetIsTurnedOn)
      (CallFunction|SetOff)
      (else
        (CallFunction|Seton)))
    (if IsMain
      (for _array_element (Variables|Default|GetAdjacents)
        (CallFunction|Toggle _array_element false)))))

(event Custom|SetOn
  (Variables|Default|SetIsTurnedOn true)
  (Rendering|Material|SetMaterial (Variables|Default|GetStaticMesh1) 0 "/Game/Models/EndoEnemy/MAT_GreenGlow.MAT_GreenGlow"))

(event Custom|SetOff
  (Variables|Default|SetIsTurnedOn false)
  (Rendering|Material|SetMaterial (Variables|Default|GetStaticMesh1) 0 "/Game/Models/EndoEnemy/MAT_RedGlow.MAT_RedGlow"))

(event Custom|SetActive
  (params (IsActive :type Boolean))
  (bind _audio (Variables|Default|GetAudio))
  (bind _childactor (Variables|Default|GetChildActor))
  (if (!= (Variables|Default|GetIsActive) IsActive)
    (bind _output_get (Variables|Default|SetIsActive IsActive))
    (Utilities|FlowControl|Sequence
      (:then_0
        (Utilities|FlowControl|Delay (Math|Random|RandomFloatinRange 0.0 0.5))
        (Audio|Components|Audio|Play _audio 0.0)
        (Audio|Components|Audio|SetPitchMultiplier _audio (Math|Random|RandomFloatinRange 0.9 1.1))
        (if _output_get
          (bind _rotation (Timeline|DeactivatedAnim ReverseFromEnd)
            (:Update
              (Transformation|SetRelativeRotation _childactor (Math|Rotator|MakeRotator 0.0 _rotation 0.0) false false)))
          (else
            (bind _rotation_2 (Timeline|ActivatedAnim PlayFromStart)
              (:Update
                (Transformation|SetRelativeRotation _childactor (Math|Rotator|MakeRotator 0.0 _rotation_2 0.0) false false))))))
      (:then_1
        (bind _asbp_light_inner_button (Utilities|Casting|CastToBP_LightInnerButton (Variables|/Script/Engine.ChildActorComponent|GetChildActor (Variables|Default|GetChildActor))))
        (Default|SetCanbeInteracted _asbp_light_inner_button _output_get)))))

(event Custom|UpdateAvailable
  (if (Variables|Default|GetIsActive)
    (Variables|Default|SetAvailable true)
    (for _array_element (Variables|Default|GetAdjacents)
      (Variables|BP_LightButton_C|SetAvailable _array_element true))))

(event Custom|SetAvaiableVisibility
  (Rendering|Material|SetMaterial (Variables|Default|GetStaticMesh1) 0 (select (Variables|Default|GetAvailable) "/Game/Models/EndoEnemy/MAT_RedGlow.MAT_RedGlow" "/Game/Materials/Instances/MI_UnlitWhite.MI_UnlitWhite")))

(event Custom|OnTriggered_Event
  (CallFunction|Toggle true))

(event EventBeginPlay
  (bind _asbp_light_inner_button (Utilities|Casting|CastToBP_LightInnerButton (Variables|/Script/Engine.ChildActorComponent|GetChildActor (Variables|Default|GetChildActor))))
  (EventDispatchers|AssignOnTriggered _asbp_light_inner_button (delegate Custom|OnTriggered_Event)))

(fn ConstructionScript)