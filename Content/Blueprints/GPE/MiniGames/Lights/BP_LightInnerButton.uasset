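; BP_LightInnerButton is an interactable press button used in the Lights minigame.
; Toggling its interactability also swaps the cylinder material between the press-button look and black.
; On interaction it fires its triggered callback, plays a sound and Niagara effect through a Multi event, and triggers a linked Node if one is valid.
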(event Custom|SetCanBeInteracted
  (params (CanInteract :type Boolean))
  (CallFunction|SetCanInteract CanInteract)
  (Rendering|Material|SetMaterial (Variables|Default|GetCylinder) 0 (select CanInteract "/Game/Materials/Instances/MI_PressButton.MI_PressButton" "/Game/Materials/Instances/MI_Black.MI_Black")))

(event Custom|Multi_PlaySound
  (Audio|Components|Audio|Play (Variables|Default|GetLeverDownEnd) 0.0)
  (Components|Activation|Activate (Variables|Default|GetInteractionNiagara) true))

(event EventInteracted
  (params (HitComponent :type Actor%20Component%20Object%20Reference%20%28by%20ref%29) (WhoInteracted :type Actor%20Object%20Reference) (HasMouseMovements :type Boolean))
  (Default|CallOnTriggered)
  (CallFunction|MultiPlaySound)
  (bind _node (Variables|Default|GetNode)
    (:then
      (Default|Trigger _node))
    (:else)))

(fn ConstructionScript)