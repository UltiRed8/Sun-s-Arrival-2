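; Manager for a five-round light-puzzle minigame where every available LightButton must be lit, confirmed by a lever.
; Each round activates a larger or different panel layout and randomly toggles more lights, re-toggling if already solved.
; A wrong confirm or expired Hardcore-only 15-second timer regenerates the current round.
; Winning saves a location-keyed checkpoint, restored on BeginPlay, triggers the VictoryNode on authority and unlocks a mode-dependent achievement.
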(event Custom|CheckForVictory
  (Variables|Default|SetAntiSpam true)
  (Utilities|VictoryChecker
    (:Incomplete
      (CallFunction|DisplayError)
      (Utilities|FlowControl|Delay 1.0)
      (CallFunction|SetupNextPad))
    (:Complete
      (bind _result (Math|Integer|IncrementInt (Variables|Default|GetScore))
        (:%20%20
          (CallFunction|DisplaySuccess _result)
          (if (>= _result 5)
            (Utilities|CheckpointSaveBool (Utilities|String|ToString(Vector) (Transformation|GetActorLocation)) true)
            (CallFunction|Completed)
            (else
              (Utilities|FlowControl|Delay 1.0)
              (CallFunction|SetupNextPad))))))))

(event Custom|DisplayError
  (bind _textrender (Variables|Default|GetTextRender))
  (bind _audio (Variables|Default|GetAudio))
  (Audio|Components|Audio|SetSound _audio "/Game/Audio/Sounds/SW_ArcadeError.SW_ArcadeError")
  (Audio|Components|Audio|Play _audio 0.0)
  (Rendering|Components|TextRender|SetText _textrender (Utilities|Text|MakeLiteralText "Not all lights 
are active. 
 
Resetting..."))
  (Rendering|SetVisibility _textrender true false)
  (Rendering|Material|SetMaterial (Variables|Default|GetStaticMesh) 1 "/Game/Materials/Instances/MI_KeycardReaderDenied.MI_KeycardReaderDenied")
  (Utilities|FlowControl|Delay 2.5)
  (Rendering|Material|SetMaterial (Variables|Default|GetStaticMesh) 1 "/Game/Materials/Instances/MI_UnlitBlack.MI_UnlitBlack")
  (Rendering|Components|TextRender|SetText (Variables|Default|GetTextRender) (Utilities|Text|FormatText "Press lever to 
confirm or 
reset."))
  (Variables|Default|SetAntiSpam false)
  (Rendering|SetVisibility (Variables|Default|GetTimerTextRender) (Variables|Default|GetHasTimer) false))

(event Custom|DisplaySuccess
  (params (Score :type Integer))
  (bind _textrender (Variables|Default|GetTextRender))
  (bind _audio (Variables|Default|GetAudio))
  (Rendering|SetVisibility (Variables|Default|GetTimerTextRender) false false)
  (Audio|Components|Audio|SetSound _audio "/Game/Audio/Sounds/SW_Achievement.SW_Achievement")
  (Audio|Components|Audio|Play _audio 0.0)
  (Rendering|Components|TextRender|SetText _textrender (Utilities|Text|FormatText "Completed! 
{Current}/5" Score))
  (Rendering|SetVisibility _textrender true false)
  (Rendering|Material|SetMaterial (Variables|Default|GetStaticMesh) 1 "/Game/Materials/Instances/MI_KeycardReaderSuccess.MI_KeycardReaderSuccess")
  (Utilities|FlowControl|Delay 5.0)
  (if (not (>= Score 5))
    (Rendering|Material|SetMaterial (Variables|Default|GetStaticMesh) 1 "/Game/Materials/Instances/MI_UnlitBlack.MI_UnlitBlack")
    (Rendering|Components|TextRender|SetText (Variables|Default|GetTextRender) (Utilities|Text|FormatText "Press lever to 
confirm or 
reset."))
    (Variables|Default|SetAntiSpam false)
    (Rendering|SetVisibility (Variables|Default|GetTimerTextRender) (Variables|Default|GetHasTimer) false)))

(event Custom|Completed
  (bind _asbp_game_instance (Utilities|GameInstance))
  (Rendering|SetVisibility (Variables|Default|GetTimerTextRender) false false)
  (Utilities|Authority
    (:Authority
      (for _array_element (Variables|Default|GetLightButtons)
        (Default|Seton _array_element)
        (Default|SetActive _array_element false))
      (bind _victorynode (Variables|Default|GetVictoryNode)
        (:then
          (Default|Trigger _victorynode))
        (:else)))
    (:Remote
      _))
  (switch Utilities|FlowControl|Switch|SwitchonE_ExtrasGamemodes (Variables|/Game/BP_GameInstance.BP_GameInstance_C|GetExtraGamemode _asbp_game_instance)
    (:NewEnumerator0
      (Default|UnlockAchievement _asbp_game_instance "ACH_MINIGAME1" :!label _label))
    (:NewEnumerator1
      (goto _label))
    (:NewEnumerator2
      (Default|UnlockAchievement _asbp_game_instance "ACH_MINIGAME1HARD"))
    (:NewEnumerator3
      (goto _label))))

(event Custom|GeneratePad
  (params (Panels :type Array%20of%20Integers))
  (bind _lightbuttons (Variables|Default|GetLightButtons))
  (for (_array_element _array_index) _lightbuttons
    (Default|SetActive _array_element (Utilities|Array|ContainsItem Panels _array_index))
    (Variables|/Game/Blueprints/GPE/MiniGames/Lights/BP_LightButton.BP_LightButton_C|SetAvailable _array_element false)
    (Default|SetOff _array_element))
  (for _array_element_2 _lightbuttons
    (Default|UpdateAvailable _array_element_2))
  (for _array_element_3 _lightbuttons
    (Default|ReplicateAvailableandSetVisibility _array_element_3 (Variables|/Game/Blueprints/GPE/MiniGames/Lights/BP_LightButton.BP_LightButton_C|GetAvailable _array_element_3)))
  (if (not (Utilities|Array|IsEmpty Panels))
    (bind _output_get (Variables|Default|SetAmountToGenerate (* (Variables|Default|GetScore) 2)))
    (while (or (>= _output_get 1) (Variables|Default|GetInstantWin))
      (bind _output_get_2 (Variables|Default|SetSelectedToggle (.OutItem (Utilities|Array|Random (Variables|Default|GetLightButtons))) :!label _label))
      (if (Variables|/Game/Blueprints/GPE/MiniGames/Lights/BP_LightButton.BP_LightButton_C|GetIsActive _output_get_2)
        (Default|Toggle _output_get_2 true)
        (Math|Integer|DecrementInt (Variables|Default|GetAmountToGenerate)
          (:%20%20
            (Utilities|VictoryChecker
              (:Incomplete
                (Variables|Default|SetInstantWin false))
              (:Complete
                (Variables|Default|SetInstantWin true)))))
        (else
          (goto _label))))
    (Variables|Default|SetTimer 15.0)
    (Rendering|SetVisibility (Variables|Default|GetTimerTextRender) (Variables|Default|GetHasTimer) false)))

(event Custom|SetupNextPad
  (CallFunction|GeneratePad)
  (Utilities|FlowControl|Delay 1.0)
  (switch int (Variables|Default|GetScore)
    (:0
      (CallFunction|GeneratePad (Utilities|Array|MakeArray 5 6 9 10)))
    (:1
      (CallFunction|GeneratePad (Utilities|Array|MakeArray 1 2 4 7 8 11 13 14)))
    (:2
      (CallFunction|GeneratePad (Utilities|Array|MakeArray 0 2 4 15 13 11 7 8)))
    (:3
      (CallFunction|GeneratePad (Utilities|Array|MakeArray 0 1 2 3 4 7 8 11 12 13 14 15)))
    (:4
      (CallFunction|GeneratePad (Utilities|Array|MakeArray 0 1 2 3 4 7 8 11 12 13 14 15 5 6 9 10)))))

(event Custom|Multi_Trigger
  (Rendering|SetVisibility (Variables|Default|GetTimerTextRender) (Variables|Default|GetHasTimer) false)
  (Utilities|Authority
    (:Authority
      (if (not (Variables|Default|GetAntiSpam))
        (Utilities|FlowControl|Sequence
          (:then_0
            (Utilities|FlowControl|Gate true :!label _label
              (:Exit
                (CallFunction|CheckforVictory))))
          (:then_1
            (Utilities|FlowControl|DoOnce false
              (:Completed
                (CallFunction|SetupNextPad)
                (CallFunction|DisplayError)
                (Utilities|FlowControl|Delay 1.0)
                (goto _label Open)))))))))

(event EventTick
  (params (DeltaSeconds :type Float%20%28single-precision%29))
  (if (Variables|Default|GetHasTimer)
    (if (> (Variables|Default|GetTimer) 0.0)
      (bind _output_get (Variables|Default|SetTimer (- (Variables|Default|GetTimer) DeltaSeconds)))
      (Rendering|Components|TextRender|SetText (Variables|Default|GetTimerTextRender) (Utilities|Text|FormatText "Timer: {Value}" (Utilities|Text|ToText(Float) (Math|Float|Clamp(Float) _output_get 0.0 15.0) "HalfToEven" false true 2 2 2 2)))
      (if (<= _output_get 0.0)
        (if (not (>= (Variables|Default|GetScore) 5))
          (if (not (Variables|Default|GetAntiSpam))
            (CallFunction|DisplayError)
            (CallFunction|SetupNextPad)))))))

(event EventTrigger
  (CallFunction|MultiTrigger)
  (|CallParentFunction))

(event EventBeginPlay
  (Utilities|FlowControl|DelayUntilNextTick)
  (Variables|Default|SetHasTimer (Utilities|Enum|Equal(Enum) (Variables|/Game/BP_GameInstance.BP_GameInstance_C|GetExtraGamemode (Utilities|GameInstance)) "NewEnumerator2"))
  (bind (_success _bool) (Utilities|CheckpointGetBool (Utilities|String|ToString(Vector) (Transformation|GetActorLocation))))
  (if _success
    (if _bool
      (Variables|Default|SetScore 5)
      (CallFunction|DisplaySuccess)
      (CallFunction|Completed))))

(fn ConstructionScript)