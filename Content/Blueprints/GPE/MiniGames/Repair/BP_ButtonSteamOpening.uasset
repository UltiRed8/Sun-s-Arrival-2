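; Steam vent prop for the repair minigame that pops open and shuts on demand.
; Open waits a short random delay, starts the opening sound, steam and looping audio, and raises a cylinder along a timeline.
; Close lowers the cylinder while dropping the loop's pitch with its height, then stops the loop.
; While open, Tick continuously spins a cube around its yaw axis.
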(event Custom|Open
  (Utilities|FlowControl|Delay (Math|Random|RandomFloatinRange 0.0 0.8))
  (Variables|Default|SetIsOpened true)
  (Audio|Components|Audio|SetPitchMultiplier (Variables|Default|GetSteamLoop) 2.0)
  (Audio|Components|Audio|Play (Variables|Default|GetOpening) 0.0)
  (bind _height (Timeline|OpenAnim PlayFromStart)
    (:Update
      (Transformation|SetRelativeLocation (Variables|Default|GetCylinder1) (Math|Vector|MakeVector 0.0 0.0 _height) false false))))

(event Custom|Close
  (bind _steamloop (Variables|Default|GetSteamLoop))
  (if (Variables|Default|GetIsOpened)
    (bind _height (Timeline|CloseAnim PlayFromStart)
      (:Update
        (Transformation|SetRelativeLocation (Variables|Default|GetCylinder1) (Math|Vector|MakeVector 0.0 0.0 _height) false false)
        (Audio|Components|Audio|SetPitchMultiplier _steamloop (* (/ (- _height 1e+01) 5e+01) 2.0)))
      (:Finished
        (Audio|Components|Audio|Stop _steamloop)
        (Variables|Default|SetIsOpened false)))))

(event EventTick
  (params (DeltaSeconds :type Float%20%28single-precision%29))
  (if (Variables|Default|GetIsOpened)
    (Transformation|AddRelativeRotation (Variables|Default|GetCube) (Math|Rotator|MakeRotator 0.0 0.0 (* DeltaSeconds 7.5e+02)) false false)))

(fn ConstructionScript)