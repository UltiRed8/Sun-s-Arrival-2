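; Repair minigame screen that flashes a calibration code one character at a time, faster as progress rises or in hardcore mode.
; A server timer finds the nearest overlapping player and sends the facing direction via Multi_SetScreenRotation; Tick eases the screen toward it with pitch-modulated sound.
; A child press button relays clicks through a dispatcher, while events drive progress text, error and success feedback, and disable the button on completion.
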(event OnComponentBeginOverlap(Sphere)
  (params (OverlappedComponent :type Primitive%20Component%20Object%20Reference) (OtherActor :type Actor%20Object%20Reference) (OtherComp :type Primitive%20Component%20Object%20Reference) (OtherBodyIndex :type Integer) (bFromSweep :type Boolean) (SweepResult :type Hit%20Result%20Structure%20%28by%20ref%29))
  (Utilities|Authority
    (:Authority
      (bind _asbp_player (Utilities|Casting|CastToBP_Player OtherActor))
      (Utilities|Array|AddUnique (Variables|Default|GetPlayersInRange) _asbp_player))))

(event OnComponentEndOverlap(Sphere)
  (params (OverlappedComponent :type Primitive%20Component%20Object%20Reference) (OtherActor :type Actor%20Object%20Reference) (OtherComp :type Primitive%20Component%20Object%20Reference) (OtherBodyIndex :type Integer))
  (Utilities|Authority
    (:Authority
      (bind _asbp_player (Utilities|Casting|CastToBP_Player OtherActor))
      (Utilities|Array|RemoveItem (Variables|Default|GetPlayersInRange) _asbp_player))))

(event Custom|GetNearestPlayer
  (bind _returnvalue (Transformation|GetActorLocation))
  (bind _playersinrange (Variables|Default|GetPlayersInRange))
  (if (Variables|Default|GetCanRotate)
    (if (Utilities|Array|IsNotEmpty _playersinrange)
      (Variables|Default|SetDistance 9999.0)
      (for _array_element _playersinrange
        (if (< (Math|Vector|Distance(Vector) (Transformation|GetActorLocation _array_element) _returnvalue) (Variables|Default|GetDistance))
          (Variables|Default|SetTargetDirection (Math|Rotator|FindLookatRotation _returnvalue (Transformation|GetActorLocation _array_element)))
          (Variables|Default|SetDistance (Math|Vector|Distance(Vector) (Transformation|GetActorLocation _array_element) _returnvalue))))
      (CallFunction|MultiSetScreenRotation (Variables|Default|GetTargetDirection)))))

(event Custom|OnTriggered_Event
  (Default|CallOnButtonClicked))

(event Custom|DisableButton
  (bind _asbp_press_button (Utilities|Casting|CastToBP_PressButton (Variables|/Script/Engine.ChildActorComponent|GetChildActor (Variables|Default|GetChildActor))))
  (Variables|/Game/Blueprints/GPE/BP_PressButton.BP_PressButton_C|SetDidIt _asbp_press_button true)
  (Rendering|Material|SetMaterial (Variables|/Game/Blueprints/GPE/BP_PressButton.BP_PressButton_C|GetCylinder _asbp_press_button) 0 "/Game/Materials/Instances/MI_Black.MI_Black")
  (Variables|/Game/Blueprints/Components/BP_CustomCursorComponent.BP_CustomCursorComponent_C|SetCursorTexture (Variables|/Game/Blueprints/GPE/BP_MouseInteractiveBase.BP_MouseInteractiveBase_C|GetBP_CustomCursorComponent _asbp_press_button) "/Game/Textures/T_CursorNormal.T_CursorNormal"))

(event Custom|ShowCode
  (params (Code :type String) (IsHardcore :type Boolean))
  (bind _codetext (Variables|Default|GetCodeText))
  (Rendering|Components|TextRender|SetText (Variables|Default|GetCalibrationText) (Utilities|Text|MakeLiteralText "Please calibrate 
using the following code:"))
  (CallFunction|PlayCodeSoundEffect 2.0)
  (Rendering|SetVisibility (Variables|Default|GetCalibrationText) true false)
  (Utilities|FlowControl|Delay 0.5)
  (CallFunction|PlayCodeSoundEffect 0.0)
  (Rendering|SetVisibility (Variables|Default|GetCalibrationText) false false)
  (Utilities|FlowControl|Delay 0.5)
  (CallFunction|PlayCodeSoundEffect 2.0)
  (Rendering|SetVisibility (Variables|Default|GetCalibrationText) true false)
  (Utilities|FlowControl|Delay 0.5)
  (CallFunction|PlayCodeSoundEffect 0.0)
  (Rendering|SetVisibility (Variables|Default|GetCalibrationText) false false)
  (Utilities|FlowControl|Delay 0.5)
  (CallFunction|PlayCodeSoundEffect 2.0)
  (Rendering|SetVisibility (Variables|Default|GetCalibrationText) true false)
  (Utilities|FlowControl|Delay 1.0)
  (bind _output_get (Variables|Default|SetCodeArray (Utilities|String|GetCharacterArrayfromString Code)))
  (if (Utilities|Array|IsNotEmpty _output_get) :!label _label
    (Rendering|Components|TextRender|SetText _codetext (Utilities|Text|ToText(String) (Utilities|Array|Get(acopy) _output_get)))
    (CallFunction|PlayCodeSoundEffect (Math|Random|RandomFloatinRange 0.0 2.0))
    (Rendering|SetVisibility _codetext true false)
    (Utilities|Array|RemoveIndex _output_get)
    (switch int (Variables|Default|GetProgress)
      (:0
        (Utilities|FlowControl|Delay (Math|Float|SelectFloat 0.6 1.0 IsHardcore))
        (goto _label))
      (:1
        (Utilities|FlowControl|Delay (Math|Float|SelectFloat 0.45 0.8 IsHardcore))
        (goto _label))
      (:2
        (Utilities|FlowControl|Delay (Math|Float|SelectFloat 0.35 0.5 IsHardcore))
        (goto _label))
      (:3
        (Utilities|FlowControl|Delay (Math|Float|SelectFloat 0.3 0.4 IsHardcore))
        (goto _label)))
    (else
      (Rendering|SetVisibility _codetext false false)
      (Utilities|FlowControl|Delay 1.0)
      (Rendering|Components|TextRender|SetText (Variables|Default|GetCalibrationText) (Utilities|Text|MakeLiteralText "Please calibrate"))
      (Default|CallOnDisplayingScoreDone)
      (CallFunction|PlayCodeSoundEffect 2.0))))

(event Custom|TurnOn
  (Rendering|Material|SetMaterial (Variables|Default|GetStaticMesh1) 1 "/Game/Materials/MAT_Static.MAT_Static")
  (Utilities|FlowControl|Delay 0.5)
  (Rendering|Material|SetMaterial (Variables|Default|GetStaticMesh1) 1 "/Game/Materials/Instances/MI_UnlitBlack.MI_UnlitBlack")
  (Rendering|SetVisibility (Variables|Default|GetProgressText) true false))

(event Custom|UpdateProgress
  (bind _progresstext (Variables|Default|GetProgressText))
  (Rendering|SetVisibility _progresstext true false)
  (Rendering|Components|TextRender|SetText _progresstext (Utilities|Text|FormatText "Progress: 
{Current}/4" (Variables|Default|GetProgress)))
  (Audio|Components|Audio|Play (Variables|Default|GetScoreUpdateSound) 0.0))

(event Custom|SetScoreProgress
  (params (Progress :type Integer))
  (bind _progresstext (Variables|Default|GetProgressText))
  (Variables|Default|SetProgress Progress)
  (Rendering|SetVisibility _progresstext true false)
  (Rendering|Components|TextRender|SetText _progresstext (Utilities|Text|FormatText "Progress: 
{Current}/4" (Variables|Default|GetProgress)))
  (Audio|Components|Audio|Play (Variables|Default|GetScoreUpdateSound) 0.0))

(event Custom|PlayCodeSoundEffect
  (params (NewPitchMultiplier :type Float%20%28single-precision%29))
  (bind _codesound (Variables|Default|GetCodeSound))
  (Audio|Components|Audio|SetPitchMultiplier _codesound NewPitchMultiplier)
  (Audio|Components|Audio|Play _codesound 0.0))

(event Custom|DisplaySuccess
  (params (ShouldReset :type Boolean))
  (bind _staticmesh2 (Variables|Default|GetStaticMesh2))
  (bind _calibrationtext (Variables|Default|GetCalibrationText))
  (Rendering|Material|SetMaterial _staticmesh2 1 "/Game/Materials/MAT_KeycardReader.MAT_KeycardReader")
  (Audio|Components|Audio|Play (Variables|Default|GetCodeSuccess) 0.0)
  (if ShouldReset
    (Utilities|FlowControl|Delay 1.0)
    (Rendering|Material|SetMaterial _staticmesh2 1 "/Engine/EngineDebugMaterials/BlackUnlitMaterial.BlackUnlitMaterial")
    (else
      (CallFunction|DisableButton)
      (Rendering|Components|TextRender|SetText _calibrationtext (Utilities|Text|MakeLiteralText "Calibration completed!"))
      (Rendering|SetVisibility _calibrationtext true false))))

(event Custom|DisplayError
  (bind _staticmesh2 (Variables|Default|GetStaticMesh2))
  (Rendering|Material|SetMaterial _staticmesh2 1 "/Game/Materials/Instances/MI_KeycardReaderDenied.MI_KeycardReaderDenied")
  (Audio|Components|Audio|Play (Variables|Default|GetCodeError) 0.0)
  (Utilities|FlowControl|Delay 1.0)
  (Rendering|Material|SetMaterial _staticmesh2 1 "/Engine/EngineDebugMaterials/BlackUnlitMaterial.BlackUnlitMaterial"))

(event Custom|Multi_SetScreenRotation
  (params (TargetDirrection :type Rotator))
  (Variables|Default|SetTargetDirection TargetDirrection))

(event EventTick
  (params (DeltaSeconds :type Float%20%28single-precision%29))
  (bind _rotatesound (Variables|Default|GetRotateSound))
  (bind _targetdirection (Variables|Default|GetTargetDirection))
  (bind _screenaxis (Variables|Default|GetScreenAxis))
  (bind _returnvalue (Math|Rotator|GetRotationXVector (Math|Rotator|MakeRotator 0.0 0.0 (.yaw _targetdirection))))
  (bind _returnvalue_2 (Audio|Components|Audio|IsPlaying _rotatesound))
  (bind _relativerotation (Variables|/Script/Engine.SceneComponent|GetRelativeRotation _screenaxis))
  (bind _returnvalue_3 (Math|Rotator|GetRotationXVector _relativerotation))
  (bind _returnvalue_4 (Math|Vector|DotProduct _returnvalue_3 _returnvalue))
  (bind _returnvalue_5 (- _returnvalue_4 1.0))
  (bind _returnvalue_6 (Math|Float|Absolute(Float) _returnvalue_5))
  (bind _returnvalue_7 (/ _returnvalue_6 2.0))
  (if (>= _returnvalue_7 0.01)
    (Transformation|SetRelativeRotation _screenaxis (Math|Interpolation|RInterpTo _relativerotation (Math|Rotator|MakeRotator 0.0 0.0 (.yaw _targetdirection)) DeltaSeconds 1.0) false false)
    (Audio|Components|Audio|SetPitchMultiplier (Variables|Default|GetRotateSound) _returnvalue_7)
    (if (not _returnvalue_2)
      (Audio|Components|Audio|Play _rotatesound 0.0))
    (elif _returnvalue_2
      (Audio|Components|Audio|Stop _rotatesound))))

(event EventBeginPlay
  (Utilities|Authority
    (:Authority
      (Utilities|Time|SetTimerbyEvent (delegate Custom|GetNearestPlayer) 0.05 true))
    (:Remote
      _))
  (bind _asbp_press_button (Utilities|Casting|CastToBP_PressButton (Variables|/Script/Engine.ChildActorComponent|GetChildActor (Variables|Default|GetChildActor))))
  (EventDispatchers|AssignOnTriggered _asbp_press_button (delegate Custom|OnTriggered_Event)))

(fn ConstructionScript)