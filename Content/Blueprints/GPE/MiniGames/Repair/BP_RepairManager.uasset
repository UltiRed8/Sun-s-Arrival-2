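; Manager for a repair minigame where the player memorises a code shown on a screen and enters it on connected buttons.
; Each round assigns buttons random unique IDs and builds a longer code from them, with Hardcore adding two-character IDs and length.
; Input is prefix-checked: errors replay the code, and screen clicks start the game or redisplay it.
; The fourth success saves a location-keyed checkpoint, triggers the conveyor and disables buttons; BeginPlay restores this state.
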(event Custom|CodeEntered
  (params (ID :type String))
  (bind _code (Variables|Default|GetCode))
  (if (not (Variables|Default|GetCompleted))
    (if (Variables|Default|GetStarted)
      (bind _output_get (Variables|Default|SetCurrentCode (Utilities|String|Append (Variables|Default|GetCurrentCode) ID)))
      (if (Utilities|String|StartsWith _code _output_get)
        (if (Utilities|Enum|Equal(Enum) _output_get _code)
          (CallFunction|Victory))
        (else
          (CallFunction|Defeat))))))

(event Custom|Victory
  (bind _conveyor (Variables|Default|GetConveyor))
  (bind _repairscreen (Variables|Default|GetRepairScreen))
  (bind _result (Math|Integer|IncrementInt (Variables|Default|GetScore))
    (:%20%20
      (Default|SetScoreProgress _repairscreen _result)
      (Default|DisplaySuccess _repairscreen (not (>= _result 4)))
      (for _array_element (Variables|Default|GetConnectedButtons)
        (Default|ClearID _array_element))
      (if (>= _result 4)
        (Variables|/Game/Blueprints/GPE/MiniGames/Repair/BP_RepairScreen.BP_RepairScreen_C|SetCanRotate (Variables|Default|GetRepairScreen) false)
        (Utilities|CheckpointSaveBool (Utilities|String|ToString(Vector) (Transformation|GetActorLocation)) true)
        (Default|Trigger _conveyor)
        (for _array_element_2 (Variables|Default|GetConnectedButtons)
          (Default|CompleteDisable _array_element_2))
        (Utilities|FlowControl|Delay 2.0)
        (Default|Trigger _conveyor)
        (else
          (Variables|Default|SetCurrentCode "")
          (CallFunction|GenerateCode)
          (Default|ShowCode (Variables|Default|GetRepairScreen) (Variables|Default|GetCode) (Variables|Default|GetIsHardcore)))))))

(event Custom|Defeat
  (bind _repairscreen (Variables|Default|GetRepairScreen))
  (Variables|Default|SetStarted false)
  (for _array_element (Variables|Default|GetConnectedButtons)
    (Default|Disable _array_element))
  (Variables|Default|SetCurrentCode "")
  (Default|DisplayError _repairscreen)
  (Utilities|FlowControl|Delay 1.2)
  (Default|ShowCode _repairscreen (Variables|Default|GetCode) (Variables|Default|GetIsHardcore)))

(event Custom|OnButtonClicked_Event
  (bind _repairscreen (Variables|Default|GetRepairScreen))
  (if (not (Variables|Default|GetCompleted))
    (if (Variables|Default|GetStarted)
      (CallFunction|RedisplayCode)
      (Variables|Default|SetStarted false)
      (else
        (Utilities|FlowControl|DoOnce false
          (:Completed
            (for _array_element (Variables|Default|GetConnectedButtons)
              (Default|Turnon _array_element))
            (CallFunction|GenerateCode)
            (Variables|/Game/Blueprints/GPE/MiniGames/Repair/BP_RepairScreen.BP_RepairScreen_C|SetCanRotate _repairscreen true)
            (Default|UpdateProgress _repairscreen)
            (bind _startednode (Variables|Default|GetStartedNode)
              (:then
                (Default|Trigger _startednode))
              (:else
                _))
            (Utilities|FlowControl|Delay 1.0)
            (Default|ShowCode (Variables|Default|GetRepairScreen) (Variables|Default|GetCode) (Variables|Default|GetIsHardcore))))))))

(event Custom|GenerateCode
  (Utilities|Array|Clear (Variables|Default|GetSelectedIDs))
  (bind _output_get (Variables|Default|SetAvailableIDs (select (Variables|Default|GetIsHardcore) (Utilities|Array|MakeArray "A" "B" "C" "D" "E" "F" "G" "H" "I" "J" "K" "L" "M" "N" "O" "P" "Q" "R" "S" "T" "U" "V" "W" "X" "Y" "Z" "0" "1" "2" "3" "4" "5" "6" "7" "8" "9" "AJ" "BU" "CT" "DW" "EP" "FC" "GA" "HW" "IZ" "JU" "KI" "LC" "MI" "NA" "OS" "PT" "QC" "RB" "SL" "TB" "UC" "VM" "WR" "XW" "YW" "ZH" "07" "11" "29" "38" "42" "53" "67" "70" "81" "94") (Utilities|Array|MakeArray "A" "B" "C" "D" "E" "F" "G" "H" "I" "J" "K" "L" "M" "N" "O" "P" "Q" "R" "S" "T" "U" "V" "W" "X" "Y" "Z" "0" "1" "2" "3" "4" "5" "6" "7" "8" "9"))))
  (for _array_element (Variables|Default|GetConnectedButtons)
    (bind _output_get_2 (Variables|Default|SetSelectedID (.OutIndex (Utilities|Array|Random _output_get))))
    (Default|SetID _array_element (Utilities|Array|Get(acopy) _output_get _output_get_2))
    (Utilities|Array|Add (Variables|Default|GetSelectedIDs) (Utilities|Array|Get(acopy) _output_get _output_get_2))
    (Utilities|Array|RemoveIndex _output_get _output_get_2))
  (Variables|Default|SetCode "")
  (for _index (range 0 (+ (Variables|Default|GetScore) (Math|Integer|SelectInt 3 2 (Variables|Default|GetIsHardcore))))
    (Variables|Default|SetCode (Utilities|String|Append (Variables|Default|GetCode) (.OutItem (Utilities|Array|Random (Variables|Default|GetSelectedIDs))))))
  (Variables|Default|SetCurrentCode ""))

(event Custom|OnDisplayingScoreDone_Event
  (for _array_element (Variables|Default|GetConnectedButtons)
    (Default|Enable _array_element))
  (Variables|Default|SetStarted true))

(event Custom|RedisplayCode
  (if (<= (Variables|Default|GetScore) 3)
    (for _array_element (Variables|Default|GetConnectedButtons)
      (Default|Disable _array_element))
    (Variables|Default|SetCurrentCode "")
    (Utilities|FlowControl|Delay 0.5)
    (Default|ShowCode (Variables|Default|GetRepairScreen) (Variables|Default|GetCode) (Variables|Default|GetIsHardcore))))

(event EventBeginPlay
  (bind _repairscreen (Variables|Default|GetRepairScreen))
  (bind _repairscreen_2 (Variables|Default|GetRepairScreen))
  (bind _conveyor (Variables|Default|GetConveyor))
  (Utilities|FlowControl|DelayUntilNextTick)
  (Variables|Default|SetIsHardcore (Utilities|Enum|Equal(Enum) (Variables|/Game/BP_GameInstance.BP_GameInstance_C|GetExtraGamemode (Utilities|GameInstance)) "NewEnumerator2"))
  (for _array_element (Variables|Default|GetConnectedButtons)
    (EventDispatchers|AssignOnButtonClicked _array_element (delegate Custom|CodeEntered)))
  (EventDispatchers|AssignOnButtonClicked _repairscreen (delegate Custom|OnButtonClicked_Event))
  (EventDispatchers|AssignOnDisplayingScoreDone _repairscreen (delegate Custom|OnDisplayingScoreDone_Event))
  (bind (_success _bool) (Utilities|CheckpointGetBool (Utilities|String|ToString(Vector) (Transformation|GetActorLocation))))
  (if _success
    (if _bool
      (Variables|Default|SetCompleted true)
      (bind _output_get (Variables|Default|SetScore 4))
      (Default|SetScoreProgress _repairscreen_2 _output_get)
      (Default|DisplaySuccess _repairscreen_2 false)
      (for _array_element_2 (Variables|Default|GetConnectedButtons)
        (Default|ClearID _array_element_2))
      (Default|Trigger _conveyor)
      (for _array_element_3 (Variables|Default|GetConnectedButtons)
        (Default|CompleteDisable _array_element_3))
      (Utilities|FlowControl|Delay 2.0)
      (Default|Trigger _conveyor))))

(fn ConstructionScript)