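; Labeled button for the Repair minigame, wrapping a child BP_PressButton and broadcasting its string ID when pressed.
; Starts with the press button locked through its DidIt flag.
; Enable and Disable toggle that lock, materials, label visibility and an optional ButtonSteamOpening.
; TurnOn and ClearID empty the ID and fall into the disabled state, while CompleteDisable blacks out the mesh and restores the normal cursor.
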(event Custom|Disable
  (Rendering|Material|SetMaterial (Variables|Default|GetStaticMesh) 1 "/Game/Materials/MAT_Static.MAT_Static")
  (bind _asbp_press_button (Utilities|Casting|CastToBP_PressButton (Variables|/Script/Engine.ChildActorComponent|GetChildActor (Variables|Default|GetChildActor))))
  (Variables|/Game/Blueprints/GPE/BP_PressButton.BP_PressButton_C|SetDidIt _asbp_press_button true)
  (Rendering|Material|SetMaterial (Variables|/Game/Blueprints/GPE/BP_PressButton.BP_PressButton_C|GetCylinder _asbp_press_button) 0 "/Game/Materials/Instances/MI_Black.MI_Black")
  (Rendering|SetVisibility (Variables|Default|GetTextRender) false false)
  (bind _buttonsteamopening (Variables|Default|GetButtonSteamOpening)
    (:then
      (Default|Close _buttonsteamopening))
    (:else)))

(event Custom|CompleteDisable
  (Rendering|Material|SetMaterial (Variables|Default|GetStaticMesh) 1 "/Game/Materials/Instances/MI_UnlitBlack.MI_UnlitBlack")
  (bind _asbp_press_button (Utilities|Casting|CastToBP_PressButton (Variables|/Script/Engine.ChildActorComponent|GetChildActor (Variables|Default|GetChildActor))))
  (Variables|/Game/Blueprints/GPE/BP_PressButton.BP_PressButton_C|SetDidIt _asbp_press_button true)
  (Rendering|Material|SetMaterial (Variables|/Game/Blueprints/GPE/BP_PressButton.BP_PressButton_C|GetCylinder _asbp_press_button) 0 "/Game/Materials/Instances/MI_Black.MI_Black")
  (Rendering|SetVisibility (Variables|Default|GetTextRender) false false)
  (Variables|/Game/Blueprints/Components/BP_CustomCursorComponent.BP_CustomCursorComponent_C|SetCursorTexture (Variables|/Game/Blueprints/GPE/BP_InteractiveBase.BP_InteractiveBase_C|GetBP_CustomCursorComponent _asbp_press_button) "/Game/Textures/T_CursorNormal.T_CursorNormal")
  (bind _buttonsteamopening (Variables|Default|GetButtonSteamOpening)
    (:then
      (Default|Close _buttonsteamopening))
    (:else)))

(event Custom|TurnOn
  (CallFunction|ClearID))

(event Custom|SetID
  (params (ID :type String))
  (bind _output_get (Variables|Default|SetID ID))
  (Rendering|Components|TextRender|SetText (Variables|Default|GetTextRender) (Utilities|Text|ToText(String) _output_get)))

(event Custom|ClearID
  (Variables|Default|SetID "")
  (Rendering|Material|SetMaterial (Variables|Default|GetStaticMesh) 1 "/Game/Materials/MAT_Static.MAT_Static")
  (bind _asbp_press_button (Utilities|Casting|CastToBP_PressButton (Variables|/Script/Engine.ChildActorComponent|GetChildActor (Variables|Default|GetChildActor))))
  (Variables|/Game/Blueprints/GPE/BP_PressButton.BP_PressButton_C|SetDidIt _asbp_press_button true)
  (Rendering|Material|SetMaterial (Variables|/Game/Blueprints/GPE/BP_PressButton.BP_PressButton_C|GetCylinder _asbp_press_button) 0 "/Game/Materials/Instances/MI_Black.MI_Black")
  (Rendering|SetVisibility (Variables|Default|GetTextRender) false false)
  (bind _buttonsteamopening (Variables|Default|GetButtonSteamOpening)
    (:then
      (Default|Close _buttonsteamopening))
    (:else)))

(event Custom|OnTriggered_Event
  (bind _id (Variables|Default|GetID))
  (if (not (Utilities|Array|IsEmpty _id))
    (Default|CallOnButtonClicked _id)))

(event Custom|Enable
  (Rendering|Material|SetMaterial (Variables|Default|GetStaticMesh) 1 "/Game/Materials/Instances/MI_KeycardReaderIdle.MI_KeycardReaderIdle")
  (bind _asbp_press_button (Utilities|Casting|CastToBP_PressButton (Variables|/Script/Engine.ChildActorComponent|GetChildActor (Variables|Default|GetChildActor))))
  (Variables|/Game/Blueprints/GPE/BP_PressButton.BP_PressButton_C|SetDidIt _asbp_press_button false)
  (Rendering|Material|SetMaterial (Variables|/Game/Blueprints/GPE/BP_PressButton.BP_PressButton_C|GetCylinder _asbp_press_button) 0 "/Game/Materials/Instances/MI_PressButton.MI_PressButton")
  (Rendering|SetVisibility (Variables|Default|GetTextRender) true false)
  (bind _buttonsteamopening (Variables|Default|GetButtonSteamOpening)
    (:then
      (Default|Open _buttonsteamopening))
    (:else)))

(event EventBeginPlay
  (bind _asbp_press_button (Utilities|Casting|CastToBP_PressButton (Variables|/Script/Engine.ChildActorComponent|GetChildActor (Variables|Default|GetChildActor))))
  (Variables|/Game/Blueprints/GPE/BP_PressButton.BP_PressButton_C|SetDidIt _asbp_press_button true)
  (Rendering|Material|SetMaterial (Variables|/Game/Blueprints/GPE/BP_PressButton.BP_PressButton_C|GetCylinder _asbp_press_button) 0 "/Game/Materials/Instances/MI_Black.MI_Black")
  (EventDispatchers|AssignOnTriggered _asbp_press_button (delegate Custom|OnTriggered_Event)))

(fn ConstructionScript)