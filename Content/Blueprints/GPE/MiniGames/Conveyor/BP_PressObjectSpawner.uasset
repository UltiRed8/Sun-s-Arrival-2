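; Object spawner for the conveyor minigame that feeds chaos actors onto the belt.
; Trigger alternately unpauses and pauses a looping timer that spawns bursts of three actors a second apart, skipping spawns while paused.
; Each actor joins the conveyor's ActorsToMove list, and a cycling counter makes one non-random with the spawner's Type and the others random.
; Reward puts a RewardObject on the same conveyor list.
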(event Custom|Spawn
  (if (not (Class|KismetSystemLibrary|IsTimerPausedHandle (Variables|Default|GetTimerRef)))
    (bind _returnvalue (Game|SpawnActorfromClass "/Game/Chaos/BP_ChaosActor.BP_ChaosActor_C" (Math|Transform|MakeTransform (Transformation|GetWorldLocation (Variables|Default|GetScene)) "0, 0, 0" "1.000000,1.000000,1.000000") "AdjustIfPossibleButAlwaysSpawn" "MultiplyWithRoot" 0 (Variables|Default|GetType) (not (== (Variables|Default|GetCounter) 0)) 0))
    (Utilities|IsValid _returnvalue
      (:Is%20Valid
        (Utilities|Array|Add (Variables|/Game/Blueprints/GPE/BP_Conveyor.BP_Conveyor_C|GetActorsToMove (Variables|Default|GetBP_Convoyer)) _returnvalue))
      (:Is%20Not%20Valid
        _))
    (bind _result (Math|Integer|DecrementInt (Variables|Default|GetCounter))
      (:%20%20
        (if (<= _result -1)
          (Variables|Default|SetCounter 2))))))

(event Custom|Reward
  (Utilities|Array|Add (Variables|/Game/Blueprints/GPE/BP_Conveyor.BP_Conveyor_C|GetActorsToMove (Variables|Default|GetBP_Convoyer)) (Variables|Default|GetRewardObject)))

(event Custom|SpawnChain
  (CallFunction|Spawn)
  (Utilities|FlowControl|Delay 1.0)
  (CallFunction|Spawn)
  (Utilities|FlowControl|Delay 1.0)
  (CallFunction|Spawn))

(event EventBeginPlay
  (bind _returnvalue (Utilities|Time|SetTimerbyFunctionName 0 "SpawnChain" 7.5 true))
  (bind _output_get (Variables|Default|SetTimerRef _returnvalue))
  (Utilities|Time|PauseTimerbyHandle _output_get))

(event EventTrigger
  (bind _timerref (Variables|Default|GetTimerRef))
  (|CallParentFunction)
  (Utilities|FlowControl|FlipFlop
    (:A
      (Utilities|Time|UnpauseTimerbyHandle _timerref))
    (:B
      (Utilities|Time|PauseTimerbyHandle _timerref))))

(fn ConstructionScript)