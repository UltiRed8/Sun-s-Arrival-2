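; Manager for the conveyor press minigame, coordinating conveyors, presses and an object spawner.
; A press starts the round, and each validated object is compared to a random target type, then multicast feedback plays and the authority pauses and rerolls.
; Reaching max score triggers rewards, achievements and a checkpoint bool keyed by actor location, restored on BeginPlay.
; Hardcore speeds up conveyors and presses, while other modes rescale fences.
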(event Custom|Validated
  (params (Type :type E_GCType%20Enum :default "NewEnumerator0"))
  (if (Utilities|Enum|Equal(Enum) Type (Variables|Default|GetType))
    (bind _result (Math|Integer|IncrementInt (Variables|Default|GetScore))
      (:%20%20
        (CallFunction|UpdateProgress)
        (if (>= _result (Variables|Default|GetMaxScore))
          (CallFunction|Victory)
          (else
            (CallFunction|MultiSuccess)))))
    (else
      (CallFunction|MultiError))))

(event Custom|SelectNextType
  (if (Math|Random|RandomBool)
    (if (Math|Random|RandomBool)
      (Variables|Default|SetType "NewEnumerator0")
      (else
        (Variables|Default|SetType "NewEnumerator1")))
    (elif (Math|Random|RandomBool)
      (Variables|Default|SetType "NewEnumerator2")
      (else
        (Variables|Default|SetType "NewEnumerator3"))))
  (CallFunction|UpdateType))

(event Custom|OnPressed
  (if (not (Variables|Default|GetIsActivated))
    (if (== (Variables|Default|GetScore) 0)
      (Variables|Default|SetIsActivated true)
      (CallFunction|SelectNextType)
      (CallFunction|ToggleConveyors)
      (Default|Trigger (Variables|Default|GetSpawnerNode)))))

(event Custom|UpdateType
  (for _array_element (Variables|Default|GetConnectedPresses)
    (Default|MultiSetType _array_element (Variables|Default|GetType)))
  (Variables|/Game/Blueprints/GPE/MiniGames/Conveyor/BP_PressObjectSpawner.BP_PressObjectSpawner_C|SetType (Variables|Default|GetObjectSpawner) (Variables|Default|GetType)))

(event Custom|ToggleConveyors
  (for _array_element (Variables|Default|GetConveyors)
    (Default|Trigger _array_element)))

(event Custom|Multi_Error
  (for _array_element (Variables|Default|GetConnectedPresses)
    (Default|PressError _array_element))
  (Networking|SwitchHasAuthority
    (:Authority
      (CallFunction|ToggleConveyors)
      (Default|Trigger (Variables|Default|GetSpawnerNode))
      (Utilities|FlowControl|Delay 1.0)
      (CallFunction|SelectNextType)
      (CallFunction|ToggleConveyors)
      (Default|Trigger (Variables|Default|GetSpawnerNode)))))

(event Custom|Multi_Success
  (for _array_element (Variables|Default|GetConnectedPresses)
    (Default|PressSuccess _array_element))
  (Networking|SwitchHasAuthority
    (:Authority
      (CallFunction|ToggleConveyors)
      (Default|Trigger (Variables|Default|GetSpawnerNode))
      (Utilities|FlowControl|Delay 1.0)
      (CallFunction|SelectNextType)
      (CallFunction|ToggleConveyors)
      (Default|Trigger (Variables|Default|GetSpawnerNode)))))

(event Custom|LoadSuccess
  (Utilities|FlowControl|Sequence
    (:then_0
      (for _array_element (Variables|Default|GetConveyors)
        (for _array_element_2 (Variables|/Game/Blueprints/GPE/BP_Conveyor.BP_Conveyor_C|GetActorsToMove _array_element)
          (bind _asbp_chaos_actor (Utilities|Casting|CastToBP_ChaosActor _array_element_2))
          (Utilities|IsValid _asbp_chaos_actor
            (:Is%20Valid
              (Default|PrepareDestroy _asbp_chaos_actor)))))
      (Utilities|FlowControl|Delay 2.0)
      (bind _asbp_press_object_spawner (Utilities|Casting|CastToBP_PressObjectSpawner (Variables|Default|GetSpawnerNode)))
      (Default|Reward _asbp_press_object_spawner))
    (:then_1
      (Utilities|FlowControl|Delay 2.0)
      (for _array_element_3 (Variables|Default|GetConveyors)
        (Variables|/Game/Blueprints/GPE/BP_Conveyor.BP_Conveyor_C|SetSpeed _array_element_3 (/ (Variables|/Game/Blueprints/GPE/BP_Conveyor.BP_Conveyor_C|GetSpeed _array_element_3) (Math|Float|SelectFloat 2.0 1.0 (Variables|Default|GetIsHardcore)))))
      (CallFunction|ToggleConveyors)
      (Utilities|FlowControl|Delay 6.0)
      (CallFunction|ToggleConveyors))))

(event Custom|SetupForDifficulty
  (switch Utilities|FlowControl|Switch|SwitchonE_ExtrasGamemodes (Variables|/Game/BP_GameInstance.BP_GameInstance_C|GetExtraGamemode (Utilities|GameInstance))
    (:NewEnumerator0
      _)
    (:NewEnumerator1
      _)
    (:NewEnumerator3
      _))
  (for _array_element (Variables|Default|GetFences)
    (Transformation|SetActorScale3D _array_element "1.000000,1.140000,3.200000")))

(event Custom|Victory
  (bind _asbp_game_instance (Utilities|GameInstance))
  (bind _asbp_player (Utilities|Casting|CastToBP_Player (Pawn|GetControlledPawn (Game|GetPlayerController 0))))
  (if (not (Variables|/Game/Blueprints/Player/BP_Player.BP_Player_C|GetIsDead _asbp_player))
    (Utilities|CheckpointSaveBool (Utilities|String|ToString(Vector) (Transformation|GetActorLocation)) true)
    (CallFunction|MultiVictory)
    (Default|Trigger (Variables|Default|GetVictoryNode))
    (CallFunction|ToggleConveyors)
    (Default|Trigger (Variables|Default|GetSpawnerNode))
    (Utilities|FlowControl|Sequence
      (:then_0
        (Utilities|FlowControl|Delay 2.0)
        (for _array_element (Variables|Default|GetConveyors)
          (Variables|/Game/Blueprints/GPE/BP_Conveyor.BP_Conveyor_C|SetSpeed _array_element (/ (Variables|/Game/Blueprints/GPE/BP_Conveyor.BP_Conveyor_C|GetSpeed _array_element) (Math|Float|SelectFloat 2.0 1.0 (Variables|Default|GetIsHardcore)))))
        (CallFunction|ToggleConveyors)
        (Utilities|FlowControl|Delay 6.0)
        (CallFunction|ToggleConveyors))
      (:then_1
        (switch Utilities|FlowControl|Switch|SwitchonE_ExtrasGamemodes (Variables|/Game/BP_GameInstance.BP_GameInstance_C|GetExtraGamemode _asbp_game_instance)
          (:NewEnumerator0
            (Default|UnlockAchievement _asbp_game_instance "ACH_MINIGAME2" :!label _label))
          (:NewEnumerator1
            (goto _label))
          (:NewEnumerator2
            (Default|UnlockAchievement _asbp_game_instance "ACH_MINIGAME2HARD"))
          (:NewEnumerator3
            (goto _label)))))))

(event Custom|Multi_Victory
  (for _array_element (Variables|Default|GetConnectedPresses)
    (Default|PressSuccess _array_element))
  (for _array_element_2 (Variables|Default|GetConveyors)
    (for _array_element_3 (Variables|/Game/Blueprints/GPE/BP_Conveyor.BP_Conveyor_C|GetActorsToMove _array_element_2)
      (bind _asbp_chaos_actor (Utilities|Casting|CastToBP_ChaosActor _array_element_3))
      (Utilities|IsValid _asbp_chaos_actor
        (:Is%20Valid
          (Default|PrepareDestroy _asbp_chaos_actor)))))
  (Utilities|FlowControl|Delay 2.0)
  (bind _asbp_press_object_spawner (Utilities|Casting|CastToBP_PressObjectSpawner (Variables|Default|GetSpawnerNode)))
  (Default|Reward _asbp_press_object_spawner))

(event Custom|UpdateProgress
  (for _array_element (Variables|Default|GetConnectedPresses)
    (Default|UpdateProgress _array_element (Variables|Default|GetScore) (Variables|Default|GetMaxScore))))

(event EventBeginPlay
  (Utilities|FlowControl|DelayUntilNextTick)
  (CallFunction|SetupforDifficulty)
  (bind _output_get (Variables|Default|SetIsHardcore (Utilities|Enum|Equal(Enum) (Variables|/Game/BP_GameInstance.BP_GameInstance_C|GetExtraGamemode (Utilities|GameInstance)) "NewEnumerator2")))
  (if _output_get
    (for _array_element (Variables|Default|GetConveyors)
      (Variables|/Game/Blueprints/GPE/BP_Conveyor.BP_Conveyor_C|SetSpeed _array_element (* (Variables|/Game/Blueprints/GPE/BP_Conveyor.BP_Conveyor_C|GetSpeed _array_element) 2.0)))
    (for _array_element_2 (Variables|Default|GetConnectedPresses)
      (Variables|/Game/Blueprints/GPE/MiniGames/Conveyor/BP_Press.BP_Press_C|SetDefaultCooldown _array_element_2 (/ (Variables|/Game/Blueprints/GPE/MiniGames/Conveyor/BP_Press.BP_Press_C|GetDefaultCooldown _array_element_2) 2.0))))
  (bind (_success _bool) (Utilities|CheckpointGetBool (Utilities|String|ToString(Vector) (Transformation|GetActorLocation))))
  (if _success
    (if _bool
      (Variables|Default|SetScore (Variables|Default|GetMaxScore))))
  (for _array_element_3 (Variables|Default|GetConnectedPresses)
    (Default|UpdateProgress _array_element_3 (Variables|Default|GetScore) (Variables|Default|GetMaxScore))
    (EventDispatchers|AssignOnPressed _array_element_3 (delegate Custom|OnPressed))
    (if (== (Variables|Default|GetScore) (Variables|Default|GetMaxScore))
      (for _array_element_4 (Variables|Default|GetConnectedPresses)
        (Default|PressSuccess _array_element_4)
        (Default|EnableScreen _array_element_4))
      (CallFunction|LoadSuccess))))

(fn ConstructionScript)