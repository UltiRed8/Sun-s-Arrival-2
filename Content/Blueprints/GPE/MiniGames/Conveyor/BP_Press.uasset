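; Press machine for the conveyor minigame, with a screen showing the body-part type, progress and success or error feedback.
; When off cooldown, a trigger fires OnPressed and a multicast timeline that lowers the press, shakes the camera, calls the parent trigger, then retracts.
; Chaos actors overlapping its box are destroyed on the server and start a cooldown.
; Tick counts the cooldown down, toggling its text, particles and sound.
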(event OnComponentBeginOverlap(Box)
  (params (OverlappedComponent :type Primitive%20Component%20Object%20Reference) (OtherActor :type Actor%20Object%20Reference) (OtherComp :type Primitive%20Component%20Object%20Reference) (OtherBodyIndex :type Integer) (bFromSweep :type Boolean) (SweepResult :type Hit%20Result%20Structure%20%28by%20ref%29))
  (Networking|SwitchHasAuthority
    (:Authority
      (bind _asbp_chaos_actor (Utilities|Casting|CastToBP_ChaosActor OtherActor))
      (Default|PrepareDestroy _asbp_chaos_actor)
      (Variables|Default|SetCooldown (Variables|Default|GetDefaultCooldown)))))

(event Custom|EnableScreen
  (Rendering|SetVisibility (Variables|Default|GetTextRender3) true false))

(event Custom|PressSuccess
  (Audio|Components|Audio|Play (Variables|Default|GetSuccessSound) 0.1)
  (Rendering|Material|SetMaterial (Variables|Default|GetDisplay) 1 "/Game/Materials/Instances/MI_KeycardReaderSuccess.MI_KeycardReaderSuccess"))

(event Custom|PressError
  (Audio|Components|Audio|Play (Variables|Default|GetErrorSound) 0.1)
  (Rendering|Material|SetMaterial (Variables|Default|GetDisplay) 1 "/Game/Materials/Instances/MI_KeycardReaderDenied.MI_KeycardReaderDenied"))

(event Custom|Multi_PressAnimation
  (bind _staticmesh (Variables|Default|GetStaticMesh))
  (bind _relativelocation (Variables|/Script/Engine.SceneComponent|GetRelativeLocation _staticmesh))
  (bind (_direction _newtrack_0) (Timeline|PressTimeline Play)
    (:Update
      (Transformation|SetRelativeLocation _staticmesh (Math|Vector|MakeVector (.x _relativelocation) (.y _relativelocation) (Math|Float|Lerp -8e+01 -1.4e+02 _newtrack_0)) false false))
    (:Finished
      (switch Utilities|FlowControl|Switch|SwitchonETimelineDirection _direction
        (:Forward
          (Default|CameraShake (Utilities|GameInstance) "/Game/Shakes/CS_Press.CS_Press_C" (Transformation|GetActorLocation) 8e+02 1.6e+03 1.0 false)
          (Audio|Components|Audio|Play (Variables|Default|GetPressed) 0.1)
          (Utilities|FlowControl|Delay 0.15)
          (|CallParentFunction)
          (Timeline|PressTimeline Reverse))))))

(event Custom|Multi_SetType
  (params (Type :type E_GCType%20Enum :default "NewEnumerator0"))
  (Rendering|Material|SetTextureParameterValue (Variables|Default|GetDynamicMaterial) "Texture" (Utilities|Select :Index Type :NewEnumerator0 "/Game/Textures/T_PressHead.T_PressHead" :NewEnumerator1 "/Game/Textures/T_PressArm.T_PressArm" :NewEnumerator2 "/Game/Textures/T_PressLeg.T_PressLeg" :NewEnumerator3 "/Game/Textures/T_PressBody.T_PressBody"))
  (Rendering|Material|SetMaterial (Variables|Default|GetDisplay) 1 (Variables|Default|GetDynamicMaterial))
  (CallFunction|EnableScreen))

(event Custom|UpdateProgress
  (params (Current :type Integer) (Max :type Integer))
  (Rendering|Components|TextRender|SetText (Variables|Default|GetTextRender) (Utilities|Text|FormatText "{Current}/{Max}" Current Max)))

(event EventBeginPlay
  (bind _returnvalue (Rendering|Material|CreateDynamicMaterialInstance (Variables|Default|GetDisplay) 1 "/Game/Materials/MAT_PressScreen.MAT_PressScreen" "None" :!class /Script/Engine.PrimitiveComponent))
  (Variables|Default|SetDynamicMaterial _returnvalue)
  (Rendering|SetVisibility (Variables|Default|GetTextRender3) false false))

(event EventTick
  (params (DeltaSeconds :type Float%20%28single-precision%29))
  (bind _textrender1 (Variables|Default|GetTextRender1))
  (bind _niagara (Variables|Default|GetNiagara))
  (bind _cooldownsound (Variables|Default|GetCooldownSound))
  (bind _output_get (Variables|Default|SetCooldown (Math|Float|Clamp(Float) (- (Variables|Default|GetCooldown) DeltaSeconds) 0.0 1e+01)))
  (Rendering|Components|TextRender|SetText (Variables|Default|GetTextRender1) (Utilities|Text|ToText(Float) _output_get "HalfToEven" false true 1 1 2 2))
  (if (== _output_get 0.0)
    (Utilities|OnceGate :!label _label
      (:OutA
        (Rendering|SetVisibility _textrender1 false false)
        (Components|Activation|Deactivate _niagara)
        (Audio|Components|Audio|Stop _cooldownsound))
      (:OutB
        (Rendering|SetVisibility _textrender1 true false)
        (Components|Activation|Activate _niagara false)
        (Audio|Components|Audio|Play _cooldownsound 0.0)))
    (else
      (goto _label InB))))

(event EventTrigger
  (if (== (Variables|Default|GetCooldown) 0.0)
    (CallFunction|MultiPressAnimation)
    (Default|CallOnPressed)))

(fn ConstructionScript)