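; Crane mini-game actor where a magnet moves on a grid to pick up and drop crates, with separate singleplayer and multiplayer layouts.
; Input drives server and multicast events that slide the magnet on Tick and play a Timeline dip to attach or release crates.
; Line traces find crates, reject gold-material ones and block obstructed moves or drops.
; Crane and crate positions save to checkpoints, restored on BeginPlay only in singleplayer.
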(event OnComponentBeginOverlap(MiniGameArea)
  (params (OverlappedComponent :type Primitive%20Component%20Object%20Reference) (OtherActor :type Actor%20Object%20Reference) (OtherComp :type Primitive%20Component%20Object%20Reference) (OtherBodyIndex :type Integer) (bFromSweep :type Boolean) (SweepResult :type Hit%20Result%20Structure%20%28by%20ref%29))
  (bind _asbp_player (Utilities|Casting|CastToBP_Player OtherActor))
  (if (Pawn|IsLocallyControlled _asbp_player)
    (Default|SetUnstuckable _asbp_player true)))

(event OnComponentEndOverlap(MiniGameArea)
  (params (OverlappedComponent :type Primitive%20Component%20Object%20Reference) (OtherActor :type Actor%20Object%20Reference) (OtherComp :type Primitive%20Component%20Object%20Reference) (OtherBodyIndex :type Integer))
  (bind _asbp_player (Utilities|Casting|CastToBP_Player OtherActor))
  (if (Pawn|IsLocallyControlled _asbp_player)
    (Default|SetUnstuckable _asbp_player false)))

(event Custom|Multi_SetPatern
  (params (IsMultiplayer :type Boolean))
  (bind _multiplayer (Variables|Default|GetMultiplayer))
  (bind _singleplayer (Variables|Default|GetSingleplayer))
  (if IsMultiplayer
    (Transformation|SetRelativeLocation _multiplayer "0, 0, 0" false false)
    (Transformation|SetRelativeLocation _singleplayer "0.000000,0.000000,-1000.000000" false false)
    (Variables|Default|SetCurrentGameTemplate _multiplayer)
    (else
      (Transformation|SetRelativeLocation _singleplayer "0, 0, 0" false false)
      (Transformation|SetRelativeLocation _multiplayer "0.000000,0.000000,-1000.000000" false false)
      (Variables|Default|SetCurrentGameTemplate _singleplayer))))

(event Custom|Input
  (params (Type :type String))
  (if (not (Variables|Default|GetLocked))
    (if (Utilities|Enum|Equal(Enum) Type "E")
      (CallFunction|ServerAct)
      (elif (Utilities|Enum|Equal(Enum) Type "U")
        (CallFunction|TryMoveOffset -1)
        (elif (Utilities|Enum|Equal(Enum) Type "D")
          (CallFunction|TryMoveOffset 1)
          (elif (Utilities|Enum|Equal(Enum) Type "L")
            (CallFunction|TryMoveOffset 0 -1)
            (elif (Utilities|Enum|Equal(Enum) Type "R")
              (CallFunction|TryMoveOffset 0 1))))))))

(event Custom|Multi_ActAnimation
  (bind _magnet (Variables|Default|GetMagnet))
  (bind _move (Variables|Default|GetMove))
  (bind _relativelocation (Variables|/Script/Engine.SceneComponent|GetRelativeLocation _magnet))
  (Components|Timeline|SetPlayRate (Variables|Default|GetTimeline) 2.0)
  (Audio|Components|Audio|Play _move 0.0)
  (bind (_direction _height) (Timeline|Timeline Play)
    (:Update
      (Transformation|SetRelativeLocation _magnet (Math|Vector|MakeVector (.x _relativelocation) (.y _relativelocation) _height) false false))
    (:Finished
      (Audio|Components|Audio|Stop _move)
      (switch Utilities|FlowControl|Switch|SwitchonETimelineDirection _direction
        (:Forward
          (Utilities|FlowControl|Delay 0.1)
          (Audio|Components|Audio|Play _move 0.0)
          (Timeline|Timeline Reverse))
        (:Backward
          (Utilities|FlowControl|Delay 0.05)
          (Variables|Default|SetLocked false))))))

(event Custom|Multi_Grab
  (bind _magnet (Variables|Default|GetMagnet))
  (bind _returnvalue (Transformation|GetWorldLocation _magnet))
  (if (not (Variables|Default|GetNeedToMove))
    (bind _outhit (Collision|LineTraceByChannel _returnvalue (+ _returnvalue (* (Transformation|GetActorUpVector) -1e+02)) "TraceTypeQuery1" false 0 "None" false "(R=0.000000,G=0.044463,B=1.000000,A=1.000000)"))
    (Audio|Components|Audio|Play (Variables|Default|GetGrab) 0.0)
    (Audio|Components|Audio|Play (Variables|Default|GetGrabIdle) 0.0)
    (Transformation|AttachComponentToComponent (.HitComponent (Collision|BreakHitResult _outhit)) (Variables|Default|GetMagnet) "None" "KeepWorld" "KeepWorld" "KeepWorld" true)
    (Variables|Default|SetHasGrabbed true)
    (Variables|Default|SetGrabbedComponent (.HitComponent (Collision|BreakHitResult _outhit)))))

(event Custom|Multi_Release
  (bind _currentposition (Variables|Default|GetCurrentPosition))
  (if (not (Variables|Default|GetNeedToMove))
    (Audio|Components|Audio|Play (Variables|Default|GetRelease) 0.0)
    (Audio|Components|Audio|Stop (Variables|Default|GetGrabIdle))
    (Transformation|AttachComponentToComponent (Variables|Default|GetGrabbedComponent) (Variables|Default|GetCurrentGameTemplate) "None" "KeepWorld" "KeepWorld" "KeepWorld" true)
    (Transformation|SetRelativeLocation (Variables|Default|GetGrabbedComponent) (Math|Vector|MakeVector (* 3e+02 (.x _currentposition)) (* -3e+02 (.y _currentposition)) -6.5e+02) false false)
    (Variables|Default|SetGrabbedComponent 0)
    (Variables|Default|SetHasGrabbed false)
    (CallFunction|SaveCrates)))

(event Custom|LoadCrates
  (for (_array_element _array_index) (Utilities|GetAllCrates)
    (bind (_success _string) (Utilities|CheckpointGetString (Utilities|String|Append "CraneCrate_" (Utilities|String|ToString(Integer) _array_index))))
    (if _success
      (Transformation|SetRelativeLocation _array_element (Math|Vector|MakeVector (Math|Conversions|ToFloat(Integer) (Utilities|Array|Get(acopy) (Utilities|String|ParseIntoArray _string "@"))) (Math|Conversions|ToFloat(Integer) (Utilities|Array|Get(acopy) (Utilities|String|ParseIntoArray _string "@") 1)) (Math|Conversions|ToFloat(Integer) (Utilities|Array|Get(acopy) (Utilities|String|ParseIntoArray _string "@") 2))) false false))))

(event Custom|LoadCrane
  (bind (_success _int) (Utilities|CheckpointGetInt "Crane_X"))
  (bind (_success_2 _int_2) (Utilities|CheckpointGetInt "Crane_Y"))
  (if (and _success_2 _success)
    (CallFunction|MultiSetDestination (Utilities|Struct|MakeIntPoint _int _int_2))))

(event Custom|LoadAll
  (CallFunction|LoadCrane)
  (CallFunction|LoadCrates))

(event Custom|Server_Act
  (if (not (Variables|Default|GetLocked))
    (if (not (Variables|Default|GetNeedToMove))
      (if (Variables|Default|GetHasGrabbed)
        (bind _returnvalue (CallFunction|CheckforCollisions))
        (if (not _returnvalue)
          (Variables|Default|SetLocked true :!label _label)
          (CallFunction|MultiActAnimation)
          (Utilities|FlowControl|Delay 0.3)
          (CallFunction|GrabRelease))
        (else
          (goto _label))))))

(event Custom|TryMoveOffset
  (params (X :type Integer) (Y :type Integer))
  (if (Math|Boolean|ANDBoolean (>= (+ X (.x (Variables|Default|GetCurrentPosition))) 0) (>= (+ Y (.y (Variables|Default|GetCurrentPosition))) 0) (<= (+ X (.x (Variables|Default|GetCurrentPosition))) (Variables|Default|GetGridYSize)) (<= (+ Y (.y (Variables|Default|GetCurrentPosition))) (Variables|Default|GetGridXSize)))
    (bind _returnvalue (CallFunction|CanMoveinDirection X Y))
    (if (not _returnvalue)
      (bind _output_get (Variables|Default|SetCurrentPosition (Utilities|Struct|MakeIntPoint (+ X (.x (Variables|Default|GetCurrentPosition))) (+ Y (.y (Variables|Default|GetCurrentPosition))))))
      (CallFunction|ServerSetDestination _output_get))))

(event Custom|SaveCrane
  (bind _currentposition (Variables|Default|GetCurrentPosition))
  (Utilities|CheckpointSaveInt "Crane_X" (.x _currentposition))
  (Utilities|CheckpointSaveInt "Crane_Y" (.y _currentposition)))

(event Custom|SetupCrates
  (CallFunction|MultiSetPatern (Default|IsinMultiplayer (Utilities|GameInstance))))

(event Custom|GrabRelease
  (bind _magnet (Variables|Default|GetMagnet))
  (bind _returnvalue (Transformation|GetWorldLocation _magnet))
  (if (not (Variables|Default|GetNeedToMove))
    (if (Variables|Default|GetHasGrabbed)
      (CallFunction|MultiRelease)
      (else
        (bind (_outhit _returnvalue_2) (Collision|LineTraceByChannel _returnvalue (+ _returnvalue (* (Transformation|GetActorUpVector) -1e+02)) "TraceTypeQuery1" false 0 "None" false "(R=0.000000,G=0.044463,B=1.000000,A=1.000000)"))
        (if _returnvalue_2
          (bind _asstatic_mesh_component (Utilities|Casting|CastToStaticMeshComponent (.HitComponent (Collision|BreakHitResult _outhit))))
          (if (not (== (Rendering|Material|GetMaterial _asstatic_mesh_component 0) "/Game/Materials/Instances/MI_Gold.MI_Gold"))
            (CallFunction|MultiGrab)))))))

(event Custom|Multi_SetDestination
  (params (CurrentPosition :type Int%20Point%20Structure))
  (Variables|Default|SetCurrentPosition CurrentPosition)
  (CallFunction|SaveCrane)
  (if (not (Variables|Default|GetNeedToMove))
    (Variables|Default|SetNeedToMove true)
    (Audio|Components|Audio|Play (Variables|Default|GetMove) (Math|Random|RandomFloatinRange 0.0 2.0))))

(event Custom|SaveCrates
  (for (_array_element _array_index) (Utilities|GetAllCrates)
    (Utilities|CheckpointSaveString (Utilities|String|Append "CraneCrate_" (Utilities|String|ToString(Integer) _array_index)) (Utilities|String|Append (Utilities|String|ToString(Float) (.x (Variables|/Script/Engine.SceneComponent|GetRelativeLocation _array_element))) "@" (Utilities|String|ToString(Float) (.y (Variables|/Script/Engine.SceneComponent|GetRelativeLocation _array_element))) "@" (Utilities|String|ToString(Float) (.z (Variables|/Script/Engine.SceneComponent|GetRelativeLocation _array_element)))))))

(event Custom|Server_SetDestination
  (params (CurrentPosition :type Int%20Point%20Structure))
  (CallFunction|MultiSetDestination CurrentPosition))

(event EventTick
  (params (DeltaSeconds :type Float%20%28single-precision%29))
  (bind _magnet (Variables|Default|GetMagnet))
  (bind _currentposition (Variables|Default|GetCurrentPosition))
  (bind _offsetx (Variables|Default|GetOffsetX))
  (bind _offsety (Variables|Default|GetOffsetY))
  (bind _returnvalue (* _offsetx (.x _currentposition)))
  (bind _returnvalue_2 (* _offsety (.y _currentposition)))
  (bind _relativelocation (Variables|/Script/Engine.SceneComponent|GetRelativeLocation _magnet))
  (bind _returnvalue_3 (Math|Vector|MakeVector _returnvalue _returnvalue_2 0.0))
  (bind _returnvalue_4 (Math|Interpolation|VInterptoConstant _relativelocation _returnvalue_3 DeltaSeconds 1.6e+03))
  (if (Variables|Default|GetNeedToMove)
    (Transformation|SetRelativeLocation (Variables|Default|GetMagnet) _returnvalue_4 false false)
    (if (Utilities|Operators|EqualEqual _relativelocation _returnvalue_4 0.1)
      (Variables|Default|SetNeedToMove false)
      (Audio|Components|Audio|Stop (Variables|Default|GetMove)))))

(event EventBeginPlay
  (bind _asbp_game_instance (Utilities|GameInstance))
  (bind _returnvalue (Default|IsinMultiplayer _asbp_game_instance))
  (Networking|SwitchHasAuthority
    (:Authority
      (CallFunction|MultiSetPatern _returnvalue)
      (if (not _returnvalue)
        (CallFunction|LoadAll)))))

(fn ConstructionScript)

(fn CheckforCollisions
  (bind _returnvalue (Transformation|GetActorUpVector))
  (bind _grabbedcomponent (Variables|Default|GetGrabbedComponent))
  (bind _returnvalue_2 (Transformation|GetWorldLocation _grabbedcomponent))
  (Utilities|IsValid _grabbedcomponent
    (:Is%20Valid
      (bind _returnvalue_3 (Collision|LineTraceByChannel (+ _returnvalue_2 (* _returnvalue -5e+01)) (+ _returnvalue_2 (* _returnvalue -1.5e+02)) "TraceTypeQuery1" false 0 "None" false "(R=0.000000,G=0.044463,B=1.000000,A=1.000000)"))
      (return _returnvalue_3))
    (:Is%20Not%20Valid
      (return false))))

(fn CanMoveinDirection
  (params (XOffset :type Integer) (YOffset :type Integer))
  (bind _defaultsceneroot (Variables|Default|GetDefaultSceneRoot))
  (bind _currentposition (Variables|Default|GetCurrentPosition))
  (bind _returnvalue (Transformation|GetWorldLocation _defaultsceneroot))
  (bind _returnvalue_2 (* (.x _currentposition) -270))
  (bind _returnvalue_3 (* (.y _currentposition) 270))
  (bind _returnvalue_4 (+ (.y _returnvalue) _returnvalue_3))
  (bind _returnvalue_5 (+ (.x _returnvalue) _returnvalue_2))
  (bind _returnvalue_6 (Math|Vector|MakeVector _returnvalue_5 _returnvalue_4 1e+02))
  (Utilities|IsValid (Variables|Default|GetGrabbedComponent)
    (:Is%20Valid
      (bind _returnvalue_7 (Collision|LineTraceByChannel _returnvalue_6 (+ _returnvalue_6 (Math|Vector|MakeVector (* XOffset -200) (* YOffset 200) 0.0)) "TraceTypeQuery1" false 0 "ForDuration" false "(R=1.000000,G=0.000000,B=0.965546,A=1.000000)" "(R=0.000000,G=1.000000,B=0.000000,A=1.000000)" 1.5))
      (return _returnvalue_7))
    (:Is%20Not%20Valid
      (return false))))