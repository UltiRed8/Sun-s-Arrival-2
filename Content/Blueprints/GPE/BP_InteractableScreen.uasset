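; Interactable screen prop that switches between on and off looks through material swaps.
; On BeginPlay it disables interaction via CanBeInteract and sets the Screen mesh's LED slot to the off material.
; TurnScreenOn and TurnScreenOff events change the Plane's display material and the LED material together; neither changes the interaction flag.
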(event Custom|TurnScreenOn
  (Rendering|Material|SetMaterial (Variables|Default|GetPlane) 0 (Variables|Default|GetScreenOnMaterial))
  (Rendering|Material|SetMaterial (Variables|Default|GetScreen) 4 "/Game/Materials/Instances/MI_ScreenLed.MI_ScreenLed"))

(event Custom|TurnScreenOff
  (Rendering|Material|SetMaterial (Variables|Default|GetPlane) 0 (Variables|Default|GetScreenOffMat))
  (Rendering|Material|SetMaterial (Variables|Default|GetScreen) 4 "/Game/Materials/Instances/MI_ScreenOffLed.MI_ScreenOffLed"))

(event EventBeginPlay
  (Variables|Default|SetCanBeInteract false)
  (Rendering|Material|SetMaterial (Variables|Default|GetScreen) 4 "/Game/Materials/Instances/MI_ScreenOffLed.MI_ScreenOffLed"))

(fn ConstructionScript)