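; Interactable pipe valve that can burst into a steam leak once, on a random chance when a player overlaps its box, becoming interactable.
; Mouse-capture and movement components let the player crank the wheel with circular motion, replicating its rotation through server and multicast calls.
; A server interaction callback marks it done, shutting off the steam and switching valve sounds and cursor.
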(event OnComponentBeginOverlap(Box)
  (params (OverlappedComponent :type Primitive%20Component%20Object%20Reference) (OtherActor :type Actor%20Object%20Reference) (OtherComp :type Primitive%20Component%20Object%20Reference) (OtherBodyIndex :type Integer) (bFromSweep :type Boolean) (SweepResult :type Hit%20Result%20Structure%20%28by%20ref%29))
  (Utilities|Casting|CastToBP_Player OtherActor)
  (if (== (Math|Random|RandomIntegerinRange 0 4) 0)
    (Utilities|FlowControl|DoOnce false
      (:Completed
        (Components|Activation|SetActive (Variables|Default|GetSteam) true false)
        (Variables|/Game/Blueprints/Components/BP_CustomCursorComponent.BP_CustomCursorComponent_C|SetCursorTexture (Variables|Default|GetBP_CustomCursorComponent) "/Game/Textures/T_CursorInteract.T_CursorInteract")
        (Variables|Default|SetCanInteract true)
        (Audio|Components|Audio|Play (Variables|Default|GetSW_PipeExplosion) 0.0)
        (Components|Activation|Activate (Variables|Default|GetSteamSound) false)
        (Audio|Components|Audio|Stop (Variables|Default|GetSteamSound1))))))

(event Custom|HandcrankAnimation
  (bind _pipevalve (Variables|Default|GetPipeValve))
  (Audio|Components|Audio|SetSound _pipevalve "/Game/Audio/Sounds/SW_PipeValveClosed.SW_PipeValveClosed")
  (Audio|Components|Audio|Play _pipevalve 0.0)
  (Variables|/Game/Blueprints/Components/BP_CustomCursorComponent.BP_CustomCursorComponent_C|SetCursorTexture (Variables|Default|GetBP_CustomCursorComponent) "/Game/Textures/T_CursorNormal.T_CursorNormal")
  (Audio|Components|Audio|Stop (Variables|Default|GetSteamSound))
  (Audio|Components|Audio|Play (Variables|Default|GetSteamSound1) 0.0))

(event Custom|Multi_SetRotation
  (params (RotationX :type Float%20%28single-precision%29))
  (Transformation|SetRelativeRotation (Variables|Default|GetWheel) (Math|Rotator|MakeRotator RotationX 0.0 0.0) false false))

(event Custom|Trigger
  (Variables|Default|SetDidIt true)
  (CallFunction|HandcrankAnimation)
  (Components|Activation|SetActive (Variables|Default|GetSteam) false false)
  (Audio|Components|Audio|Play (Variables|Default|GetPipeValve) 0.0))

(event Custom|Server_SetRotation
  (params (RotationX :type Float%20%28single-precision%29))
  (CallFunction|MultiSetRotation RotationX))

(event Custom|OnMouseMoved_Event
  (params (Angle :type Float%20%28double-precision%29) (Direction :type Vector%202D%20Structure))
  (bind _wheel (Variables|Default|GetWheel))
  (bind _pipevalve (Variables|Default|GetPipeValve))
  (if (> Angle 0.0)
    (Transformation|AddRelativeRotation _wheel (Math|Rotator|MakeRotator (* (Math|Trig|RadiansToDegrees Angle) 1.0) 0.0 0.0) false false)
    (CallFunction|ServerSetRotation (.roll (Variables|/Script/Engine.SceneComponent|GetRelativeRotation _wheel)))
    (if (Audio|Components|Audio|IsPlaying _pipevalve)
      _
      (else
        (Audio|Components|Audio|Play _pipevalve 0.0)))
    (Utilities|FlowControl|RetriggerableDelay 0.1)
    (if (not (Variables|Default|GetDidIt))
      (Audio|Components|Audio|Stop _pipevalve))))

(event Custom|OnMouseCapture_Event
  (Variables|/Game/Blueprints/Components/BP_CustomCursorComponent.BP_CustomCursorComponent_C|SetCursorTexture (Variables|Default|GetBP_CustomCursorComponent) "/Game/Textures/T_CursorMouseCircle.T_CursorMouseCircle"))

(event Custom|OnMouseUncaptured_Event
  (Variables|/Game/Blueprints/Components/BP_CustomCursorComponent.BP_CustomCursorComponent_C|SetCursorTexture (Variables|Default|GetBP_CustomCursorComponent) (select (Variables|Default|GetDidIt) "/Game/Textures/T_CursorNormal.T_CursorNormal" "/Game/Textures/T_CursorInteract.T_CursorInteract")))

(event EventBeginPlay
  (bind _bp_mousemovementcomponent (Variables|Default|GetBP_MouseMovementComponent))
  (Utilities|RegisterInteractable)
  (|CallParentFunction)
  (EventDispatchers|AssignOnMouseMoved _bp_mousemovementcomponent (delegate Custom|OnMouseMoved_Event))
  (EventDispatchers|AssignOnMouseCapture _bp_mousemovementcomponent (delegate Custom|OnMouseCapture_Event))
  (EventDispatchers|AssignOnMouseUncaptured _bp_mousemovementcomponent (delegate Custom|OnMouseUncaptured_Event)))

(event EventServerInteract
  (params (WhoInteracted :type Actor%20Object%20Reference))
  (if (Variables|Default|GetCanInteract)
    (Actor|SetOwner WhoInteracted)
    (if (not (Variables|Default|GetDidIt))
      (bind _asbp_player (Utilities|Casting|CastToBP_Player WhoInteracted))
      (Default|FromServerInteractwith _asbp_player self))))

(event EventOntoServerInteract
  (params (MethodName :type String))
  (CallFunction|Trigger))

(event EventDestroyed
  (Utilities|UnregisterInteractable))

(event EventClientInteract
  (Default|StartCapturing (Variables|Default|GetBP_MouseMovementComponent)))

(fn ConstructionScript)