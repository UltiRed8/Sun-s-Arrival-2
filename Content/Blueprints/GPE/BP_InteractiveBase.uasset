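; BP_InteractiveBase is an interactive gameplay actor, named as a base class, that is triggered by mouse movement gestures.
; It counts successful movements reported by its BPMouseMovementComponent until they reach a required threshold.
; Each success from that threshold onward asks the controlled BP_Player to interact with it through the server, optionally soft-stopping mouse capture.
; Releasing mouse capture resets the count.
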(event Custom|MouseMovementSuccess
  (params (Angle :type Float%20%28double-precision%29) (Direction :type Vector%202D%20Structure))
  (bind _result (Math|Integer|IncrementInt (Variables|Default|GetCurrentMovementSuccess))
    (:%20%20
      (if (>= _result (Variables|Default|GetNeededMovementSuccess))
        (bind _asbp_player (Utilities|Casting|CastToBP_Player (Pawn|GetControlledPawn (Game|GetPlayerController 0))))
        (Default|OntoServerInteractwith _asbp_player self)
        (if (Variables|Default|GetStopMouseCaptureAtSucceess)
          (Default|SoftStopCapturing (Variables|Default|GetBP_MouseMovementComponent)))))))

(event Custom|OnMouseUncaptured
  (Variables|Default|SetCurrentMovementSuccess 0))

(event EventBeginPlay
  (bind _bp_mousemovementcomponent (Variables|Default|GetBP_MouseMovementComponent))
  (EventDispatchers|AssignOnMouseMoved _bp_mousemovementcomponent (delegate Custom|MouseMovementSuccess))
  (EventDispatchers|AssignOnMouseUncaptured _bp_mousemovementcomponent (delegate Custom|OnMouseUncaptured)))

(fn ConstructionScript)