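; Interactable toilet prop with a hinged lid and lid top that open and close, plus a flush sound.
; Interaction branches on the hit component's name, defaulting to the flush.
; Timelines rotate each hinge's pitch, interlocked so the lid only lifts when the top is up and the top only lowers when the lid is down.
; CanBeInteract blocks input until each action completes, and lid sounds play as animations finish.
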(event Custom|LidTopInteract
  (if (Variables|Default|GetIsLidTopOnTop)
    (if (Variables|Default|GetIsLidDown)
      (Variables|Default|SetIsLidTopOnTop false)
      (bind (_direction _lidtop) (Timeline|LidTopInteraction Reverse)
        (:Update
          (Transformation|SetRelativeRotation (Variables|Default|GetAxisLidTop) (Math|Rotator|MakeRotator 0.0 _lidtop 0.0) false false))
        (:Finished
          (Variables|Default|SetCanBeInteract true :!label _label)
          (switch Utilities|FlowControl|Switch|SwitchonETimelineDirection _direction
            (:Forward
              (Audio|Components|Audio|Play (Variables|Default|GetSW_ToiletLidOpen) 0.0))
            (:Backward
              (Audio|Components|Audio|Play (Variables|Default|GetSW_ToiletLidClose) 0.0)))))
      (else
        (goto _label)))
    (else
      (Variables|Default|SetIsLidTopOnTop true)
      (Timeline|LidTopInteraction PlayFromStart))))

(event Custom|LidInteract
  (if (Variables|Default|GetIsLidDown)
    (if (Variables|Default|GetIsLidTopOnTop)
      (Variables|Default|SetIsLidDown false)
      (bind _lid (Timeline|LidInteraction PlayFromStart)
        (:Update
          (Transformation|SetRelativeRotation (Variables|Default|GetAxisLid) (Math|Rotator|MakeRotator 0.0 _lid 0.0) false false))
        (:Finished
          (Variables|Default|SetCanBeInteract true :!label _label)
          (switch Utilities|FlowControl|Switch|SwitchonETimelineDirection "Forward"
            (:Forward
              (Audio|Components|Audio|Play (Variables|Default|GetSW_ToiletLidOpen) 0.0))
            (:Backward
              (Audio|Components|Audio|Play (Variables|Default|GetSW_ToiletLidClose) 0.0)))))
      (else
        (goto _label)))
    (else
      (Variables|Default|SetIsLidDown true)
      (Timeline|LidInteraction Reverse))))

(event Custom|PlayToiletSound
  (Audio|Components|Audio|Play (Variables|Default|GetSW_ToiletFlush) 0.0)
  (Variables|Default|SetCanBeInteract true))

(event EventBeginPlay
  (|CallParentFunction))

(event EventInteraction
  (|CallParentFunction)
  (if (Variables|Default|GetCanBeInteract)
    (Variables|Default|SetCanBeInteract false)
    (switch string (Utilities|GetObjectName (Variables|Default|GetInteractComponent))
      (:Default
        (CallFunction|PlayToiletSound))
      (:Lid
        (CallFunction|LidInteract))
      (:LidTop
        (CallFunction|LidTopInteract)))))

(fn ConstructionScript
  (|CallParentFunction))