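; Segmented security door that opens from front and back buttons when enabled, optionally auto-closes, and saves its enabled state to checkpoints keyed by location.
; Replayed timelines slide the panels one by one with alarm, slam and steam effects, while status light and camera-visible map plane change color.
; Endo AI able to open it halt in EndoBox, scream to open it if closed or wait out transitions, then resume toward their destination.
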(event OnComponentBeginOverlap(EndoBox)
  (params (OverlappedComponent :type Primitive%20Component%20Object%20Reference) (OtherActor :type Actor%20Object%20Reference) (OtherComp :type Primitive%20Component%20Object%20Reference) (OtherBodyIndex :type Integer) (bFromSweep :type Boolean) (SweepResult :type Hit%20Result%20Structure%20%28by%20ref%29))
  (if (Variables|Default|GetIsEnabled)
    (if (not (Variables|Default|GetForceOpen))
      (bind _asbp_endo_base (Utilities|Casting|CastToBP_EndoBase OtherActor))
      (if (not (Utilities|Array|ContainsItem (Variables|Default|GetOverlappedEndo) _asbp_endo_base))
        (if (Variables|/Game/Blueprints/Enemies/BP_EndoBase.BP_EndoBase_C|GetCanOpenSAS _asbp_endo_base)
          (Utilities|Array|Add (Variables|Default|GetOverlappedEndo) _asbp_endo_base)
          (if (Variables|Default|GetIsOnTransition)
            (Class|NavMovementInterface|StopActiveMovement (Variables|/Script/Engine.Character|GetCharacterMovement _asbp_endo_base))
            (Variables|Default|SetEndoDestination (Variables|/Game/Blueprints/Enemies/BP_EndoBase.BP_EndoBase_C|GetDestination _asbp_endo_base))
            (Variables|/Game/Blueprints/Enemies/BP_EndoBase.BP_EndoBase_C|SetCanPatrol _asbp_endo_base false)
            (Variables|Default|SetHasStoppedAI true)
            (Utilities|FlowControl|Delay 0.1 :!label _label)
            (if (Variables|Default|GetIsOnTransition)
              (goto _label)
              (elif (Variables|Default|GetIsClose)
                (Variables|Default|SetHasStoppedAI false :!label _label_2)
                (if (not (Variables|Default|GetForceOpen))
                  (Variables|Default|SetForceOpen true)
                  (Class|NavMovementInterface|StopActiveMovement (Variables|/Script/Engine.Character|GetCharacterMovement _asbp_endo_base))
                  (Variables|Default|SetEndoDestination (Variables|/Game/Blueprints/Enemies/BP_EndoBase.BP_EndoBase_C|GetDestination _asbp_endo_base))
                  (Variables|/Game/Blueprints/Enemies/BP_EndoBase.BP_EndoBase_C|SetCanPatrol _asbp_endo_base false)
                  (Animation|PlayAnimMontage _asbp_endo_base "/Game/Animations/Endo/AM_Scream.AM_Scream" 1.0 "None")
                  (CallFunction|Open)
                  (Utilities|FlowControl|Delay 3.5)
                  (bind _outhit (Collision|LineTraceByChannel (Transformation|GetActorLocation _asbp_endo_base) (+ (Transformation|GetActorLocation _asbp_endo_base) (* (Transformation|GetActorForwardVector _asbp_endo_base) 1e+02)) "TraceTypeQuery1" false (Utilities|Array|MakeArray self) "None"))
                  (bind _movementresult (AI|AIMoveTo _asbp_endo_base (Variables|Default|GetEndoDestination) 0 5.0 false :!label _label_3)
                    (:then
                      (Variables|/Game/Blueprints/Enemies/BP_EndoBase.BP_EndoBase_C|SetCanPatrol _asbp_endo_base true)
                      (bind _asbp_endo_chase (Utilities|Casting|CastToBP_EndoChase _asbp_endo_base)
                        (:then
                          (Utilities|FlowControl|DelayUntilNextTick)
                          (if (Variables|/Game/Blueprints/Enemies/BP_EndoChase.BP_EndoChase_C|GetIsChasing _asbp_endo_chase)
                            _
                            (else
                              (Default|DefaultState _asbp_endo_base :!label _label_4))))
                        (:CastFailed
                          (goto _label_4)))
                      (Variables|Default|SetForceOpen false)
                      (Utilities|Array|RemoveItem (Variables|Default|GetOverlappedEndo) _asbp_endo_base)
                      (if (Variables|Default|GetClosesAutomatically)
                        (Utilities|FlowControl|Delay 4.5)
                        (CallFunction|Close)))
                    (:OnFail
                      (switch Utilities|FlowControl|Switch|SwitchonEPathFollowingResult _movementresult
                        (:Blocked
                          (Utilities|FlowControl|DelayUntilNextTick)
                          (goto _label_3))))))
                (else
                  (if (Variables|Default|GetHasStoppedAI) :!label _label_5
                    (Variables|Default|SetHasStoppedAI false)
                    (AI|AIMoveTo _asbp_endo_base (Variables|Default|GetEndoDestination) 0 5.0 false
                      (:then
                        (Variables|/Game/Blueprints/Enemies/BP_EndoBase.BP_EndoBase_C|SetCanPatrol _asbp_endo_base true)
                        (bind _asbp_endo_chase_2 (Utilities|Casting|CastToBP_EndoChase _asbp_endo_base)
                          (:then
                            (Utilities|FlowControl|DelayUntilNextTick)
                            (if (Variables|/Game/Blueprints/Enemies/BP_EndoChase.BP_EndoChase_C|GetIsChasing _asbp_endo_chase_2)
                              _
                              (else
                                (Default|DefaultState _asbp_endo_base :!label _label_6))))
                          (:CastFailed
                            (goto _label_6)))
                        (Utilities|Array|RemoveItem (Variables|Default|GetOverlappedEndo) _asbp_endo_base)))))))
            (elif (Variables|Default|GetIsClose)
              (goto _label_2)
              (else
                (Variables|Default|SetEndoDestination (Variables|/Game/Blueprints/Enemies/BP_EndoBase.BP_EndoBase_C|GetDestination _asbp_endo_base))
                (goto _label_5)))))))))

(event OnComponentEndOverlap(EndoBox)
  (params (OverlappedComponent :type Primitive%20Component%20Object%20Reference) (OtherActor :type Actor%20Object%20Reference) (OtherComp :type Primitive%20Component%20Object%20Reference) (OtherBodyIndex :type Integer))
  (bind _asbp_endo_base (Utilities|Casting|CastToBP_EndoBase OtherActor))
  (if (Utilities|Array|ContainsItem (Variables|Default|GetOverlappedEndo) _asbp_endo_base)
    (Utilities|Array|RemoveItem (Variables|Default|GetOverlappedEndo) _asbp_endo_base)))

(event Custom|SetupMapMaterial
  (bind _asbp_camera_visible_actor (Utilities|Casting|CastToBP_CameraVisibleActor (Variables|/Script/Engine.ChildActorComponent|GetChildActor (Variables|Default|GetChildActor))))
  (Rendering|Material|SetMaterial (Variables|/Game/Blueprints/Player/BP_CameraVisibleActor.BP_CameraVisibleActor_C|GetPlane _asbp_camera_visible_actor) 0 (select (Variables|Default|GetIsEnabled) "/Game/Materials/Instances/MI_Red.MI_Red" "/Game/Materials/Instances/MI_Black.MI_Black")))

(event Custom|SetupButtons
  (for _array_element (Utilities|Array|MakeArray (Variables|Default|GetCA_ButtonBack) (Variables|Default|GetCA_ButtonFront))
    (bind _asbp_press_button (Utilities|Casting|CastToBP_PressButton (Variables|/Script/Engine.ChildActorComponent|GetChildActor _array_element)))
    (EventDispatchers|AssignOnTriggered _asbp_press_button (delegate Custom|OnTriggered_Event))))

(event Custom|StartAlarm
  (bind _asbp_camera_visible_actor (Utilities|Casting|CastToBP_CameraVisibleActor (Variables|/Script/Engine.ChildActorComponent|GetChildActor (Variables|Default|GetChildActor))))
  (Rendering|Material|SetMaterial (Variables|/Game/Blueprints/Player/BP_CameraVisibleActor.BP_CameraVisibleActor_C|GetPlane _asbp_camera_visible_actor) 0 "/Game/Materials/Instances/MI_Yellow.MI_Yellow")
  (Variables|Default|SetAlarm true)
  (Audio|PlaySoundatLocation "/Game/Audio/Sounds/SW_SasAlarm.SW_SasAlarm" (Transformation|GetWorldLocation (Variables|Default|GetStaticMesh)) "0, 0, 0" 1.0 1.0 0.0 "/Game/Audio/Attenuations/SA_SasAttenuation.SA_SasAttenuation" 0 0 0 :!label _label)
  (Utilities|FlowControl|Delay 0.9)
  (if (Variables|Default|GetAlarm)
    (goto _label)))

(event Custom|OnTriggered_Event
  (CallFunction|Trigger))

(event Custom|Trigger
  (if (Variables|Default|GetIsEnabled)
    (if (not (Variables|Default|GetCooldown))
      (if (not (Variables|Default|GetIsOnTransition))
        (Variables|Default|SetCooldown true)
        (CallFunction|Open)
        (if (Variables|Default|GetClosesAutomatically)
          (Utilities|FlowControl|Delay 8.0)
          (CallFunction|Close))))))

(event Custom|SetEnabled
  (params (IsEnabled :type Boolean))
  (bind _output_get (Variables|Default|SetIsEnabled IsEnabled))
  (Rendering|Material|SetMaterial (Variables|Default|GetStaticMesh) 3 (select _output_get "/Game/Models/EndoEnemy/MAT_RedGlow.MAT_RedGlow" "/Game/Materials/Instances/MI_UnlitBlack.MI_UnlitBlack"))
  (bind _asbp_camera_visible_actor (Utilities|Casting|CastToBP_CameraVisibleActor (Variables|/Script/Engine.ChildActorComponent|GetChildActor (Variables|Default|GetChildActor)))
    (:then
      (Rendering|Material|SetMaterial (Variables|/Game/Blueprints/Player/BP_CameraVisibleActor.BP_CameraVisibleActor_C|GetPlane _asbp_camera_visible_actor) 0 (select _output_get "/Game/Materials/Instances/MI_Red.MI_Red" "/Game/Materials/Instances/MI_Black.MI_Black")))
    (:CastFailed
      _))
  (Utilities|CheckpointSaveBool (Utilities|String|ToString(Vector) (Transformation|GetActorLocation)) _output_get)
  (for _array_element (Utilities|Array|MakeArray (Variables|/Script/Engine.ChildActorComponent|GetChildActor (Variables|Default|GetCA_ButtonFront)) (Variables|/Script/Engine.ChildActorComponent|GetChildActor (Variables|Default|GetCA_ButtonBack)))
    (bind _asbp_press_button (Utilities|Casting|CastToBP_PressButton _array_element))
    (Rendering|Material|SetMaterial (Variables|/Game/Blueprints/GPE/BP_PressButton.BP_PressButton_C|GetCylinder _asbp_press_button) 0 (select (Variables|Default|GetIsEnabled) "/Game/Materials/Instances/MI_PressButton.MI_PressButton" "/Game/Materials/Instances/MI_Black.MI_Black"))))

(event Custom|ForceEvent
  (bind _ns_sassteam0 (Variables|Default|GetNS_SasSteam0))
  (Rendering|Material|SetMaterial (Variables|Default|GetStaticMesh) 3 "/Game/Materials/Instances/MI_YellowBlinking.MI_YellowBlinking")
  (CallFunction|StartAlarm)
  (Utilities|FlowControl|Delay 1.6)
  (Audio|PlaySoundatLocation "/Game/Audio/Sounds/SW_SasOpening.SW_SasOpening" (Transformation|GetActorLocation) "0, 0, 0" 1.0 2.0 0.0 "/Game/Audio/Attenuations/SA_SasAttenuation.SA_SasAttenuation" 0 0 0)
  (Utilities|FlowControl|Delay 0.4)
  (Variables|Default|SetPartIndex 0)
  (bind _position (Timeline|Timeline_0 PlayFromStart)
    (:Update
      (Transformation|SetRelativeLocation (Utilities|Array|Get(acopy) (Utilities|Array|MakeArray (Variables|Default|GetDoorPart7) (Variables|Default|GetDoorPart6) (Variables|Default|GetDoorPart5) (Variables|Default|GetDoorPart4) (Variables|Default|GetDoorPart3) (Variables|Default|GetDoorPart2) 0) (Variables|Default|GetPartIndex)) (Math|Vector|MakeVector _position 0.0 0.0) false false))
    (:Finished
      (Audio|PlaySoundatLocation "/Game/Audio/Sounds/SW_MetalDoorSlam.SW_MetalDoorSlam" (Transformation|GetActorLocation) "0, 0, 0" 0.5 2.0 0.0 "/Game/Audio/Attenuations/SA_SasAttenuation.SA_SasAttenuation" 0 0 0)
      (Variables|Default|SetIsClose false)
      (Utilities|FlowControl|Delay 0.05)
      (bind _result (Math|Integer|IncrementInt (Variables|Default|GetPartIndex))
        (:%20%20
          (if (not (<= _result 5))
            (Components|Activation|Activate _ns_sassteam0 false)
            (Audio|PlaySoundatLocation "/Game/Audio/Sounds/SW_Steam.SW_Steam" (Transformation|GetActorLocation) "0, 0, 0" 5.0 1.0 0.0 "/Game/Audio/Attenuations/SA_SasAttenuation.SA_SasAttenuation" 0 0 0)
            (Utilities|FlowControl|Delay 0.5)
            (Components|Activation|Deactivate _ns_sassteam0)
            (Variables|Default|SetAlarm false)
            (Utilities|FlowControl|Delay 0.5)
            (Rendering|Material|SetMaterial (Variables|Default|GetStaticMesh) 3 "/Game/Models/EndoEnemy/MAT_GreenGlow.MAT_GreenGlow")
            (bind _asbp_camera_visible_actor (Utilities|Casting|CastToBP_CameraVisibleActor (Variables|/Script/Engine.ChildActorComponent|GetChildActor (Variables|Default|GetChildActor))))
            (Rendering|Material|SetMaterial (Variables|/Game/Blueprints/Player/BP_CameraVisibleActor.BP_CameraVisibleActor_C|GetPlane _asbp_camera_visible_actor) 0 "/Game/Materials/Instances/MI_Green.MI_Green")))))))

(event Custom|Close
  (bind _ns_sassteam0 (Variables|Default|GetNS_SasSteam0))
  (Rendering|Material|SetMaterial (Variables|Default|GetStaticMesh) 3 "/Game/Materials/Instances/MI_YellowBlinking.MI_YellowBlinking")
  (CallFunction|StartAlarm)
  (Utilities|FlowControl|Delay 1.6)
  (Audio|PlaySoundatLocation "/Game/Audio/Sounds/SW_SasClosing.SW_SasClosing" (Transformation|GetActorLocation) "0, 0, 0" 2.0 2.0 0.0 "/Game/Audio/Attenuations/SA_SasAttenuation.SA_SasAttenuation" 0 0 0)
  (Utilities|FlowControl|Delay 0.4)
  (Variables|Default|SetPartIndex 5)
  (Variables|Default|SetIsOnTransition true)
  (bind _position (Timeline|Timeline ReverseFromEnd)
    (:Update
      (Transformation|SetRelativeLocation (Utilities|Array|Get(acopy) (Utilities|Array|MakeArray (Variables|Default|GetDoorPart7) (Variables|Default|GetDoorPart6) (Variables|Default|GetDoorPart5) (Variables|Default|GetDoorPart4) (Variables|Default|GetDoorPart3) (Variables|Default|GetDoorPart2) (Variables|Default|GetDoorPart1)) (Variables|Default|GetPartIndex)) (Math|Vector|MakeVector _position 0.0 0.0) false false))
    (:Finished
      (Audio|PlaySoundatLocation "/Game/Audio/Sounds/SW_MetalDoorSlam.SW_MetalDoorSlam" (Transformation|GetActorLocation) "0, 0, 0" 0.5 2.0 0.0 "/Game/Audio/Attenuations/SA_SasAttenuation.SA_SasAttenuation" 0 0 0)
      (Variables|Default|SetIsClose true)
      (Utilities|FlowControl|Delay 0.05)
      (bind _result (Math|Integer|DecrementInt (Variables|Default|GetPartIndex))
        (:%20%20
          (if (>= _result 0)
            (Timeline|Timeline ReverseFromEnd)
            (else
              (Components|Activation|Activate _ns_sassteam0 false)
              (Audio|PlaySoundatLocation "/Game/Audio/Sounds/SW_Steam.SW_Steam" (Transformation|GetActorLocation) "0, 0, 0" 5.0 1.0 0.0 "/Game/Audio/Attenuations/SA_SasAttenuation.SA_SasAttenuation" 0 0 0)
              (Utilities|FlowControl|Delay 0.5)
              (Components|Activation|Deactivate _ns_sassteam0)
              (Variables|Default|SetAlarm false)
              (Utilities|FlowControl|Delay 0.5)
              (Rendering|Material|SetMaterial (Variables|Default|GetStaticMesh) 3 "/Game/Models/EndoEnemy/MAT_RedGlow.MAT_RedGlow")
              (Variables|Default|SetCooldown false)
              (Variables|Default|SetIsOnTransition false)
              (bind _asbp_camera_visible_actor (Utilities|Casting|CastToBP_CameraVisibleActor (Variables|/Script/Engine.ChildActorComponent|GetChildActor (Variables|Default|GetChildActor))))
              (Rendering|Material|SetMaterial (Variables|/Game/Blueprints/Player/BP_CameraVisibleActor.BP_CameraVisibleActor_C|GetPlane _asbp_camera_visible_actor) 0 "/Game/Materials/Instances/MI_Red.MI_Red"))))))))

(event Custom|Open
  (bind _ns_sassteam0 (Variables|Default|GetNS_SasSteam0))
  (if (not (Variables|Default|GetIsOnTransition))
    (Rendering|Material|SetMaterial (Variables|Default|GetStaticMesh) 3 "/Game/Materials/Instances/MI_YellowBlinking.MI_YellowBlinking")
    (CallFunction|StartAlarm)
    (Utilities|FlowControl|Delay 1.6)
    (Audio|PlaySoundatLocation "/Game/Audio/Sounds/SW_SasOpening.SW_SasOpening" (Transformation|GetActorLocation) "0, 0, 0" 1.0 2.0 0.0 "/Game/Audio/Attenuations/SA_SasAttenuation.SA_SasAttenuation" 0 0 0)
    (Utilities|FlowControl|Delay 0.4)
    (Variables|Default|SetPartIndex 0)
    (Variables|Default|SetIsOnTransition true)
    (bind _position (Timeline|PartOpening PlayFromStart)
      (:Update
        (Transformation|SetRelativeLocation (Utilities|Array|Get(acopy) (Utilities|Array|MakeArray (Variables|Default|GetDoorPart7) (Variables|Default|GetDoorPart6) (Variables|Default|GetDoorPart5) (Variables|Default|GetDoorPart4) (Variables|Default|GetDoorPart3) (Variables|Default|GetDoorPart2) (Variables|Default|GetDoorPart1)) (Variables|Default|GetPartIndex)) (Math|Vector|MakeVector _position 0.0 0.0) false false))
      (:Finished
        (Audio|PlaySoundatLocation "/Game/Audio/Sounds/SW_MetalDoorSlam.SW_MetalDoorSlam" (Transformation|GetActorLocation) "0, 0, 0" 0.5 2.0 0.0 "/Game/Audio/Attenuations/SA_SasAttenuation.SA_SasAttenuation" 0 0 0)
        (Variables|Default|SetIsClose false)
        (Utilities|FlowControl|Delay 0.05)
        (bind _result (Math|Integer|IncrementInt (Variables|Default|GetPartIndex))
          (:%20%20
            (if (<= _result 5)
              (Timeline|PartOpening PlayFromStart)
              (else
                (Components|Activation|Activate _ns_sassteam0 false)
                (Audio|PlaySoundatLocation "/Game/Audio/Sounds/SW_Steam.SW_Steam" (Transformation|GetActorLocation) "0, 0, 0" 5.0 1.0 0.0 "/Game/Audio/Attenuations/SA_SasAttenuation.SA_SasAttenuation" 0 0 0)
                (Utilities|FlowControl|Delay 0.5)
                (Components|Activation|Deactivate _ns_sassteam0)
                (Variables|Default|SetAlarm false)
                (Utilities|FlowControl|Delay 0.5)
                (Rendering|Material|SetMaterial (Variables|Default|GetStaticMesh) 3 "/Game/Models/EndoEnemy/MAT_GreenGlow.MAT_GreenGlow")
                (Variables|Default|SetIsOnTransition false)
                (bind _asbp_camera_visible_actor (Utilities|Casting|CastToBP_CameraVisibleActor (Variables|/Script/Engine.ChildActorComponent|GetChildActor (Variables|Default|GetChildActor))))
                (Rendering|Material|SetMaterial (Variables|/Game/Blueprints/Player/BP_CameraVisibleActor.BP_CameraVisibleActor_C|GetPlane _asbp_camera_visible_actor) 0 "/Game/Materials/Instances/MI_Green.MI_Green")))))))))

(event EventBeginPlay
  (bind _doorpart1 (Variables|Default|GetDoorPart1))
  (if (Variables|Default|GetIsEnabled)
    (Collision|SetCollisionResponsetoChannel _doorpart1 "ECC_Pawn" "ECR_Overlap")
    (Collision|SetCollisionResponsetoChannel _doorpart1 "ECC_Vehicle" "ECR_Overlap"))
  (CallFunction|SetupMapMaterial)
  (CallFunction|SetupButtons)
  (bind (_success _bool) (Utilities|CheckpointGetBool (Utilities|String|ToString(Vector) (Transformation|GetActorLocation))))
  (if _success
    (CallFunction|SetEnabled _bool))
  (for _array_element (Utilities|Array|MakeArray (Variables|/Script/Engine.ChildActorComponent|GetChildActor (Variables|Default|GetCA_ButtonFront)) (Variables|/Script/Engine.ChildActorComponent|GetChildActor (Variables|Default|GetCA_ButtonBack)))
    (bind _asbp_press_button (Utilities|Casting|CastToBP_PressButton _array_element))
    (Rendering|Material|SetMaterial (Variables|/Game/Blueprints/GPE/BP_PressButton.BP_PressButton_C|GetCylinder _asbp_press_button) 0 (select (Variables|Default|GetIsEnabled) "/Game/Materials/Instances/MI_PressButton.MI_PressButton" "/Game/Materials/Instances/MI_Black.MI_Black"))))

(fn ConstructionScript
  (CallFunction|SetEnabled (Variables|Default|GetIsEnabled)))