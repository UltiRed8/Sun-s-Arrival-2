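; BP_Clock is a clock prop that displays the real-world time with rotating second, minute and hour hands.
; BeginPlay starts a looping timer that calls Update every tenth of a second and is cleared on Destroyed.
; Update converts the current Now() time into stepped yaw rotations for each hand, with a fixed offset on the hour hand.
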(event Custom|Update
  (bind _returnvalue (Math|DateTime|Now))
  (bind (_year _month _day _hour _minute _second) (Math|DateTime|BreakDateTime _returnvalue))
  (Transformation|SetRelativeRotation (Variables|Default|GetHandSeconds) (Math|Rotator|MakeRotator 0.0 0.0 (* (/ (Math|Conversions|ToFloat(Integer) _second) 6e+01) 3.6e+02)) false false)
  (Transformation|SetRelativeRotation (Variables|Default|GetHandMinutes) (Math|Rotator|MakeRotator 0.0 0.0 (* (/ (Math|Conversions|ToFloat(Integer) _minute) 6e+01) 3.6e+02)) false false)
  (Transformation|SetRelativeRotation (Variables|Default|GetHandHours) (Math|Rotator|MakeRotator 0.0 0.0 (+ (* (/ (Math|Conversions|ToFloat(Integer) _hour) 12.0) 3.6e+02) -2e+01)) false false))

(event EventBeginPlay
  (|CallParentFunction)
  (bind _returnvalue (Utilities|Time|SetTimerbyEvent (delegate Custom|Update) 0.1 true))
  (Variables|Default|SetTimer _returnvalue))

(event EventDestroyed
  (|CallParentFunction)
  (Utilities|Time|ClearandInvalidateTimerbyHandle (Variables|Default|GetTimer)))

(fn ConstructionScript)