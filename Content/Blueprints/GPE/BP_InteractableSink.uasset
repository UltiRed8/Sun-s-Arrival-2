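; Interactable sink Blueprint that runs water effects and sound when the player interacts with it.
; Interaction calls the parent, then triggers MultiToggleFX if CanBeInteract is set, otherwise just re-enables the flag.
; MultiToggleFX clears the flag, plays the sound and activates WaterFX, then deactivates it after a fixed delay.
; PlayWaterSound restores the flag immediately when Audio is valid, so the sink is not locked during that delay.
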(event Custom|PlayWaterSound
  (Utilities|IsValid (Variables|Default|GetAudio)
    (:Is%20Valid
      (Audio|Components|Audio|Play (Variables|Default|GetAudio) 0.0)
      (Variables|Default|SetCanBeInteract true))))

(event Custom|MultiToggleFX
  (Variables|Default|SetCanBeInteract false)
  (CallFunction|PlayWaterSound)
  (Components|Activation|Activate (Variables|Default|GetWaterFX) false)
  (Utilities|FlowControl|Delay 8.0)
  (Components|Activation|Deactivate (Variables|Default|GetWaterFX)))

(event EventBeginPlay
  (|CallParentFunction))

(event EventInteraction
  (|CallParentFunction)
  (if (Variables|Default|GetCanBeInteract)
    (CallFunction|MultiToggleFX)
    (else
      (Variables|Default|SetCanBeInteract true))))

(fn ConstructionScript)