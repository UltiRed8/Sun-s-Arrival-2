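; BP_InteractableFireExtinguisher is an interactable fire extinguisher prop that sprays when used.
; It registers as an interactable on begin play and unregisters when destroyed.
; When interacted with while interaction is allowed, a multicast event plays its audio and activates a Niagara spray, deactivated after a short retriggerable delay so repeated uses extend it.
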(event Custom|Multi_PlaySound
  (bind _ns_fireextinguisher (Variables|Default|GetNS_FireExtinguisher))
  (Audio|Components|Audio|Play (Variables|Default|GetAudio) 0.0)
  (Components|Activation|Activate _ns_fireextinguisher false)
  (Utilities|FlowControl|RetriggerableDelay 1.2)
  (Components|Activation|Deactivate _ns_fireextinguisher))

(event EventBeginPlay
  (Utilities|RegisterInteractable))

(event EventInteraction
  (|CallParentFunction)
  (if (Variables|Default|GetCanBeInteract)
    (CallFunction|MultiPlaySound)))

(event EventDestroyed
  (Utilities|UnregisterInteractable))

(fn ConstructionScript)