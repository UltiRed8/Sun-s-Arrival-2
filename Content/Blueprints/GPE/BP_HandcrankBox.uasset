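; Interactable handcrank box that takes a crank item from inventory, then triggers a linked Node once used.
; Interaction runs server-to-client, starting mouse-capture cranking with replicated handle rotation or, with that setting off, calling back to the server.
; Triggering plays the crank animation and fires the Node after a delay.
; Crank placement and completion persist as checkpoint bools keyed by actor location.
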(event Custom|HandcrankAnimation
  (bind _rotated (Variables|Default|GetRotated))
  (Variables|/Game/Blueprints/Components/BP_CustomCursorComponent.BP_CustomCursorComponent_C|SetCursorTexture (Variables|Default|GetBP_CustomCursorComponent) "/Game/Textures/T_CursorNormal.T_CursorNormal")
  (bind _rotation (Timeline|DoorOpening Play)
    (:Update
      (Transformation|SetRelativeRotation (Variables|Default|GetHandlePivot) (Math|Rotator|MakeRotator _rotation 0.0 0.0) false false)
      (if (not (Audio|Components|Audio|IsPlaying _rotated))
        (Audio|Components|Audio|Play _rotated 0.0)))
    (:Finished
      (Audio|Components|Audio|Stop _rotated))))

(event Custom|Multi_PlaceHandcrank
  (Rendering|SetVisibility (Variables|Default|GetHandlePivot) true true)
  (Audio|Components|Audio|Play (Variables|Default|GetPlaced) 0.0)
  (Variables|/Game/Blueprints/Components/BP_CustomCursorComponent.BP_CustomCursorComponent_C|SetCursorTexture (Variables|Default|GetBP_CustomCursorComponent) "/Game/Textures/T_CursorInteract.T_CursorInteract"))

(event Custom|CheckInventory
  (bind _inventory (Utilities|Inventory))
  (bind _handcrankid (Variables|Default|GetHandcrankID))
  (bind _returnvalue (Utilities|String|MakeLiteralString _handcrankid))
  (bind _returnvalue_2 (Default|HasItem _inventory _returnvalue))
  (if _returnvalue_2
    (Default|RemoveItem _inventory _returnvalue)
    (Variables|Default|SetHasHandcrank true)
    (CallFunction|MultiPlaceHandcrank)
    (Utilities|CheckpointSaveBool (Utilities|String|Append (Utilities|String|ToString(Vector) (Transformation|GetActorLocation)) "_HandCrank") true)))

(event Custom|Multi_SetRotation
  (params (RotationX :type Float%20%28single-precision%29))
  (Transformation|SetRelativeRotation (Variables|Default|GetHandlePivot) (Math|Rotator|MakeRotator RotationX 0.0 0.0) false false))

(event Custom|Trigger
  (Variables|Default|SetDidIt true)
  (Utilities|CheckpointSaveBool (Utilities|String|ToString(Vector) (Transformation|GetActorLocation)) true)
  (CallFunction|HandcrankAnimation)
  (Utilities|FlowControl|Delay 2.0)
  (bind _node (Variables|Default|GetNode)
    (:then
      (Default|Trigger _node))
    (:else)))

(event Custom|Server_SetRotation
  (params (RotationX :type Float%20%28single-precision%29))
  (CallFunction|MultiSetRotation RotationX))

(event Custom|OnMouseMoved_Event
  (params (Angle :type Float%20%28double-precision%29) (Direction :type Vector%202D%20Structure))
  (bind _rotated (Variables|Default|GetRotated))
  (bind _handlepivot (Variables|Default|GetHandlePivot))
  (if (> Angle 0.0)
    (Transformation|AddRelativeRotation _handlepivot (Math|Rotator|MakeRotator (* (Math|Trig|RadiansToDegrees Angle) -1.0) 0.0 0.0) false false)
    (CallFunction|ServerSetRotation (.roll (Variables|/Script/Engine.SceneComponent|GetRelativeRotation _handlepivot)))
    (if (Audio|Components|Audio|IsPlaying _rotated)
      _
      (else
        (Audio|Components|Audio|Play _rotated 0.0)))
    (Utilities|FlowControl|RetriggerableDelay 0.1)
    (Audio|Components|Audio|Stop _rotated)))

(event Custom|OnMouseCapture_Event
  (Variables|/Game/Blueprints/Components/BP_CustomCursorComponent.BP_CustomCursorComponent_C|SetCursorTexture (Variables|Default|GetBP_CustomCursorComponent) "/Game/Textures/T_CursorMouseCircle.T_CursorMouseCircle"))

(event Custom|OnMouseUncaptured_Event
  (Variables|/Game/Blueprints/Components/BP_CustomCursorComponent.BP_CustomCursorComponent_C|SetCursorTexture (Variables|Default|GetBP_CustomCursorComponent) (select (Variables|Default|GetDidIt) "/Game/Textures/T_CursorNormal.T_CursorNormal" "/Game/Textures/T_CursorInteract.T_CursorInteract")))

(event EventServerInteract
  (params (WhoInteracted :type Actor%20Object%20Reference))
  (Actor|SetOwner WhoInteracted)
  (if (not (Variables|Default|GetDidIt))
    (if (Variables|Default|GetHasHandcrank)
      (bind _asbp_player (Utilities|Casting|CastToBP_Player WhoInteracted))
      (Default|FromServerInteractwith _asbp_player self)
      (else
        (CallFunction|CheckInventory)))))

(event EventOntoServerInteract
  (params (MethodName :type String))
  (CallFunction|Trigger))

(event EventDestroyed
  (Utilities|UnregisterInteractable))

(event EventBeginPlay
  (bind _bp_customcursorcomponent (Variables|Default|GetBP_CustomCursorComponent))
  (bind _bp_mousemovementcomponent (Variables|Default|GetBP_MouseMovementComponent))
  (Utilities|RegisterInteractable)
  (|CallParentFunction)
  (EventDispatchers|AssignOnMouseMoved _bp_mousemovementcomponent (delegate Custom|OnMouseMoved_Event))
  (EventDispatchers|AssignOnMouseCapture _bp_mousemovementcomponent (delegate Custom|OnMouseCapture_Event))
  (EventDispatchers|AssignOnMouseUncaptured _bp_mousemovementcomponent (delegate Custom|OnMouseUncaptured_Event))
  (if (Variables|Default|GetHasHandcrank)
    (Variables|/Game/Blueprints/Components/BP_CustomCursorComponent.BP_CustomCursorComponent_C|SetCursorTexture _bp_customcursorcomponent "/Game/Textures/T_CursorInteract.T_CursorInteract")
    (else
      (Variables|/Game/Blueprints/Components/BP_CustomCursorComponent.BP_CustomCursorComponent_C|SetCursorTexture _bp_customcursorcomponent "/Game/Textures/T_CursorInteract.T_CursorInteract")))
  (bind (_success _bool) (Utilities|CheckpointGetBool (Utilities|String|Append (Utilities|String|ToString(Vector) (Transformation|GetActorLocation)) "_HandCrank")))
  (if _success
    (if _bool
      (Variables|Default|SetHasHandcrank true)
      (CallFunction|MultiPlaceHandcrank)))
  (bind (_success_2 _bool_2) (Utilities|CheckpointGetBool (Utilities|String|ToString(Vector) (Transformation|GetActorLocation))))
  (if _success_2
    (Variables|Default|SetDidIt _bool_2)
    (Variables|/Game/Blueprints/Components/BP_CustomCursorComponent.BP_CustomCursorComponent_C|SetCursorTexture (Variables|Default|GetBP_CustomCursorComponent) "/Game/Textures/T_CursorNormal.T_CursorNormal")))

(event EventClientInteract
  (if (Variables|/Game/Saves/SG_Settings.SG_Settings_C|GetMouseInteractions (Variables|/Game/BP_GameInstance.BP_GameInstance_C|GetSettings (Utilities|GameInstance)))
    (Default|StartCapturing (Variables|Default|GetBP_MouseMovementComponent))
    (else
      (bind _asbp_player (Utilities|Casting|CastToBP_Player (Pawn|GetControlledPawn (Game|GetPlayerController 0))))
      (Default|OntoServerInteractwith _asbp_player self))))

(fn ConstructionScript
  (Rendering|SetVisibility (Variables|Default|GetHandlePivot) (Variables|Default|GetHasHandcrank) true))