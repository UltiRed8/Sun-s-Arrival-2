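; Interactable computer that toggles a set of linked screens on and off when the player uses it.
; It extends a parent interactable's Interaction event and, when interaction is allowed, plays an optional sound at its location.
; A FlipFlop alternates each use between turning every valid screen in AllScreensLinked on and turning them off, starting with on.
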(event Custom|PlayComputerSound
  (Utilities|IsValid (Variables|Default|GetInteractSound)
    (:Is%20Valid
      (Audio|PlaySoundatLocation (Variables|Default|GetInteractSound) (Transformation|GetActorLocation) "0, 0, 0" 1.0 1.0 0.0 0 0 0 0))))

(event EventBeginPlay
  (|CallParentFunction))

(event EventInteraction
  (|CallParentFunction)
  (if (Variables|Default|GetCanBeInteract)
    (CallFunction|PlayComputerSound)
    (if (Utilities|Array|IsNotEmpty (Variables|Default|GetAllScreensLinked))
      (Utilities|FlowControl|FlipFlop
        (:A
          (for _array_element (Variables|Default|GetAllScreensLinked)
            (Utilities|IsValid _array_element
              (:Is%20Valid
                (Default|TurnScreenon _array_element)))))
        (:B
          (for _array_element_2 (Variables|Default|GetAllScreensLinked)
            (Utilities|IsValid _array_element_2
              (:Is%20Valid
                (Default|TurnScreenOff _array_element_2)))))))))

(fn ConstructionScript)