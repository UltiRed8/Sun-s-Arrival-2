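; Interactable chest of drawers whose three drawers slide open and closed individually along their local X axis.
; Interaction locks re-entry, ignores hits on the case, and routes the hit component to that drawer's move event, defaulting to the third drawer.
; Each move event plays a sound at the drawer's relative location, then flip-flops its own timeline forward or in reverse, unlocking interaction on finish.
; An older switch on component name remains disconnected.
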(event Custom|MoveDrawer3
  (params (Drawer :type Static%20Mesh%20Component%20Object%20Reference))
  (bind _relativelocation (Variables|/Script/Engine.SceneComponent|GetRelativeLocation Drawer))
  (Audio|PlaySoundatLocation (Variables|Default|GetInteractSound) (Variables|/Script/Engine.SceneComponent|GetRelativeLocation Drawer) "0, 0, 0" 1.0 1.0 0.0 0 0 0 0)
  (Utilities|FlowControl|FlipFlop
    (:A
      (bind _movex (Timeline|Timeline_4 PlayFromStart)
        (:Update
          (Transformation|SetRelativeLocation Drawer (Math|Vector|MakeVector _movex (.y _relativelocation) (.z _relativelocation)) false false))
        (:Finished
          (Variables|Default|SetCanBeInteract true))))
    (:B
      (Timeline|Timeline_4 Reverse))))

(event Custom|MoveDrawer1
  (params (Drawer :type Static%20Mesh%20Component%20Object%20Reference))
  (bind _relativelocation (Variables|/Script/Engine.SceneComponent|GetRelativeLocation Drawer))
  (Audio|PlaySoundatLocation (Variables|Default|GetInteractSound) (Variables|/Script/Engine.SceneComponent|GetRelativeLocation Drawer) "0, 0, 0" 1.0 1.0 0.0 0 0 0 0)
  (Utilities|FlowControl|FlipFlop
    (:A
      (bind _movex (Timeline|Timeline_2 PlayFromStart)
        (:Update
          (Transformation|SetRelativeLocation Drawer (Math|Vector|MakeVector _movex (.y _relativelocation) (.z _relativelocation)) false false))
        (:Finished
          (Variables|Default|SetCanBeInteract true))))
    (:B
      (Timeline|Timeline_2 Reverse))))

(event Custom|MoveDrawer2
  (params (Drawer :type Static%20Mesh%20Component%20Object%20Reference))
  (bind _relativelocation (Variables|/Script/Engine.SceneComponent|GetRelativeLocation Drawer))
  (Audio|PlaySoundatLocation (Variables|Default|GetInteractSound) (Variables|/Script/Engine.SceneComponent|GetRelativeLocation Drawer) "0, 0, 0" 1.0 1.0 0.0 0 0 0 0)
  (Utilities|FlowControl|FlipFlop
    (:A
      (bind _movex (Timeline|Timeline_3 PlayFromStart)
        (:Update
          (Transformation|SetRelativeLocation Drawer (Math|Vector|MakeVector _movex (.y _relativelocation) (.z _relativelocation)) false false))
        (:Finished
          (Variables|Default|SetCanBeInteract true))))
    (:B
      (Timeline|Timeline_3 Reverse))))

(event EventInteraction
  (bind _interactcomponent (Variables|Default|GetInteractComponent))
  (bind _drawer2 (Variables|Default|GetDrawer2))
  (bind _drawer1 (Variables|Default|GetDrawer1))
  (|CallParentFunction)
  (if (Variables|Default|GetCanBeInteract)
    (Variables|Default|SetCanBeInteract false)
    (if (== (Variables|Default|GetInteractComponent) (Variables|Default|GetCase))
      (Variables|Default|SetCanBeInteract true)
      (elif (== _interactcomponent _drawer1)
        (CallFunction|MoveDrawer1 _drawer1)
        (elif (== _interactcomponent _drawer2)
          (CallFunction|MoveDrawer2 _drawer2)
          (else
            (CallFunction|MoveDrawer3 (Variables|Default|GetDrawer3))))))))

(event EventBeginPlay
  (|CallParentFunction))

(fn ConstructionScript)