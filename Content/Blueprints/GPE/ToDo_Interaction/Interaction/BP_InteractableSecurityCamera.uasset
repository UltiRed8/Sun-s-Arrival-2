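; Interactable security camera whose pivot mimics the look movement of a nearby player after a delay.
; Sphere overlaps maintain the player list and select its first entry; on entry, that player's control rotation and a look-at rotation toward them are stored as baselines.
; While interactable, Tick buffers control rotations over DelayTime, sized by frame delta, then applies the oldest's pitch and yaw offsets to the camera baseline, with zero roll.
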(event OnComponentBeginOverlap(Sphere)
  (params (OverlappedComponent :type Primitive%20Component%20Object%20Reference) (OtherActor :type Actor%20Object%20Reference) (OtherComp :type Primitive%20Component%20Object%20Reference) (OtherBodyIndex :type Integer) (bFromSweep :type Boolean) (SweepResult :type Hit%20Result%20Structure%20%28by%20ref%29))
  (bind _asbp_player (Utilities|Casting|CastToBP_Player OtherActor))
  (Utilities|Array|Add (Variables|Default|GetAllPlayers) _asbp_player)
  (bind _output_get (Variables|Default|SetSelectedPlayer (Utilities|Array|Get(acopy) (Variables|Default|GetAllPlayers))))
  (Utilities|IsValid _output_get
    (:Is%20Valid
      (Variables|Default|SetBasePlayerRotation (Pawn|GetControlRotation _output_get :!class /Script/Engine.Pawn))
      (Variables|Default|SetBaseCameraRotation (Math|Rotator|FindLookatRotation (Transformation|GetActorLocation) (Transformation|GetActorLocation _output_get))))))

(event OnComponentEndOverlap(Sphere)
  (params (OverlappedComponent :type Primitive%20Component%20Object%20Reference) (OtherActor :type Actor%20Object%20Reference) (OtherComp :type Primitive%20Component%20Object%20Reference) (OtherBodyIndex :type Integer))
  (bind _asbp_player (Utilities|Casting|CastToBP_Player OtherActor))
  (Utilities|Array|RemoveItem (Variables|Default|GetAllPlayers) _asbp_player)
  (Variables|Default|SetSelectedPlayer (Utilities|Array|Get(acopy) (Variables|Default|GetAllPlayers))))

(event EventTick
  (params (DeltaSeconds :type Float%20%28single-precision%29))
  (bind _rotationhistory (Variables|Default|GetRotationHistory))
  (bind _rotationhistory_2 (Variables|Default|GetRotationHistory))
  (bind _baseplayerrotation (Variables|Default|GetBasePlayerRotation))
  (bind _basecamerarotation (Variables|Default|GetBaseCameraRotation))
  (bind (_roll _pitch _yaw) (Math|Rotator|BreakRotator _baseplayerrotation))
  (bind (_roll_2 _pitch_2 _yaw_2) (Math|Rotator|BreakRotator _basecamerarotation))
  (bind _output (Utilities|Array|Get(acopy) _rotationhistory_2))
  (bind (_roll_3 _pitch_3 _yaw_3) (Math|Rotator|BreakRotator _output))
  (if (Variables|Default|GetCanBeInteract)
    (if (not (Utilities|Array|IsEmpty (Variables|Default|GetAllPlayers)))
      (Utilities|IsValid (Variables|Default|GetSelectedPlayer)
        (:Is%20Valid
          (Utilities|Array|Add (Variables|Default|GetRotationHistory) (Pawn|GetControlRotation (Variables|Default|GetSelectedPlayer) :!class /Script/Engine.Pawn))
          (Variables|Default|SetHistoryMaxSize (Math|Float|Round (/ (Variables|Default|GetDelayTime) DeltaSeconds)))
          (if (> (Utilities|Array|Length (Variables|Default|GetRotationHistory)) (Variables|Default|GetHistoryMaxSize))
            (Utilities|Array|RemoveItem _rotationhistory (Utilities|Array|Get(acopy) _rotationhistory)))
          (if (>= (Utilities|Array|Length (Variables|Default|GetRotationHistory)) (Variables|Default|GetHistoryMaxSize))
            (Transformation|SetWorldRotation (Variables|Default|GetPivot) (Math|Rotator|MakeRotator 0.0 (+ _pitch_2 (- _pitch_3 _pitch)) (+ _yaw_2 (- _yaw_3 _yaw))) false false)))))))

(fn ConstructionScript)