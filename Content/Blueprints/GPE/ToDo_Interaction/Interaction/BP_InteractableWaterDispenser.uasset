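; Interactable water dispenser that toggles a water effect and plays a sound when the player uses it.
; It extends a parent interactable: Interaction calls the parent, then runs MultiToggleFX, where a FlipFlop alternately activates and deactivates WaterFX.
; CanBeInteract locks during the toggle and resets once the sound is triggered; without a valid sound, the next interaction only re-enables it.
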(event Custom|PlayWaterSound
  (Utilities|IsValid (Variables|Default|GetInteractSound)
    (:Is%20Valid
      (Audio|PlaySoundatLocation (Variables|Default|GetInteractSound) (Transformation|GetActorLocation) "0, 0, 0" 1.0 1.0 0.0 0 0 0 0)
      (Variables|Default|SetCanBeInteract true))))

(event Custom|MultiToggleFX
  (Variables|Default|SetCanBeInteract false)
  (Utilities|IsValid (Variables|Default|GetWaterFX)
    (:Is%20Valid
      (Utilities|FlowControl|FlipFlop
        (:A
          (Components|Activation|Activate (Variables|Default|GetWaterFX) false))
        (:B
          (Components|Activation|Deactivate (Variables|Default|GetWaterFX)))))
    (:Is%20Not%20Valid
      _))
  (CallFunction|PlayWaterSound))

(event EventBeginPlay
  (|CallParentFunction))

(event EventInteraction
  (|CallParentFunction)
  (if (Variables|Default|GetCanBeInteract)
    (CallFunction|MultiToggleFX)
    (else
      (Variables|Default|SetCanBeInteract true))))

(fn ConstructionScript)