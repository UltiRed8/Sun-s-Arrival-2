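; Interactable toilet prop with two hinged lid parts and a base that plays a sound when used.
; Interaction branches on the targeted component, swinging the top lid or lid via timeline-driven pitch rotation of its axis component, or playing the sound.
; State flags enforce hinge order: the lid only raises when the top lid is up, and the top lid only lowers when the lid is down.
; CanBeInteract blocks input until each action finishes.
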(event Custom|LidTopInteract
  (if (Variables|Default|GetIsLidTopOnTop)
    (if (Variables|Default|GetIsLidDown)
      (Variables|Default|SetIsLidTopOnTop false)
      (bind _lidtop (Timeline|LidTopInteraction Reverse)
        (:Update
          (Transformation|SetRelativeRotation (Variables|Default|GetAxisLidTop) (Math|Rotator|MakeRotator 0.0 _lidtop 0.0) false false))
        (:Finished
          (Variables|Default|SetCanBeInteract true :!label _label)))
      (else
        (goto _label)))
    (else
      (Variables|Default|SetIsLidTopOnTop true)
      (Timeline|LidTopInteraction PlayFromStart))))

(event Custom|LidInteract
  (if (Variables|Default|GetIsLidDown)
    (if (Variables|Default|GetIsLidTopOnTop)
      (Variables|Default|SetIsLidDown false)
      (bind _lid (Timeline|LidInteraction PlayFromStart)
        (:Update
          (Transformation|SetRelativeRotation (Variables|Default|GetAxisLid) (Math|Rotator|MakeRotator 0.0 _lid 0.0) false false))
        (:Finished
          (Variables|Default|SetCanBeInteract true :!label _label)))
      (else
        (goto _label)))
    (else
      (Variables|Default|SetIsLidDown true)
      (Timeline|LidInteraction Reverse))))

(event Custom|PlayToiletSound
  (Audio|PlaySoundatLocation (Variables|Default|GetInteractSound) (Transformation|GetActorLocation) "0, 0, 0" 1.0 1.0 0.0 0 0 0 0)
  (Variables|Default|SetCanBeInteract true))

(event EventBeginPlay
  (|CallParentFunction))

(event EventInteraction
  (|CallParentFunction)
  (if (Variables|Default|GetCanBeInteract)
    (Variables|Default|SetCanBeInteract false)
    (if (== (Variables|Default|GetInteractComponent) (Variables|Default|GetLidTop))
      (CallFunction|LidTopInteract)
      (elif (== (Variables|Default|GetInteractComponent) (Variables|Default|GetBase))
        (CallFunction|PlayToiletSound)
        (else
          (CallFunction|LidInteract))))))

(fn ConstructionScript
  (|CallParentFunction))