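; BP_InteractableDeskLight is an interactable desk light that switches its point light between two intensities.
; Interaction calls the parent, then uses a FlipFlop to alternate FirstIntensity and SecondIntensity and plays InteractSound at the actor's location.
; CanBeInteract gates the toggle and resets immediately after the sound starts.
; Without a valid sound it stays false, so the following interaction only re-enables it.
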(event Custom|PlayLightSound
  (Utilities|IsValid (Variables|Default|GetInteractSound)
    (:Is%20Valid
      (Audio|PlaySoundatLocation (Variables|Default|GetInteractSound) (Transformation|GetActorLocation) "0, 0, 0" 1.0 1.0 0.0 0 0 0 0)
      (Variables|Default|SetCanBeInteract true))))

(event EventInteraction
  (bind _pointlight (Variables|Default|GetPointLight))
  (|CallParentFunction)
  (if (Variables|Default|GetCanBeInteract)
    (Variables|Default|SetCanBeInteract false)
    (Utilities|FlowControl|FlipFlop
      (:A
        (Rendering|Components|Light|SetIntensity _pointlight (Variables|Default|GetFirstIntensity)))
      (:B
        (Rendering|Components|Light|SetIntensity _pointlight (Variables|Default|GetSecondIntensity))))
    (CallFunction|PlayLightSound)
    (else
      (Variables|Default|SetCanBeInteract true))))

(fn ConstructionScript)