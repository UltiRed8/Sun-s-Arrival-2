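; BP_InteractableCoin is an interactable coin pickup that adds to the player's coin balance.
; On BeginPlay it finds the BP_GlobalInventory actor in the level and caches it.
; When interacted with and allowed, it plays a sound at its location, increments CoinsBalance in that inventory and destroys itself.
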(event EventBeginPlay
  (|CallParentFunction)
  (bind _returnvalue (Actor|GetActorOfClass "/Game/Blueprints/Inventory/BP_GlobalInventory.BP_GlobalInventory_C"))
  (Variables|Default|SetInventory _returnvalue))

(event EventInteraction
  (|CallParentFunction)
  (if (Variables|Default|GetCanBeInteract)
    (Audio|PlaySoundatLocation (Variables|Default|GetInteractSound) (Transformation|GetActorLocation) "0, 0, 0" 1.0 1.0 0.0 0 0 0 0)
    (Math|Integer|IncrementInt (Variables|/Game/Blueprints/Inventory/BP_GlobalInventory.BP_GlobalInventory_C|GetCoinsBalance (Variables|Default|GetInventory))
      (:%20%20
        (Actor|DestroyActor)))))

(fn ConstructionScript)