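; Interactable vending machine that spends one coin from the global inventory to dispense the next actor in its reward list.
; A coin timeline animates the insertion, then a second timeline pushes the reward out before it gets physics and leaves the list.
; Interactions while busy, empty or short of coins play feedback sounds.
; When disabled, the construction script strips its lights and idle sound component and blacks out one material.
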(event EventBeginPlay
  (|CallParentFunction)
  (bind _returnvalue (Actor|GetActorOfClass "/Game/Blueprints/Inventory/BP_GlobalInventory.BP_GlobalInventory_C"))
  (Variables|Default|SetGlobalInventory _returnvalue))

(event EventInteraction
  (bind _coin (Variables|Default|GetCoin))
  (bind _coin_2 (Variables|Default|GetCoin))
  (bind _relativelocation (Variables|/Script/Engine.SceneComponent|GetRelativeLocation _coin_2))
  (|CallParentFunction)
  (if (Variables|Default|GetIsEnabled)
    (if (Variables|Default|GetCanBeInteract)
      (if (Utilities|Array|IsEmpty (Variables|Default|GetAllRewards))
        (Audio|PlaySoundatLocation (Variables|Default|GetNoInteractionSound) (Transformation|GetActorLocation) "0, 0, 0" 1.0 1.0 0.0 0 0 0 0 :!label _label)
        (else
          (Utilities|IsValid (Variables|Default|GetGlobalInventory)
            (:Is%20Valid
              (if (>= (Variables|/Game/Blueprints/Inventory/BP_GlobalInventory.BP_GlobalInventory_C|GetCoinsBalance (Variables|Default|GetGlobalInventory)) 1)
                (Variables|Default|SetActualReward (Utilities|Array|Get(acopy) (Variables|Default|GetAllRewards)))
                (Math|Integer|DecrementInt (Variables|/Game/Blueprints/Inventory/BP_GlobalInventory.BP_GlobalInventory_C|GetCoinsBalance (Variables|Default|GetGlobalInventory))
                  (:%20%20
                    (Variables|Default|SetCanBeInteract false)
                    (Rendering|SetVisibility (Variables|Default|GetCoin) true false)
                    (bind _movement (Timeline|CoinMovement PlayFromStart)
                      (:Update
                        (Transformation|SetRelativeLocation _coin_2 (Math|Vector|MakeVector _movement (.y _relativelocation) (.z _relativelocation)) false false))
                      (:Finished
                        (Audio|PlaySoundatLocation (Variables|Default|GetInteractSound) (Transformation|GetActorLocation) "0, 0, 0" 1.0 1.0 0.0 0 0 0 0)
                        (Rendering|SetVisibility _coin false false)
                        (Transformation|SetRelativeLocation _coin (Math|Vector|MakeVector 9e+01 0.0 2.2e+02) false false)
                        (Utilities|IsValid (Variables|Default|GetActualReward)
                          (:Is%20Valid
                            (bind _move (Timeline|Timeline PlayFromStart)
                              (:Update
                                (Transformation|SetActorRelativeLocation (Variables|Default|GetActualReward) (Math|Vector|MakeVector (Math|Float|Lerp (.x (Transformation|GetActorLocation (Variables|Default|GetActualReward))) (+ (.x (Transformation|GetActorLocation (Variables|Default|GetActualReward))) 2.0) _move) (.y (Transformation|GetActorLocation (Variables|Default|GetActualReward))) (.z (Transformation|GetActorLocation (Variables|Default|GetActualReward))))))
                              (:Finished
                                (Variables|Default|SetCanBeInteract true)
                                (Utilities|IsValid (Actor|GetComponentbyClass (Variables|Default|GetActualReward) "/Script/Engine.StaticMeshComponent")
                                  (:Is%20Valid
                                    (Physics|SetSimulatePhysics (Actor|GetComponentbyClass (Variables|Default|GetActualReward) "/Script/Engine.StaticMeshComponent") true))
                                  (:Is%20Not%20Valid
                                    _))
                                (Variables|Default|SetActualReward 0)
                                (Utilities|Array|RemoveIndex (Variables|Default|GetAllRewards)))))
                          (:Is%20Not%20Valid
                            (Development|PrintString "Reward not valid")))))))
                (else
                  (Audio|PlaySoundatLocation (Variables|Default|GetNotEnoughCoinsSound) (Transformation|GetActorLocation) "0, 0, 0" 1.0 1.0 0.0 0 0 0 0)))))))
      (else
        (goto _label)))))

(fn ConstructionScript
  (|CallParentFunction)
  (if (not (Variables|Default|GetIsEnabled))
    (Components|DestroyComponent (Variables|Default|GetRectLight1))
    (Rendering|Material|SetMaterial (Variables|Default|GetVendingMachine) 3 "/Game/Materials/Instances/MI_UnlitBlack.MI_UnlitBlack")))