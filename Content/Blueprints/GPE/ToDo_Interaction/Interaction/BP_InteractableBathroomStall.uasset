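; Interactable bathroom stall whose door swings open and closed on alternating interactions, building on a parent interactable's logic.
; Interaction relays through server and multicast events, so the door motion is meant to play for all players.
; A FlipFlop plays or reverses a timeline driving the yaw of the Axis component when the interacted component is the Door.
; Further interaction is blocked until the timeline finishes.
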(event Custom|Multi_OpenDoor
  (Variables|Default|SetCanBeInteract false)
  (if (== (Variables|Default|GetInteractComponent) (Variables|Default|GetDoor))
    (Utilities|FlowControl|FlipFlop
      (:A
        (bind _opendoortrack (Timeline|OpenDoor PlayFromStart)
          (:Update
            (Transformation|SetRelativeRotation (Variables|Default|GetAxis) (Math|Rotator|MakeRotator 0.0 0.0 _opendoortrack) false false))
          (:Finished
            (Variables|Default|SetCanBeInteract true :!label _label))))
      (:B
        (Timeline|OpenDoor Reverse)))
    (else
      (goto _label))))

(event Custom|Server_OpenDoor
  (CallFunction|MultiOpenDoor))

(event EventBeginPlay
  (|CallParentFunction))

(event EventInteraction
  (|CallParentFunction)
  (if (Variables|Default|GetCanBeInteract)
    (CallFunction|ServerOpenDoor)))

(fn ConstructionScript)