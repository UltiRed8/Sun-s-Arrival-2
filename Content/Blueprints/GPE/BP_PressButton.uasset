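; BP_PressButton is an interactable push-button gameplay element that fires a trigger when used.
; It registers as an interactable on BeginPlay and unregisters when destroyed.
; On server interaction, it calls OnTriggered, fires the multicast feedback event and triggers its linked Node if valid.
; The multicast plays the LeverDownEnd sound and a particle effect.
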(event Custom|Multi_PlaySound
  (Audio|Components|Audio|Play (Variables|Default|GetLeverDownEnd) 0.0)
  (CallFunction|PlayParticle))

(event EventBeginPlay
  (Utilities|RegisterInteractable))

(event EventServerInteract
  (params (WhoInteracted :type Actor%20Object%20Reference))
  (Default|CallOnTriggered)
  (CallFunction|MultiPlaySound)
  (bind _node (Variables|Default|GetNode)
    (:then
      (Default|Trigger _node))
    (:else)))

(event EventDestroyed
  (Utilities|UnregisterInteractable))

(fn ConstructionScript)