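; Chaos destructible actor that becomes one of four random body pieces (head, arm, leg or main) and later breaks apart and disappears.
; On BeginPlay the authority picks the type and multicasts it, so the other three GC components get destroyed.
; PrepareDestroy removes collision, enables physics on the remaining piece, then after a short delay a timeline drives its scale before the actor is destroyed.
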(event Custom|PrepareDestroy
  (Components|DestroyComponent (Variables|Default|GetCollision))
  (CallFunction|EnablePhysics)
  (Utilities|FlowControl|Delay 1.0)
  (bind _size (Timeline|DestroyTimeline PlayFromStart)
    (:Update
      (CallFunction|UpdateScale _size))
    (:Finished
      (Actor|DestroyActor))))

(event Custom|EnablePhysics
  (for _array_element (Variables|Default|GetAllGC)
    (Utilities|IsValid _array_element
      (:Is%20Valid
        (Physics|SetSimulatePhysics _array_element true)))))

(event Custom|UpdateScale
  (params (ScaleValue :type Float%20%28double-precision%29))
  (bind _returnvalue (* ScaleValue 0.05))
  (for _array_element (Variables|Default|GetAllGC)
    (Utilities|IsValid _array_element
      (:Is%20Valid
        (Transformation|SetRelativeScale3D _array_element (Math|Vector|MakeVector _returnvalue _returnvalue _returnvalue))))))

(event Custom|Multi_SetupElement
  (params (Enumerator :type E_GCType%20Enum :default "NewEnumerator0"))
  (bind _gc_head (Variables|Default|GetGC_Head))
  (Variables|Default|SetType Enumerator)
  (switch Utilities|FlowControl|Switch|SwitchonE_GCType (Variables|Default|GetType)
    (:NewEnumerator0
      (Components|DestroyComponent (Variables|Default|GetGC_Arm)))
    (:NewEnumerator1
      (Components|DestroyComponent _gc_head))
    (:NewEnumerator2
      (Components|DestroyComponent _gc_head))
    (:NewEnumerator3
      (Components|DestroyComponent (Variables|Default|GetGC_Leg))))
  (Variables|Default|SetAllGC (Utilities|Array|MakeArray (Variables|Default|GetGC_Head) (Variables|Default|GetGC_Arm) (Variables|Default|GetGC_Leg) (Variables|Default|GetGC_Main))))

(event EventBeginPlay
  (Networking|SwitchHasAuthority
    (:Authority
      (if (Math|Random|RandomBool)
        (if (Math|Random|RandomBool)
          (Variables|Default|SetType "NewEnumerator0")
          (else
            (Variables|Default|SetType "NewEnumerator1")))
        (elif (Math|Random|RandomBool)
          (Variables|Default|SetType "NewEnumerator2")
          (else
            (Variables|Default|SetType "NewEnumerator3"))))
      (CallFunction|MultiSetupElement (Variables|Default|GetType)))))

(fn ConstructionScript)