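; PC_GameBase is a base player controller that handles shared input setup, input device detection and the pause action.
; On the local controller it adds the IMC_Player Enhanced Input mapping context at BeginPlay and removes it when destroyed.
; Any key press tells the game instance whether a gamepad is in use, and IA_Pause calls the game instance's EscapeEvent.
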(event Input|EnhancedActionEvents|EnhancedInputActionIA_Pause
  (params (ActionValue :type Boolean) (ElapsedSeconds :type Float%20%28double-precision%29) (TriggeredSeconds :type Float%20%28double-precision%29) (InputAction :type Input%20Action%20Object%20Reference :default "/Game/Inputs/Actions/IA_Pause.IA_Pause"))
  (:Started
    (Default|EscapeEvent (Utilities|GameInstance))))

(event EventBeginPlay
  (bind _returnvalue (PlayerController|LocalPlayerSubsystems|GetEnhancedInputLocalPlayerSubsystem))
  (bind _self self)
  (if (Pawn|IsLocalController)
    (Utilities|IsValid _returnvalue
      (:Is%20Valid
        (Input|AddMappingContext _returnvalue "/Game/Inputs/IMC_Player.IMC_Player" 0 (Utilities|Struct|MakeModifyContextOptions true false true)))
      (:Is%20Not%20Valid
        _)))
  (Input|EnableInput _self _self))

(event EventDestroyed
  (bind _returnvalue (PlayerController|LocalPlayerSubsystems|GetEnhancedInputLocalPlayerSubsystem))
  (if (Pawn|IsLocalController)
    (Utilities|IsValid _returnvalue
      (:Is%20Valid
        (Input|RemoveMappingContext _returnvalue "/Game/Inputs/IMC_Player.IMC_Player" (Utilities|Struct|MakeModifyContextOptions true false true))))))

(event Input|KeyboardEvents|AnyKey
  (params (Key :type Key%20Structure :default "None"))
  (:Pressed
    (Default|SetUsingController (Utilities|GameInstance) (Class|KismetInputLibrary|KeyIsGamepadKey Key))))

(fn ConstructionScript)