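; Player controller that passes the player's username and color customization to the controlled BP_Player pawn.
; On BeginPlay it calls the parent, reads username, hue shift, brightness and saturation from the game instance, and sends them to Server_SetPlayerData.
; That event casts the controlled pawn to BP_Player and writes the values to it, doing nothing if the cast fails.
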(event Custom|Server_SetPlayerData
  (params (Username :type String) (HueShift :type Float%20%28double-precision%29) (Brightness :type Float%20%28double-precision%29) (Saturation :type Float%20%28double-precision%29))
  (bind _asbp_player (Utilities|Casting|CastToBP_Player (Pawn|GetControlledPawn)))
  (Variables|/Game/Blueprints/Player/BP_Player.BP_Player_C|SetHueShift _asbp_player HueShift)
  (Variables|/Game/Blueprints/Player/BP_Player.BP_Player_C|SetUsername _asbp_player Username)
  (Variables|/Game/Blueprints/Player/BP_Player.BP_Player_C|SetBrightness _asbp_player Brightness)
  (Variables|/Game/Blueprints/Player/BP_Player.BP_Player_C|SetSaturation _asbp_player Saturation))

(event EventBeginPlay
  (bind _asbp_game_instance (Utilities|GameInstance))
  (bind (_hueshift _brightness _saturation) (Default|GetCustomization _asbp_game_instance))
  (|CallParentFunction)
  (CallFunction|ServerSetPlayerData (Default|GetUsername _asbp_game_instance) _hueshift _brightness _saturation))

(fn ConstructionScript)